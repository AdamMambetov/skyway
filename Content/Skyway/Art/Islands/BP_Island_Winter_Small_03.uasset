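; Small winter island Blueprint for Skyway that procedurally places static meshes along a cable strung between two log meshes.
; The construction script adds one mesh per inner cable segment, using the cable component's segment count.
; Each position is linearly interpolated between the two logs' relative locations, with a lowered start point, fixed sideways offsets and a shared rotation and scale.
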(fn `UserConstructionScript`
  (bind _numsegments (`CableComponent.NumSegments` (`self.CableActor_CableComponent0`)))
  (for _index (range 2 _numsegments)
    (`AddComponent|NODE_AddStaticMeshComponent-2` :`RelativeTransform` (`KismetMathLibrary.MakeTransform` (`KismetMathLibrary.MakeVector` (+ (.x (`|EaseFunction` "Linear" (`KismetMathLibrary.NormalizeToRange` (`KismetMathLibrary.Conv_IntToDouble` _index) 1.0 (`KismetMathLibrary.Conv_IntToDouble` _numsegments)) (`KismetMathLibrary.MakeVector` (.x (`SceneComponent.RelativeLocation` (`self.Log_low4_StaticMeshComponent0`))) (.y (`SceneComponent.RelativeLocation` (`self.Log_low4_StaticMeshComponent0`))) (- (.z (`SceneComponent.RelativeLocation` (`self.Log_low4_StaticMeshComponent0`))) 46.1)) (`SceneComponent.RelativeLocation` (`self.Log_low2_StaticMeshComponent0`)))) 90.0) (+ (.y (`|EaseFunction` "Linear" (`KismetMathLibrary.NormalizeToRange` (`KismetMathLibrary.Conv_IntToDouble` _index) 1.0 (`KismetMathLibrary.Conv_IntToDouble` _numsegments)) (`KismetMathLibrary.MakeVector` (.x (`SceneComponent.RelativeLocation` (`self.Log_low4_StaticMeshComponent0`))) (.y (`SceneComponent.RelativeLocation` (`self.Log_low4_StaticMeshComponent0`))) (- (.z (`SceneComponent.RelativeLocation` (`self.Log_low4_StaticMeshComponent0`))) 46.1)) (`SceneComponent.RelativeLocation` (`self.Log_low2_StaticMeshComponent0`)))) 30.0) (.z (`|EaseFunction` "Linear" (`KismetMathLibrary.NormalizeToRange` (`KismetMathLibrary.Conv_IntToDouble` _index) 1.0 (`KismetMathLibrary.Conv_IntToDouble` _numsegments)) (`KismetMathLibrary.MakeVector` (.x (`SceneComponent.RelativeLocation` (`self.Log_low4_StaticMeshComponent0`))) (.y (`SceneComponent.RelativeLocation` (`self.Log_low4_StaticMeshComponent0`))) (- (.z (`SceneComponent.RelativeLocation` (`self.Log_low4_StaticMeshComponent0`))) 46.1)) (`SceneComponent.RelativeLocation` (`self.Log_low2_StaticMeshComponent0`))))) (struct :`Yaw` 30.0) (2.0 2.0 2.0)))))