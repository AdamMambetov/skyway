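; BP_Island_Base is a base island actor that populates itself with NPCs and cleans itself up by distance.
; On BeginPlay it spawns a BP_NpcSpawnerBase at SpawnerLocation, passing through its NPC class, radius, count and respawn settings plus a random team ID.
; Tick measures distance to the island's owner and, once beyond DistanceForDestroy, destroys the spawner and the island through a DoOnce.
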(event `self.ReceiveBeginPlay`
  (bind _returnvalue (`|SpawnActorFromClass` "/Game/Skyway/Core/AI/Spawners/BP_NpcSpawnerBase.BP_NpcSpawnerBase_C" (`SceneComponent.K2_GetComponentToWorld` (`self.SpawnerLocation`)) "Undefined" "OverrideRootScale" self (`self.NpcToSpawn`) (`KismetMathLibrary.RandomIntegerInRange` 1 999) (`self.RespawnNpcAfterDeth`) null (`self.SpawnRadius`) (`self.MinAmountOfSpawnActor`) (`self.MaxAmountOfSpawnActor`) null)))

(event `self.ReceiveTick`
  (params (DeltaSeconds :type "Float (single-precision)"))
  (`parent.ReceiveTick` DeltaSeconds)
  (if (> (`KismetMathLibrary.Vector_Distance` (`self.K2_GetActorLocation` (`self.GetOwner`)) (`self.K2_GetActorLocation`)) (`self.DistanceForDestroy`))
    (`/Engine/EditorBlueprintResources/StandardMacros.DoOnce` false
      (:`Completed`
        (`self.K2_DestroyActor` (stale `self.ReceiveBeginPlay` _returnvalue))
        (`self.K2_DestroyActor`)))))

(fn `UserConstructionScript`)