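; Camera component that manages a character's first-person and third-person view modes and tracks camera target points.
; Tick re-assigns ViewMode to itself, then caches the owner's transform as PivotTarget and the mesh's first-person socket location as FPTarget.
; ChangeViewMode toggles the mode, forcing third person when the owner's AC_StatComponent reports death.
; SetViewMode sets it directly, and the ViewMode RepNotify broadcasts OnViewModeChange.
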(event `self.ReceiveTick`
  (params (DeltaSeconds :type "Float (single-precision)"))
  (bind _returnvalue (`self.GetOwner`))
  (bind _ownermesh (`self.OwnerMesh`))
  (set `self.ViewMode` (`self._ViewMode`))
  (`/Engine/EditorBlueprintResources/StandardMacros.IsValid` _returnvalue
    (:`Is Valid`
      (set `self.PivotTarget` (`Actor.GetTransform` _returnvalue))
      (`/Engine/EditorBlueprintResources/StandardMacros.IsValid` _ownermesh
        (:`Is Valid`
          (set `self.FP_Target` (`SceneComponent.GetSocketLocation` _ownermesh (`self.FirstPersonCameraSocket`))))))))

(fn `ChangeViewMode`
  (if (not (`/Game/Skyway/Core/Stats/AC_StatComponent.IsDead` (`Actor.GetComponentByClass` (`self.GetOwner`) "/Game/Skyway/Core/Stats/AC_StatComponent.AC_StatComponent_C")))
    (set `self._ViewMode` (select `/Game/Skyway/Core/Engine/E_ViewMode` (`self._ViewMode`) :`NewEnumerator0` "NewEnumerator1" :`NewEnumerator1` "NewEnumerator0" :!type "/Game/Skyway/Core/Engine/E_ViewMode Enum"))
    (else
      (set `self._ViewMode` "NewEnumerator1"))))

(fn `OnRep__ViewMode`
  (`self.OnViewModeChange` (`self._ViewMode`)))

(fn `SetViewMode`
  (params (_ViewMode :type "/Game/Skyway/Core/Engine/E_ViewMode Enum" :default "NewEnumerator0"))
  (set `self._ViewMode` _ViewMode))