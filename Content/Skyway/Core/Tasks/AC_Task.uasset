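; Task component that runs the player's training quest chains from DT_TaskChains, showing task descriptions and granting experience, flash and item rewards.
; Once the world loads, it restores saved chains and binds to inventory, crafting, upgrade and ship-building events, mapping gameplay tags to action completions.
; Progress blends item counts with completed actions, saving on every update.
; Completed tasks advance the chain, and finished training chains unlock the next.
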(event `self.ReceiveBeginPlay`
  (bind _asgm_main (cast `/Game/Skyway/Core/Engine/GM_Main` (`GameplayStatics.GetGameMode`)))
  (set `self.GM_Main` _asgm_main))

(event `self.ReceiveTick`
  (params (DeltaSeconds :type "Float (single-precision)"))
  (bind _gm_main (`self.GM_Main`)
    (:`then`
      (if (`/Game/Skyway/Core/Engine/GM_Main.bWorldLoaded` _gm_main)
        (`|ExecutionSequence`
          (:`then_0`
            (`/Engine/EditorBlueprintResources/StandardMacros.DoOnce` false :!label _label
              (:`Completed`
                (bind _returnvalue (message `/Game/Skyway/Core/Engine/BPI_GameMode.GetSaveGame` (`GameplayStatics.GetGameMode`)))
                (`/Game/Skyway/Core/Engine/BPI_CanSave.LoadToPlayer` _returnvalue)
                (`KismetSystemLibrary.DelayUntilNextTick`)
                (`self.NewGameBegin`)
                (bind _output_get (set `self.OwnerInventoryComp` (`Actor.GetComponentByClass` (`self.GetOwner`) "/Game/Skyway/Core/Inventory/AC_Inventory.AC_Inventory_C")))
                (set `self.OwnerExpComp` (`Actor.GetComponentByClass` (`self.GetOwner`) "/Game/Skyway/Core/Expereance/AC_Expereance.AC_Expereance_C"))
                (bind _output_get_2 (set `self.OwnerCraftingComp` (`Actor.GetComponentByClass` (`self.GetOwner`) "/Game/Skyway/Core/Crafting/AC_Crafting.AC_Crafting_C")))
                (bind _output_get_3 (set `self.OwnerUpgradeComp` (`Actor.GetComponentByClass` (`self.GetOwner`) "/Game/Skyway/Core/Upgrade/AC_Upgrade.AC_Upgrade_C")))
                (add `/Game/Skyway/Core/Upgrade/AC_Upgrade.OnUpgradeActivate` _output_get_3 (`|CreateDelegate` :!event `OnUpgradeActivate`))
                (add `/Game/Skyway/Core/Crafting/AC_Crafting.OnStudyRecipe` _output_get_2 (`|CreateDelegate` :!event `OnStudyRecipe`))
                (bind _returnvalue_2 (`GameplayStatics.GetActorOfClass` "/Game/Skyway/Core/Ship/BP_Ship_Test.BP_Ship_Test_C"))
                (`/Engine/EditorBlueprintResources/StandardMacros.IsValid` _returnvalue_2
                  (:`Is Valid`
                    (bind _output_get_4 (set `self.PlayerShip` _returnvalue_2))
                    (add `/Game/Skyway/Core/Ship/BP_Ship_Base.OnBuildingSpawned` _output_get_4 (`|CreateDelegate` :!event `OnBuildingPlaced`)))
                  (:`Is Not Valid`
                    _))
                (add `/Game/Skyway/Core/Inventory/AC_Storage.OnItemAdded` _output_get (`|CreateDelegate` :!event `OnItemAdded_Event`))
                (add `self.OnTaskCompletePercentUpdate` (`|CreateDelegate` :!event `OnTaskCompletePercentUpdate_Event`))))))
        (else
          (goto _label :!via `Reset`))))
    (:`else`)))

(event `OnItemAdded_Event`
  (params (SlotInfo :type "/Game/Skyway/Core/Inventory/S_Slot_Info Structure") (AddedCount :type Integer))
  (`self.OnCraftItem` (`.ID_71_BA06E0BD4E97D16461377CB9BF36CE2D` (break `/Game/Skyway/Core/Inventory/S_Item_Info` (`.ItemInfo_14_7E8F48144F0F01654500E084A85436C5` (break `/Game/Skyway/Core/Inventory/S_Slot_Info` SlotInfo)))))
  (`self.CalcTaskProgress`))

(event `/Game/Skyway/Core/Engine/BPI_CanSave.SaveToPlayer`
  (params (SaveGame :type "SaveGame Object Reference"))
  (bind (_returnvalue _playerinfo) (message `/Game/Skyway/Core/Engine/BPI_SaveGame.LoadPlayer` SaveGame (`FileManager.GetPlayerName`)))
  (if _returnvalue
    (bind _structout (setmembers `/Game/Skyway/Core/Engine/S_PlayerInfo` :`StructRef` _playerinfo :`AllTaskChains` (`self.AllTaskChains`) :`CurrentTaskChain` (`self.CurrentTaskChain`)))
    (message `/Game/Skyway/Core/Engine/BPI_SaveGame.SavePlayer` SaveGame _structout)
    (else
      (bind _structout_2 (setmembers `/Game/Skyway/Core/Engine/S_PlayerInfo` :`StructRef` (`/Game/Skyway/Core/Engine/MLBP_Defaults.DEFAULT`) :`Name` (`FileManager.GetPlayerName`) :`AllTaskChains` (`self.AllTaskChains`) :`CurrentTaskChain` (`self.CurrentTaskChain`)))
      (message `/Game/Skyway/Core/Engine/BPI_SaveGame.SavePlayer` SaveGame _structout_2))))

(event `/Game/Skyway/Core/Engine/BPI_CanSave.LoadToPlayer`
  (params (SaveGame :type "SaveGame Object Reference"))
  (bind (_returnvalue _playerinfo) (message `/Game/Skyway/Core/Engine/BPI_SaveGame.LoadPlayer` SaveGame (`FileManager.GetPlayerName`)))
  (if _returnvalue
    (bind ((`AllTaskChains_25_F45CB33A4984185D6FA4E0AFF9C2034B` _alltaskchains) (`CurrentTaskChain_28_B8A39BB2437E86EE33F412ACE89125DC` _currenttaskchain)) (break `/Game/Skyway/Core/Engine/S_PlayerInfo` _playerinfo))
    (set `self.AllTaskChains` _alltaskchains)
    (set `self.CurrentTaskChain` _currenttaskchain)
    (`self.CalcTaskProgress`)))

(event `OnTaskCompletePercentUpdate_Event`
  (bind _returnvalue (message `/Game/Skyway/Core/Engine/BPI_GameMode.GetSaveGame` (`GameplayStatics.GetGameMode`)))
  (`self.SaveToPlayer` _returnvalue))

(fn `AddCompletePercentToCurrentTask`
  (params (Percent :type "Float (double-precision)"))
  (bind ((`Task_37_F243B44D4B614EEEE1517DBCEF91E53D` _task) (`CurrentTaskIndex_11_0FD1030F4BBB9E7445CBB486176018B2` _currenttaskindex)) (break `/Game/Skyway/Core/Tasks/S_TaskChain` (`self.CurrentTaskChain`)))
  (bind ((`Task_37_F243B44D4B614EEEE1517DBCEF91E53D` _task_2) (`CurrentTaskIndex_11_0FD1030F4BBB9E7445CBB486176018B2` _currenttaskindex_2)) (break `/Game/Skyway/Core/Tasks/S_TaskChain` (`self.CurrentTaskChain`)))
  (bind _output (`|GetArrayItem` _task _currenttaskindex))
  (bind _returnvalue (+ (`.CompletePercent_17_5764B4A843FB2668BDE1F1AEDDF87098` (break `/Game/Skyway/Core/Tasks/S_Task` (`|GetArrayItem` _task_2 _currenttaskindex_2))) (`local.Percent`)))
  (if (`KismetArrayLibrary.Array_IsValidIndex` _task_2 _currenttaskindex_2)
    (if (or (> _returnvalue 1.0) (`KismetMathLibrary.NearlyEqual_FloatFloat` _returnvalue 1.0 1e-05))
      (set `self.ProgressPercent` 1.0)
      (setmembers `/Game/Skyway/Core/Tasks/S_Task` :`StructRef` _output :`CompletePercent` 1.0)
      (set `self.CurrentTaskChain` (`self.CurrentTaskChain`))
      (`self.OnTaskCompletePercentUpdate`)
      (`KismetSystemLibrary.K2_SetTimer` null "CompleteCurrentTask" 1.0)
      (else
        (set `self.ProgressPercent` _returnvalue)
        (setmembers `/Game/Skyway/Core/Tasks/S_Task` :`StructRef` _output :`CompletePercent` _returnvalue)
        (set `self.CurrentTaskChain` (`self.CurrentTaskChain`))
        (`self.OnTaskCompletePercentUpdate`)))))

(fn `BeginTaskChain`)

(fn `CalcTaskProgress`
  (locals (L_AllItemsCount :type Integer) (L_InventoryItemsCount :type Integer) (L_AllActionsCount :type Integer) (L_CompleteActionsCount :type Integer))
  (bind ((`Task_37_F243B44D4B614EEEE1517DBCEF91E53D` _task) (`CurrentTaskIndex_11_0FD1030F4BBB9E7445CBB486176018B2` _currenttaskindex)) (break `/Game/Skyway/Core/Tasks/S_TaskChain` (`self.CurrentTaskChain`)))
  (bind ((`Task_37_F243B44D4B614EEEE1517DBCEF91E53D` _task_2) (`CurrentTaskIndex_11_0FD1030F4BBB9E7445CBB486176018B2` _currenttaskindex_2)) (break `/Game/Skyway/Core/Tasks/S_TaskChain` (`self.CurrentTaskChain`)))
  (bind ((`Task_37_F243B44D4B614EEEE1517DBCEF91E53D` _task_3) (`CurrentTaskIndex_11_0FD1030F4BBB9E7445CBB486176018B2` _currenttaskindex_3)) (break `/Game/Skyway/Core/Tasks/S_TaskChain` (`self.CurrentTaskChain`)))
  (bind ((`Task_37_F243B44D4B614EEEE1517DBCEF91E53D` _task_4) (`CurrentTaskIndex_11_0FD1030F4BBB9E7445CBB486176018B2` _currenttaskindex_4)) (break `/Game/Skyway/Core/Tasks/S_TaskChain` (`self.CurrentTaskChain`)))
  (bind ((`Task_37_F243B44D4B614EEEE1517DBCEF91E53D` _task_5) (`CurrentTaskIndex_11_0FD1030F4BBB9E7445CBB486176018B2` _currenttaskindex_5)) (break `/Game/Skyway/Core/Tasks/S_TaskChain` (`self.CurrentTaskChain`)))
  (bind _returnvalue (!= (`local.L_AllItemsCount`) 0))
  (bind _returnvalue_2 (/ (`KismetMathLibrary.Conv_IntToDouble` (`local.L_InventoryItemsCount`)) (`KismetMathLibrary.Conv_IntToDouble` (`local.L_AllItemsCount`))))
  (bind _returnvalue_3 (/ (`KismetMathLibrary.Conv_IntToDouble` (`local.L_CompleteActionsCount`)) (`KismetMathLibrary.Conv_IntToDouble` (`local.L_AllActionsCount`))))
  (bind ((`CompletePercent_17_5764B4A843FB2668BDE1F1AEDDF87098` _completepercent)) (break `/Game/Skyway/Core/Tasks/S_Task` (`|GetArrayItem` _task_2 _currenttaskindex_2)))
  (if (`KismetArrayLibrary.Array_IsValidIndex` _task _currenttaskindex)
    (for (_array_element _array_index) (`.ItemsForComplete_21_741010A140C025BC8475BC9FB3A2EC41` (break `/Game/Skyway/Core/Tasks/S_Task` (`|GetArrayItem` _task_4 _currenttaskindex_4)))
      (bind (_count _currentcount _itemid) (break `/Game/Skyway/Core/Tasks/S_ItemForCompleteTask` _array_element))
      (set `local.L_AllItemsCount` (+ _count (`local.L_AllItemsCount`)))
      (bind _ownerinventorycomp (`self.OwnerInventoryComp`)
        (:`then`
          (bind _returnvalue_4 (`/Game/Skyway/Core/Inventory/AC_Storage.FindCountItemById` _ownerinventorycomp _itemid))
          (bind _returnvalue_5 (select `bool` (> _currentcount _returnvalue_4) :`false` _returnvalue_4 :`true` _currentcount))
          (bind _returnvalue_6 (select `bool` (> _returnvalue_5 _count) :`false` _returnvalue_5 :`true` _count))
          (set `local.L_InventoryItemsCount` (+ (`local.L_InventoryItemsCount`) _returnvalue_6))
          (setmembers `/Game/Skyway/Core/Tasks/S_ItemForCompleteTask` :`StructRef` (`|GetArrayItem` (`.ItemsForComplete_21_741010A140C025BC8475BC9FB3A2EC41` (break `/Game/Skyway/Core/Tasks/S_Task` (`|GetArrayItem` _task_3 _currenttaskindex_3))) _array_index) :`CurrentCount` _returnvalue_6)
          (set `self.CurrentTaskChain` (`self.CurrentTaskChain`)))
        (:`else`)))
    (for _array_element_2 (`.ActionsForComplete_30_429583314AF60E279DEA538AEB7C6E5F` (break `/Game/Skyway/Core/Tasks/S_Task` (`|GetArrayItem` _task_5 _currenttaskindex_5)))
      (`/Engine/EditorBlueprintResources/StandardMacros.IncrementInt` (`local.L_AllActionsCount`)
        (:`  `
          (if (`.ActionComplete_5_A24780C84284573A2418D39EE8927255` (break `/Game/Skyway/Core/Tasks/S_TaskAction` _array_element_2))
            (`/Engine/EditorBlueprintResources/StandardMacros.IncrementInt` (`local.L_CompleteActionsCount`))))))
    (if (and _returnvalue (!= (`local.L_AllActionsCount`) 0))
      (`self.AddCompletePercentToCurrentTask` (- (/ (+ _returnvalue_2 _returnvalue_3) 2.0) _completepercent))
      (else
        (`self.AddCompletePercentToCurrentTask` (select `bool` _returnvalue :`false` (- _returnvalue_3 _completepercent) :`true` (- _returnvalue_2 _completepercent)))))))

(fn `CompleteActionById`
  (params (ActionId :type "GameplayTag Structure") (Anyway :type Boolean))
  (bind _alltaskchains (`self.AllTaskChains`))
  (bind ((`Task_37_F243B44D4B614EEEE1517DBCEF91E53D` _task) (`CurrentTaskIndex_11_0FD1030F4BBB9E7445CBB486176018B2` _currenttaskindex)) (break `/Game/Skyway/Core/Tasks/S_TaskChain` (`self.CurrentTaskChain`)))
  (bind ((`ActionsForComplete_30_429583314AF60E279DEA538AEB7C6E5F` _actionsforcomplete)) (break `/Game/Skyway/Core/Tasks/S_Task` (`|GetArrayItem` _task _currenttaskindex)))
  (if Anyway
    (for (_array_element _array_index) _alltaskchains
      (for (_array_element_2 _array_index_2) (`.Task_37_F243B44D4B614EEEE1517DBCEF91E53D` (break `/Game/Skyway/Core/Tasks/S_TaskChain` _array_element))
        (for (_array_element_3 _array_index_3) (`.ActionsForComplete_30_429583314AF60E279DEA538AEB7C6E5F` (break `/Game/Skyway/Core/Tasks/S_Task` _array_element_2))
          (if (== (`.ActionId_8_8DB485394FD92C3AC4CBCCAC68E81455` (break `/Game/Skyway/Core/Tasks/S_TaskAction` _array_element_3)) (`local.ActionId`))
            (setmembers `/Game/Skyway/Core/Tasks/S_TaskAction` :`StructRef` (`|GetArrayItem` (`.ActionsForComplete_30_429583314AF60E279DEA538AEB7C6E5F` (break `/Game/Skyway/Core/Tasks/S_Task` (`|GetArrayItem` (`.Task_37_F243B44D4B614EEEE1517DBCEF91E53D` (break `/Game/Skyway/Core/Tasks/S_TaskChain` (`|GetArrayItem` _alltaskchains _array_index))) _array_index_2))) _array_index_3) :`ActionComplete` true)
            (for _array_element_4 (`self.AllTaskChains`)
              (if (== (`.TaskChainId_2_5890888C4B297BFE194416978D2CB025` (break `/Game/Skyway/Core/Tasks/S_TaskChain` _array_element_4)) (`.TaskChainId_2_5890888C4B297BFE194416978D2CB025` (break `/Game/Skyway/Core/Tasks/S_TaskChain` (`self.CurrentTaskChain`))))
                (set `self.CurrentTaskChain` _array_element_4)
                (`self.CalcTaskProgress`)
                (return)))))))
    (elif (`KismetArrayLibrary.Array_IsValidIndex` _task _currenttaskindex)
      (for (_array_element_5 _array_index_4) _actionsforcomplete
        (if (== (`.ActionId_8_8DB485394FD92C3AC4CBCCAC68E81455` (break `/Game/Skyway/Core/Tasks/S_TaskAction` _array_element_5)) (`local.ActionId`))
          (setmembers `/Game/Skyway/Core/Tasks/S_TaskAction` :`StructRef` (`|GetArrayItem` _actionsforcomplete _array_index_4) :`ActionComplete` true)
          (set `self.CurrentTaskChain` (`self.CurrentTaskChain`))
          (`self.CalcTaskProgress`)
          (return))))))

(fn `CompleteCurrentTask`
  (bind _currenttaskchain (`self.CurrentTaskChain`))
  (bind ((`Task_37_F243B44D4B614EEEE1517DBCEF91E53D` _task) (`CurrentTaskIndex_11_0FD1030F4BBB9E7445CBB486176018B2` _currenttaskindex)) (break `/Game/Skyway/Core/Tasks/S_TaskChain` (`self.CurrentTaskChain`)))
  (bind ((`Task_37_F243B44D4B614EEEE1517DBCEF91E53D` _task_2) (`CurrentTaskIndex_11_0FD1030F4BBB9E7445CBB486176018B2` _currenttaskindex_2)) (break `/Game/Skyway/Core/Tasks/S_TaskChain` _currenttaskchain))
  (bind _output (`|GetArrayItem` _task _currenttaskindex))
  (bind ((`Name_10_77E568F24A2CC371C0627790A404173D` _name) (`Description_12_F8C4236B460F77C1C5BDE59B78E4CB1C` _description) (`ItemsForComplete_21_741010A140C025BC8475BC9FB3A2EC41` _itemsforcomplete) (`ActionsForComplete_30_429583314AF60E279DEA538AEB7C6E5F` _actionsforcomplete) (`Reward_24_2CFBAD1C4F3686789C5865A46F2DCBD5` _reward)) (break `/Game/Skyway/Core/Tasks/S_Task` (`|GetArrayItem` _task_2 _currenttaskindex_2)))
  (bind (_expereance _flash _items) (break `/Game/Skyway/Core/Tasks/S_Reward` (`.Reward_24_2CFBAD1C4F3686789C5865A46F2DCBD5` (break `/Game/Skyway/Core/Tasks/S_Task` _output))))
  (if (`KismetArrayLibrary.Array_IsValidIndex` _task _currenttaskindex)
    (`/Game/Skyway/Core/Expereance/AC_Expereance.AddExpereance` (`self.OwnerExpComp`) _expereance)
    (`/Game/Skyway/Core/Expereance/AC_Expereance.AddFlash` (`self.OwnerExpComp`) _flash)
    (for _array_element _items
      (bind (_itemid _amount) (break `/Game/Skyway/Core/Tasks/S_Item` _array_element))
      (`/Game/Skyway/Core/Inventory/AC_Storage.AddItem` (`self.OwnerInventoryComp`) _itemid _amount))
    (setmembers `/Game/Skyway/Core/Tasks/S_Task` :`StructRef` _output :`CompletePercent` 1.0)
    (setmembers `/Game/Skyway/Core/Tasks/S_TaskChain` :`StructRef` _currenttaskchain :`CurrentTaskIndex` (+ _currenttaskindex_2 1))
    (set `self.CurrentTaskChain` (`self.CurrentTaskChain`))
    (`self.OnTaskComplete`)
    (`self.CalcTaskProgress`)
    (if (not (`KismetArrayLibrary.Array_IsValidIndex` _task_2 _currenttaskindex_2))
      (`self.CompleteCurrentTaskChain`)
      (else
        (bind _returnvalue (`|CreateWidget` "/Game/Skyway/Core/UI/Task/WBP_TaskDescription.WBP_TaskDescription_C" null _itemsforcomplete _description _name _actionsforcomplete _reward))
        (`UserWidget.AddToViewport` _returnvalue 0)))
    (return)
    (else
      (`self.CompleteCurrentTaskChain`)
      (return))))

(fn `CompleteCurrentTaskChain`
  (bind _alltaskchains (`self.AllTaskChains`))
  (bind _currenttaskchain (`self.CurrentTaskChain`))
  (bind _alltaskchains_2 (`self.AllTaskChains`))
  (bind ((`Task_37_F243B44D4B614EEEE1517DBCEF91E53D` _task)) (break `/Game/Skyway/Core/Tasks/S_TaskChain` (`self.CurrentTaskChain`)))
  (for (_ _array_index) _task
    (setmembers `/Game/Skyway/Core/Tasks/S_Task` :`StructRef` (`|GetArrayItem` _task _array_index) :`CompletePercent` 1.0))
  (setmembers `/Game/Skyway/Core/Tasks/S_TaskChain` :`StructRef` _currenttaskchain :`CurrentTaskIndex` -1)
  (set `self.CurrentTaskChain` _currenttaskchain)
  (`self.OnTaskChainComplete`)
  (if (== (`.TaskChainId_2_5890888C4B297BFE194416978D2CB025` (break `/Game/Skyway/Core/Tasks/S_TaskChain` _currenttaskchain)) (struct :`TagName` "Task.Train"))
    (for (_array_element _array_index_2) _alltaskchains_2
      (bind ((`TaskChainId_2_5890888C4B297BFE194416978D2CB025` _taskchainid)) (break `/Game/Skyway/Core/Tasks/S_TaskChain` _array_element))
      (if (== _taskchainid (struct :`TagName` "Task.Train2"))
        (setmembers `/Game/Skyway/Core/Tasks/S_TaskChain` :`StructRef` (`|GetArrayItem` _alltaskchains_2 _array_index_2) :`Available` true)
        (`self.SetCurrentTaskChain` _taskchainid)))
    (elif (== (`.TaskChainId_2_5890888C4B297BFE194416978D2CB025` (break `/Game/Skyway/Core/Tasks/S_TaskChain` (`self.CurrentTaskChain`))) (struct :`TagName` "Task.Train2"))
      (for (_array_element_2 _array_index_3) _alltaskchains
        (bind ((`TaskChainId_2_5890888C4B297BFE194416978D2CB025` _taskchainid_2)) (break `/Game/Skyway/Core/Tasks/S_TaskChain` _array_element_2))
        (if (== _taskchainid_2 (struct :`TagName` "Task.Train3"))
          (setmembers `/Game/Skyway/Core/Tasks/S_TaskChain` :`StructRef` (`|GetArrayItem` _alltaskchains _array_index_3) :`Available` true)
          (`self.SetCurrentTaskChain` _taskchainid_2))))))

(fn `InitAllTaskChains`
  (bind _outrownames (`DataTableFunctionLibrary.GetDataTableRowNames` "/Game/Skyway/Core/Tasks/DT_TaskChains.DT_TaskChains"))
  (for _array_element _outrownames
    (bind _returnvalue (`|GetDataTableRow` "/Game/Skyway/Core/Tasks/DT_TaskChains.DT_TaskChains" _array_element)
      (:`then`
        (`KismetArrayLibrary.Array_Add` (`self.AllTaskChains`) _returnvalue)))))

(fn `NewGameBegin`
  (if (not (`BlueprintGameplayTagLibrary.IsGameplayTagValid` (`.TaskChainId_2_5890888C4B297BFE194416978D2CB025` (break `/Game/Skyway/Core/Tasks/S_TaskChain` (`self.CurrentTaskChain`)))))
    (cast `/Game/Skyway/Core/AI/NPC/BP_MainMenuNpc` (`self.GetOwner`)
      (:`CastFailed`
        (bind _returnvalue (`|GetDataTableRow` "/Game/Skyway/Core/Tasks/DT_TaskChains.DT_TaskChains" "Task.Train")
          (:`then`
            (bind _output_get (set `self.CurrentTaskChain` _returnvalue))
            (`self.InitAllTaskChains`)
            (bind ((`Task_37_F243B44D4B614EEEE1517DBCEF91E53D` _task) (`CurrentTaskIndex_11_0FD1030F4BBB9E7445CBB486176018B2` _currenttaskindex)) (break `/Game/Skyway/Core/Tasks/S_TaskChain` _output_get))
            (bind ((`Name_10_77E568F24A2CC371C0627790A404173D` _name) (`Description_12_F8C4236B460F77C1C5BDE59B78E4CB1C` _description) (`ItemsForComplete_21_741010A140C025BC8475BC9FB3A2EC41` _itemsforcomplete) (`ActionsForComplete_30_429583314AF60E279DEA538AEB7C6E5F` _actionsforcomplete) (`Reward_24_2CFBAD1C4F3686789C5865A46F2DCBD5` _reward)) (break `/Game/Skyway/Core/Tasks/S_Task` (`|GetArrayItem` _task _currenttaskindex)))
            (bind _returnvalue_2 (`|CreateWidget` "/Game/Skyway/Core/UI/Task/WBP_TaskDescription.WBP_TaskDescription_C" null _itemsforcomplete _description _name _actionsforcomplete _reward))
            (`UserWidget.AddToViewport` _returnvalue_2 0)))))))

(fn `OnBuildingPlaced`
  (params (SpawnedBuilding :type "/Game/Skyway/Core/Building/AC_Building_Base Object Reference") (Parent :type "/Game/Skyway/Core/Building/AC_Building_Base Object Reference"))
  (if (`KismetMathLibrary.ClassIsChildOf` (`GameplayStatics.GetObjectClass` (`local.SpawnedBuilding`)) "/Game/Skyway/Core/Building/AC_PlacedBuilding_Base.AC_PlacedBuilding_Base_C")
    (`|SwitchGameplayTag` (`/Game/Skyway/Core/Building/AC_Building_Base.BuildingId` (`local.SpawnedBuilding`))
      (:`Item.Building.Furnace_2`
        (`self.CompleteActionById` (struct :`TagName` "Action.PlaceFurnace_2") true))
      (:`Item.Building.Accumulator`
        (`self.CompleteActionById` (struct :`TagName` "Action.PlaceAcum") true))
      (:`Item.Building.Furnace`
        (`self.CompleteActionById` (struct :`TagName` "Action.PlaceShredderOrFurnace") true :!label _label))
      (:`Item.Building.Shredder`
        (goto _label))
      (:`Item.Building.Generator`
        (`self.CompleteActionById` (struct :`TagName` "Action.PlaceGenerator") true))
      (:`Item.Building.Engine`
        (`self.CompleteActionById` (struct :`TagName` "Action.PlaceEngine") true))
      (:`Item.Building.Windmill`
        (`self.CompleteActionById` (struct :`TagName` "Action.PlaceWindmill") true)))
    (else
      (`|SwitchGameplayTag` (`/Game/Skyway/Core/Building/AC_Building_Base.BuildingId` (`local.SpawnedBuilding`))
        (:`Item.Building.FoundationTriangular`
          _)
        (:`Item.Building.Foundation`
          _))
      (`self.CompleteActionById` (struct :`TagName` "Action.PlaceShipBuilding")))))

(fn `OnCraftItem`
  (params (Selection :type "GameplayTag Structure"))
  (`|SwitchGameplayTag` Selection
    (:`Item.Building.Furnace`
      (`self.CompleteActionById` (struct :`TagName` "Action.CraftFurnaceOrShredder") true :!label _label))
    (:`Item.Building.Shredder`
      (goto _label))
    (:`Item.Building.Generator`
      (`self.CompleteActionById` (struct :`TagName` "Action.CraftGenerator") true))
    (:`Item.Building.Accumulator`
      (`self.CompleteActionById` (struct :`TagName` "Action.CraftAccum") true))
    (:`Item.Building.Windmill`
      (`self.CompleteActionById` (struct :`TagName` "Action.CraftWindmill") true))
    (:`Item.Building.Engine`
      (`self.CompleteActionById` (struct :`TagName` "Action.CraftEngine") true))))

(fn `OnRep_CurrentTaskChain`
  (for (_array_element _array_index) (`self.AllTaskChains`)
    (if (== (`.TaskChainId_2_5890888C4B297BFE194416978D2CB025` (break `/Game/Skyway/Core/Tasks/S_TaskChain` (`self.CurrentTaskChain`))) (`.TaskChainId_2_5890888C4B297BFE194416978D2CB025` (break `/Game/Skyway/Core/Tasks/S_TaskChain` _array_element)))
      (`KismetArrayLibrary.Array_Set` (`self.AllTaskChains`) _array_index (`self.CurrentTaskChain`))
      (return))))

(fn `OnStudyRecipe`
  (params (RecipeId :type "GameplayTag Structure"))
  (`|SwitchGameplayTag` RecipeId
    (:`Recipe.Player.Furnace_2`
      (`self.CompleteActionById` (struct :`TagName` "Action.StudyFurnace_2") true))
    (:`Recipe.Player.Furnace`
      (`self.CompleteActionById` (struct :`TagName` "Action.StudyFurnaceOrShredder") true :!label _label))
    (:`Recipe.Player.Shredder`
      (goto _label))
    (:`Recipe.Player.Generator`
      (`self.CompleteActionById` (struct :`TagName` "Action.StudyGenerator") true))
    (:`Recipe.Player.Accum`
      (`self.CompleteActionById` (struct :`TagName` "Action.StudyAcum") true))))

(fn `OnUpgradeActivate`
  (params (UpgradeInfo :type "/Game/Skyway/Core/Upgrade/S_UpgradeInfo Structure"))
  (`self.CompleteActionById` (struct :`TagName` "Action.FirstUpgrade") true)
  (`|SwitchGameplayTag` (`.Id_16_C698D4794DE27ACE1B0B23BCD391E817` (break `/Game/Skyway/Core/Upgrade/S_UpgradeInfo` UpgradeInfo))))

(fn `SetCurrentTaskChain`
  (params (TaskChainId :type "GameplayTag Structure"))
  (for _array_element (`self.AllTaskChains`)
    (bind ((`TaskChainId_2_5890888C4B297BFE194416978D2CB025` _taskchainid) (`Task_37_F243B44D4B614EEEE1517DBCEF91E53D` _task) (`CurrentTaskIndex_11_0FD1030F4BBB9E7445CBB486176018B2` _currenttaskindex)) (break `/Game/Skyway/Core/Tasks/S_TaskChain` _array_element))
    (if (== _taskchainid (`local.TaskChainId`))
      (if (and (!= _currenttaskindex -1) (`.Available_16_7D6A1A994DCDFCF060E03B94841EB89F` (break `/Game/Skyway/Core/Tasks/S_TaskChain` _array_element)))
        (set `self.CurrentTaskChain` _array_element)
        (`self.CalcTaskProgress`)
        (`self.OnTaskChainUpdate`)
        (return)))))