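; Ship Blueprint that manages the player's respawn point on a buildable ship and switches music for raids.
; The respawn component attaches to newly spawned charging stations; when its parent is destroyed it seeks another, falling back to random floor or foundation pieces if still on the root.
; The parent building's GUID persists through save/load, and the player teleports there once the world loads.
; Raid events start battle music and damp it afterwards.
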(event `self.ReceiveBeginPlay`
  (bind _spawnresources (`self.SpawnResources`))
  (`parent.ReceiveBeginPlay`)
  (add `/Game/Skyway/Core/Ship/Spawn/AC_SpawnResources.OnRaidBegin` _spawnresources (`|CreateDelegate` :!event `OnRaidBegin_Event`))
  (add `/Game/Skyway/Core/Ship/Spawn/AC_SpawnResources.OnRaidEnd` _spawnresources (`|CreateDelegate` :!event `OnRaidEnd_Event`))
  (bind _asgm_main (cast `/Game/Skyway/Core/Engine/GM_Main` (`GameplayStatics.GetGameMode`)))
  (set `self.GM_Main` _asgm_main))

(event `self.OnWeatherChange`
  (params (Speed :type "Float (double-precision)") (Direction :type "Vector Structure"))
  (`parent.OnWeatherChange` Speed Direction))

(event `TeleportPlayer_SERVER`
  (params (Player :type "Pawn Object Reference"))
  (`self.K2_SetActorLocation` Player (`SceneComponent.K2_GetComponentLocation` (`self.RespawnLocation`)) false true))

(event `/Game/Skyway/Core/Engine/BPI_CanSave.Save`
  (params (SaveGame :type "SaveGame Object Reference"))
  (bind _returnvalue (message `/Game/Skyway/Core/Building/BPI_Build.GetShipBuildingInfo` (`SceneComponent.GetAttachParent` (`self.RespawnLocation`))))
  (setmembers `/Game/Skyway/Core/Engine/S_ShipInfo` :`StructRef` (`self.ShipInfo`) :`RespawnBuildingGuid` (`.Guid_51_E783821C442F8F3AEE949A989634E84B` (break `/Game/Skyway/Core/Engine/S_ShipBuildingInfo` _returnvalue)))
  (`parent.Save` SaveGame))

(event `/Game/Skyway/Core/Engine/BPI_CanSave.Load`
  (params (SaveGame :type "SaveGame Object Reference"))
  (`parent.Load` SaveGame)
  (bind (_returnvalue _findbuilding) (`self.FindBuildingByGuid` (`.RespawnBuildingGuid_22_DFBEE2774485E509A52902A22C7745DF` (break `/Game/Skyway/Core/Engine/S_ShipInfo` (`self.ShipInfo`)))))
  (`self.AttachRespawnLocationComponent` _findbuilding))

(event `self.ReceiveTick`
  (params (DeltaSeconds :type "Float (single-precision)"))
  (`parent.ReceiveTick` DeltaSeconds)
  (`|ExecutionSequence`
    (:`then_0`
      (if (`/Game/Skyway/Core/Engine/GM_Main.bWorldLoaded` (`self.GM_Main`))
        (`/Engine/EditorBlueprintResources/StandardMacros.DoOnce` false :!label _label
          (:`Completed`
            (`self.TeleportPlayer_SERVER` (`GameplayStatics.GetPlayerCharacter` 0))))
        (else
          (goto _label :!via `Reset`))))))

(event `OnRaidBegin_Event`
  (`|ExecutionSequence`
    (:`then_0`
      (`AudioComponent.SetSound` (`/Game/Skyway/Core/Engine/GM_Main.Audio` (`self.GM_Main`)) "/Game/Skyway/Audio/Cues/battle-skyway_Cue.battle-skyway_Cue")
      (`AudioComponent.Play` (`/Game/Skyway/Core/Engine/GM_Main.Audio` (`self.GM_Main`)) 0.0))
    (:`then_1`
      (goto _label_2 :!via `Reset`))))

(event `OnRaidEnd_Event`
  (`/Engine/EditorBlueprintResources/StandardMacros.DoOnce` false :!label _label_2
    (:`Completed`
      (`/Game/Skyway/Core/Engine/GM_Main.DampingCurrentSound` (`self.GM_Main`) 15.0))))

(fn `AttachRespawnLocationComponent`
  (params (Parent :type "SceneComponent Object Reference"))
  (locals (L_RespawnOffset :type "Vector Structure" :default (0.0 0.0 100.0)))
  (`SceneComponent.K2_AttachToComponent` (`self.RespawnLocation`) Parent "None" "SnapToTarget" "SnapToTarget" "SnapToTarget" true)
  (`SceneComponent.K2_SetRelativeLocation` (`self.RespawnLocation`) (+ (`SceneComponent.RelativeLocation` (`self.RespawnLocation`)) (`local.L_RespawnOffset`)) false false)
  (bind _returnvalue (message `/Game/Skyway/Core/Building/BPI_Build.GetShipBuildingInfo` (`local.Parent`)))
  (setmembers `/Game/Skyway/Core/Engine/S_ShipInfo` :`StructRef` (`self.ShipInfo`) :`RespawnBuildingGuid` (`.Guid_51_E783821C442F8F3AEE949A989634E84B` (break `/Game/Skyway/Core/Engine/S_ShipBuildingInfo` _returnvalue))))

(fn `OnBuildingSpawned_Event`
  (params (SpawnedBuilding :type "/Game/Skyway/Core/Building/AC_Building_Base Object Reference") (Parent :type "/Game/Skyway/Core/Building/AC_Building_Base Object Reference"))
  (`parent.OnBuildingSpawned_Event` SpawnedBuilding Parent)
  (if (== "/Game/Skyway/Core/Building/AC_Building_ChargingStation.AC_Building_ChargingStation_C" (`GameplayStatics.GetObjectClass` (`local.SpawnedBuilding`)))
    (`self.UpdateRespawnLocation` (`local.SpawnedBuilding`))))

(fn `OnDestroyBuilding_Event`
  (params (DestroyedBuilding :type "/Game/Skyway/Core/Building/AC_Building_Base Object Reference"))
  (`|ExecutionSequence`
    (:`then_0`
      (if (== (`local.DestroyedBuilding`) (`SceneComponent.GetAttachParent` (`self.RespawnLocation`)))
        (`self.UpdateRespawnLocation` null)
        (return)
        (else
          (return))))
    (:`then_1`
      (`parent.OnDestroyBuilding_Event` (`local.DestroyedBuilding`))
      (return))))

(fn `UpdateRespawnLocation`
  (params (NewChargingStation :type "/Game/Skyway/Core/Building/AC_Building_Base Object Reference"))
  (locals (L_RandomBuilding :type "/Game/Skyway/Core/Building/AC_Building_Base Object Reference") (L_RespawnOffset :type "Vector Structure" :default (0.0 0.0 100.0)))
  (bind _returnvalue (`GameplayStatics.GetObjectClass` (`local.L_RandomBuilding`)))
  (`/Engine/EditorBlueprintResources/StandardMacros.IsValid` NewChargingStation
    (:`Is Valid`
      (`self.AttachRespawnLocationComponent` (`local.NewChargingStation`))
      (return))
    (:`Is Not Valid`
      (for _array_element (`self.Buildings`)
        (if (== (`GameplayStatics.GetObjectClass` _array_element) "/Game/Skyway/Core/Building/AC_Building_ChargingStation.AC_Building_ChargingStation_C")
          (`self.AttachRespawnLocationComponent` _array_element)
          (return)))
      (while (== (`SceneComponent.GetAttachParent` (`self.RespawnLocation`)) (`self.DefaultSceneRoot`))
        (set `local.L_RandomBuilding` (`KismetArrayLibrary.Array_Random` (`self.Buildings`)))
        (if (or (== _returnvalue "/Game/Skyway/Core/Building/ShipBuildings/AC_Building_Foundation.AC_Building_Foundation_C") (== _returnvalue "/Game/Skyway/Core/Building/ShipBuildings/AC_Building_Foundation_Triangular.AC_Building_Foundation_Triangular_C") (== _returnvalue "/Game/Skyway/Core/Building/ShipBuildings/AC_Building_Floor.AC_Building_Floor_C") (== _returnvalue "/Game/Skyway/Core/Building/ShipBuildings/AC_Building_Floor_Triangular.AC_Building_Floor_Triangular_C"))
          (`self.AttachRespawnLocationComponent` (`local.L_RandomBuilding`))))
      (return))))

(fn `UserConstructionScript`
  (`parent.UserConstructionScript`))