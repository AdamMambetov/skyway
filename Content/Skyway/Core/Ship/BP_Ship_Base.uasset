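; Base player-buildable ship: building components attach at runtime through server events and form a GUID parent/child tree.
; Each tick it sums active engine thrust and BP_Wind weather, subtracts a per-foundation speed penalty and moves the actor; an active island-locked harpoon stops it.
; Removal is refused for the workbench, parents of placed devices or at one foundation, otherwise children re-parent.
; Save/Load rebuilds buildings from saved ShipInfo.
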(event `self.ReceiveBeginPlay`
  (`parent.ReceiveBeginPlay`)
  (add `self.OnBuildingSpawned` (`|CreateDelegate` :!event `OnBuildingSpawned_Event`))
  (`KismetArrayLibrary.Array_Clear` (`self.Buildings`))
  (set `self.FoundationCount` 0)
  (for _array_element (`SceneComponent.GetChildrenComponents` (`self.DefaultSceneRoot`) true)
    (bind _asac_building_base (cast `/Game/Skyway/Core/Building/AC_Building_Base` _array_element))
    (`KismetArrayLibrary.Array_AddUnique` (`self.Buildings`) _asac_building_base)
    (if (`/Game/Skyway/Core/Engine/FLBP_Defaults.IsPlacedBuilding` (`/Game/Skyway/Core/Building/AC_Building_Base.BuildingId` _asac_building_base))
      (`KismetArrayLibrary.Array_Add` (`self.Devices`) (cast `/Game/Skyway/Core/Building/AC_PlacedBuilding_Base` _asac_building_base :!pure true))
      (else
        (bind _returnvalue (`GameplayStatics.GetObjectClass` _asac_building_base))
        (if (or (== _returnvalue "/Game/Skyway/Core/Building/ShipBuildings/AC_Building_Foundation.AC_Building_Foundation_C") (== _returnvalue "/Game/Skyway/Core/Building/ShipBuildings/AC_Building_Foundation_Triangular.AC_Building_Foundation_Triangular_C"))
          (set `self.FoundationCount` (+ 1 (`self.FoundationCount`)))))))
  (bind _returnvalue_2 (`GameplayStatics.GetActorOfClass` "/Game/Skyway/Core/Weather/BP_Wind.BP_Wind_C"))
  (`/Engine/EditorBlueprintResources/StandardMacros.IsValid` _returnvalue_2
    (:`Is Valid`
      (set `self.WeatherSpeed` (`/Game/Skyway/Core/Weather/BP_Wind.Speed` _returnvalue_2))
      (set `self.WeatherDirection` (`/Game/Skyway/Core/Weather/BP_Wind.Direction` _returnvalue_2))
      (add `/Game/Skyway/Core/Weather/BP_Wind.OnWeatherChange` _returnvalue_2 (`|CreateDelegate` :!event `OnWeatherChange`))
      (bind _returnvalue_3 (message `/Game/Skyway/Core/Engine/BPI_GameMode.GetSaveGame` (`GameplayStatics.GetGameMode`)))
      (`/Engine/EditorBlueprintResources/StandardMacros.IsValid` _returnvalue_3
        (:`Is Valid`
          (bind _returnvalue_4 (message `/Game/Skyway/Core/Engine/BPI_SaveGame.LoadShip` _returnvalue_3))
          (if _returnvalue_4
            (`/Game/Skyway/Core/Engine/BPI_CanSave.Load` _returnvalue_3)))))))

(event `self.ReceiveTick`
  (params (DeltaSeconds :type "Float (single-precision)"))
  (`self.CalculateDirectionAndSpeed`)
  (`self.Move`)
  (`/Game/Skyway/Core/Ship/Spawn/AC_SpawnResources.SetSpawnDirection` (`self.SpawnResources`) (`self.Direction`)))

(event `OnWeatherChange`
  (params (Speed :type "Float (double-precision)") (Direction :type "Vector Structure"))
  (set `self.WeatherSpeed` Speed)
  (set `self.WeatherDirection` Direction))

(event `Build_SERVER`
  (params (BuildingInfo :type "/Game/Skyway/Core/Inventory/S_Building_Info Structure") (HitBuildingComp :type "SceneComponent Object Reference") (BuildingWorldTransform :type "Transform Structure"))
  (bind ((`Class_9_55C23E17411E821DD83085AA79CC3C29` _class)) (break `/Game/Skyway/Core/Inventory/S_Building_Info` BuildingInfo))
  (bind ((`Class_9_55C23E17411E821DD83085AA79CC3C29` _class_2)) (break `/Game/Skyway/Core/Inventory/S_Building_Info` BuildingInfo))
  (bind _returnvalue (`/Game/Skyway/Core/Engine/FLBP_Defaults.ConvertWorldTransformToRelative` (`self.GetTransform`) BuildingWorldTransform))
  (bind _returnvalue_2 (`|AddComponentByClass` _class_2 false _returnvalue (make `/Game/Skyway/Core/Engine/S_ShipBuildingInfo` :`Class` _class_2 :`RelativeTransform` _returnvalue :`Guid` (`KismetGuidLibrary.NewGuid`) :`ParentGuid` (`.Guid_51_E783821C442F8F3AEE949A989634E84B` (break `/Game/Skyway/Core/Engine/S_ShipBuildingInfo` (`/Game/Skyway/Core/Building/AC_Building_Base.ShipBuildingInfo` (cast `/Game/Skyway/Core/Building/AC_Building_Base` (select `bool` (`KismetSystemLibrary.DoesImplementInterface` HitBuildingComp "/Game/Skyway/Core/Building/BPI_Build.BPI_Build_C") :`false` (`SceneComponent.GetAttachParent` HitBuildingComp) :`true` HitBuildingComp) :!pure true)))))))
  (`KismetArrayLibrary.Array_Add` (`self.Buildings`) _returnvalue_2)
  (`|ExecutionSequence`
    (:`then_0`
      (`self.OnBuildingSpawned` _returnvalue_2 (cast `/Game/Skyway/Core/Building/AC_Building_Base` (select `bool` (`KismetSystemLibrary.DoesImplementInterface` HitBuildingComp "/Game/Skyway/Core/Building/BPI_Build.BPI_Build_C") :`false` (`SceneComponent.GetAttachParent` HitBuildingComp) :`true` HitBuildingComp) :!pure true)))
    (:`then_1`
      (if (`KismetMathLibrary.ClassIsChildOf` (`.Class_9_55C23E17411E821DD83085AA79CC3C29` (break `/Game/Skyway/Core/Inventory/S_Building_Info` BuildingInfo)) "/Game/Skyway/Core/Building/AC_PlacedBuilding_Base.AC_PlacedBuilding_Base_C")
        (if (`/Game/Skyway/Core/Engine/FLBP_Defaults.IsPlacedBuilding` (`/Game/Skyway/Core/Building/AC_Building_Base.BuildingId` _returnvalue_2))
          (`KismetArrayLibrary.Array_Add` (`self.Devices`) (cast `/Game/Skyway/Core/Building/AC_PlacedBuilding_Base` _returnvalue_2 :!pure true)))
        (elif (or (== _class null) (== _class null))
          (`self.AddFoundationCount_SERVER`))))))

(event `UpdateAllBuildingCollisions_SERVER`
  (`self.UpdateAllBuildingCollisions`))

(event `DestroyComponent_SERVER`
  (params (Component :type "ActorComponent Object Reference"))
  (`ActorComponent.K2_DestroyComponent` Component)
  (if (`KismetSystemLibrary.DoesImplementInterface` Component "/Game/Skyway/Core/Building/BPI_Build.BPI_Build_C")
    (bind _asac_building_base (cast `/Game/Skyway/Core/Building/AC_Building_Base` Component))
    (`KismetArrayLibrary.Array_RemoveItem` (`self.Buildings`) _asac_building_base)
    (bind _asac_placed_building_base (cast `/Game/Skyway/Core/Building/AC_PlacedBuilding_Base` Component))
    (`KismetArrayLibrary.Array_RemoveItem` (`self.Devices`) _asac_placed_building_base)))

(event `AddFoundationCount_SERVER`
  (set `self.FoundationCount` (+ (`self.FoundationCount`) 1)))

(event `/Game/Skyway/Core/Engine/BPI_CanSave.Save`
  (params (SaveGame :type "SaveGame Object Reference"))
  (set `self.ShipInfo` (`/Game/Skyway/Core/Engine/MLBP_Defaults.DEFAULT`))
  (`/Game/Skyway/Core/Engine/FLBP_Defaults.SaveActorComponents` self SaveGame)
  (message `/Game/Skyway/Core/Engine/BPI_SaveGame.SaveShip` SaveGame (`self.ShipInfo`)))

(event `/Game/Skyway/Core/Engine/BPI_CanSave.Load`
  (params (SaveGame :type "SaveGame Object Reference"))
  (bind (_returnvalue _shipinfo) (message `/Game/Skyway/Core/Engine/BPI_SaveGame.LoadShip` SaveGame))
  (if _returnvalue
    (`self.DestroyAllBuildings`)
    (bind _output_get (set `self.ShipInfo` _shipinfo))
    (for _array_element (`.ShipBuildingsInfo_18_ECE6E3D64E66EC500AF7D7931B9A275F` (break `/Game/Skyway/Core/Engine/S_ShipInfo` _output_get))
      (bind ((`Class_2_EE10482842247968BBA769AB25C96EE5` _class) (`RelativeTransform_61_ADB221C3429CCCF8EB6D4EBC279E2078` _relativetransform)) (break `/Game/Skyway/Core/Engine/S_ShipBuildingInfo` _array_element))
      (bind _returnvalue_2 (`|AddComponentByClass` _class false _relativetransform _array_element))
      (`KismetArrayLibrary.Array_Add` (`self.Buildings`) _returnvalue_2)
      (if (`KismetMathLibrary.ClassIsChildOf` _class "/Game/Skyway/Core/Building/AC_PlacedBuilding_Base.AC_PlacedBuilding_Base_C")
        (if (`/Game/Skyway/Core/Engine/FLBP_Defaults.IsPlacedBuilding` (`/Game/Skyway/Core/Building/AC_Building_Base.BuildingId` _returnvalue_2))
          (`KismetArrayLibrary.Array_Add` (`self.Devices`) (cast `/Game/Skyway/Core/Building/AC_PlacedBuilding_Base` _returnvalue_2 :!pure true)))
        (elif (or (== _class null) (== _class null))
          (set `self.FoundationCount` (+ 1 (`self.FoundationCount`))))))
    (`/Game/Skyway/Core/Engine/FLBP_Defaults.LoadActorComponents` self SaveGame)))

(event `/Game/Skyway/Core/Ship/BPI_Ship.SetShipBuildingInfo`
  (params (ShipBuildingInfo :type "/Game/Skyway/Core/Engine/S_ShipBuildingInfo Structure"))
  (bind ((`Guid_51_E783821C442F8F3AEE949A989634E84B` _guid)) (break `/Game/Skyway/Core/Engine/S_ShipBuildingInfo` ShipBuildingInfo))
  (if (`KismetGuidLibrary.IsValid_Guid` _guid)
    (bind (_returnvalue _index) (`/Game/Skyway/Core/Ship/BPI_Ship.GetShipBuildingInfo` _guid))
    (if (!= _index -1)
      (`KismetArrayLibrary.Array_Set` (`.ShipBuildingsInfo_18_ECE6E3D64E66EC500AF7D7931B9A275F` (break `/Game/Skyway/Core/Engine/S_ShipInfo` (`self.ShipInfo`))) _index ShipBuildingInfo)
      (else
        (`KismetArrayLibrary.Array_Add` (`.ShipBuildingsInfo_18_ECE6E3D64E66EC500AF7D7931B9A275F` (break `/Game/Skyway/Core/Engine/S_ShipInfo` (`self.ShipInfo`))) ShipBuildingInfo)))))

(event `OnBuildingSpawned_Event` :!signature `self.OnBuildingSpawned`
  (params (SpawnedBuilding :type "/Game/Skyway/Core/Building/AC_Building_Base Object Reference") (Parent :type "/Game/Skyway/Core/Building/AC_Building_Base Object Reference"))
  (bind _shipbuildinginfo (`/Game/Skyway/Core/Building/AC_Building_Base.ShipBuildingInfo` Parent))
  (bind _structout (setmembers `/Game/Skyway/Core/Engine/S_ShipBuildingInfo` :`StructRef` (`/Game/Skyway/Core/Building/AC_Building_Base.ShipBuildingInfo` SpawnedBuilding) :`ParentGuid` (`.Guid_51_E783821C442F8F3AEE949A989634E84B` (break `/Game/Skyway/Core/Engine/S_ShipBuildingInfo` _shipbuildinginfo))))
  (`KismetArrayLibrary.Array_Add` (`.GuidOfChildren_55_2B4951EC46466E24FBB4398102287EB0` (break `/Game/Skyway/Core/Engine/S_ShipBuildingInfo` _shipbuildinginfo)) (`.Guid_51_E783821C442F8F3AEE949A989634E84B` (break `/Game/Skyway/Core/Engine/S_ShipBuildingInfo` _structout))))

(fn `Build`
  (params (BuildingInfo :type "/Game/Skyway/Core/Inventory/S_Building_Info Structure") (HitBuildingComponent :type "SceneComponent Object Reference") (BuildingWorldTransform :type "Transform Structure"))
  (locals (L_Building :type "Object Object Reference"))
  (`self.Build_SERVER` BuildingInfo HitBuildingComponent BuildingWorldTransform))

(fn `CalculateDirectionAndSpeed`
  (locals (L_EngineId :type "GameplayTag Structure" :default (struct :`TagName` "Item.Building.Engine")) (L_Engine :type "/Game/Skyway/Core/Building/Consumers/AC_Building_Engine Object Reference") (L_FinalDirection :type "Vector Structure" :default (0.0 0.0 0.0)) (L_FinalSpeed :type "Float (double-precision)" :default 0.0) (L_HarpoonId :type "GameplayTag Structure" :default (struct :`TagName` "Item.Building.Teleport")))
  (bind _l_engine (`local.L_Engine`))
  (bind _returnvalue (- (+ (`local.L_FinalSpeed`) (`self.WeatherSpeed`)) (* (`self.FoundationCount`) 5.0)))
  (for _array_element (`self.Devices`)
    (if (== (`/Game/Skyway/Core/Building/AC_Building_Base.BuildingId` _array_element) (`local.L_HarpoonId`))
      (bind _asac_placed_building_teleport (cast `/Game/Skyway/Core/Building/AC_PlacedBuilding_Teleport` _array_element))
      (if (and (`/Game/Skyway/Core/Building/AC_PlacedBuilding_Base.Active` _asac_placed_building_teleport) (`/Game/Skyway/Core/Building/AC_PlacedBuilding_Teleport.bFindIsland` _asac_placed_building_teleport))
        (set `self.Speed` 0.0)
        (return))))
  (for _array_element_2 (`self.Devices`)
    (if (== (`/Game/Skyway/Core/Building/AC_Building_Base.BuildingId` _array_element_2) (`local.L_EngineId`))
      (bind _asac_building_engine (cast `/Game/Skyway/Core/Building/Consumers/AC_Building_Engine` _array_element_2))
      (set `local.L_Engine` _asac_building_engine)
      (if (`/Game/Skyway/Core/Building/AC_PlacedBuilding_Base.Active` _l_engine)
        (set `local.L_FinalDirection` (+ (`local.L_FinalDirection`) (`/Game/Skyway/Core/Building/Consumers/AC_Building_Engine.Direction` _l_engine)))
        (set `local.L_FinalSpeed` (+ (`local.L_FinalSpeed`) (`/Game/Skyway/Core/Building/Consumers/AC_Building_Engine.Speed` (`local.L_Engine`)))))))
  (set `self.Direction` (+ (`local.L_FinalDirection`) (`self.WeatherDirection`)))
  (set `self.Speed` (select `bool` (< _returnvalue 0.0) :`false` _returnvalue)))

(fn `DestroyAllBuildings`
  (locals (L_Childrens :type "Array of SceneComponent Object Reference"))
  (bind _output_get (set `local.L_Childrens` (`SceneComponent.GetChildrenComponents` (`self.DefaultSceneRoot`) true)))
  (for _array_element _output_get
    (if (`KismetSystemLibrary.DoesImplementInterface` _array_element "/Game/Skyway/Core/Building/BPI_Build.BPI_Build_C")
      (bind _returnarray (message `/Game/Skyway/Core/Building/BPI_Build.GetBuildingCollisions` _array_element))
      (for _array_element_2 _returnarray
        (`ActorComponent.K2_DestroyComponent` _array_element_2))
      (`ActorComponent.K2_DestroyComponent` _array_element)))
  (`KismetArrayLibrary.Array_Clear` (`self.Buildings`))
  (set `self.FoundationCount` 0)
  (set `self.ShipInfo` (struct)))

(fn `DestroyBuilding`
  (params (Building :type "ActorComponent Object Reference"))
  (returns (ReturnValue :type Boolean))
  (locals (L_Building :type "/Game/Skyway/Core/Building/AC_Building_Base Object Reference"))
  (bind ((`Guid_51_E783821C442F8F3AEE949A989634E84B` _guid) (`ParentGuid_58_D8A5A7A8421A51374A145C9D344F54A2` _parentguid)) (break `/Game/Skyway/Core/Engine/S_ShipBuildingInfo` (`/Game/Skyway/Core/Building/AC_Building_Base.ShipBuildingInfo` (`local.L_Building`))))
  (bind _asac_building_base (cast `/Game/Skyway/Core/Building/AC_Building_Base` Building))
  (set `local.L_Building` _asac_building_base)
  (if (and (`KismetSystemLibrary.IsValid` (`local.L_Building`)) (!= (`KismetArrayLibrary.Array_Find` (`self.Buildings`) (`local.L_Building`)) -1) (> (`self.FoundationCount`) 1) (!= (`GameplayStatics.GetObjectClass` (`local.L_Building`)) "/Game/Skyway/Core/Building/AC_Building_Workbench.AC_Building_Workbench_C"))
    (for _array_element (`.GuidOfChildren_55_2B4951EC46466E24FBB4398102287EB0` (break `/Game/Skyway/Core/Engine/S_ShipBuildingInfo` (`/Game/Skyway/Core/Building/AC_Building_Base.ShipBuildingInfo` (`local.L_Building`))))
      (bind (_returnvalue _findbuilding) (`self.FindBuildingByGuid` _array_element))
      (if _returnvalue
        (if (`KismetMathLibrary.ClassIsChildOf` (`GameplayStatics.GetObjectClass` _findbuilding) "/Game/Skyway/Core/Building/AC_PlacedBuilding_Base.AC_PlacedBuilding_Base_C")
          (return false))))
    (bind _returnarray (`/Game/Skyway/Core/Building/BPI_Build.GetBuildingCollisions` (`local.L_Building`)))
    (for _array_element_2 _returnarray
      (`self.DestroyComponent_SERVER` _array_element_2))
    (bind (_returnvalue_2 _findbuilding_2) (`self.FindBuildingByGuid` _parentguid))
    (if _returnvalue_2
      (`KismetArrayLibrary.Array_RemoveItem` (`.GuidOfChildren_55_2B4951EC46466E24FBB4398102287EB0` (break `/Game/Skyway/Core/Engine/S_ShipBuildingInfo` (`/Game/Skyway/Core/Building/AC_Building_Base.ShipBuildingInfo` _findbuilding_2))) _guid))
    (for _array_element_3 (`.GuidOfChildren_55_2B4951EC46466E24FBB4398102287EB0` (break `/Game/Skyway/Core/Engine/S_ShipBuildingInfo` (`/Game/Skyway/Core/Building/AC_Building_Base.ShipBuildingInfo` (`local.L_Building`))))
      (bind (_returnvalue_3 _findbuilding_3) (`self.FindBuildingByGuid` _array_element_3))
      (if _returnvalue_3
        (setmembers `/Game/Skyway/Core/Engine/S_ShipBuildingInfo` :`StructRef` (`/Game/Skyway/Core/Building/AC_Building_Base.ShipBuildingInfo` _findbuilding_3) :`ParentGuid` (select `bool` _returnvalue_2 :`true` (`.ParentGuid_58_D8A5A7A8421A51374A145C9D344F54A2` (break `/Game/Skyway/Core/Engine/S_ShipBuildingInfo` (`/Game/Skyway/Core/Building/AC_Building_Base.ShipBuildingInfo` (`local.L_Building`))))))))
    (`self.DestroyComponent_SERVER` (`local.L_Building`))
    (return true)
    (else
      (return false))))

(fn `FindBuildingByGuid`
  (params (BuildingGuid :type "Guid Structure (by ref)"))
  (returns (ReturnValue :type Boolean) (FindBuilding :type "/Game/Skyway/Core/Building/AC_Building_Base Object Reference"))
  (if (`KismetGuidLibrary.IsValid_Guid` (`local.BuildingGuid`))
    (for _array_element (`self.Buildings`)
      (if (== (`.Guid_51_E783821C442F8F3AEE949A989634E84B` (break `/Game/Skyway/Core/Engine/S_ShipBuildingInfo` (`/Game/Skyway/Core/Building/AC_Building_Base.ShipBuildingInfo` _array_element))) (`local.BuildingGuid`))
        (return true _array_element)))))

(fn `GetShipBuildingInfo`
  (params (BuildingGuid :type "Guid Structure"))
  (returns (ReturnValue :type "/Game/Skyway/Core/Engine/S_ShipBuildingInfo Structure") (Index :type Integer))
  (if (`KismetGuidLibrary.IsValid_Guid` BuildingGuid)
    (for (_array_element _array_index) (`.ShipBuildingsInfo_18_ECE6E3D64E66EC500AF7D7931B9A275F` (break `/Game/Skyway/Core/Engine/S_ShipInfo` (`self.ShipInfo`)))
      (if (== (`.Guid_51_E783821C442F8F3AEE949A989634E84B` (break `/Game/Skyway/Core/Engine/S_ShipBuildingInfo` _array_element)) (`local.BuildingGuid`))
        (return _array_element _array_index)))
    (return (`/Game/Skyway/Core/Engine/MLBP_Defaults.DEFAULT`) -1)
    (else
      (return (`/Game/Skyway/Core/Engine/MLBP_Defaults.DEFAULT`) -1))))

(fn `GetShipInfo`
  (returns (ReturnValue :type "/Game/Skyway/Core/Engine/S_ShipInfo Structure"))
  (return (`self.ShipInfo`)))

(fn `Move`
  (`self.K2_SetActorLocation` (+ (`self.K2_GetActorLocation`) (* (* (`self.Direction`) (`self.Speed`)) (`GameplayStatics.GetWorldDeltaSeconds`)))))

(fn `UpdateAllBuildingCollisions`
  (locals (L_CollisionCount :type Integer))
  (for _array_element (`self.Buildings`)
    (`/Engine/EditorBlueprintResources/StandardMacros.IsValid` _array_element
      (:`Is Valid`
        (bind _returnarray (`/Game/Skyway/Core/Building/BPI_Build.GetBuildingCollisions` _array_element))
        (for _array_element_2 _returnarray
          (`/Engine/EditorBlueprintResources/StandardMacros.IsValid` _array_element_2
            (:`Is Valid`
              (`ActorComponent.K2_DestroyComponent` _array_element_2))))
        (`/Game/Skyway/Core/Building/AC_Building_Base.SpawnCollisions_SERVER` _array_element)))))

(fn `UserConstructionScript`)