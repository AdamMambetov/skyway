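; Actor component, apparently for the ship, that scatters random resource pickups around its owner and schedules flying robot raids.
; Pickups come from DT_Raws and spawn in a box offset along a set direction, throttled by delay and a live-count cap.
; A save-restored timer drives raids, which grow more frequent and larger as world time advances.
; OnRep writes TimeToRaid back to the save; level-based resource selection is unused.
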(event `self.ReceiveBeginPlay`
  (bind _returnvalue (`GameplayStatics.GetGameMode`))
  (`self.SortResourcesByLevel`)
  (if (`self.bCanSpawn`)
    (for _ (range 51)
      (set `self.bCanSpawn` true)
      (`self.SpawnRandomResourcesInRadius_SERVER`)
      (set `self.bCanSpawn` true))
    (bind _returnvalue_2 (message `/Game/Skyway/Core/Engine/BPI_GameMode.GetSaveGame` _returnvalue))
    (`/Engine/EditorBlueprintResources/StandardMacros.IsValid` _returnvalue_2
      (:`Is Valid`
        (bind _timetoraid (message `/Game/Skyway/Core/Engine/BPI_SaveGame.GetTimeToRaid` _returnvalue_2))
        (set `self.TimeToRaid` _timetoraid)
        (`KismetSystemLibrary.K2_SetTimerDelegate` (`|CreateDelegate` :!event `Spawn Flying Robots`) (`self.TimeToRaid`) true)
        (set `self.Loaded` true))
      (:`Is Not Valid`
        (bind _asgm_main (cast `/Game/Skyway/Core/Engine/GM_Main` _returnvalue))
        (add `/Game/Skyway/Core/Engine/GM_Main.OnSaveGameLoaded` _asgm_main (`|CreateDelegate` :!event `OnGameLoaded_Event`))))))

(event `self.ReceiveTick`
  (params (DeltaSeconds :type "Float (single-precision)"))
  (`self.SpawnRandomResourcesInRadius_SERVER`)
  (if (`self.Loaded`)
    (set `self.TimeToRaid` (- (`self.TimeToRaid`) DeltaSeconds))
    (bind _returnvalue (message `/Game/Skyway/Core/Engine/BPI_GameMode.GetSaveGame` (`GameplayStatics.GetGameMode`)))
    (bind _worldtime (message `/Game/Skyway/Core/Engine/BPI_SaveGame.GetCurrentWorldTime` _returnvalue))
    (if (> _worldtime 5400.0)
      (set `self.MaxTimeToSpawnFlyingRobots` 300.0)
      (set `self.MinTimeToSpawnFlyingRobots` 180.0)
      (set `self.MaxCountRaidNpc` 3)
      (elif (> _worldtime 2400.0)
        (set `self.MaxTimeToSpawnFlyingRobots` 480.0)
        (set `self.MinTimeToSpawnFlyingRobots` 300.0)
        (set `self.MaxCountRaidNpc` 2)
        (else
          (set `self.MaxTimeToSpawnFlyingRobots` 600.0)
          (set `self.MinTimeToSpawnFlyingRobots` 480.0)
          (set `self.MaxCountRaidNpc` 1))))))

(event `SpawnRandomResourcesInRadius_SERVER`
  (if (and (`self.bCanSpawn`) (< (`KismetArrayLibrary.Array_Length` (`self.SpawnedResources`)) 60))
    (bind _returnvalue (`self.SpawnRandomResourcesInRadius` 4500.0 (`KismetMathLibrary.RandomIntegerInRange` 1 3) (`self.Direction`)))
    (if _returnvalue
      (set `self.bCanSpawn` false)
      (`KismetSystemLibrary.Delay` (`self.DurationOfSpawn`))
      (set `self.bCanSpawn` true))))

(event `OnDestroyed_Event`
  (params (DestroyedActor :type "Actor Object Reference"))
  (`KismetArrayLibrary.Array_RemoveItem` (`self.SpawnedResources`) DestroyedActor))

(event `OnRaidActorDeth_Event`
  (params (Npc :type "/Game/Skyway/Core/AI/NPC/BP_BaseNPC Object Reference"))
  (bind _asbp_flying_robot (cast `/Game/Skyway/Core/AI/NPC/BP_FlyingRobot` Npc))
  (`KismetArrayLibrary.Array_RemoveItem` (`self.RaidActors`) _asbp_flying_robot)
  (if (== (`KismetArrayLibrary.Array_Length` (`self.RaidActors`)) 0)
    (`self.OnRaidEnd`)))

(event `OnRaidEnd_Event`
  (`self.OnRaidEnd`))

(event `OnGameLoaded_Event`
  (params (SaveGame :type "SaveGame Object Reference"))
  (bind _timetoraid (message `/Game/Skyway/Core/Engine/BPI_SaveGame.GetTimeToRaid` SaveGame))
  (set `self.TimeToRaid` _timetoraid)
  (`KismetSystemLibrary.K2_SetTimerDelegate` (`|CreateDelegate` :!event `Spawn Flying Robots`) (`self.TimeToRaid`) true)
  (set `self.Loaded` true))

(fn `OnRep_TimeToRaid`
  (bind _returnvalue (message `/Game/Skyway/Core/Engine/BPI_GameMode.GetSaveGame` (`GameplayStatics.GetGameMode`)))
  (message `/Game/Skyway/Core/Engine/BPI_SaveGame.SetTimeToRaid` _returnvalue (`self.TimeToRaid`)))

(fn `SetSpawnDirection`
  (params (Direction :type "Vector Structure"))
  (set `self.Direction` Direction))

(fn `SortResourcesByLevel`
  (bind _outrownames (`DataTableFunctionLibrary.GetDataTableRowNames` "/Game/Skyway/Core/Inventory/DT_Raws.DT_Raws"))
  (for _array_element _outrownames
    (bind _returnvalue (`|GetDataTableRow` "/Game/Skyway/Core/Inventory/DT_Raws.DT_Raws" _array_element)
      (:`then`
        (if (!= -1 (`.Lvl_5_F4DBF3354965105D0BF32887533C8DC1` (break `/Game/Skyway/Core/Inventory/S_Raw_Info` _returnvalue)))
          (`KismetArrayLibrary.Array_Add` (`self.Resources`) _returnvalue))))))

(fn `Spawn Flying Robots`
  (locals (L_Id :type Integer :default 0))
  (bind (_returnvalue_x _returnvalue_y) (`KismetMathLibrary.BreakVector` (`KismetMathLibrary.RandomUnitVector`)))
  (bind (_returnvalue_x_2 _returnvalue_y_2 _returnvalue_z) (`KismetMathLibrary.BreakVector` (`Actor.K2_GetActorLocation` (`self.GetOwner`))))
  (set `local.L_Id` (`KismetMathLibrary.RandomIntegerInRange` 1 100000000))
  (for _ (range 1 (+ (`KismetMathLibrary.RandomIntegerInRange` 1 (`self.MaxCountRaidNpc`)) 1))
    (bind _returnvalue (`|SpawnActorFromClass` "/Game/Skyway/Core/AI/NPC/BP_FlyingRobot.BP_FlyingRobot_C" (`KismetMathLibrary.MakeTransform` (`KismetMathLibrary.MakeVector_NetQuantize` (* _returnvalue_x 10000.0) (* _returnvalue_y 10000.0) (+ _returnvalue_z 3000.0))) "Undefined" "MultiplyWithRoot" null null))
    (`KismetArrayLibrary.Array_Add` (`self.RaidActors`) _returnvalue)
    (set `BaseCharacter.ID` (`local.L_Id`) _returnvalue)
    (add `/Game/Skyway/Core/AI/NPC/BP_FlyingRobot.OnRaidEnd` _returnvalue (`|CreateDelegate` :!event `OnRaidEnd_Event`))
    (add `/Game/Skyway/Core/AI/NPC/BP_BaseNPC.OnNpcDeth` _returnvalue (`|CreateDelegate` :!event `OnRaidActorDeth_Event`)))
  (bind _output_get (set `self.TimeToRaid` (`KismetMathLibrary.RandomFloatInRange` (`self.MinTimeToSpawnFlyingRobots`) (`self.MaxTimeToSpawnFlyingRobots`))))
  (`KismetSystemLibrary.K2_SetTimerDelegate` (`|CreateDelegate` :!event `Spawn Flying Robots`) _output_get)
  (`self.OnRaidBegin`))

(fn `SpawnRandomResourcesInRadius`
  (params (SpawnRadius :type "Float (double-precision)") (LVL :type Integer) (Direction :type "Vector Structure"))
  (returns (ReturnValue :type Boolean))
  (locals (L_RandomLocation :type "Vector Structure") (L_EndLocation :type "Vector Structure"))
  (bind _spawnedresources (`self.SpawnedResources`))
  (bind _resources (`self.Resources`))
  (bind _returnvalue (/ (`local.SpawnRadius`) 2.0))
  (bind ((`ItemInfo_2_96BFBB67441ABC75F13542B20097FC01` _iteminfo) (`PickupClass_16_8EC98BA448AF05C0A6A44BBA159DB3E1` _pickupclass)) (break `/Game/Skyway/Core/Inventory/S_Raw_Info` (`|GetArrayItem` _resources (`self.ResourceIndex`))))
  (set `local.L_EndLocation` (+ (* (`self.Direction`) (`local.SpawnRadius`)) (`Actor.K2_GetActorLocation` (`self.GetOwner`))))
  (set `local.L_RandomLocation` (`KismetMathLibrary.RandomPointInBoundingBox` (`local.L_EndLocation`) (`KismetMathLibrary.MakeVector` _returnvalue _returnvalue 500.0)))
  (if (> (`KismetMathLibrary.Vector_Distance` (`local.L_EndLocation`) (`local.L_RandomLocation`)) (`self.MIN_SPAWN_DISTANCE`))
    (set `self.ResourceIndex` (`KismetMathLibrary.RandomIntegerInRange` 0 (`KismetArrayLibrary.Array_Length` _resources)))
    (bind _returnvalue_2 (`|SpawnActorFromClass` _pickupclass (`KismetMathLibrary.MakeTransform` (`local.L_RandomLocation`) (`KismetMathLibrary.RandomRotator` true) (`/Game/Skyway/Core/Engine/MLBP_Defaults.DEFAULT_SCALE`)) "Undefined" "SelectDefaultAtRuntime" (`self.GetOwner`) (`.ID_71_BA06E0BD4E97D16461377CB9BF36CE2D` (break `/Game/Skyway/Core/Inventory/S_Item_Info` _iteminfo)) 1 null))
    (bind _returnvalue_3 (`KismetArrayLibrary.Array_Add` _spawnedresources _returnvalue_2))
    (bind _output (`|GetArrayItem` _spawnedresources _returnvalue_3))
    (`/Engine/EditorBlueprintResources/StandardMacros.IsValid` _output
      (:`Is Valid`
        (add `Actor.OnDestroyed` _output (`|CreateDelegate` :!event `OnDestroyed_Event`))
        (return true)))
    (else
      (return false))))