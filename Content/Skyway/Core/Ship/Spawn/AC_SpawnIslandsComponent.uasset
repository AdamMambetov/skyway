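; Ship component that populates the sky around its owner with random islands from DT_Islands, up to a maximum count.
; BeginPlay loads the table through a server event; Tick prunes invalid islands and requests server spawns.
; Spawn points are re-rolled until their distance from the owner is within range, with height offset from the owner's Z.
; Each island receives its class-default DistanceForDestroy and is tracked in SpawnedIslands.
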(event `self.ReceiveBeginPlay`
  (`parent.ReceiveBeginPlay`)
  (`self.InitIslands_SERVER`)
  (`self.SpawnIsland`))

(event `InitIslands_SERVER`
  (`self.InitIslands`))

(event `SpawnIsland_SERVER`
  (`self.SpawnIsland`))

(event `UpdateIslands_SERVER`
  (`self.UpdateIslands`))

(event `self.ReceiveTick`
  (params (DeltaSeconds :type "Float (single-precision)"))
  (`self.UpdateIslands`)
  (`self.SpawnIsland_SERVER`))

(fn `CanSpawnIsland`
  (returns (ReturnValue :type Boolean))
  (return (and (< (`KismetArrayLibrary.Array_Length` (`self.SpawnedIslands`)) (`self.MAX_ISLAND_COUNT`)) true)))

(fn `GenerateIslandZ`
  (returns (ReturnValue :type "Float (double-precision)"))
  (locals (L_Z :type "Float (double-precision)" :default 400.0))
  (return (- (.z (`Actor.K2_GetActorLocation` (`self.GetOwner`))) (`local.L_Z`))))

(fn `InitIslands`
  (`KismetArrayLibrary.Array_Clear` (`self.Islands`))
  (bind _outrownames (`DataTableFunctionLibrary.GetDataTableRowNames` "/Game/Skyway/Core/Island/DT_Islands.DT_Islands"))
  (for _array_element _outrownames
    (bind _returnvalue (`|GetDataTableRow` "/Game/Skyway/Core/Island/DT_Islands.DT_Islands" _array_element)
      (:`then`
        (`KismetArrayLibrary.Array_Add` (`self.Islands`) _returnvalue)))))

(fn `SpawnIsland`
  (locals (L_SpawnLocation :type "Vector Structure") (L_MinRange :type "Float (double-precision)" :default 40000.0) (L_MaxRange :type "Float (double-precision)" :default 45000.0) (L_Count :type Integer))
  (bind ((`Class_5_9CA15E4848F3AD39B49791B4493688E8` _class)) (break `/Game/Skyway/Core/Island/S_Island_Info` (`KismetArrayLibrary.Array_Random` (`self.Islands`))))
  (if (`self.CanSpawnIsland`)
    (`|ExecutionSequence`
      (:`then_0`
        (set `local.L_SpawnLocation` (`KismetMathLibrary.MakeVector` (.x (+ (* (`KismetMathLibrary.RandomUnitVector`) (`KismetMathLibrary.RandomFloatInRange` (`local.L_MinRange`) (`local.L_MaxRange`))) (`Actor.K2_GetActorLocation` (`self.GetOwner`)))) (.y (+ (* (`KismetMathLibrary.RandomUnitVector`) (`KismetMathLibrary.RandomFloatInRange` (`local.L_MinRange`) (`local.L_MaxRange`))) (`Actor.K2_GetActorLocation` (`self.GetOwner`)))) (`self.GenerateIslandZ`)) :!label _label)
        (`/Engine/EditorBlueprintResources/StandardMacros.IncrementInt` (`local.L_Count`)))
      (:`then_1`
        (while (not (`KismetMathLibrary.InRange_FloatFloat` (`KismetMathLibrary.Vector_Distance` (`Actor.K2_GetActorLocation` (`self.GetOwner`)) (`local.L_SpawnLocation`)) (`local.L_MinRange`) (`local.L_MaxRange`)))
          (goto _label))
        (bind _returnvalue (`|SpawnActorFromClass` _class (`KismetMathLibrary.MakeTransform` (`local.L_SpawnLocation`) (`/Game/Skyway/Core/Engine/MLBP_Defaults.DEFAULT`) (`/Game/Skyway/Core/Engine/MLBP_Defaults.DEFAULT_SCALE`)) "Undefined" "OverrideRootScale" (`self.GetOwner`) (defaults `Object` _class) null))
        (`KismetArrayLibrary.Array_Add` (`self.SpawnedIslands`) _returnvalue)))))

(fn `UpdateIslands`
  (for _array_element (`self.SpawnedIslands`)
    (`/Engine/EditorBlueprintResources/StandardMacros.IsValid` _array_element
      (:`Is Not Valid`
        (`KismetArrayLibrary.Array_RemoveItem` (`self.SpawnedIslands`) _array_element)))))