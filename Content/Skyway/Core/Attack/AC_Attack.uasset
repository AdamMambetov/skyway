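; Attack component for Skyway characters that handles the equipped weapon and melee or ranged attacks with combos.
; Weapon slot updates from AC_Storage spawn or destroy the weapon actor from DT_Weapons, visible only in BattleMode.
; Attack IDs follow weapon type and character; server RPCs check and spend Energy, then multicast the attack start.
; Input during an attack sets SaveCombo, letting SaveCombo() chain the next child gameplay tag from the attack table.
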(event `self.ReceiveTick`
  (params (DeltaSeconds :type "Float (single-precision)"))
  (bind _ownerref (`self.OwnerRef`)
    (:`then`
      (set `self.CharacterState` (`BaseCharacter.CharacterState` _ownerref)))
    (:`else`)))

(event `self.ReceiveBeginPlay`
  (add `self.OnAttackEnd` (`|CreateDelegate` :!event `OnAttackEnd_SERVER`))
  (bind _asbase_character (cast `BaseCharacter` (`self.GetOwner`)))
  (bind _output_get (set `self.OwnerRef` _asbase_character))
  (set `self.CurrentCharacter` (`BaseCharacter.Character` _output_get))
  (if (`KismetSystemLibrary.IsValid` (`Actor.GetComponentByClass` (`self.GetOwner`) "/Game/Skyway/Core/Inventory/AC_Storage.AC_Storage_C"))
    (`self.Bind`)
    (else
      (bind _returnvalue (`KismetSystemLibrary.K2_SetTimerDelegate` (`|CreateDelegate` :!event `Bind`) 0.01 true)))))

(event `Bind`
  (bind _returnvalue (`Actor.GetComponentByClass` (`self.GetOwner`) "/Game/Skyway/Core/Inventory/AC_Storage.AC_Storage_C"))
  (bind _output (`|GetArrayItem` (`/Game/Skyway/Core/Inventory/AC_Storage.GetSlotsAtItemType` _returnvalue (struct :`TagName` "SlotContainer.Weapon") (`/Game/Skyway/Core/Engine/MLBP_Defaults.DEFAULT`))))
  (if (`KismetSystemLibrary.IsValid` (`Actor.GetComponentByClass` (`self.GetOwner`) "/Game/Skyway/Core/Inventory/AC_Storage.AC_Storage_C"))
    (`KismetSystemLibrary.K2_ClearAndInvalidateTimerHandle` (stale `self.ReceiveBeginPlay` _returnvalue))
    (add `/Game/Skyway/Core/Inventory/AC_Storage.OnSlotUpdated` _returnvalue (`|CreateDelegate` :!event `OnSlotUpdated_Event`))
    (`KismetSystemLibrary.PrintString` (`BlueprintGameplayTagLibrary.GetDebugStringFromGameplayTag` (`.ID_71_BA06E0BD4E97D16461377CB9BF36CE2D` (break `/Game/Skyway/Core/Inventory/S_Item_Info` (`.ItemInfo_14_7E8F48144F0F01654500E084A85436C5` (break `/Game/Skyway/Core/Inventory/S_Slot_Info` _output))))))
    (`self.OnSlotUpdated_Event` _output)
    (set `self.OwningStatComp` (`Actor.GetComponentByClass` (`self.GetOwner`) "/Game/Skyway/Core/Stats/AC_StatComponent.AC_StatComponent_C"))
    (bind _asbp_main_character (cast `/Game/Skyway/Core/Characters/BP_MainCharacter` (`self.GetOwner`)))
    (add `/Game/Skyway/Core/Characters/BP_MainCharacter.OnCharacterStateChanged` _asbp_main_character (`|CreateDelegate` :!event `OnCharacterStateChanged_Event`))))

(event `AttackById_SERVER`
  (params (AttackId :type "GameplayTag Structure" :default (struct :`TagName` "Attack")))
  (`self.AttackById` AttackId))

(event `OnSlotUpdated_Event`
  (params (SlotInfo :type "/Game/Skyway/Core/Inventory/S_Slot_Info Structure"))
  (bind ((`ItemInfo_14_7E8F48144F0F01654500E084A85436C5` _iteminfo) (`Type_32_DA6EC9A74765E8D199FD1FABBE3B74F3` _type)) (break `/Game/Skyway/Core/Inventory/S_Slot_Info` SlotInfo))
  (bind ((`ID_71_BA06E0BD4E97D16461377CB9BF36CE2D` _id)) (break `/Game/Skyway/Core/Inventory/S_Item_Info` _iteminfo))
  (switch `/Game/Skyway/Core/Inventory/E_SlotType` _type
    (:`NewEnumerator3`
      (if (`/Game/Skyway/Core/Engine/FLBP_Defaults.IsValidItemId` _id)
        (`self.AddWeapon_SERVER` _id)
        (else
          (`self.RemoveWeapon_SERVER`))))))

(event `OnAttackStart_SERVER`
  (`self.OnAttackStart_MULTI`))

(event `OnAttackStart_MULTI`
  (`self.OnAttackStart` (`self.AttackInfo`)))

(event `OnCharacterStateChanged_Event`
  (params (CharacterState :type "ECharacterState Enum" :default "HookMode"))
  (bind _output_get (set `self.CharacterState` CharacterState))
  (`Actor.SetActorHiddenInGame` (`self.Weapon`) (`|EnumInequality` _output_get "BattleMode")))

(event `OnAttackEnd_SERVER` :!signature `self.OnAttackEnd`
  (params (AttackInfo :type "/Game/Skyway/Core/Attack/F_AttackInfo Structure"))
  (`self.AttackEnd` AttackInfo))

(event `AddWeapon_SERVER`
  (params (WeaponId :type "GameplayTag Structure"))
  (`self.AddWeapon` WeaponId))

(event `RemoveWeapon_SERVER`
  (`self.RemoveWeapon`))

(event `WeaponAttack`
  (bind _weapon (`self.Weapon`)
    (:`then`
      (`/Game/Skyway/Core/Inventory/BP_Weapon_Base.Attack_SERVER` _weapon))
    (:`else`)))

(event `SetAttackState_SERVER`
  (params (NewAttackState :type "/Game/Skyway/Core/Attack/E_AttackState Enum" :default "NewEnumerator0"))
  (set `self.AttackState` NewAttackState))

(fn `AddWeapon`
  (params (WeaponId :type "GameplayTag Structure"))
  (bind _returnvalue (`|GetDataTableRow` "/Game/Skyway/Core/Inventory/DT_Weapons.DT_Weapons" (`BlueprintGameplayTagLibrary.GetTagName` (`local.WeaponId`)))
    (:`then`
      (bind _returnvalue_2 (`|SpawnActorFromClass` (`.Class_24_289B5396421C23CA42D335845D0EDA29` (break `/Game/Skyway/Core/Inventory/S_Weapon_Info` _returnvalue)) (`/Game/Skyway/Core/Engine/MLBP_Defaults.DEFAULT`) (`/Game/Skyway/Core/Engine/MLBP_Defaults.DEFAULT`) "SelectDefaultAtRuntime" (`self.GetOwner`) (`local.WeaponId`) 1 null))
      (bind _output_get (set `self.Weapon` _returnvalue_2))
      (`Actor.SetActorHiddenInGame` _output_get (`|EnumInequality` (`self.CharacterState`) "BattleMode")))))

(fn `Attack`
  (if (and (`KismetSystemLibrary.IsValid` (`self.Weapon`)) (`|EnumEquality` (`self.CharacterState`) (enumliteral `ECharacterState` "BattleMode")))
    (switch `/Game/Skyway/Core/Attack/E_AttackState` (`self.AttackState`)
      (:`NewEnumerator0`
        (`self.AttackById_SERVER` (`self.GenerateAttackId`)))
      (:`NewEnumerator1`
        (`self.SetAttackState_SERVER` "NewEnumerator2"))
      (:`NewEnumerator2`
        (if (not (`AnimInstance.IsAnyMontagePlaying` (`SkeletalMeshComponent.GetAnimInstance` (`Character.Mesh` (`self.OwnerRef`)))))
          (`self.OnAttackEnd` (`self.AttackInfo`))
          (`self.AttackById_SERVER` (`self.GenerateAttackId`)))))))

(fn `AttackById`
  (params (AttackId :type "GameplayTag Structure" :default (struct :`TagName` "Attack")))
  (set `self.NewAttackId` AttackId)
  (if (`self.CanAttack`)
    (set `self.CurrentAttackId` (`self.NewAttackId`))
    (set `self.AttackState` "NewEnumerator1")
    (bind (_returnvalue _attackinfo) (`/Game/Skyway/Core/Engine/FLBP_Defaults.GetAttackInfoById` (`self.CurrentAttackId`)))
    (if _returnvalue
      (set `self.AttackInfo` _attackinfo)
      (set `self.ComboCount` (`.ComboCount_22_07E59F884B9F8A91BB68EEBA56EB3E46` (break `/Game/Skyway/Core/Attack/F_AttackInfo` (`self.AttackInfo`))))
      (`self.OnAttackStart_SERVER`)
      (bind _owningstatcomp (`self.OwningStatComp`)
        (:`then`
          (`/Game/Skyway/Core/Stats/AC_StatComponent.ChangeStatValueById_SERVER` _owningstatcomp (make `/Game/Skyway/Core/Stats/S_StatModifier` :`Id` (struct :`TagName` "Stat.Energy") :`Value` (* -1.0 (`.EnergyCost_29_8585DDA14ED53E7C5D966DB1BB269479` (break `/Game/Skyway/Core/Inventory/S_Weapon_Info` (`/Game/Skyway/Core/Inventory/BP_Weapon_Base.WeaponInfo` (`self.Weapon`))))) :`TypeContainer` (struct :`GameplayTags` (struct :`(TagName` "StatModifier.Immediately"))))))
        (:`else`)))))

(fn `AttackEnd`
  (params (AttackInfo :type "/Game/Skyway/Core/Attack/F_AttackInfo Structure"))
  (if (`self.IsAttackEnd` (`local.AttackInfo`))
    (set `self.AttackState` "NewEnumerator0")
    (set `self.CurrentAttackId` (struct))
    (set `self.ComboCount` 0)
    (`/Game/Skyway/Core/Inventory/BP_Weapon_Base.DisableCollision_SERVER` (`self.Weapon`))))

(fn `CanAttack`
  (returns (ReturnValue :type Boolean))
  (if (and (`|EnumInequality` (`self.AttackState`) "NewEnumerator1") (`/Game/Skyway/Core/Engine/FLBP_Defaults.IsValidAttackId` (`self.NewAttackId`)))
    (if (not (`KismetMathLibrary.NearlyEqual_FloatFloat` (`.EnergyCost_29_8585DDA14ED53E7C5D966DB1BB269479` (break `/Game/Skyway/Core/Inventory/S_Weapon_Info` (`/Game/Skyway/Core/Inventory/BP_Weapon_Base.WeaponInfo` (`self.Weapon`)))) 0.0 0.001))
      (bind _owningstatcomp (`self.OwningStatComp`)
        (:`then`
          (bind (_returnvalue _statinfo) (`/Game/Skyway/Core/Stats/AC_StatComponent.GetStatInfoById` _owningstatcomp (struct :`TagName` "Stat.Energy")))
          (return (and _returnvalue (>= (`.CurrentValue_4_DE51577F455957135DBA8EAD967FB78D` (break `/Game/Skyway/Core/Stats/S_StatInfo` _statinfo)) (`.EnergyCost_29_8585DDA14ED53E7C5D966DB1BB269479` (break `/Game/Skyway/Core/Inventory/S_Weapon_Info` (`/Game/Skyway/Core/Inventory/BP_Weapon_Base.WeaponInfo` (`self.Weapon`))))))))
        (:`else`))
      (else
        (return true)))))

(fn `GenerateAttackId`
  (returns (ReturnValue :type "GameplayTag Structure"))
  (switch `/Game/Skyway/Core/Inventory/E_WeaponType` (`.Type_25_742DF51A4E96C15CAA15F3A5D0E18F2C` (break `/Game/Skyway/Core/Inventory/S_Weapon_Info` (`/Game/Skyway/Core/Inventory/BP_Weapon_Base.WeaponInfo` (`self.Weapon`))))
    (:`NewEnumerator0`
      (return (select `ECharacters` (`self.CurrentCharacter`) :`Bouncer` (struct :`TagName` "Attack.Bouncer.Fist.Attack_1") :!type "GameplayTag Structure")))
    (:`NewEnumerator1`
      (return (select `ECharacters` (`self.CurrentCharacter`) :`Bot` (struct :`TagName` "Attack.Bot.Blaster.Shoot") :!type "GameplayTag Structure")))
    (:`NewEnumerator2`
      (return (select `ECharacters` (`self.CurrentCharacter`) :`Bot` (struct :`TagName` "Attack.Bot.Baton.Attack.1") :!type "GameplayTag Structure")))))

(fn `GetNextComboAttackId`
  (returns (ReturnValue :type "GameplayTag Structure"))
  (locals (L_ComboAttacks :type "Array of GameplayTag Structure"))
  (if (`/Game/Skyway/Core/Engine/FLBP_Defaults.IsValidAttackId` (`.ID_14_7DE4D21A47D6F6091D9B8E8389E399A2` (break `/Game/Skyway/Core/Attack/F_AttackInfo` (`self.AttackInfo`))))
    (set `local.L_ComboAttacks` (`CppDefaults.GetChildrensByTag` (`.ComboId_19_34D78E7141F59EC9988981B7C0990F5D` (break `/Game/Skyway/Core/Attack/F_AttackInfo` (`self.AttackInfo`))) "/Game/Skyway/Core/Engine/DT_Attacks_GT.DT_Attacks_GT"))
    (if (`KismetArrayLibrary.Array_IsValidIndex` (`local.L_ComboAttacks`) (`self.ComboCount`))
      (return (`|GetArrayItem` (`local.L_ComboAttacks`) (`self.ComboCount`)))
      (else
        (return (`|GetArrayItem` (`local.L_ComboAttacks`)))))))

(fn `GetWeaponInfo`
  (returns (ReturnValue :type "/Game/Skyway/Core/Inventory/S_Weapon_Info Structure"))
  (return (`/Game/Skyway/Core/Inventory/BP_Weapon_Base.WeaponInfo` (`self.Weapon`))))

(fn `GetWeaponType`
  (returns (ReturnValue :type "/Game/Skyway/Core/Inventory/E_WeaponType Enum"))
  (bind _weapon (`self.Weapon`)
    (:`then`
      (return (`.Type_25_742DF51A4E96C15CAA15F3A5D0E18F2C` (break `/Game/Skyway/Core/Inventory/S_Weapon_Info` (`/Game/Skyway/Core/Inventory/BP_Weapon_Base.WeaponInfo` _weapon)))))
    (:`else`)))

(fn `IsAttackEnd`
  (params (AttackInfo :type "/Game/Skyway/Core/Attack/F_AttackInfo Structure"))
  (returns (ReturnValue :type Boolean))
  (return (and (`|EnumEquality` (`self.AttackState`) "NewEnumerator1") (== (`.ID_14_7DE4D21A47D6F6091D9B8E8389E399A2` (break `/Game/Skyway/Core/Attack/F_AttackInfo` (`local.AttackInfo`))) (`self.CurrentAttackId`)))))

(fn `OnRep_AttackState`
  (`self.OnAttackStateChanged` (`self.AttackState`)))

(fn `RemoveWeapon`
  (`/Engine/EditorBlueprintResources/StandardMacros.IsValid` (`self.Weapon`)
    (:`Is Valid`
      (`Actor.K2_DestroyActor` (`self.Weapon`))
      (set `self.Weapon` null))))

(fn `SaveCombo`
  (if (`|EnumEquality` (`self.AttackState`) (enumliteral `/Game/Skyway/Core/Attack/E_AttackState` "NewEnumerator2"))
    (`self.SetAttackState_SERVER` "NewEnumerator0")
    (`self.AttackById_SERVER` (`self.GetNextComboAttackId`))))