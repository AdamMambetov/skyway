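; BP_Projectile is a weapon projectile that damages what it hits.
; The construction script looks up the WeaponId tag's row in DT_Weapons, caches it as WeaponInfo and sets the projectile movement's initial and max speed from it.
; On sphere overlap, the server alone applies the weapon's damage to any actor other than the owner, then destroys the projectile.
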(event `self.Sphere.OnComponentBeginOverlap`
  (params (OverlappedComponent :type "PrimitiveComponent Object Reference") (OtherActor :type "Actor Object Reference") (OtherComp :type "PrimitiveComponent Object Reference") (OtherBodyIndex :type Integer) (bFromSweep :type Boolean) (SweepResult :type "HitResult Structure (by ref)"))
  (`/Engine/EditorBlueprintResources/ActorMacros.Switch Has Authority`
    (:`Authority`
      (if (!= OtherActor (`self.GetOwner`))
        (`GameplayStatics.ApplyDamage` OtherActor (`.Damage_9_E157A1A343752171738AF58207467496` (break `/Game/Skyway/Core/Inventory/S_Weapon_Info` (`self.WeaponInfo`))))
        (`self.K2_DestroyActor`)))))

(fn `UserConstructionScript`
  (bind _returnvalue (`|GetDataTableRow` "/Game/Skyway/Core/Inventory/DT_Weapons.DT_Weapons" (`BlueprintGameplayTagLibrary.GetTagName` (`self.WeaponId`)))
    (:`then`
      (bind _output_get (set `self.WeaponInfo` _returnvalue))
      (bind ((`Class_24_289B5396421C23CA42D335845D0EDA29` _class) (`Type_25_742DF51A4E96C15CAA15F3A5D0E18F2C` _type) (`ProjectileSpeed_21_69F9401441B1F6E861D3B990F0B6DCF6` _projectilespeed)) (break `/Game/Skyway/Core/Inventory/S_Weapon_Info` _output_get))
      (set `ProjectileMovementComponent.MaxSpeed` _projectilespeed (`self.ProjectileMovement`))
      (set `ProjectileMovementComponent.InitialSpeed` _projectilespeed (`self.ProjectileMovement`)))))