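; Weather system actor that runs a looping day/night clock, scaled by a configurable day length in minutes, and drives sun, precipitation and sky.
; Tick advances the time and calls UpdateWeather, which samples time-keyed curves to blend sun intensity by weather type, pitch the sun, and toggle light-shaft bloom, rain and snow.
; It then refreshes the sky sphere material.
; Fog and skylight logic is present but unconnected.
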(event `self.ReceiveBeginPlay`
  (set `self.OneHour` (/ (* (`self.DayLengthInMinutes`) (`self.ONE_HOUR_IN_MINUTES`)) (`self.ONE_DAY_IN_HOURS`))))

(event `self.ReceiveTick`
  (params (DeltaSeconds :type "Float (single-precision)"))
  (if (> (`self.CalculateCurrentTime`) 0.0)
    (if (or (< (`self.CalculateCurrentTime`) (`self.ONE_DAY_IN_HOURS`)) (`KismetMathLibrary.NearlyEqual_FloatFloat` (`self.CalculateCurrentTime`)))
      (`self.SetCurrentTime` (`self.CalculateCurrentTime`))
      (else
        (`self.SetCurrentTime` (`KismetMathLibrary.Abs` (- (`self.ONE_DAY_IN_HOURS`) (`self.CalculateCurrentTime`))))))
    (`self.UpdateWeather`)
    (bind _asmaterial_instance_dynamic (cast `MaterialInstanceDynamic` (`PrimitiveComponent.GetMaterial` (`/Engine/EngineSky/BP_Sky_Sphere.SkySphereMesh` (`self.SkySphereActor`)) 0)))
    (`MaterialInstanceDynamic.K2_GetVectorParameterValue` _asmaterial_instance_dynamic "Horizon color")))

(event `SetCurrentTime`
  (params (CurrentTime :type "Float (double-precision)"))
  (set `self.CurrentTime` CurrentTime))

(fn `CalculateCurrentTime`
  (returns (ReturnValue :type "Float (double-precision)"))
  (return (+ (`KismetMathLibrary.SafeDivide` (`GameplayStatics.GetWorldDeltaSeconds`) (`self.OneHour`)) (`self.CurrentTime`))))

(fn `SpawnActors`
  (bind _returnvalue (`|SpawnActorFromClass` "/Script/Engine.DirectionalLight" (`/Game/Skyway/Core/Engine/MLBP_Defaults.DEFAULT`) (`/Game/Skyway/Core/Engine/MLBP_Defaults.DEFAULT`) "OverrideRootScale" self null))
  (bind _output_get (set `self.SunActor` _returnvalue))
  (`self.K2_AttachToActor` _output_get self "None" "SnapToTarget" "SnapToTarget" "SnapToTarget" true)
  (bind _returnvalue_2 (`|SpawnActorFromClass` "/Engine/EngineSky/BP_Sky_Sphere.BP_Sky_Sphere_C" (`/Game/Skyway/Core/Engine/MLBP_Defaults.DEFAULT`) (`/Game/Skyway/Core/Engine/MLBP_Defaults.DEFAULT`) "OverrideRootScale" self null))
  (bind _output_get_2 (set `self.SkySphereActor` _returnvalue_2))
  (set `/Engine/EngineSky/BP_Sky_Sphere.Directional light actor` (`self.SunActor`) _output_get_2))

(fn `UpdateWeather`
  (locals (L_WeatherType :type "Float (single-precision)" :default 0.0) (L_Enable :type "Float (double-precision)" :default 1.0))
  (bind (_returnvalue_x _returnvalue_y) (`KismetMathLibrary.BreakVector` (`CurveVector.GetVectorValue` (`self.SunIntensityCurve`) (`self.CurrentTime`))))
  (`|ExecutionSequence`
    (:`then_0`
      ;[1 1 1] Variables
      (set `local.L_WeatherType` (`CurveFloat.GetFloatValue` (`self.WeatherTypeCurve`) (`self.CurrentTime`))))
    (:`then_1`
      ;[1 1 1] Sun
      (`LightComponent.SetIntensity` (`Light.LightComponent` (`self.SunActor`)) (`KismetMathLibrary.Lerp` _returnvalue_x _returnvalue_y (`local.L_WeatherType`)))
      (`self.K2_SetActorRelativeRotation` (`self.SunActor`) (`KismetMathLibrary.MakeRotator` 0.0 (`CurveFloat.GetFloatValue` (`self.DayLengthCurve`) (`self.CurrentTime`))) false false)
      (`LightComponent.SetEnableLightShaftBloom` (`Light.LightComponent` (`self.SunActor`)) (`KismetMathLibrary.InRange_FloatFloat` (`self.CurrentTime`) (`self.SUNRISE_TIME`) (`self.SUNSET_TIME`))))
    (:`then_2`)
    (:`then_3`)
    (:`then_4`
      ;[1 1 1] Rain
      (if (and (`self.bRain`) (`KismetMathLibrary.NearlyEqual_FloatFloat` (`CurveFloat.GetFloatValue` (`self.RainTimelineCurve`) (`self.CurrentTime`)) (`local.L_Enable`)))
        (`ActorComponent.Activate` (`self.Rain`) false)
        (else
          (`ActorComponent.Deactivate` (`self.Rain`)))))
    (:`then_5`
      ;[1 1 1] Snow
      (if (and (`self.bSnow`) (`KismetMathLibrary.NearlyEqual_FloatFloat` (`CurveFloat.GetFloatValue` (`self.SnowTimelineCurve`) (`self.CurrentTime`)) (`local.L_Enable`)))
        (`ActorComponent.Activate` (`self.Snow`) false)
        (else
          (`ActorComponent.Deactivate` (`self.Snow`)))))
    (:`then_6`
      ;[1 1 1] Sky Sphere
      (bind _skysphereactor (`self.SkySphereActor`)
        (:`then`
          (`/Engine/EngineSky/BP_Sky_Sphere.RefreshMaterial` _skysphereactor))
        (:`else`)))))

(fn `UserConstructionScript`
  (`self.K2_SetActorLocationAndRotation` (`KismetMathLibrary.Conv_IntVectorToVector` (`GameplayStatics.GetWorldOriginLocation`)) (`/Game/Skyway/Core/Engine/MLBP_Defaults.DEFAULT`))
  (`self.UpdateWeather`))