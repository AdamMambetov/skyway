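; Wind actor that periodically picks a new random horizontal wind direction and speed, then blends toward them over time.
; A looping timer derives the direction from a random cone vector and the actor's location, folding half of Z into X/Y, and picks a speed within the min/max range.
; Tick lerps from the current values using a growing alpha.
; Speed and Direction RepNotifies broadcast OnWeatherChange with both values.
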(event `self.ReceiveTick`
  (params (DeltaSeconds :type "Float (single-precision)"))
  (bind _alpha (`self.Alpha`))
  (if (and (< _alpha 1.0) (!= (`self.NewDirection`) (0.0 0.0 0.0)))
    (set `self.Alpha` (+ (* DeltaSeconds (`self.DirectionSpeed`)) _alpha))
    (set `self.Direction` (`KismetMathLibrary.VLerp` (`self.Direction`) (`self.NewDirection`) (`self.Alpha`)))
    (set `self.Speed` (`KismetMathLibrary.Lerp` (`self.Speed`) (`self.NewSpeed`) (`self.Alpha`)))))

(event `self.ReceiveBeginPlay`
  (`self.CalculateWeatherDirection`)
  (`KismetSystemLibrary.K2_SetTimer` null "CalculateWeatherDirection" (`self.RefreshDirectionTime`) true)
  (bind _returnvalue (`/Game/Skyway/Core/Engine/FLBP_Defaults.GetDebugUseCase`))
  (set `self.bDebug` _returnvalue))

(fn `CalculateDirectionInCone`
  (returns (ReturnValue :type "Vector Structure"))
  (locals (L_NewDirection :type "Vector Structure" :default (0.0 0.0 0.0)))
  (bind _x (.x (`local.L_NewDirection`)))
  (bind _y (.y (`local.L_NewDirection`)))
  (bind _returnvalue (/ (.z (`local.L_NewDirection`)) 2.0))
  (bind _returnvalue_2 (/ (.z (`local.L_NewDirection`)) 2.0))
  (set `local.L_NewDirection` (`KismetMathLibrary.GetDirectionUnitVector` (`KismetMathLibrary.RandomUnitVectorInConeInDegrees` (`SceneComponent.GetForwardVector` (`self.DefaultSceneRoot`)) 300.0) (`self.K2_GetActorLocation`)))
  (bind _output_get (set `local.L_NewDirection` (`KismetMathLibrary.MakeVector` (select `bool` (> _x 0.0) :`false` (- _x _returnvalue_2) :`true` (+ _x _returnvalue_2)) (select `bool` (> _y 0.0) :`false` (- _y _returnvalue) :`true` (+ _y _returnvalue)))))
  (return _output_get))

(fn `CalculateWeatherDirection`
  (set `self.NewDirection` (`self.CalculateDirectionInCone`))
  (set `self.NewSpeed` (`KismetMathLibrary.RandomFloatInRange` (`self.MinSpeed`) (`self.MaxSpeed`)))
  (set `self.Alpha` 0.0))

(fn `OnRep_Direction`
  (`self.OnWeatherChange` (`self.Speed`) (`self.Direction`)))

(fn `OnRep_Speed`
  (`self.OnWeatherChange` (`self.Speed`) (`self.Direction`)))

(fn `UserConstructionScript`
  (set `self.Direction` (`self.GetActorForwardVector`)))