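; Windmill building component that sets its energy speed according to the current wind.
; It finds the BP_Wind actor on begin play, then each tick normalizes that wind's speed between its min and max.
; The scaled result, multiplied by frame delta time, adds a bonus on top of the base energy speed.
; Its energy activation check always passes.
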(event `self.ReceiveBeginPlay`
  (`parent.ReceiveBeginPlay`)
  (bind _returnvalue (`GameplayStatics.GetActorOfClass` "/Game/Skyway/Core/Weather/BP_Wind.BP_Wind_C"))
  (set `self.WindRef` _returnvalue))

(event `self.ReceiveTick`
  (params (DeltaSeconds :type "Float (single-precision)"))
  (bind _baseenergyspeed (`self.BaseEnergySpeed`))
  (`parent.ReceiveTick` DeltaSeconds)
  (bind _windref (`self.WindRef`)
    (:`then`
      (set `self.EnergySpeed` (+ (* _baseenergyspeed (* (`KismetMathLibrary.NormalizeToRange` (`/Game/Skyway/Core/Weather/BP_Wind.Speed` _windref) (`/Game/Skyway/Core/Weather/BP_Wind.MinSpeed` _windref) (`/Game/Skyway/Core/Weather/BP_Wind.MaxSpeed` _windref)) 10.0) (`GameplayStatics.GetWorldDeltaSeconds`)) _baseenergyspeed)))
    (:`else`)))

(fn `CanActivateEnergy`
  (returns (ReturnValue :type Boolean))
  (return true))