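; AC_PlacedVender_Base is a base class for placed Vender buildings that generate energy and pass it to their outputs.
; Each tick it first distributes stored energy, then, if active, adds energy at a frame-rate independent rate until it reaches its maximum.
; Distribution moves a fixed per-second amount to each output in turn, only while enough energy is stored and that output has room for it.
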(event `self.ReceiveTick`
  (params (DeltaSeconds :type "Float (single-precision)"))
  (`parent.ReceiveTick` DeltaSeconds)
  (`self.GenerateEnergy`))

(fn `EnergyManagement`
  (bind _returnvalue (* (`self.MenegmentSpeed`) (`GameplayStatics.GetWorldDeltaSeconds`)))
  (for _array_element (`self.Outputs`)
    (bind _energy (`/Game/Skyway/Core/Building/AC_PlacedBuilding_Base.Energy` _array_element))
    (bind _maxenergy (`/Game/Skyway/Core/Building/AC_PlacedBuilding_Base.MaxEnergy` _array_element))
    (if (and (> (`self.Energy`) (* (`self.MenegmentSpeed`) (`GameplayStatics.GetWorldDeltaSeconds`))) (< _energy _maxenergy) (<= (+ (`/Game/Skyway/Core/Building/AC_PlacedBuilding_Base.Energy` _array_element) (* (`self.MenegmentSpeed`) (`GameplayStatics.GetWorldDeltaSeconds`))) _maxenergy))
      (set `/Game/Skyway/Core/Building/AC_PlacedBuilding_Base.Energy` (+ _energy _returnvalue) _array_element)
      (set `self.Energy` (- (`self.Energy`) _returnvalue)))))

(fn `GenerateEnergy`
  (`self.EnergyManagement`)
  (if (`self.Active`)
    (if (<= (`self.Energy`) (`self.MaxEnergy`))
      (set `self.Energy` (+ (`self.Energy`) (* (`GameplayStatics.GetWorldDeltaSeconds`) (`self.EnergySpeed`)))))))