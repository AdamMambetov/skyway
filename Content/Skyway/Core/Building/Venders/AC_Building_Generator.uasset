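; Generator building component that consumes fuel items from its own storage and gates energy activation on fuel stock and energy capacity.
; On BeginPlay it adds an AC_Storage to its owner and attaches a smoke Niagara effect shown only while active.
; Tick drains fuel progress even when inactive, consuming one item to refill it once empty and active.
; Storage contents save and load with the ship's building info.
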(event `self.ReceiveBeginPlay`
  (`parent.ReceiveBeginPlay`)
  (bind _returnvalue (`NiagaraFunctionLibrary.SpawnSystemAttached` "/Game/Skyway/Art/VFX/Smoke/NS_Smoke_2.NS_Smoke_2" self "SmokeSocket" (0.0 0.0 0.0) (struct) "KeepRelativeOffset"))
  (set `self.NS_Smoke` _returnvalue)
  (bind _returnvalue_2 (`|AddComponentByClass` :`self` (`self.GetOwner`) :`Class` "/Game/Skyway/Core/Inventory/AC_Storage.AC_Storage_C" :`InitSlotContainers` (`self.InitSlotContainers`)))
  (set `self.Storage` _returnvalue_2))

(event `self.ReceiveTick`
  (params (DeltaSeconds :type "Float (single-precision)"))
  (`parent.ReceiveTick` DeltaSeconds)
  (`self.SetVisibility` (`self.NS_Smoke`) (`self.Active`) false)
  (`self.Update Fuel`))

(event `/Game/Skyway/Core/Engine/BPI_CanSave.SaveToShip`
  (params (SaveGame :type "SaveGame Object Reference"))
  (`parent.SaveToShip` SaveGame)
  (bind _structout (setmembers `/Game/Skyway/Core/Engine/S_ShipBuildingInfo` :`StructRef` (`self.ShipBuildingInfo`) :`StorageSlotContainers` (`/Game/Skyway/Core/Inventory/AC_Storage.GetSlotContainers` (`self.Storage`))))
  (message `/Game/Skyway/Core/Ship/BPI_Ship.SetShipBuildingInfo` (`self.GetOwner`) _structout))

(event `/Game/Skyway/Core/Engine/BPI_CanSave.LoadToShip`
  (params (SaveGame :type "SaveGame Object Reference") (ShipBuildingInfo :type "/Game/Skyway/Core/Engine/S_ShipBuildingInfo Structure"))
  (`parent.LoadToShip` SaveGame ShipBuildingInfo)
  (`/Game/Skyway/Core/Engine/BPI_CanSave.LoadToShip` (`self.Storage`) SaveGame ShipBuildingInfo))

(fn `CanActivateEnergy`
  (returns (ReturnValue :type Boolean))
  (return (and (> (`.Amount_49_D1E29AF04498C178B74986AAD5610193` (break `/Game/Skyway/Core/Inventory/S_Item_Info` (`.ItemInfo_14_7E8F48144F0F01654500E084A85436C5` (break `/Game/Skyway/Core/Inventory/S_Slot_Info` (`|GetArrayItem` (`/Game/Skyway/Core/Inventory/AC_Storage.GetSlotsAtItemType` (`self.Storage`) (struct :`TagName` "SlotContainer.Storage") "NewEnumerator5")))))) 0) (<= (`self.Energy`) (`self.MaxEnergy`)))))

(fn `Update Fuel`
  (if (and (< (`self.FuelProgressBarPercent`) 0.0) (`self.Active`))
    (`/Game/Skyway/Core/Inventory/AC_Storage.RemoveSlot` (`self.Storage`) (`|GetArrayItem` (`/Game/Skyway/Core/Inventory/AC_Storage.GetSlotsAtItemType` (`self.Storage`) (struct :`TagName` "SlotContainer.Storage") "NewEnumerator5")) 1)
    (set `self.FuelProgressBarPercent` 1.0)
    (else
      (set `self.FuelProgressBarPercent` (- (`self.FuelProgressBarPercent`) (* (/ 1.0 (`self.FuelBurnSpeed`)) (`GameplayStatics.GetWorldDeltaSeconds`)))))))