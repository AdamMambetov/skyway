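; Accumulator building component for ships that stores energy and passes it between linked devices.
; EnergyManagement pulls energy from Inputs and pushes it to Outputs at a frame-time-scaled speed, gated by simple empty and full checks.
; Saving records linked devices' GUIDs in the ship building info.
; Loading matches those GUIDs against the owning ship's Devices and re-compounds each link on both ends with opposite directions.
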(event `self.ReceiveBeginPlay`
  (`parent.ReceiveBeginPlay`))

(event `self.ReceiveTick`
  (params (DeltaSeconds :type "Float (single-precision)"))
  (`parent.ReceiveTick` DeltaSeconds)
  (set `self.CompoundCable` null)
  (set `self.WBP_CompoundColor` null))

(event `/Game/Skyway/Core/Engine/BPI_CanSave.SaveToShip`
  (params (SaveGame :type "SaveGame Object Reference"))
  (`parent.SaveToShip` SaveGame)
  (bind (_inputdevices _outputdevices) (`self.GetInputAndOutputDevicesInQueue`))
  (bind _structout (setmembers `/Game/Skyway/Core/Engine/S_ShipBuildingInfo` :`StructRef` (`self.ShipBuildingInfo`) :`AccumulatorInputDevices` _inputdevices :`AccumulatorOutputDevices` _outputdevices))
  (message `/Game/Skyway/Core/Ship/BPI_Ship.SetShipBuildingInfo` (`self.GetOwner`) _structout))

(event `/Game/Skyway/Core/Engine/BPI_CanSave.LoadToShip`
  (params (SaveGame :type "SaveGame Object Reference") (ShipBuildingInfo :type "/Game/Skyway/Core/Engine/S_ShipBuildingInfo Structure"))
  (`parent.LoadToShip` SaveGame ShipBuildingInfo)
  (`self.LoadInputAndOutputDevices` ShipBuildingInfo))

(fn `EnergyManagement`
  (bind _returnvalue (* (`self.EnergySpeed`) (`GameplayStatics.GetWorldDeltaSeconds`)))
  (bind _returnvalue_2 (* (`self.EnergySpeed`) (`GameplayStatics.GetWorldDeltaSeconds`)))
  (for _array_element (`self.Inputs`)
    (bind _energy (`/Game/Skyway/Core/Building/AC_PlacedBuilding_Base.Energy` _array_element))
    (if (and (< (`self.Energy`) (`self.MaxEnergy`)) (> _energy 0.0))
      (set `/Game/Skyway/Core/Building/AC_PlacedBuilding_Base.Energy` (- _energy _returnvalue_2) _array_element)
      (set `self.Energy` (+ (`self.Energy`) _returnvalue_2))))
  (for _array_element_2 (`self.Outputs`)
    (bind _energy_2 (`/Game/Skyway/Core/Building/AC_PlacedBuilding_Base.Energy` _array_element_2))
    (if (and (> (`self.Energy`) 0.0) (< _energy_2 (`/Game/Skyway/Core/Building/AC_PlacedBuilding_Base.MaxEnergy` _array_element_2)))
      (set `/Game/Skyway/Core/Building/AC_PlacedBuilding_Base.Energy` (+ _energy_2 _returnvalue) _array_element_2)
      (set `self.Energy` (- (`self.Energy`) _returnvalue)))))

(fn `GetInputAndOutputDevicesInQueue`
  (returns (InputDevices :type "Array of Guid Structure") (OutputDevices :type "Array of Guid Structure"))
  (locals (L_Inputs :type "Array of Guid Structure") (L_Outputs :type "Array of Guid Structure"))
  (for _array_element (`self.Inputs`)
    (`KismetArrayLibrary.Array_Add` (`local.L_Inputs`) (`.Guid_51_E783821C442F8F3AEE949A989634E84B` (break `/Game/Skyway/Core/Engine/S_ShipBuildingInfo` (`/Game/Skyway/Core/Building/AC_Building_Base.ShipBuildingInfo` _array_element)))))
  (for _array_element_2 (`self.Outputs`)
    (`KismetArrayLibrary.Array_Add` (`local.L_Outputs`) (`.Guid_51_E783821C442F8F3AEE949A989634E84B` (break `/Game/Skyway/Core/Engine/S_ShipBuildingInfo` (`/Game/Skyway/Core/Building/AC_Building_Base.ShipBuildingInfo` _array_element_2)))))
  (return (`local.L_Inputs`) (`local.L_Outputs`)))

(fn `LoadInputAndOutputDevices`
  (params (S_ShipBuildingInfo :type "/Game/Skyway/Core/Engine/S_ShipBuildingInfo Structure (by ref)"))
  (locals (L_BuildingGuid :type "Guid Structure") (L_Device :type "/Game/Skyway/Core/Building/AC_PlacedBuilding_Base Object Reference"))
  (bind _asbp_ship_base (cast `/Game/Skyway/Core/Ship/BP_Ship_Base` (`self.GetOwner`)))
  (for _array_element (`/Game/Skyway/Core/Ship/BP_Ship_Base.Devices` _asbp_ship_base)
    (set `local.L_Device` _array_element)
    (set `local.L_BuildingGuid` (`.Guid_51_E783821C442F8F3AEE949A989634E84B` (break `/Game/Skyway/Core/Engine/S_ShipBuildingInfo` (`/Game/Skyway/Core/Building/AC_Building_Base.ShipBuildingInfo` (`local.L_Device`)))))
    (for _array_element_2 (`.AccumulatorInputDevices_59_855EADE74D9B97A6DE678EA8CF7F6978` (break `/Game/Skyway/Core/Engine/S_ShipBuildingInfo` (`local.S_ShipBuildingInfo`)))
      (if (== _array_element_2 (`local.L_BuildingGuid`))
        (`self.Compound` (`local.L_Device`) true (`self.Compound Color`))
        (`self.Compound` (`local.L_Device`) self false (`self.Compound Color`))
        (break)))
    (for _array_element_3 (`.AccumulatorOutputDevices_60_0FF201194437439BEE2500ABE645FA0B` (break `/Game/Skyway/Core/Engine/S_ShipBuildingInfo` (`local.S_ShipBuildingInfo`)))
      (if (== _array_element_3 (`local.L_BuildingGuid`))
        (`self.Compound` (`local.L_Device`) false (`self.Compound Color`))
        (`self.Compound` (`local.L_Device`) self true (`self.Compound Color`))
        (break)))))