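; Base component for buildings placed on a ship, handling links between devices and an Active energy state that child classes decide through CanActivateEnergy.
; It loads its DataTable row by BuildingId and adds a screen-space color widget to the owner.
; Compound and Decompound manage limited input/output slots and colored grapple cables, whose visibility can be toggled across linked devices.
; Energy saves and loads through the ship's building info.
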(event `self.ReceiveBeginPlay`
  (bind _returnvalue (`self.GetOwner`))
  (bind (_returnvalue_x _returnvalue_y) (`KismetMathLibrary.BreakVector` (`KismetMathLibrary.InverseTransformLocation` (`Actor.GetTransform` _returnvalue) (.location (`self.K2_GetComponentToWorld`)))))
  (`parent.ReceiveBeginPlay`)
  (`self.SetCollisionObjectType` "ECC_GameTraceChannel13")
  (bind _returnvalue_2 (`|GetDataTableRow` "/Game/Skyway/Core/Building/DT_Buildings_Placed.DT_Buildings_Placed" (`BlueprintGameplayTagLibrary.GetTagName` (`self.BuildingId`)))
    (:`then`
      (set `self.BuildingInfo` _returnvalue_2)
      (`KismetSystemLibrary.Delay` 1e-06)
      (bind _returnvalue_3 (`|CreateWidget` "/Game/Skyway/Core/UI/PlacedBuildingInterfaces/WBP_DeviceColor.WBP_DeviceColor_C" null (`self.Compound Color`)))
      (set `self.WBP_CompoundColor` _returnvalue_3)
      (bind _returnvalue_4 (`|AddComponentByClass` _returnvalue "/Script/UMG.WidgetComponent" false (`KismetMathLibrary.MakeTransform` (`KismetMathLibrary.MakeVector` _returnvalue_x _returnvalue_y 150.0) (.rotation (`self.K2_GetComponentToWorld`)) (.scale (`self.K2_GetComponentToWorld`)))))
      (set `self.CompoundColorComp` _returnvalue_4)
      (`self.SetCollisionEnabled` _returnvalue_4 "NoCollision")
      (`WidgetComponent.SetWidgetSpace` _returnvalue_4 "Screen")
      (`WidgetComponent.SetWidget` _returnvalue_4 _returnvalue_3)
      (`WidgetComponent.SetDrawSize` _returnvalue_4 (150.0 150.0))
      (`self.SetCompoundColorVisibility` false))))

(event `self.ReceiveTick`
  (params (DeltaSeconds :type "Float (single-precision)"))
  (if (!= (`self.CanActivateEnergy`) (`self.Active`))
    (set `self.Active` (`self.CanActivateEnergy`))))

(event `/Game/Skyway/Core/Engine/BPI_CanSave.SaveToShip`
  (params (SaveGame :type "SaveGame Object Reference"))
  (`parent.SaveToShip` SaveGame)
  (bind _returnvalue (message `/Game/Skyway/Core/Ship/BPI_Ship.GetShipBuildingInfo` (`self.GetOwner`) (`.Guid_51_E783821C442F8F3AEE949A989634E84B` (break `/Game/Skyway/Core/Engine/S_ShipBuildingInfo` (`self.ShipBuildingInfo`)))))
  (bind _structout (setmembers `/Game/Skyway/Core/Engine/S_ShipBuildingInfo` :`StructRef` _returnvalue :`Energy` (`self.Energy`)))
  (message `/Game/Skyway/Core/Ship/BPI_Ship.SetShipBuildingInfo` (`self.GetOwner`) _structout))

(event `/Game/Skyway/Core/Engine/BPI_CanSave.LoadToShip`
  (params (SaveGame :type "SaveGame Object Reference") (ShipBuildingInfo :type "/Game/Skyway/Core/Engine/S_ShipBuildingInfo Structure"))
  (`parent.LoadToShip` SaveGame ShipBuildingInfo)
  (set `self.Energy` (`.Energy_48_13505A3C40FFE0ABF3DC7FB5AB736F63` (break `/Game/Skyway/Core/Engine/S_ShipBuildingInfo` ShipBuildingInfo))))

(fn `CanActivateEnergy`
  (returns (ReturnValue :type Boolean))
  (return false))

(fn `Compound`
  (params (CompoundDevice :type "/Game/Skyway/Core/Building/AC_PlacedBuilding_Base Object Reference") (In :type Boolean) (CompoundColor :type "LinearColor Structure"))
  (returns (ReturnValue :type Boolean))
  (set `self.Compound Color` CompoundColor)
  (if (> (`KismetMathLibrary.SelectInt` (`self.FreeInputCount`) (`self.FreeOutputCount`) (`local.In`)) 0)
    (`KismetArrayLibrary.Array_Add` (select `bool` (`local.In`) :`false` (`self.Outputs`) :`true` (`self.Inputs`)) (`local.CompoundDevice`))
    (`/Engine/EditorBlueprintResources/StandardMacros.DecrementInt` (select `bool` (`local.In`) :`false` (`self.FreeOutputCount`) :`true` (`self.FreeInputCount`))
      (:`  `
        (`self.CreateCompoundCable` (`local.CompoundDevice`))
        (return true)))
    (else
      (return false))))

(fn `CreateCompoundCable`
  (params (CompoundDevice :type "SceneComponent Object Reference"))
  (bind _returnvalue (`|SpawnActorFromClass` "/Game/Skyway/Core/Hook/BP_GrappleCable.BP_GrappleCable_C" (`/Game/Skyway/Core/Engine/MLBP_Defaults.DEFAULT`) "Undefined" "OverrideRootScale" null null))
  (`Actor.K2_AttachToComponent` _returnvalue self "None" "KeepRelative" "KeepRelative" "KeepRelative" true)
  (bind _cablecomponent (`CableActor.CableComponent` _returnvalue))
  (`CableComponent.SetAttachEndToComponent` _cablecomponent CompoundDevice "None")
  (`Actor.K2_SetActorLocation` _returnvalue (+ (`Actor.K2_GetActorLocation` _returnvalue) (0.0 0.0 50.0)) false false)
  (set `CableComponent.EndLocation` (0.0 0.0 50.0) _cablecomponent)
  (`/Game/Skyway/Core/Hook/BP_GrappleCable.SetCableColor` _returnvalue (`self.Compound Color`))
  (`Actor.SetActorHiddenInGame` _returnvalue (not (`self.ConpoundCableVisibility`)))
  (set `self.CompoundCable` _returnvalue))

(fn `Decompound`
  (params (DecompoundDevice :type "/Game/Skyway/Core/Building/AC_PlacedBuilding_Base Object Reference"))
  (returns (ReturnValue :type Boolean))
  (set `self.Compound Color` (struct))
  (bind _compoundcable (`self.CompoundCable`)
    (:`then`
      (`Actor.K2_DestroyActor` _compoundcable))
    (:`else`
      _))
  (bind _returnvalue (`KismetArrayLibrary.Array_RemoveItem` (`self.Outputs`) DecompoundDevice))
  (if _returnvalue
    (`/Engine/EditorBlueprintResources/StandardMacros.IncrementInt` (`self.FreeOutputCount`)
      (:`  `
        (`self.Decompound` DecompoundDevice self)
        (return true)))
    (else
      (bind _returnvalue_2 (`KismetArrayLibrary.Array_RemoveItem` (`self.Inputs`) DecompoundDevice))
      (if _returnvalue_2
        (`/Engine/EditorBlueprintResources/StandardMacros.IncrementInt` (`self.FreeInputCount`)
          (:`  `
            (`self.Decompound` DecompoundDevice self)
            (return true)))
        (else
          (return false))))))

(fn `Interact`
  (returns (ReturnValue :type "/Game/Skyway/Core/Inventory/S_Building_Info Structure"))
  (return (`self.BuildingInfo`)))

(fn `OnDeviceColorClicked`
  (params (FingerIndex :type "ETouchIndex Enum" :default "Touch1") (TouchedComponent :type "PrimitiveComponent Object Reference"))
  (`KismetSystemLibrary.PrintString` "Hello")
  (`self.SetVisibilityCompoundCable` (not (`self.ConpoundCableVisibility`))))

(fn `OnRep_Compound Color`
  (bind (_r _g _b _a) (break `LinearColor` (`self.Compound Color`)))
  (`self.WBP_CompoundColor`
    (:`then`
      (setmembers `LinearColor` :`StructRef` (`/Game/Skyway/Core/UI/PlacedBuildingInterfaces/WBP_DeviceColor.Color` (`self.WBP_CompoundColor`)) :`R` _r :`G` _g :`B` _b :`A` (- _a 0.3))
      (`WidgetComponent.SetWidget` (`self.CompoundColorComp`) (`self.WBP_CompoundColor`)))
    (:`else`)))

(fn `SetCompoundColorVisibility`
  (params (Visible :type Boolean))
  (bind _wbp_compoundcolor (`self.WBP_CompoundColor`))
  (`/Engine/EditorBlueprintResources/StandardMacros.IsValid` _wbp_compoundcolor
    (:`Is Valid`
      (`Widget.SetVisibility` (`/Game/Skyway/Core/UI/PlacedBuildingInterfaces/WBP_DeviceColor.Image_18` _wbp_compoundcolor) (select `bool` Visible :`false` "Hidden" :`true` "Visible" :!type "ESlateVisibility Enum"))
      (`WidgetComponent.SetWidget` (`self.CompoundColorComp`) (`self.WBP_CompoundColor`)))))

(fn `SetVisibilityCompoundCable`
  (params (NewVisibility :type Boolean))
  (bind _compoundcable (`self.CompoundCable`))
  (set `self.ConpoundCableVisibility` NewVisibility)
  (`/Engine/EditorBlueprintResources/StandardMacros.IsValid` _compoundcable
    (:`Is Valid`
      (`Actor.SetActorHiddenInGame` _compoundcable (not NewVisibility)))
    (:`Is Not Valid`
      _))
  (for _array_element (`self.Outputs`)
    (bind _compoundcable_2 (`/Game/Skyway/Core/Building/AC_PlacedBuilding_Base.CompoundCable` _array_element)
      (:`then`
        (set `/Game/Skyway/Core/Building/AC_PlacedBuilding_Base.ConpoundCableVisibility` NewVisibility _array_element)
        (`Actor.SetActorHiddenInGame` _compoundcable_2 (not NewVisibility)))
      (:`else`)))
  (for _array_element_2 (`self.Inputs`)
    (bind _compoundcable_3 (`/Game/Skyway/Core/Building/AC_PlacedBuilding_Base.CompoundCable` _array_element_2)
      (:`then`
        (set `/Game/Skyway/Core/Building/AC_PlacedBuilding_Base.ConpoundCableVisibility` NewVisibility _array_element_2)
        (`Actor.SetActorHiddenInGame` _compoundcable_3 (not NewVisibility)))
      (:`else`))))