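; Triangular floor piece component for the building system, providing the collision components for its floor and wall sides.
; SpawnCollisions runs the parent version, then adds an AC_BuildingCollision to the owner for each entry in CollisionPositions and stores it in Collisions.
; An older per-side spawn chain with debug collisions is left unconnected.
; GetBuildingCollisions still returns the six named variables that only that chain assigns, rather than the Collisions array.
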(fn `GetBuildingCollisions`
  (returns (ReturnArray :type "Array of /Game/Skyway/Core/Building/AC_BuildingCollision Object Reference"))
  (return (`|MakeArray` (`self.FloorCollisionBackward`) (`self.FloorCollisionLeft`) (`self.FloorCollisionRight`) (`self.WallCollisionBackward`) (`self.WallCollisionLeft`) (`self.WallCollisionRight`))))

(fn `SpawnCollisions`
  (`parent.SpawnCollisions`)
  (for _array_element (`self.CollisionPositions`)
    (bind _returnvalue (`|AddComponentByClass` (`self.GetOwner`) "/Game/Skyway/Core/Building/AC_BuildingCollision.AC_BuildingCollision_C" false (`/Game/Skyway/Core/Engine/MLBP_Defaults.DEFAULT`) _array_element self))
    (`KismetArrayLibrary.Array_Add` (`self.Collisions`) _returnvalue)))