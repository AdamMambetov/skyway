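; Base Blueprint for placed venders in the Skyway building system that accumulates energy over time.
; While Active, Tick calls GenerateEnergy, which adds EnergySpeed scaled by world delta seconds to Energy.
; Accumulation stops once Energy exceeds MaxEnergy, with no clamp, so the value can slightly overshoot the limit.
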(event `self.ReceiveTick`
  (params (DeltaSeconds :type "Float (single-precision)"))
  (`parent.ReceiveTick` DeltaSeconds)
  (if (`self.Active`)
    (`self.GenerateEnergy`)))

(fn `GenerateEnergy`
  (if (<= (`self.Energy`) (`self.MaxEnergy`))
    (set `self.Energy` (+ (`self.Energy`) (* (`GameplayStatics.GetWorldDeltaSeconds`) (`self.EnergySpeed`))))))