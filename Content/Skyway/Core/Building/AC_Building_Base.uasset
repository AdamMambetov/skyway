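; Base component for ship building pieces, which generates collision components marking the socket positions on its static mesh.
; On BeginPlay it maps the mesh sockets it finds to position enums through server events, then spawns an AC_BuildingCollision for each via multicast.
; It also sets its collision channel, offers a debug arrow-and-label helper, and leaves SetMesh, GetHit and Interact as stubs.
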(event `self.ReceiveBeginPlay`
  (`self.InitCollisionPositions_SERVER`)
  (`self.SpawnCollisions_SERVER`)
  (`self.SetCollisionObjectType` "ECC_GameTraceChannel12"))

(event `SpawnCollisions_SERVER`
  (`self.SpawnCollisions_MULTI`))

(event `SpawnCollisions_MULTI`
  (`self.SpawnCollisions`))

(event `InitCollisionPositions_SERVER`
  (`self.InitCollisionPositions`))

(event `/Game/Skyway/Core/Building/BPI_Build.SetMesh`
  (params (Mesh :type "StaticMesh Object Reference")))

(fn `CreateDebugCollision`
  (params (Collision :type "BoxComponent Object Reference") (CollisionDirection :type Text))
  (locals (L_DebugArrow :type "ArrowComponent Object Reference") (L_DebugText :type "TextRenderComponent Object Reference"))
  (bind _returnvalue (`/Game/Skyway/Core/Engine/FLBP_Defaults.GetDebugUseCase`))
  (if _returnvalue
    (bind _returnvalue_2 (`|AddComponentByClass` (`self.GetOwner`) "/Script/Engine.ArrowComponent" false (`/Game/Skyway/Core/Engine/MLBP_Defaults.DEFAULT`)))
    (bind _output_get (set `local.L_DebugArrow` _returnvalue_2))
    (`self.K2_AttachToComponent` _output_get (`local.Collision`) "None" "KeepRelative" "KeepRelative" "KeepRelative" true)
    (`self.SetHiddenInGame` (`local.L_DebugArrow`) false false)
    (bind _returnvalue_3 (`|AddComponentByClass` (`self.GetOwner`) "/Script/Engine.TextRenderComponent" false (`/Game/Skyway/Core/Engine/MLBP_Defaults.DEFAULT`)))
    (bind _output_get_2 (set `local.L_DebugText` _returnvalue_3))
    (`self.K2_AttachToComponent` _output_get_2 (`local.Collision`) "None" "KeepRelative" "KeepRelative" "KeepRelative" true)
    (`TextRenderComponent.SetTextRenderColor` :`self` (`local.L_DebugText`))
    (`TextRenderComponent.K2_SetText` (`local.L_DebugText`) (`local.CollisionDirection`))))

(fn `GetBuildingCollisions`
  (returns (ReturnArray :type "Array of /Game/Skyway/Core/Building/AC_BuildingCollision Object Reference"))
  (return (`self.Collisions`)))

(fn `GetHit`
  (returns (HitMesh :type Boolean))
  (return false))

(fn `GetShip`
  (returns (ReturnValue :type "/Game/Skyway/Core/Ship/BP_Ship_Base Object Reference"))
  (bind _asbp_ship_base (cast `/Game/Skyway/Core/Ship/BP_Ship_Base` (`self.GetOwner`)))
  (return _asbp_ship_base))

(fn `InitCollisionPositions`
  (`KismetArrayLibrary.Array_Clear` (`self.CollisionPositions`))
  (for (_array_element _array_index) (`self.AllBuildingSockets`)
    (if (`KismetSystemLibrary.IsValid` (`StaticMesh.FindSocket` (`self.StaticMesh`) _array_element))
      (`KismetArrayLibrary.Array_Add` (`self.CollisionPositions`) (cast `/Game/Skyway/Core/Building/E_BuildingCollisionPosition` (`KismetMathLibrary.Conv_IntToByte` _array_index))))))

(fn `Interact`
  (returns (ReturnValue :type "/Game/Skyway/Core/Inventory/S_Building_Info Structure"))
  (return))

(fn `SpawnCollisions`
  (`KismetArrayLibrary.Array_Clear` (`self.Collisions`))
  (for _array_element (`self.CollisionPositions`)
    (bind _returnvalue (`|AddComponentByClass` (`self.GetOwner`) "/Game/Skyway/Core/Building/AC_BuildingCollision.AC_BuildingCollision_C" false (`/Game/Skyway/Core/Engine/MLBP_Defaults.DEFAULT`) _array_element self))
    (`KismetArrayLibrary.Array_Add` (`self.Collisions`) _returnvalue)))