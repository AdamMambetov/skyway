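; Building component for a fuel-burning generator that consumes stored items while active.
; On BeginPlay it adds an AC_Storage component with a Piece-item container to its owner.
; Each tick it drains a fuel progress bar, removing one fuel item and refilling the bar when it drops below zero while active.
; CanActivateEnergy allows activation only when fuel is stored and energy does not exceed its maximum.
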(event `self.ReceiveBeginPlay`
  (`parent.ReceiveBeginPlay`)
  (bind _returnvalue (`|AddComponentByClass` (`self.GetOwner`) "/Game/Skyway/Core/Inventory/AC_Storage.AC_Storage_C" (`|MakeArray` (make `/Game/Skyway/Core/Inventory/S_SlotContainer_Info` :`Id` (struct :`TagName` "SlotContainer.Storage") :`StoredItemTypes` (struct :`GameplayTags` (struct :`(TagName` "Item.Piece")))))))
  (set `self.Storage` _returnvalue))

(event `self.ReceiveTick`
  (params (DeltaSeconds :type "Float (single-precision)"))
  (`parent.ReceiveTick` DeltaSeconds)
  (`self.Update Fuel`))

(fn `CanActivateEnergy`
  (returns (ReturnValue :type Boolean))
  (return (and (> (`.Amount_49_D1E29AF04498C178B74986AAD5610193` (break `/Game/Skyway/Core/Inventory/S_Item_Info` (`.ItemInfo_14_7E8F48144F0F01654500E084A85436C5` (break `/Game/Skyway/Core/Inventory/S_Slot_Info` (`|GetArrayItem` (`/Game/Skyway/Core/Inventory/AC_Storage.GetSlotsAtItemType` (`self.Storage`) (struct :`TagName` "SlotContainer.Storage") "NewEnumerator5")))))) 0) (<= (`self.Energy`) (`self.MaxEnergy`)))))

(fn `Update Fuel`
  (if (and (< (`self.FuelProgressBarPercent`) 0.0) (`self.Active`))
    (`/Game/Skyway/Core/Inventory/AC_Storage.RemoveSlot` (`self.Storage`) (`|GetArrayItem` (`/Game/Skyway/Core/Inventory/AC_Storage.GetSlotsAtItemType` (`self.Storage`) (struct :`TagName` "SlotContainer.Storage") "NewEnumerator5")) 1)
    (set `self.FuelProgressBarPercent` 1.0)
    (else
      (set `self.FuelProgressBarPercent` (- (`self.FuelProgressBarPercent`) (* (`self.FuelBurnSpeed`) (`GameplayStatics.GetWorldDeltaSeconds`)))))))