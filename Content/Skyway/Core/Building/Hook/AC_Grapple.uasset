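; Grappling hook component for a Character that fires a hook projectile with an attached cable actor.
; Hits on actors tagged CanBeGrappled reel them toward the owner; other hits launch the owner toward the hook with gravity, friction and air control zeroed.
; Tick updates cable length and pull, destroying the hook on distance limits or when the owner passes it.
; Hook destruction, including cancel, removes the cable and restores hard-coded movement values.
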(event `self.ReceiveBeginPlay`
  (bind _ascharacter (cast `Character` (`self.GetOwner`)))
  (set `self.OwnerCharacterMovement` (`Character.CharacterMovement` _ascharacter))
  (bind _asbp_main_character (cast `/Game/Skyway/Core/Engine/BP_MainCharacter` (`GameplayStatics.GetPlayerCharacter` 0)))
  (set `self.MainCharacterRef` _asbp_main_character))

(event `self.ReceiveTick`
  (params (DeltaSeconds :type "Float (single-precision)"))
  (bind _returnvalue (* (* (* (`self.ToGrappleHook`) -1.0) (`self.GrappleSpeed`)) (`GameplayStatics.GetWorldDeltaSeconds`)))
  (switch `/Game/Skyway/Core/Building/Hook/E_HookState` (`self.GrappleState`)
    (:`NewEnumerator1`
      (bind _grapplecable (`self.GrappleCable`)
        (:`then`
          (set `CableComponent.CableLength` (- (`self.CalculateCableLength`) 100.0) (`CableActor.CableComponent` _grapplecable))
          (if (> (`self.CalculateCableLength`) (+ (`self.MinGrappleDistace`) 1000.0))
            (`self.DestroyCable`)))
        (:`else`)))
    (:`NewEnumerator2`
      (bind _grapplecable_2 (`self.GrappleCable`)
        (:`then`
          (set `CableComponent.CableLength` 0.0 (`CableActor.CableComponent` _grapplecable_2))
          (`CharacterMovementComponent.AddForce` (`self.OwnerCharacterMovement`) (* (`self.ToGrappleHook`) 100000.0))
          (`self.DestroyCable`))
        (:`else`)))
    (:`NewEnumerator3`
      (bind _grapplecable_3 (`self.GrappleCable`)
        (:`then`
          (set `CableComponent.CableLength` 0.0 (`CableActor.CableComponent` _grapplecable_3))
          (`Actor.K2_AddActorWorldOffset` (`self.HitActor`) _returnvalue false false)
          (`Actor.K2_AddActorWorldOffset` (`self.GrappleHook`) _returnvalue false false)
          (`self.DestroyCable`))
        (:`else`)))))

(fn `CancelGrapple`
  (bind _grapplehook (`self.GrappleHook`)
    (:`then`
      (`Actor.K2_DestroyActor` _grapplehook))
    (:`else`)))

(fn `DestroyCable`
  (bind _returnvalue (`KismetMathLibrary.Vector_Distance` (`Actor.K2_GetActorLocation` (`self.GrappleHook`)) (`Actor.K2_GetActorLocation` (`self.GetOwner`))))
  (if (or (> _returnvalue (`self.MaxGrappleDistace`)) (< _returnvalue (`self.MinGrappleDistace`)))
    (`Actor.K2_DestroyActor` (`self.GrappleHook`))
    (elif (and (`|EnumInequality` (`self.GrappleState`) "NewEnumerator1") (< (`KismetMathLibrary.Dot_VectorVector` (`self.InitialHookDirection2D`) (`self.ToGrappleHook2D`)) 0.0) (`|EnumInequality` (`self.GrappleState`) "NewEnumerator3"))
      (`Actor.K2_DestroyActor` (`self.GrappleHook`)))))

(fn `FireGrapple`
  (params (TargetLocation :type "Vector Structure") (LocalOffset :type "Vector Structure"))
  (locals (L_FireDirection :type "Vector Structure" :default (0.0 0.0 0.0)))
  (if (not (`self.IsUse?`))
    (set `self.GrappleState` "NewEnumerator1")
    (set `local.L_FireDirection` (`KismetMathLibrary.Normal` (- (`local.TargetLocation`) (`self.CableStartLocation` (`local.LocalOffset`)))))
    (bind _returnvalue (`|SpawnActorFromClass` "/Game/Skyway/Core/Building/Hook/BP_GrappleHook.BP_GrappleHook_C" (`KismetMathLibrary.MakeTransform` (`self.CableStartLocation` (`local.LocalOffset`))) "Undefined" "OverrideRootScale" null (* (`local.L_FireDirection`) (`self.HookSpeed`)) null))
    (bind _output_get (set `self.GrappleHook` _returnvalue))
    (add `Actor.OnActorHit` _output_get (`|CreateDelegate` :!event `OnGrappleHit`))
    (add `Actor.OnDestroyed` (`self.GrappleHook`) (`|CreateDelegate` :!event `OnGrappleDestroyed`))
    (bind _returnvalue_2 (`|SpawnActorFromClass` "/Game/Skyway/Core/Building/Hook/BP_GrappleCable.BP_GrappleCable_C" (`KismetMathLibrary.MakeTransform` (`self.CableStartLocation` (`local.LocalOffset`)) (`KismetMathLibrary.MakeRotFromX` (`local.L_FireDirection`))) "Undefined" "OverrideRootScale" null null))
    (set `CharacterMovementComponent.MaxWalkSpeed` 150.0 (`self.OwnerCharacterMovement`))
    (bind _output_get_2 (set `self.GrappleCable` _returnvalue_2))
    (`Actor.K2_AttachToActor` _output_get_2 (`self.GetOwner`) "None" "KeepWorld" "KeepWorld" "KeepWorld" true)
    (`CableComponent.SetAttachEndTo` (`CableActor.CableComponent` (`self.GrappleCable`)) (`self.GrappleHook`) "None" "None")
    (set `CableComponent.EndLocation` (0.0 0.0 0.0) (`CableActor.CableComponent` (`self.GrappleCable`)))))

(fn `IsUse?`
  (returns (ReturnValue :type Boolean))
  (return (select `/Game/Skyway/Core/Building/Hook/E_HookState` (`self.GrappleState`) :`NewEnumerator1` true :`NewEnumerator2` true :`NewEnumerator3` true)))

(fn `OnGrappleDestroyed`
  (params (DestroyedActor :type "Actor Object Reference"))
  (set `self.GrappleHook` null)
  (set `self.GrappleState` "NewEnumerator0")
  (`|ExecutionSequence`
    (:`then_0`
      (bind _grapplecable (`self.GrappleCable`)
        (:`then`
          (`Actor.K2_DestroyActor` _grapplecable)
          (set `self.GrappleCable` null))
        (:`else`)))
    (:`then_1`
      (bind _ascharacter (cast `Character` (`self.GetOwner`)))
      (bind _charactermovement (`Character.CharacterMovement` _ascharacter))
      (set `CharacterMovementComponent.GroundFriction` 8.0 _charactermovement)
      (set `CharacterMovementComponent.GravityScale` 3.0 _charactermovement)
      (set `CharacterMovementComponent.AirControl` 1.0 _charactermovement)
      (set `CharacterMovementComponent.MaxWalkSpeed` 1500.0 _charactermovement))))

(fn `OnGrappleHit`
  (params (SelfActor :type "Actor Object Reference") (OtherActor :type "Actor Object Reference") (NormalImpulse :type "Vector Structure") (Hit :type "HitResult Structure (by ref)"))
  (bind (_bblockinghit _binitialoverlap _time _distance _location _impactpoint _normal _impactnormal _physmat _hitactor) (`GameplayStatics.BreakHitResult` Hit))
  (if (not (`Actor.ActorHasTag` _hitactor "CanBeGrappled"))
    (set `self.GrappleState` "NewEnumerator2")
    (bind _ascharacter (cast `Character` (`self.GetOwner`)))
    (bind _charactermovement (`Character.CharacterMovement` _ascharacter))
    (set `CharacterMovementComponent.GroundFriction` 0.0 _charactermovement)
    (set `CharacterMovementComponent.GravityScale` 0.0 _charactermovement)
    (set `CharacterMovementComponent.AirControl` 0.0 _charactermovement)
    (set `CharacterMovementComponent.MaxWalkSpeed` 1500.0 _charactermovement)
    (set `MovementComponent.Velocity` (* (`self.ToGrappleHook`) (`self.GrappleSpeed`)) _charactermovement)
    (`Character.Jump` (`self.MainCharacterRef`))
    (set `self.InitialHookDirection2D` (`self.ToGrappleHook2D`))
    (else
      (set `self.HitActor` _hitactor)
      (set `self.GrappleState` "NewEnumerator3"))))