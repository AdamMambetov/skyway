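; BP_GrappleHook is the projectile actor for a grappling hook, destroying itself once it travels beyond the grapple's range.
; On BeginPlay it applies its Velocity variable to the ProjectileMovement component and records its starting location.
; Each Tick it compares the distance from that start with the max distance read from its Grapple reference.
; The file contains no hit or attach logic.
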(event `self.ReceiveBeginPlay`
  (set `MovementComponent.Velocity` (`self.Velocity`) (`self.ProjectileMovement`))
  (set `self.StartLocation` (`self.K2_GetActorLocation`)))

(event `self.ReceiveTick`
  (params (DeltaSeconds :type "Float (single-precision)"))
  (if (< (`/Game/Skyway/Core/Building/Hook/AC_Grapple.MaxGrappleDistace` (`self.Grapple`)) (`KismetMathLibrary.Vector_Distance` (`self.StartLocation`) (`self.K2_GetActorLocation`)))
    (`self.K2_DestroyActor`)))

(fn `UserConstructionScript`)