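; Building component for a charging station that restores Energy and Health to an actor standing within its range.
; On BeginPlay it adds a box collision to its owner, raised above the component, and has the ship destroy it on EndPlay.
; Overlap serves one actor with a stat component at a time, running a looping timer that applies immediate server-side stat modifiers scaled by the interval until that actor leaves.
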(event `self.ReceiveBeginPlay`
  (bind (_returnvalue_location _returnvalue_rotation _returnvalue_scale) (`KismetMathLibrary.BreakTransform` (`self.GetRelativeTransform`)))
  (`parent.ReceiveBeginPlay`)
  (bind _returnvalue (`|AddComponentByClass` (`self.GetOwner`) "/Script/Engine.BoxComponent" false (`KismetMathLibrary.MakeTransform` (+ _returnvalue_location (0.0 0.0 100.0)) _returnvalue_rotation _returnvalue_scale)))
  (set `self.BoxCollision` _returnvalue)
  (`BoxComponent.SetBoxExtent` (`self.BoxCollision`) (`self.In Box Extent`) true)
  (add `PrimitiveComponent.OnComponentBeginOverlap` (`self.BoxCollision`) (`|CreateDelegate` :!event `OnComponentBeginOverlap_Event`))
  (add `PrimitiveComponent.OnComponentEndOverlap` (`self.BoxCollision`) (`|CreateDelegate` :!event `OnComponentEndOverlap_Event`)))

(event `self.ReceiveEndPlay`
  (params (EndPlayReason :type "EEndPlayReason Enum" :default "Destroyed"))
  (bind _returnvalue (`self.GetShip`))
  (`/Game/Skyway/Core/Ship/BP_Ship_Base.DestroyComponent_SERVER` _returnvalue (`self.BoxCollision`)))

(fn `OnComponentBeginOverlap_Event`
  (params (OverlappedComponent :type "PrimitiveComponent Object Reference") (OtherActor :type "Actor Object Reference") (OtherComp :type "PrimitiveComponent Object Reference") (OtherBodyIndex :type Integer) (bFromSweep :type Boolean) (SweepResult :type "HitResult Structure (by ref)"))
  (locals (L_OverlappedActorStatComp :type "/Game/Skyway/Core/Stats/AC_StatComponent Object Reference"))
  (set `local.L_OverlappedActorStatComp` (`Actor.GetComponentByClass` OtherActor "/Game/Skyway/Core/Stats/AC_StatComponent.AC_StatComponent_C"))
  (if (and (`KismetSystemLibrary.IsValid` (`local.L_OverlappedActorStatComp`)) (not (`KismetSystemLibrary.IsValid` (`self.OverlappedActorStatComp`))))
    (set `self.OverlappedActorStatComp` (`local.L_OverlappedActorStatComp`))
    (bind _returnvalue (`KismetSystemLibrary.K2_SetTimerDelegate` (`|CreateDelegate` :!event `RestoreTimerFunc`) (`self.Time`) true))
    (set `self.RestoreTimerHandle` _returnvalue)))

(fn `OnComponentEndOverlap_Event`
  (params (OverlappedComponent :type "PrimitiveComponent Object Reference") (OtherActor :type "Actor Object Reference") (OtherComp :type "PrimitiveComponent Object Reference") (OtherBodyIndex :type Integer))
  (if (== (`self.OverlappedActorStatComp`) (`Actor.GetComponentByClass` (`local.OtherActor`) "/Game/Skyway/Core/Stats/AC_StatComponent.AC_StatComponent_C"))
    (set `self.OverlappedActorStatComp` null)
    (`KismetSystemLibrary.K2_ClearAndInvalidateTimerHandle` (`self.RestoreTimerHandle`))))

(fn `RestoreTimerFunc`
  (bind _overlappedactorstatcomp (`self.OverlappedActorStatComp`)
    (:`then`
      (`/Game/Skyway/Core/Stats/AC_StatComponent.ChangeStatValueById_SERVER` _overlappedactorstatcomp (make `/Game/Skyway/Core/Stats/S_StatModifier` :`Id` (struct :`TagName` "Stat.Energy") :`Value` (* (`self.RestoreValue`) (`self.Time`)) :`TypeContainer` (struct :`GameplayTags` (struct :`(TagName` "StatModifier.Immediately")))))
      (`/Game/Skyway/Core/Stats/AC_StatComponent.ChangeStatValueById_SERVER` (`self.OverlappedActorStatComp`) (make `/Game/Skyway/Core/Stats/S_StatModifier` :`Id` (struct :`TagName` "Stat.Health") :`Value` (* (`self.RestoreValue`) (`self.Time`)) :`TypeContainer` (struct :`GameplayTags` (struct :`(TagName` "StatModifier.Immediately"))))))
    (:`else`)))