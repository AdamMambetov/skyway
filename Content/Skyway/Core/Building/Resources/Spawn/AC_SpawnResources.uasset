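; Actor component that spawns random resource pickups around a point offset from its owner along a settable direction.
; On BeginPlay it sorts DT_Raws rows into per-level arrays, re-adding the accumulated list after each row, so earlier rows repeat.
; Tick calls a server event that spawns level-1 pickups in a box, rejecting points too near its center.
; A delay throttles successful spawns, and a capped list drops pickups when destroyed.
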(event `self.ReceiveBeginPlay`
  (`self.SortResourcesByLevel`))

(event `self.ReceiveTick`
  (params (DeltaSeconds :type "Float (single-precision)"))
  (`self.SpawnRandomResourcesInRadius_SERVER`))

(event `SpawnRandomResourcesInRadius_SERVER`
  (if (and (`self.bCanSpawn`) (< (`KismetArrayLibrary.Array_Length` (`self.SpawnedResources`)) 50))
    (bind _returnvalue (`self.SpawnRandomResourcesInRadius` 5000.0 1 (`self.Direction`)))
    (if _returnvalue
      (set `self.bCanSpawn` false)
      (`KismetSystemLibrary.Delay` (`self.DurationOfSpawn`))
      (set `self.bCanSpawn` true))))

(event `OnDestroyed_Event`
  (params (DestroyedActor :type "Actor Object Reference"))
  (`KismetArrayLibrary.Array_RemoveItem` (`self.SpawnedResources`) DestroyedActor))

(fn `SetSpawnDirection`
  (params (Direction :type "Vector Structure"))
  (set `self.Direction` Direction))

(fn `SortResourcesByLevel`
  (bind _outrownames (`DataTableFunctionLibrary.GetDataTableRowNames` "/Game/Skyway/Core/Inventory/DT_Raws.DT_Raws"))
  (for _array_element _outrownames
    (bind _returnvalue (`|GetDataTableRow` "/Game/Skyway/Core/Inventory/DT_Raws.DT_Raws" _array_element)
      (:`then`
        (`KismetArrayLibrary.Array_Add` (`self.Resources`) _returnvalue)
        (for _array_element_2 (`self.Resources`)
          (`KismetArrayLibrary.Array_Add` (select `int` (`.Lvl_5_F4DBF3354965105D0BF32887533C8DC1` (break `/Game/Skyway/Core/Inventory/S_Raw_Info` _array_element_2)) :`0` _ :`1` (`self.Resources1LVL`) :`2` (`self.Resources2LVL`) :`3` (`self.Resources3LVL`)) _array_element_2))))))

(fn `SpawnRandomResourcesInRadius`
  (params (SpawnRadius :type "Float (double-precision)") (LVL :type Integer) (Direction :type "Vector Structure"))
  (returns (ReturnValue :type Boolean))
  (locals (L_RandomLocation :type "Vector Structure") (L_EndLocation :type "Vector Structure"))
  (bind _spawnedresources (`self.SpawnedResources`))
  (bind _returnvalue (/ (`local.SpawnRadius`) 2.0))
  (bind _returnvalue_2 (select `int` (`local.LVL`) :`0` _ :`1` (`self.Resources1LVL`) :`2` (`self.Resources2LVL`) :`3` (`self.Resources3LVL`)))
  (set `local.L_EndLocation` (+ (* (`self.Direction`) (`local.SpawnRadius`)) (`Actor.K2_GetActorLocation` (`self.GetOwner`))))
  (set `local.L_RandomLocation` (`KismetMathLibrary.RandomPointInBoundingBox` (`local.L_EndLocation`) (`KismetMathLibrary.MakeVector` _returnvalue _returnvalue 500.0)))
  (if (> (`KismetMathLibrary.Vector_Distance` (`local.L_EndLocation`) (`local.L_RandomLocation`)) (`self.MIN_SPAWN_DISTANCE`))
    (set `self.ResourceIndex` (`KismetMathLibrary.RandomInteger` (`KismetArrayLibrary.Array_Length` _returnvalue_2)))
    (bind _returnvalue_3 (`|SpawnActorFromClass` (`.PickupClass_16_8EC98BA448AF05C0A6A44BBA159DB3E1` (break `/Game/Skyway/Core/Inventory/S_Raw_Info` (`|GetArrayItem` _returnvalue_2 (`self.ResourceIndex`)))) (`KismetMathLibrary.MakeTransform` (`local.L_RandomLocation`) (`KismetMathLibrary.RandomRotator` true) (`/Game/Skyway/Core/Engine/MLBP_Defaults.DEFAULT_SCALE`)) "Undefined" "OverrideRootScale" null null))
    (bind _returnvalue_4 (`KismetArrayLibrary.Array_Add` _spawnedresources _returnvalue_3))
    (add `Actor.OnDestroyed` (`|GetArrayItem` _spawnedresources _returnvalue_4) (`|CreateDelegate` :!event `OnDestroyed_Event`))
    (return true)
    (else
      (return false))))