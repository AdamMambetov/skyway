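; Ship building component for a charging machine that uses energy to craft charged batteries through a recycle recipe.
; It adds storage and crafting components at BeginPlay, and its energy check tests recycle input, output slot and energy level.
; Tick pauses or resumes crafting with the Active state and plays electric audio, while each craft end requests another.
; Storage persists with the ship, with slot updates triggering a fast save.
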(event `self.ReceiveBeginPlay`
  (`parent.ReceiveBeginPlay`)
  (bind _returnvalue (`|AddComponentByClass` :`self` (`self.GetOwner`) :`Class` "/Game/Skyway/Core/Inventory/AC_Storage.AC_Storage_C" :`InitSlotContainers` (`self.InitSlotContainers`)))
  (bind _output_get (set `self.Storage` _returnvalue))
  (add `/Game/Skyway/Core/Inventory/AC_Storage.OnSlotUpdated` _output_get (`|CreateDelegate` :!event `OnStorageSlotUpdate`))
  (bind _returnvalue_2 (`|AddComponentByClass` (`self.GetOwner`) "/Game/Skyway/Core/Crafting/AC_Crafting.AC_Crafting_C"))
  (bind _output_get_2 (set `self.Crafting` _returnvalue_2))
  (add `/Game/Skyway/Core/Crafting/AC_Crafting.CraftEnd` _output_get_2 (`|CreateDelegate` :!event `CraftEnd_Event`)))

(event `self.ReceiveTick`
  (params (DeltaSeconds :type "Float (single-precision)"))
  (bind _audiocomp (`self.AudioComp`))
  (`parent.ReceiveTick` DeltaSeconds)
  (if (and (not (`AudioComponent.IsPlaying` (`self.AudioComp`))) (`self.Active`))
    (`AudioComponent.SetSound` _audiocomp "/Game/Skyway/Audio/Cues/ElectricSound_Cue.ElectricSound_Cue")
    (`AudioComponent.Play` _audiocomp 0.0))
  (if (`self.Active`)
    (`/Game/Skyway/Core/Crafting/AC_Crafting.CraftUnpause` (`self.Crafting`))
    (`|ExecutionSequence`
      (:`then_0`
        (`/Engine/EditorBlueprintResources/StandardMacros.DoOnce` false :!label _label
          (:`Completed`
            (`self.CraftRequest`))))
      (:`then_1`
        (goto _label_2 :!via `Reset`)))
    (else
      (`/Game/Skyway/Core/Crafting/AC_Crafting.CraftPause` (`self.Crafting`))
      (`|ExecutionSequence`
        (:`then_0`
          (`/Engine/EditorBlueprintResources/StandardMacros.DoOnce` false :!label _label_2))
        (:`then_1`
          (goto _label :!via `Reset`))))))

(event `CraftEnd_Event`
  (`self.CraftRequest`))

(event `/Game/Skyway/Core/Engine/BPI_CanSave.SaveToShip`
  (params (SaveGame :type "SaveGame Object Reference"))
  (setmembers `/Game/Skyway/Core/Engine/S_ShipBuildingInfo` :`StructRef` (`self.ShipBuildingInfo`) :`StorageSlotContainers` (`/Game/Skyway/Core/Inventory/AC_Storage.GetSlotContainers` (`self.Storage`)))
  (`parent.SaveToShip` SaveGame))

(event `/Game/Skyway/Core/Engine/BPI_CanSave.LoadToShip`
  (params (SaveGame :type "SaveGame Object Reference") (ShipBuildingInfo :type "/Game/Skyway/Core/Engine/S_ShipBuildingInfo Structure"))
  (`parent.LoadToShip` SaveGame ShipBuildingInfo)
  (`/Game/Skyway/Core/Engine/BPI_CanSave.LoadToShip` (`self.Storage`) SaveGame ShipBuildingInfo))

(fn `CanActivateEnergy`
  (returns (ReturnValue :type Boolean))
  (bind _returnarray (`/Game/Skyway/Core/Inventory/AC_Storage.GetSlotsAtItemType` (`self.Storage`) (struct :`TagName` "SlotContainer.Recycle") "NewEnumerator5"))
  (bind ((`Amount_49_D1E29AF04498C178B74986AAD5610193` _amount) (`MaxAmount_42_B9C41EB0416DBFA24E1E75A6CD16E5AA` _maxamount)) (break `/Game/Skyway/Core/Inventory/S_Item_Info` (`.ItemInfo_14_7E8F48144F0F01654500E084A85436C5` (break `/Game/Skyway/Core/Inventory/S_Slot_Info` (`|GetArrayItem` _returnarray 1)))))
  (bind ((`Amount_49_D1E29AF04498C178B74986AAD5610193` _amount_2) (`ID_71_BA06E0BD4E97D16461377CB9BF36CE2D` _id)) (break `/Game/Skyway/Core/Inventory/S_Item_Info` (`.ItemInfo_14_7E8F48144F0F01654500E084A85436C5` (break `/Game/Skyway/Core/Inventory/S_Slot_Info` (`|GetArrayItem` (`/Game/Skyway/Core/Inventory/AC_Storage.GetSlotsAtItemType` (`self.Storage`) (struct :`TagName` "SlotContainer.Storage") "NewEnumerator5"))))))
  (return (and (> (`.Amount_49_D1E29AF04498C178B74986AAD5610193` (break `/Game/Skyway/Core/Inventory/S_Item_Info` (`.ItemInfo_14_7E8F48144F0F01654500E084A85436C5` (break `/Game/Skyway/Core/Inventory/S_Slot_Info` (`|GetArrayItem` _returnarray))))) 0) (or (== _amount 0) (< _amount _maxamount)) (> (`self.Energy`) 1.0) (or (== (struct :`TagName` "Item.Consumable.ChargedBattery") _id) (< _amount_2 1)))))

(fn `CraftRequest`
  (returns (ReturnValue :type Boolean))
  (bind ((`Amount_49_D1E29AF04498C178B74986AAD5610193` _amount) (`ID_71_BA06E0BD4E97D16461377CB9BF36CE2D` _id)) (break `/Game/Skyway/Core/Inventory/S_Item_Info` (`.ItemInfo_14_7E8F48144F0F01654500E084A85436C5` (break `/Game/Skyway/Core/Inventory/S_Slot_Info` (`|GetArrayItem` (`/Game/Skyway/Core/Inventory/AC_Storage.GetSlotsAtItemType` (`self.Storage`) (struct :`TagName` "SlotContainer.Storage") "NewEnumerator5"))))))
  (if (or (== (struct :`TagName` "Item.Consumable.ChargedBattery") _id) (< _amount 1))
    (if (or (`KismetSystemLibrary.K2_IsTimerPausedHandle` (`/Game/Skyway/Core/Crafting/AC_Crafting.CraftTimerHandle` (`self.Crafting`))) (`KismetSystemLibrary.K2_IsValidTimerHandle` (`/Game/Skyway/Core/Crafting/AC_Crafting.CraftTimerHandle` (`self.Crafting`))))
      (`/Game/Skyway/Core/Crafting/AC_Crafting.CraftUnpause` (`self.Crafting`))
      (return true)
      (else
        (bind _returnvalue (`/Game/Skyway/Core/Crafting/AC_Crafting.CraftRequest` :`self` (`self.Crafting`) :`RecipeId` (struct :`TagName` "Recipe.Recycle.ChargedBattery") :`RequesterStorage` (`self.Storage`)))
        (return _returnvalue)))))

(fn `GetStorage`
  (returns (ReturnValue :type "/Game/Skyway/Core/Inventory/AC_Storage Object Reference"))
  (return (`self.Storage`)))

(fn `OnStorageSlotUpdate`
  (params (SlotInfo :type "/Game/Skyway/Core/Inventory/S_Slot_Info Structure"))
  (locals (L_SaveGame :type "SaveGame Object Reference"))
  (bind _returnvalue (message `/Game/Skyway/Core/Engine/BPI_GameMode.GetSaveGame` (`GameplayStatics.GetGameMode`)))
  (bind _output_get (set `local.L_SaveGame` _returnvalue))
  (`/Game/Skyway/Core/Engine/BPI_CanSave.SaveToShip` _output_get)
  (bind _returnvalue_2 (message `/Game/Skyway/Core/Ship/BPI_Ship.GetShipInfo` (`self.GetOwner`)))
  (message `/Game/Skyway/Core/Engine/BPI_SaveGame.SaveShip` (`local.L_SaveGame`) _returnvalue_2)
  (message `/Game/Skyway/Core/Engine/BPI_GameMode.FastSaveGame` (`GameplayStatics.GetGameMode`)))

(fn `SpendEnergy`
  (`parent.SpendEnergy`))