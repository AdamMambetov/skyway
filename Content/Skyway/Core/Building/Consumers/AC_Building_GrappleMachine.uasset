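; Powered ship building component for a grapple machine that automatically hooks nearby pickups into its own storage.
; On BeginPlay it builds the skeletal mesh, storage and grapple components, plus a looping timer for targeting.
; Targeting sphere-traces for untagged pickups with clear line to the hook, tags one, then Tick turns the AnimBP toward it and fires once.
; Tick also pauses the timer when inactive and swaps green/red materials; storage persists through ship saves.
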(event `self.ReceiveBeginPlay`
  (bind _skeletalmesh (`self.SkeletalMesh`))
  (`parent.ReceiveBeginPlay`)
  (bind _returnvalue (`|AddComponentByClass` :`self` (`self.GetOwner`) :`Class` "/Script/Engine.SkeletalMeshComponent"))
  (bind _output_get (set `self.SkeletalMesh` _returnvalue))
  (`self.K2_AttachToComponent` _output_get self "None" "KeepRelative" "KeepRelative" "KeepRelative" true)
  (`SkinnedMeshComponent.SetSkinnedAssetAndUpdate` _output_get (`.SkeletalMesh_51_44579ECC489E180B8BC740AADCECDAAF` (break `/Game/Skyway/Core/Inventory/S_Item_Info` (`.ItemInfo_2_96BFBB67441ABC75F13542B20097FC01` (break `/Game/Skyway/Core/Inventory/S_Building_Info` (`self.BuildingInfo`))))) true)
  (`self.SetHiddenInGame` true)
  (`SkeletalMeshComponent.SetAnimInstanceClass` _skeletalmesh "/Game/Skyway/Art/Building/GrappleMachine/ABP_GrappleMachine.ABP_GrappleMachine_C")
  (bind _asabp_grapple_machine (cast `/Game/Skyway/Art/Building/GrappleMachine/ABP_GrappleMachine` (`SkeletalMeshComponent.GetAnimInstance` _skeletalmesh)))
  (set `self.ABP_GrappleMachine` _asabp_grapple_machine)
  (bind _returnvalue_2 (`|AddComponentByClass` :`self` (`self.GetOwner`) :`Class` "/Game/Skyway/Core/Inventory/AC_Storage.AC_Storage_C" :`InitSlotContainers` (`self.InitSlotContainers`)))
  (bind _output_get_2 (set `self.Storage` _returnvalue_2))
  (add `/Game/Skyway/Core/Inventory/AC_Storage.OnSlotUpdated` _output_get_2 (`|CreateDelegate` :!event `OnStorageSlotUpdate`))
  (bind _returnvalue_3 (`|AddComponentByClass` (`self.GetOwner`) "/Game/Skyway/Core/Hook/AC_Grapple.AC_Grapple_C" (`self.SkeletalMesh`) (`self.Storage`)))
  (set `self.Grapple` _returnvalue_3)
  (bind _returnvalue_4 (`KismetSystemLibrary.K2_SetTimerDelegate` (`|CreateDelegate` :!event `FindTargetAndFireGrapple`) 4.0 true))
  (set `self.FireGrappleHandle` _returnvalue_4))

(event `self.ReceiveTick`
  (params (DeltaSeconds :type "Float (single-precision)"))
  (bind _alfadirection (`self.AlfaDirection`))
  (bind _returnvalue (`Actor.K2_GetActorLocation` (`self.ClosestActor`)))
  (`parent.ReceiveTick` DeltaSeconds)
  (`self.UpdateAppereance`)
  (if (and (not (`AudioComponent.IsPlaying` (`self.AudioComp`))) (`self.Active`))
    _
    (else
      _))
  (if (`self.Active`)
    (`KismetSystemLibrary.K2_UnPauseTimerHandle` (`self.FireGrappleHandle`))
    (if (< (`self.AlfaDirection`) 1.0)
      (set `self.Direction` (`KismetMathLibrary.Lerp` (`self.Direction`) (`self.NewDirection`) _alfadirection))
      (set `self.AlfaDirection` (+ _alfadirection (* (`self.RotateTime`) (`GameplayStatics.GetWorldDeltaSeconds`))))
      (set `/Game/Skyway/Art/Building/GrappleMachine/ABP_GrappleMachine.Direction` (`self.Direction`) (`self.ABP_GrappleMachine`))
      (goto _label :!via `Reset`)
      (else
        (`/Engine/EditorBlueprintResources/StandardMacros.DoOnce` true :!label _label
          (:`Completed`
            (`/Game/Skyway/Core/Hook/AC_Grapple.FireGrapple_SERVER` (`self.Grapple`) _returnvalue (`KismetMathLibrary.GetDirectionUnitVector` (`self.GetSocketLocation` (`self.SkeletalMesh`) "HookSocket") _returnvalue) 1.0)))))
    (else
      (`KismetSystemLibrary.K2_PauseTimerHandle` (`self.FireGrappleHandle`)))))

(event `/Game/Skyway/Core/Engine/BPI_CanSave.SaveToShip`
  (params (SaveGame :type "SaveGame Object Reference"))
  (setmembers `/Game/Skyway/Core/Engine/S_ShipBuildingInfo` :`StructRef` (`self.ShipBuildingInfo`) :`StorageSlotContainers` (`/Game/Skyway/Core/Inventory/AC_Storage.GetSlotContainers` (`self.Storage`)))
  (`parent.SaveToShip` SaveGame))

(event `/Game/Skyway/Core/Engine/BPI_CanSave.LoadToShip`
  (params (SaveGame :type "SaveGame Object Reference") (ShipBuildingInfo :type "/Game/Skyway/Core/Engine/S_ShipBuildingInfo Structure"))
  (`parent.LoadToShip` SaveGame ShipBuildingInfo)
  (`/Game/Skyway/Core/Engine/BPI_CanSave.LoadToShip` (`self.Storage`) SaveGame ShipBuildingInfo))

(fn `CanActivateEnergy`
  (returns (ReturnValue :type Boolean))
  (return (> (`self.Energy`) (`self.EnergyToWork`))))

(fn `FindTargetAndFireGrapple`
  (locals (L_ClosestActor :type "Actor Object Reference") (L_BestDistance :type "Float (double-precision)" :default 9999999999.0))
  (bind _returnvalue (`self.K2_GetComponentLocation`))
  (bind (_returnvalue_roll _returnvalue_pitch _returnvalue_yaw) (`KismetMathLibrary.BreakRotator` (`KismetMathLibrary.FindLookAtRotation` (`Actor.K2_GetActorLocation` (`self.ClosestActor`)) (`self.GetSocketLocation` (`self.SkeletalMesh`) "HookSocket"))))
  (bind (_outhits _returnvalue_2) (`KismetSystemLibrary.SphereTraceMultiForObjects` :`Start` _returnvalue :`End` _returnvalue :`Radius` 3000.0 :`ObjectTypes` (`|MakeArray` "ObjectTypeQuery4" :!type "EObjectTypeQuery Enum") :`DrawTime` 4.0))
  (if _returnvalue_2
    (for _array_element _outhits
      (bind (_bblockinghit _binitialoverlap _time _distance _location _impactpoint _normal _impactnormal _physmat _hitactor) (`GameplayStatics.BreakHitResult` _array_element))
      (if (`KismetMathLibrary.ClassIsChildOf` (`GameplayStatics.GetObjectClass` _hitactor) "/Game/Skyway/Core/Inventory/BP_Pickup_Base.BP_Pickup_Base_C")
        (bind (_outhit _returnvalue_3) (`KismetSystemLibrary.CapsuleTraceSingleForObjects` (`Actor.K2_GetActorLocation` _hitactor) (`self.GetSocketLocation` (`self.SkeletalMesh`) "HookSocket") 10.0 10.0 (`|MakeArray` "ObjectTypeQuery1" "ObjectTypeQuery2" "ObjectTypeQuery11" "ObjectTypeQuery10" "ObjectTypeQuery4" :!type "EObjectTypeQuery Enum") false (`|MakeArray` _hitactor) "None" false (struct :`R` 0.233506 :`G` 1.0 :`A` 1.0) (struct :`R` 1.0 :`A` 1.0)))
        (if (and (not _returnvalue_3) (not (`Actor.ActorHasTag` _hitactor "Grappled")))
          (set `self.ClosestActor` _hitactor)
          (break))))
    (bind _closestactor (`self.ClosestActor`)
      (:`then`
        (`KismetArrayLibrary.Array_Add` (`Actor.Tags` _closestactor) "Grappled")
        (set `self.NewDirection` (mod _returnvalue_yaw 180.0))
        (set `self.AlfaDirection` 0.0))
      (:`else`))))

(fn `GetStorage`
  (returns (ReturnValue :type "/Game/Skyway/Core/Inventory/AC_Storage Object Reference"))
  (return (`self.Storage`)))

(fn `OnStorageSlotUpdate`
  (params (SlotInfo :type "/Game/Skyway/Core/Inventory/S_Slot_Info Structure"))
  (locals (L_SaveGame :type "SaveGame Object Reference"))
  (bind _returnvalue (message `/Game/Skyway/Core/Engine/BPI_GameMode.GetSaveGame` (`GameplayStatics.GetGameMode`)))
  (bind _output_get (set `local.L_SaveGame` _returnvalue))
  (`/Game/Skyway/Core/Engine/BPI_CanSave.SaveToShip` _output_get)
  (bind _returnvalue_2 (message `/Game/Skyway/Core/Ship/BPI_Ship.GetShipInfo` (`self.GetOwner`)))
  (message `/Game/Skyway/Core/Engine/BPI_SaveGame.SaveShip` (`local.L_SaveGame`) _returnvalue_2)
  (message `/Game/Skyway/Core/Engine/BPI_GameMode.FastSaveGame` (`GameplayStatics.GetGameMode`)))

(fn `SpendEnergy`
  (`parent.SpendEnergy`))

(fn `UpdateAppereance`
  (locals (L_Materials :type "Array of MaterialInterface Object Reference"))
  (bind _skeletalmesh (`self.SkeletalMesh`))
  (bind _output_get (set `local.L_Materials` (`self.GetMaterials` _skeletalmesh)))
  (for (_ _array_index) _output_get
    (`self.SetMaterial` _skeletalmesh _array_index (select `bool` (`self.Active`) :`false` "/Game/Skyway/Art/Building/GrappleMachine/MI_GrappleMachine_Red.MI_GrappleMachine_Red" :`true` "/Game/Skyway/Art/Building/GrappleMachine/MI_GrappleMachine_Green.MI_GrappleMachine_Green" :!type "MaterialInterface Object Reference"))))