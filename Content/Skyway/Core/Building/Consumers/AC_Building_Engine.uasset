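; Engine building component that consumes energy, shown as an animated engine with two fire effects and a steerable rotation.
; On begin play it hides itself, adds a skeletal mesh to its owner at its transform and attaches Niagara fire to two sockets.
; Tick derives Direction from Rotation and syncs Active to fire visibility and the anim blueprint.
; SetRotation wraps angles toward ±180, and Rotation's RepNotify feeds the anim blueprint.
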(event `self.ReceiveBeginPlay`
  (`parent.ReceiveBeginPlay`)
  (`KismetSystemLibrary.DelayUntilNextTick`)
  (bind _returnvalue (`|AddComponentByClass` (`self.GetOwner`) "/Script/Engine.SkeletalMeshComponent" false (`/Game/Skyway/Core/Engine/FLBP_Defaults.ConvertWorldTransformToRelative` (`Actor.GetTransform` (`self.GetOwner`)) (`self.K2_GetComponentToWorld`))))
  (bind _output_get (set `self.EngineSkeletalMeshRef` _returnvalue))
  (`SkinnedMeshComponent.SetSkinnedAssetAndUpdate` _output_get "/Game/Skyway/Art/Building/Engine/SK_Engine.SK_Engine" true)
  (`SkeletalMeshComponent.SetAnimInstanceClass` (`self.EngineSkeletalMeshRef`) "/Game/Skyway/Art/Building/Engine/ABP_Engine.ABP_Engine_C")
  (`self.SetVisibility` false)
  (bind _returnvalue_2 (`NiagaraFunctionLibrary.SpawnSystemAttached` "/Game/Skyway/Art/VFX/Fire/NS_Fire.NS_Fire" (`self.EngineSkeletalMeshRef`) "FireLeftSocket" (0.0 0.0 0.0) (struct) "KeepRelativeOffset"))
  (set `self.NS_FireLeft` _returnvalue_2)
  (bind _returnvalue_3 (`NiagaraFunctionLibrary.SpawnSystemAttached` "/Game/Skyway/Art/VFX/Fire/NS_Fire.NS_Fire" (`self.EngineSkeletalMeshRef`) "FireRightSocket" (0.0 0.0 0.0) (struct) "KeepRelativeOffset"))
  (set `self.NS_FireRight` _returnvalue_3)
  (bind _asabp_engine (cast `/Game/Skyway/Art/Building/Engine/ABP_Engine` (`SkeletalMeshComponent.GetAnimInstance` (`self.EngineSkeletalMeshRef`))))
  (set `self.EngineAnimBP` _asabp_engine))

(event `self.ReceiveTick`
  (params (DeltaSeconds :type "Float (single-precision)"))
  (`parent.ReceiveTick` DeltaSeconds)
  (set `self.Direction` (`.Y` (`KismetMathLibrary.BreakRotIntoAxes` (`KismetMathLibrary.MakeRotator` 0.0 0.0 (`self.Rotation`)))))
  (`|ExecutionSequence`
    (:`then_0`
      (`self.NS_FireRight`
        (:`then`
          (`self.NS_FireLeft`
            (:`then`
              (if (!= (`self.Active`) (`self.IsVisible` (`self.NS_FireLeft`)))
                (`self.SetVisibility` (`self.NS_FireLeft`) (`self.Active`) false)
                (`self.SetVisibility` (`self.NS_FireRight`) (`self.Active`) false)))
            (:`else`)))
        (:`else`)))
    (:`then_1`
      (bind _engineanimbp (`self.EngineAnimBP`)
        (:`then`
          (if (!= (`self.Active`) (`/Game/Skyway/Art/Building/Engine/ABP_Engine.IsActive` _engineanimbp))
            (set `/Game/Skyway/Art/Building/Engine/ABP_Engine.IsActive` (`self.Active`) (`self.EngineAnimBP`))))
        (:`else`)))))

(event `/Game/Skyway/Core/Building/BPI_Build.SetRotation`
  (params (NewRotation :type "Float (double-precision)"))
  (bind _output_get (set `self.Rotation` NewRotation))
  (if (> _output_get 180.0)
    (set `self.Rotation` (+ -360.0 (`self.Rotation`)))
    (if (> (`self.Rotation`) 180.0)
      (`/Game/Skyway/Core/Building/BPI_Build.SetRotation` (`self.Rotation`)))
    (elif (< (`self.Rotation`) -180.0)
      (set `self.Rotation` (+ 360.0 (`self.Rotation`)))
      (if (< (`self.Rotation`) -180.0)
        (`/Game/Skyway/Core/Building/BPI_Build.SetRotation` (`self.Rotation`))))))

(fn `CanActivateEnergy`
  (returns (ReturnValue :type Boolean))
  (return (>= (`self.Energy`) (`self.EnergyToWork`))))

(fn `GetRotation`
  (returns (ReturnValue :type "Float (double-precision)"))
  (return (`self.Rotation`)))

(fn `OnRep_Rotation`
  (set `/Game/Skyway/Art/Building/Engine/ABP_Engine.Rotation` (`self.Rotation`) (`self.EngineAnimBP`)))