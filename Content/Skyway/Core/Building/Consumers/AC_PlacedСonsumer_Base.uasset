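; Base class for placed energy consumers in the Skyway building system, draining stored energy while active.
; Each Tick calls the parent, then runs SpendEnergy when Active is set.
; SpendEnergy subtracts EnergySpeed scaled by world delta time while Energy is non-negative, without clamping, so it can dip below zero.
; The CanActivateEnergy override simply returns the parent's result.
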(event `self.ReceiveTick`
  (params (DeltaSeconds :type "Float (single-precision)"))
  (`parent.ReceiveTick` DeltaSeconds)
  (if (`self.Active`)
    (`self.SpendEnergy`)))

(fn `CanActivateEnergy`
  (returns (ReturnValue :type Boolean))
  (return (`parent.CanActivateEnergy`)))

(fn `SpendEnergy`
  (if (>= (`self.Energy`) 0.0)
    (set `self.Energy` (- (`self.Energy`) (* (`self.EnergySpeed`) (`GameplayStatics.GetWorldDeltaSeconds`))))))