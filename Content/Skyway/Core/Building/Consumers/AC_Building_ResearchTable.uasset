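; Building component for a research table that consumes energy in the Skyway building system.
; On BeginPlay it adds an AC_Crafting component to its owning actor and keeps a reference to it.
; Energy activation requires stored energy above the working threshold and an active research timer on that crafting component.
; Tick checks the active state but does nothing with it.
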(event `self.ReceiveBeginPlay`
  (`parent.ReceiveBeginPlay`)
  (bind _returnvalue (`|AddComponentByClass` (`self.GetOwner`) "/Game/Skyway/Core/Crafting/AC_Crafting.AC_Crafting_C"))
  (set `self.Crafting` _returnvalue))

(event `self.ReceiveTick`
  (params (DeltaSeconds :type "Float (single-precision)"))
  (`parent.ReceiveTick` DeltaSeconds)
  (if (`self.Active`)
    _))

(fn `CanActivateEnergy`
  (returns (ReturnValue :type Boolean))
  (return (and (> (`self.Energy`) (`self.EnergyToWork`)) (`KismetSystemLibrary.K2_IsTimerActiveHandle` (`/Game/Skyway/Core/Crafting/AC_Crafting.ResearchHandle` (`self.Crafting`))))))