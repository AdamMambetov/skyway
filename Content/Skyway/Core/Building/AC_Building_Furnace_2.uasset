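; Furnace building component for ships that burns fuel to craft each input item's DT_Pieces recipe, with smoke and sound while active.
; It adds Storage and Crafting components to its owner; Tick drains fuel and pauses or resumes crafting with Active, and craft completion requests the next.
; CanActivateEnergy checks fuel, input, energy and output slot compatibility, while SpendEnergy is empty.
; Storage persists in ship building info, and slot updates trigger a fast save.
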(event `self.ReceiveBeginPlay`
  (`parent.ReceiveBeginPlay`)
  (bind _returnvalue (`NiagaraFunctionLibrary.SpawnSystemAttached` "/Game/Skyway/Art/VFX/Smoke/NS_Smoke_2.NS_Smoke_2" self "SmokeSocket" (0.0 0.0 0.0) (struct) "KeepRelativeOffset"))
  (set `self.NS Smoke` _returnvalue)
  (bind _returnvalue_2 (`|AddComponentByClass` :`self` (`self.GetOwner`) :`Class` "/Game/Skyway/Core/Inventory/AC_Storage.AC_Storage_C" :`InitSlotContainers` (`self.InitSlotContainers`)))
  (set `self.Storage` _returnvalue_2)
  (bind _returnvalue_3 (`|AddComponentByClass` (`self.GetOwner`) "/Game/Skyway/Core/Crafting/AC_Crafting.AC_Crafting_C"))
  (bind _output_get (set `self.Crafting` _returnvalue_3))
  (add `/Game/Skyway/Core/Crafting/AC_Crafting.CraftEnd` _output_get (`|CreateDelegate` :!event `CraftEnd_Event`))
  (add `/Game/Skyway/Core/Inventory/AC_Storage.OnSlotUpdated` (`self.Storage`) (`|CreateDelegate` :!event `OnStorageSlotUpdated_Event`)))

(event `self.ReceiveTick`
  (params (DeltaSeconds :type "Float (single-precision)"))
  (bind _active (`self.Active`))
  (bind _audiocomp (`self.AudioComp`))
  (`parent.ReceiveTick` DeltaSeconds)
  (if (and (not (`AudioComponent.IsPlaying` (`self.AudioComp`))) (`self.Active`))
    (`AudioComponent.SetSound` _audiocomp "/Game/Skyway/Audio/Cues/двигатели__Cue.двигатели__Cue")
    (`AudioComponent.Play` _audiocomp 0.0))
  (`self.SetVisibility` (`self.NS Smoke`) _active false)
  (`self.Update Fuel`)
  (if _active
    (`/Game/Skyway/Core/Crafting/AC_Crafting.CraftUnpause` (`self.Crafting`))
    (else
      (`/Game/Skyway/Core/Crafting/AC_Crafting.CraftPause` (`self.Crafting`)))))

(event `CraftEnd_Event`
  (`self.CraftRequest`))

(event `/Game/Skyway/Core/Engine/BPI_CanSave.SaveToShip`
  (params (SaveGame :type "SaveGame Object Reference"))
  (setmembers `/Game/Skyway/Core/Engine/S_ShipBuildingInfo` :`StructRef` (`self.ShipBuildingInfo`) :`StorageSlotContainers` (`/Game/Skyway/Core/Inventory/AC_Storage.GetSlotContainers` (`self.Storage`)))
  (`parent.SaveToShip` SaveGame))

(event `/Game/Skyway/Core/Engine/BPI_CanSave.LoadToShip`
  (params (SaveGame :type "SaveGame Object Reference") (ShipBuildingInfo :type "/Game/Skyway/Core/Engine/S_ShipBuildingInfo Structure"))
  (`parent.LoadToShip` SaveGame ShipBuildingInfo)
  (`/Game/Skyway/Core/Engine/BPI_CanSave.LoadToShip` (`self.Storage`) SaveGame ShipBuildingInfo))

(fn `CanActivateEnergy`
  (returns (ReturnValue :type Boolean))
  (bind _returnvalue (<= (`self.Energy`) (`self.MaxEnergy`)))
  (bind ((`Amount_49_D1E29AF04498C178B74986AAD5610193` _amount) (`ID_71_BA06E0BD4E97D16461377CB9BF36CE2D` _id)) (break `/Game/Skyway/Core/Inventory/S_Item_Info` (`.ItemInfo_14_7E8F48144F0F01654500E084A85436C5` (break `/Game/Skyway/Core/Inventory/S_Slot_Info` (`|GetArrayItem` (`/Game/Skyway/Core/Inventory/AC_Storage.GetSlotsAtItemType` (`self.Storage`) (struct :`TagName` "SlotContainer.Storage") "NewEnumerator5"))))))
  (bind _returnvalue_2 (< _amount 1))
  (bind _returnvalue_3 (> (`.Amount_49_D1E29AF04498C178B74986AAD5610193` (break `/Game/Skyway/Core/Inventory/S_Item_Info` (`.ItemInfo_14_7E8F48144F0F01654500E084A85436C5` (break `/Game/Skyway/Core/Inventory/S_Slot_Info` (`|GetArrayItem` (`/Game/Skyway/Core/Inventory/AC_Storage.GetSlotsAtItemType` (`self.Storage`) (struct :`TagName` "SlotContainer.Recycle") (`/Game/Skyway/Core/Engine/MLBP_Defaults.DEFAULT`)) 1))))) 0))
  (bind _returnvalue_4 (or (> (`.Amount_49_D1E29AF04498C178B74986AAD5610193` (break `/Game/Skyway/Core/Inventory/S_Item_Info` (`.ItemInfo_14_7E8F48144F0F01654500E084A85436C5` (break `/Game/Skyway/Core/Inventory/S_Slot_Info` (`|GetArrayItem` (`/Game/Skyway/Core/Inventory/AC_Storage.GetSlotsAtItemType` (`self.Storage`) (struct :`TagName` "SlotContainer.Recycle") (`/Game/Skyway/Core/Engine/MLBP_Defaults.DEFAULT`))))))) 0) (> (`self.FuelProgressBarPercent`) 0.0)))
  (bind _returnvalue_5 (`|GetDataTableRow` "/Game/Skyway/Core/Inventory/DT_Pieces.DT_Pieces" (`BlueprintGameplayTagLibrary.GetTagName` (`.ID_71_BA06E0BD4E97D16461377CB9BF36CE2D` (break `/Game/Skyway/Core/Inventory/S_Item_Info` (`.ItemInfo_14_7E8F48144F0F01654500E084A85436C5` (break `/Game/Skyway/Core/Inventory/S_Slot_Info` (`|GetArrayItem` (`/Game/Skyway/Core/Inventory/AC_Storage.GetSlotsAtItemType` (`self.Storage`) (struct :`TagName` "SlotContainer.Recycle") "NewEnumerator5") 1)))))))
    (:`then`
      (bind _returnvalue_6 (`|GetDataTableRow` "/Game/Skyway/Core/Crafting/DT_Recipes.DT_Recipes" (`BlueprintGameplayTagLibrary.GetTagName` (`.RecipeId_25_3797D7844273B4CF8F7EB1842ED1659C` (break `/Game/Skyway/Core/Inventory/S_Piece_Info` _returnvalue_5))))
        (:`then`
          (if _returnvalue_2
            (return (and _returnvalue_4 _returnvalue _returnvalue_3 _returnvalue_2))
            (else
              (return (and (== (`.Result_23_1B532DAD43B20A155E0A209CC428568B` (break `/Game/Skyway/Core/Crafting/S_Recipe` _returnvalue_6)) _id) _returnvalue_4 _returnvalue_3 _returnvalue)))))
        (:`RowNotFound`
          _)))
    (:`RowNotFound`
      _))
  (return (and _returnvalue_4 _returnvalue_3 _returnvalue)))

(fn `CraftRequest`
  (returns (ReturnValue :type Boolean))
  (bind ((`Amount_49_D1E29AF04498C178B74986AAD5610193` _amount) (`ID_71_BA06E0BD4E97D16461377CB9BF36CE2D` _id)) (break `/Game/Skyway/Core/Inventory/S_Item_Info` (`.ItemInfo_14_7E8F48144F0F01654500E084A85436C5` (break `/Game/Skyway/Core/Inventory/S_Slot_Info` (`|GetArrayItem` (`/Game/Skyway/Core/Inventory/AC_Storage.GetSlotsAtItemType` (`self.Storage`) (struct :`TagName` "SlotContainer.Storage") "NewEnumerator5"))))))
  (bind _returnvalue (`|GetDataTableRow` "/Game/Skyway/Core/Inventory/DT_Pieces.DT_Pieces" (`BlueprintGameplayTagLibrary.GetTagName` (`.ID_71_BA06E0BD4E97D16461377CB9BF36CE2D` (break `/Game/Skyway/Core/Inventory/S_Item_Info` (`.ItemInfo_14_7E8F48144F0F01654500E084A85436C5` (break `/Game/Skyway/Core/Inventory/S_Slot_Info` (`|GetArrayItem` (`/Game/Skyway/Core/Inventory/AC_Storage.GetSlotsAtItemType` (`self.Storage`) (struct :`TagName` "SlotContainer.Recycle") "NewEnumerator5") 1)))))))
    (:`then`
      (bind ((`RecipeId_25_3797D7844273B4CF8F7EB1842ED1659C` _recipeid)) (break `/Game/Skyway/Core/Inventory/S_Piece_Info` _returnvalue))
      (bind _returnvalue_2 (`|GetDataTableRow` "/Game/Skyway/Core/Crafting/DT_Recipes.DT_Recipes" (`BlueprintGameplayTagLibrary.GetTagName` _recipeid))
        (:`then`
          (if (or (== (`.Result_23_1B532DAD43B20A155E0A209CC428568B` (break `/Game/Skyway/Core/Crafting/S_Recipe` _returnvalue_2)) _id) (< _amount 1))
            (if (or (`KismetSystemLibrary.K2_IsTimerPausedHandle` (`/Game/Skyway/Core/Crafting/AC_Crafting.CraftTimerHandle` (`self.Crafting`))) (`KismetSystemLibrary.K2_IsValidTimerHandle` (`/Game/Skyway/Core/Crafting/AC_Crafting.CraftTimerHandle` (`self.Crafting`))))
              (`/Game/Skyway/Core/Crafting/AC_Crafting.CraftUnpause` (`self.Crafting`))
              (return true)
              (else
                (bind _returnvalue_3 (`/Game/Skyway/Core/Crafting/AC_Crafting.CraftRequest` :`self` (`self.Crafting`) :`RecipeId` _recipeid :`RequesterStorage` (`self.Storage`)))
                (return _returnvalue_3)))))))))

(fn `GetStorage`
  (returns (ReturnValue :type "/Game/Skyway/Core/Inventory/AC_Storage Object Reference"))
  (return (`self.Storage`)))

(fn `OnStorageSlotUpdated_Event`
  (params (SlotInfo :type "/Game/Skyway/Core/Inventory/S_Slot_Info Structure"))
  (locals (L_SaveGame :type "SaveGame Object Reference"))
  (bind _returnvalue (message `/Game/Skyway/Core/Engine/BPI_GameMode.GetSaveGame` (`GameplayStatics.GetGameMode`)))
  (bind _output_get (set `local.L_SaveGame` _returnvalue))
  (`/Game/Skyway/Core/Engine/BPI_CanSave.SaveToShip` _output_get)
  (bind _returnvalue_2 (message `/Game/Skyway/Core/Ship/BPI_Ship.GetShipInfo` (`self.GetOwner`)))
  (message `/Game/Skyway/Core/Engine/BPI_SaveGame.SaveShip` (`local.L_SaveGame`) _returnvalue_2)
  (message `/Game/Skyway/Core/Engine/BPI_GameMode.FastSaveGame` (`GameplayStatics.GetGameMode`)))

(fn `SpendEnergy`)

(fn `Update Fuel`
  (if (`self.Active`)
    (if (<= (`self.FuelProgressBarPercent`) 0.0)
      (`/Game/Skyway/Core/Inventory/AC_Storage.RemoveSlot` (`self.Storage`) (`|GetArrayItem` (`/Game/Skyway/Core/Inventory/AC_Storage.GetSlotsAtItemType` (`self.Storage`) (struct :`TagName` "SlotContainer.Recycle") "NewEnumerator5")) 1)
      (set `self.FuelProgressBarPercent` 1.0)
      (else
        (set `self.FuelProgressBarPercent` (- (`self.FuelProgressBarPercent`) (* (/ 1.0 (`self.FuelBurnSpeed`)) (`GameplayStatics.GetWorldDeltaSeconds`))))))))