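; Triangular foundation piece for the building system, providing snap collision boxes on its three edges for attaching other pieces.
; SpawnCollisions extends the parent, creating a foundation box and a wall box on the left, backward and right sides, each with a debug collision.
; Foundation and wall boxes get separate extents and block different custom trace channels.
; ReturnBoxes returns all six boxes.
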(fn `ReturnBoxes`
  (returns (Boxes :type "Array of BoxComponent Object Reference"))
  (return (`|MakeArray` (`self.FoundationCollisionLeft`) (`self.FoundationCollisionBackward`) (`self.FoundationCollisionRight`) (`self.WallCollisionLeft`) (`self.WallCollisionBackward`) (`self.WallCollisionRight`))))

(fn `SpawnCollisions`
  (`parent.SpawnCollisions`)
  (`|ExecutionSequence`
    (:`then_0`
      ;[1 1 1] Foundation Left
      (bind _returnvalue (`self.CreateCollision` (`self.FOUNDATION_LOCATION_LEFT`) (`self.FOUNDATION_ROTATION_LEFT`)))
      (bind _output_get (set `self.FoundationCollisionLeft` _returnvalue))
      (`self.CreateDebugCollision` _output_get "Left"))
    (:`then_1`
      ;[1 1 1] Foundation Backward
      (bind _returnvalue_2 (`self.CreateCollision` (`self.FOUNDATION_LOCATION_BACKWARD`) (`self.FOUNDATION_ROTATION_BACKWARD`)))
      (bind _output_get_2 (set `self.FoundationCollisionBackward` _returnvalue_2))
      (`self.CreateDebugCollision` _output_get_2 "Backward"))
    (:`then_2`
      ;[1 1 1] Foundation Right
      (bind _returnvalue_3 (`self.CreateCollision` (`self.FOUNDATION_LOCATION_RIGHT`) (`self.FOUNDATION_ROTATION_RIGHT`)))
      (bind _output_get_3 (set `self.FoundationCollisionRight` _returnvalue_3))
      (`self.CreateDebugCollision` _output_get_3 "Right"))
    (:`then_3`
      ;[1 1 1] Wall Left
      (bind _returnvalue_4 (`self.CreateCollision` (`self.WALL_LOCATION_LEFT`) (`self.WALL_ROTATION_LEFT`)))
      (bind _output_get_4 (set `self.WallCollisionLeft` _returnvalue_4))
      (`self.CreateDebugCollision` _output_get_4 "Left"))
    (:`then_4`
      ;[1 1 1] Wall Backward
      (bind _returnvalue_5 (`self.CreateCollision` (`self.WALL_LOCATION_BACKWARD`) (`self.WALL_ROTATION_BACKWARD`)))
      (bind _output_get_5 (set `self.WallCollisionBackward` _returnvalue_5))
      (`self.CreateDebugCollision` _output_get_5 "Backward"))
    (:`then_5`
      ;[1 1 1] Wall Right
      (bind _returnvalue_6 (`self.CreateCollision` (`self.WALL_LOCATION_RIGHT`) (`self.WALL_ROTATION_RIGHT`)))
      (bind _output_get_6 (set `self.WallCollisionRight` _returnvalue_6))
      (`self.CreateDebugCollision` _output_get_6 "Right"))
    (:`then_6`
      ;[1 1 1] Foundation Default Settings
      (`BoxComponent.SetBoxExtent` (`self.FoundationCollisionBackward`) (`self.FOUNDATION_BOX_EXTEND`) true)
      (`BoxComponent.SetBoxExtent` (`self.FoundationCollisionLeft`) (`self.FOUNDATION_BOX_EXTEND`) true)
      (`BoxComponent.SetBoxExtent` (`self.FoundationCollisionRight`) (`self.FOUNDATION_BOX_EXTEND`) true)
      (`self.SetCollisionResponseToChannel` (`self.FoundationCollisionLeft`) "ECC_GameTraceChannel2" "ECR_Block")
      (`self.SetCollisionResponseToChannel` (`self.FoundationCollisionBackward`) "ECC_GameTraceChannel2" "ECR_Block")
      (`self.SetCollisionResponseToChannel` (`self.FoundationCollisionRight`) "ECC_GameTraceChannel2" "ECR_Block")
      (`self.SetCollisionResponseToChannel` (`self.FoundationCollisionLeft`) "ECC_GameTraceChannel3" "ECR_Block")
      (`self.SetCollisionResponseToChannel` (`self.FoundationCollisionBackward`) "ECC_GameTraceChannel3" "ECR_Block")
      (`self.SetCollisionResponseToChannel` (`self.FoundationCollisionRight`) "ECC_GameTraceChannel3" "ECR_Block"))
    (:`then_7`
      ;[1 1 1] Wall Default Settings
      (`BoxComponent.SetBoxExtent` (`self.WallCollisionBackward`) (`self.WALL_BOX_EXTEND`) true)
      (`BoxComponent.SetBoxExtent` (`self.WallCollisionLeft`) (`self.WALL_BOX_EXTEND`) true)
      (`BoxComponent.SetBoxExtent` (`self.WallCollisionRight`) (`self.WALL_BOX_EXTEND`) true)
      (`self.SetCollisionResponseToChannel` (`self.WallCollisionLeft`) "ECC_GameTraceChannel4" "ECR_Block")
      (`self.SetCollisionResponseToChannel` (`self.WallCollisionBackward`) "ECC_GameTraceChannel4" "ECR_Block")
      (`self.SetCollisionResponseToChannel` (`self.WallCollisionRight`) "ECC_GameTraceChannel4" "ECR_Block"))))