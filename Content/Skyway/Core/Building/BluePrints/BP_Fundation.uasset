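; BP_Fundation is a foundation piece for the Skyway building system.
; ReturnBoxes exposes nine components as one array: four foundation, four wall and one ladder, which by name appear to be attachment boxes for neighboring pieces.
; GetHit returns the piece's HitMesh, while Floating and the construction script are empty.
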(fn `Floating`)

(fn `GetHit`
  (returns (HitMesh :type Boolean))
  (return (`self.Hit Mesh`)))

(fn `ReturnBoxes`
  (returns (Boxes :type "Array of BoxComponent Object Reference"))
  (return (`|MakeArray` (`self.Fundation1`) (`self.Fundation2`) (`self.Fundation3`) (`self.Fundation4`) (`self.Wall1`) (`self.Wall2`) (`self.Wall3`) (`self.Wall4`) (`self.Ladder`))))

(fn `UserConstructionScript`)