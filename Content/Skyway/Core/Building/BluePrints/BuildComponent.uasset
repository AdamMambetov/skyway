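; Build-mode component for BP_MainCharacter that previews and places pieces from DT_Buildables.
; A self-repeating BuildCycle, delayed by frame delta, traces from the camera to move a ghost mesh, snapping it to matching build boxes on the hit actor.
; Box-trace overlap checks, varying by mesh, set CanBuild and tint the ghost green or red.
; SpawnBuild passes the buildable and hit box to the ship through messages, then disables that box's collision.
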(event `self.ReceiveBeginPlay`
  (bind _asbp_main_character (cast `/Game/Skyway/Core/Engine/BP_MainCharacter` (`self.GetOwner`)))
  (set `self.PlayerRef` _asbp_main_character)
  (bind _outrownames (`DataTableFunctionLibrary.GetDataTableRowNames` "/Game/Skyway/Core/Building/DT_Buildables.DT_Buildables"))
  (for _array_element _outrownames
    (bind _returnvalue (`|GetDataTableRow` "/Game/Skyway/Core/Building/DT_Buildables.DT_Buildables" _array_element)
      (:`then`
        (`KismetArrayLibrary.Array_Add` (`self.Buildables`) _returnvalue)))))

(event `BuildDelay`
  (bind _buildghost (`self.BuildGhost`))
  (if (`self.IsBuildModeOn`)
    (`KismetSystemLibrary.Delay` (`GameplayStatics.GetWorldDeltaSeconds`))
    (`self.BuildCycle`)
    (else
      (set `self.IsBuildModeOn` false :!label _label)
      (set `self.CanBuild` false)
      (`/Engine/EditorBlueprintResources/StandardMacros.IsValid` _buildghost
        (:`Is Valid`
          (`/Game/Skyway/Core/Engine/BP_MainCharacter.DestroyComponent` (`self.PlayerRef`) _buildghost))))))

(event `StopBuildMode`
  (goto _label))

(event `LaunchBuildMode`
  (if (`self.IsBuildModeOn`)
    (`self.StopBuildMode`)
    (else
      (set `self.IsBuildModeOn` true)
      (`self.BuildCycle`))))

(fn `BuildCycle`
  (bind _camera (`self.Camera`))
  (bind (_buildtransform_location _buildtransform_rotation _buildtransform_scale) (`KismetMathLibrary.BreakTransform` (`self.BuildTransform`)))
  (bind _buildghost (`self.BuildGhost`))
  (bind _returnvalue (`SceneComponent.K2_GetComponentLocation` _camera))
  (bind _returnvalue_2 (not (`self.CanBuild`)))
  (bind (_returnvalue_roll _returnvalue_pitch _returnvalue_yaw) (`KismetMathLibrary.BreakRotator` (`SceneComponent.K2_GetComponentRotation` (`self.Camera`))))
  (bind (_output_mesh _output_tracechannel) (break `/Game/Skyway/Core/Building/S_Buildables` (`|GetArrayItem` (`self.Buildables`) (`self.BuildID`))))
  (bind (_outhit _returnvalue_3) (`KismetSystemLibrary.LineTraceSingle` _returnvalue (+ _returnvalue (* (`SceneComponent.GetForwardVector` _camera) 1000)) _output_tracechannel))
  (if _returnvalue_3
    (if _returnvalue_2
      _
      (else
        _))
    (set `self.Ghost Rotation` (`KismetMathLibrary.MakeRotator` _returnvalue_roll 0.0 _returnvalue_yaw))
    (bind (_bblockinghit _binitialoverlap _time _distance _location _impactpoint _normal _impactnormal _physmat _hitactor _hitcomponent _hitbonename _hititem _elementindex _faceindex _tracestart _traceend) (`GameplayStatics.BreakHitResult` _outhit))
    (set `self.BuildTransform` (`KismetMathLibrary.MakeTransform` _location _buildtransform_rotation _buildtransform_scale))
    (set `self.Hit Actor` _hitactor)
    (set `self.Hit Component` _hitcomponent)
    (`/Engine/EditorBlueprintResources/StandardMacros.IsValid` _buildghost
      (:`Is Valid`
        (bind (_found _transform) (`self.DetectBuildBoxes`))
        (if _found
          (set `self.BuildTransform` _transform))
        (bind _hit (`self.Check for Overlap `))
        (bind _hit_2 (`self.Check for Overlap `))
        (if (and _hit _hit_2)
          (`self.Give Build Color` false)
          (else
            (`self.Give Build Color` true)))
        (`self.BuildDelay`))
      (:`Is Not Valid`
        (`self.SpawnBuildGhost` :!label _label)
        (`self.BuildDelay` :!label _label_2)))
    (else
      (if _returnvalue_2
        (set `self.BuildTransform` (`KismetMathLibrary.MakeTransform` _traceend _buildtransform_rotation _buildtransform_scale)))
      (`/Engine/EditorBlueprintResources/StandardMacros.IsValid` _buildghost
        (:`Is Valid`
          (`self.Give Build Color` false)
          (goto _label_2))
        (:`Is Not Valid`
          (goto _label))))))

(fn `Change Mesh`
  (bind _output_mesh (break `/Game/Skyway/Core/Building/S_Buildables` (`|GetArrayItem` (`self.Buildables`) (`self.BuildID`))))
  (bind _buildghost (`self.BuildGhost`)
    (:`then`
      (`StaticMeshComponent.SetStaticMesh` _buildghost _output_mesh))
    (:`else`)))

(fn `Check for Overlap `
  (returns (Hit :type Boolean))
  (bind _buildghost (`self.BuildGhost`))
  (bind _buildghost_2 (`self.BuildGhost`))
  (bind _origin (`KismetSystemLibrary.GetComponentBounds` _buildghost))
  (bind (_min _max) (`StaticMeshComponent.GetLocalBounds` _buildghost))
  (bind (_min_2 _max_2) (`StaticMeshComponent.GetLocalBounds` _buildghost_2))
  (bind _origin_2 (`KismetSystemLibrary.GetComponentBounds` _buildghost_2))
  (bind _output_mesh (break `/Game/Skyway/Core/Building/S_Buildables` (`|GetArrayItem` (`self.Buildables`) (`self.BuildID`))))
  (bind (_returnvalue_x _returnvalue_y _returnvalue_z) (`KismetMathLibrary.BreakVector` (/ (- _min_2 _max_2) 9.0)))
  (bind (_returnvalue_x_2 _returnvalue_y_2 _returnvalue_z_2) (`KismetMathLibrary.BreakVector` (/ (- _min _max) 2.5)))
  (bind _returnvalue (`|GetDataTableRow` "/Game/Skyway/Core/Building/DT_Buildables.DT_Buildables" (`self.Row Name_0`))
    (:`then`
      (bind _returnvalue_2 (`|GetDataTableRow` "/Game/Skyway/Core/Building/DT_Buildables.DT_Buildables" (`self.Row Name`))
        (:`then`
          (if (or (== _output_mesh (break `/Game/Skyway/Core/Building/S_Buildables` _returnvalue_2)) (== (break `/Game/Skyway/Core/Building/S_Buildables` _returnvalue) _output_mesh))
            (bind (_outhit _returnvalue_3) (`KismetSystemLibrary.BoxTraceSingle` :`Start` _origin_2 :`End` _origin_2 :`HalfSize` (+ (`KismetMathLibrary.MakeVector` (* -1 _returnvalue_x) (* -1 _returnvalue_y) (* -1 _returnvalue_z)) (0.0 0.0 20.0)) :`TraceChannel` "TraceTypeQuery1" :`TraceColor` (struct :`R` 0.990895 :`B` 1.0 :`A` 1.0) :`TraceHitColor` (struct :`R` 1.0 :`A` 1.0) :`DrawTime` 0.1))
            (return _returnvalue_3)
            (else
              (set `self.HalfSize` (0.0 0.0 0.0))
              (bind (_outhit_2 _returnvalue_4) (`KismetSystemLibrary.BoxTraceSingleForObjects` :`Start` _origin :`End` _origin :`HalfSize` (`KismetMathLibrary.MakeVector` (* -1 _returnvalue_x_2) (* -1 _returnvalue_y_2) (* -1 _returnvalue_z_2)) :`Orientation` (`SceneComponent.K2_GetComponentRotation` _buildghost) :`ObjectTypes` (`|MakeArray` "ObjectTypeQuery1" "ObjectTypeQuery3" :!type "EObjectTypeQuery Enum") :`DrawTime` 0.1))
              (return _returnvalue_4))))))))

(fn `DetectBuildBoxes`
  (returns (Found :type Boolean) (Transform :type "Transform Structure"))
  (locals (L_Found :type Boolean))
  (bind _boxes (message `/Game/Skyway/Core/Building/BluePrints/BPI_Build.ReturnBoxes` (`self.Hit Actor`)))
  (for _array_element _boxes
    (set `self.Hit Box` _array_element)
    (if (== _array_element (`self.Hit Component`))
      (set `local.L_Found` true)
      (break)))
  (return (`local.L_Found`) (`SceneComponent.K2_GetComponentToWorld` (`self.Hit Component`))))

(fn `Give Build Color`
  (params (IsGreen :type Boolean))
  (set `self.CanBuild` IsGreen)
  (for _index (range (`PrimitiveComponent.GetNumMaterials` (`self.BuildGhost`)))
    (if IsGreen
      (`PrimitiveComponent.SetMaterial` (`self.BuildGhost`) _index "/Game/Skyway/Core/Building/GreenColor.GreenColor")
      (else
        (`PrimitiveComponent.SetMaterial` (`self.BuildGhost`) _index "/Game/Skyway/Core/Building/RedColor.RedColor"))))
  (`SceneComponent.K2_SetWorldTransform` (`self.BuildGhost`) (`self.BuildTransform`) false false))

(fn `Spawn Build`
  (bind _returnvalue (message `/Game/Skyway/Core/Building/BluePrints/BPI_Build.GetShip` (`self.Hit Actor`)))
  (message `/Game/Skyway/Core/Engine/Ship/BPI_Ship.Build` _returnvalue (`|GetArrayItem` (`self.Buildables`) (`self.BuildID`)) (`self.Hit Box`))
  (bind _hit_box (`self.Hit Box`)
    (:`then`
      (`PrimitiveComponent.SetCollisionEnabled` _hit_box "NoCollision"))
    (:`else`)))

(fn `SpawnBuildGhost`
  (bind _output_mesh (break `/Game/Skyway/Core/Building/S_Buildables` (`|GetArrayItem` (`self.Buildables`) (`self.BuildID`))))
  (bind _returnvalue (`|AddComponentByClass` (`self.PlayerRef`) "/Script/Engine.StaticMeshComponent" false (`self.BuildTransform`)))
  (bind _output_get (set `self.BuildGhost` _returnvalue))
  (`StaticMeshComponent.SetStaticMesh` _output_get _output_mesh)
  (`PrimitiveComponent.SetCollisionEnabled` (`self.BuildGhost`) "NoCollision"))