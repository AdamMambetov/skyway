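; BP_Floor is a building piece Blueprint for a floor section in the Skyway building system.
; Its ReturnBoxes function returns an array of its ladder, four floor and four wall components, presumably boxes used as attachment points for other pieces.
; The construction script is empty, and the file contains no other logic.
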(fn `ReturnBoxes`
  (returns (Boxes :type "Array of BoxComponent Object Reference"))
  (return (`|MakeArray` (`self.Ladder`) (`self.Floor1`) (`self.Floor2`) (`self.Floor3`) (`self.Floor4`) (`self.Wall1`) (`self.Wall4`) (`self.Wall3`) (`self.Wall2`))))

(fn `UserConstructionScript`)