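; Box collision component that marks an attachment point on a ship building piece, apparently for building snapping.
; On BeginPlay it attaches to the socket for its CollisionPosition, sets that slot's extent and blocking trace channels, then caches the building's data-table row.
; Foundation and floor slots block paired square and triangular channels.
; UpdateCollisionEnabled box-traces to disable collision on overlapping listed building classes, but its event-graph call is unwired.
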(event `self.ReceiveBeginPlay`
  (`self.InitCollision`)
  (bind _returnvalue (`|GetDataTableRow` "/Game/Skyway/Core/Building/DT_Buildings.DT_Buildings" (`BlueprintGameplayTagLibrary.GetTagName` (`/Game/Skyway/Core/Building/AC_Building_Base.BuildingId` (`self.AttachedBuilding`))))
    (:`then`
      (set `self.AttachedBuildingInfo` _returnvalue))))

(event `self.ReceiveTick`
  (params (DeltaSeconds :type "Float (single-precision)")))

(fn `InitCollision`
  (bind _returnvalue (enumliteral `ECollisionChannel` "ECC_GameTraceChannel2"))
  (bind _returnvalue_2 (enumliteral `ECollisionChannel` "ECC_GameTraceChannel7"))
  (bind _returnvalue_3 (enumliteral `ECollisionChannel` "ECC_GameTraceChannel4"))
  (bind _returnvalue_4 (enumliteral `ECollisionChannel` "ECC_GameTraceChannel2"))
  (bind _returnvalue_5 (enumliteral `ECollisionChannel` "ECC_GameTraceChannel4"))
  (bind _returnvalue_6 (enumliteral `ECollisionChannel` "ECC_GameTraceChannel3"))
  (bind _returnvalue_7 (enumliteral `ECollisionChannel` "ECC_GameTraceChannel4"))
  (bind _returnvalue_8 (enumliteral `ECollisionChannel` "ECC_GameTraceChannel6"))
  (bind _returnvalue_9 (enumliteral `ECollisionChannel` "ECC_GameTraceChannel4"))
  (bind _returnvalue_10 (enumliteral `ECollisionChannel` "ECC_GameTraceChannel7"))
  (bind _returnvalue_11 (enumliteral `ECollisionChannel` "ECC_GameTraceChannel4"))
  (bind _returnvalue_12 (enumliteral `ECollisionChannel` "ECC_GameTraceChannel3"))
  (bind _returnvalue_13 (enumliteral `ECollisionChannel` "ECC_GameTraceChannel6"))
  (bind _returnvalue_14 (enumliteral `ECollisionChannel` "ECC_GameTraceChannel4"))
  (bind _returnvalue_15 (enumliteral `ECollisionChannel` "ECC_GameTraceChannel6"))
  (bind _returnvalue_16 (enumliteral `ECollisionChannel` "ECC_GameTraceChannel7"))
  (bind _returnvalue_17 (enumliteral `ECollisionChannel` "ECC_GameTraceChannel4"))
  (bind _returnvalue_18 (enumliteral `ECollisionChannel` "ECC_GameTraceChannel4"))
  (bind _returnvalue_19 (`/Game/Skyway/Core/Engine/MLBP_Defaults.DEFAULT`))
  (bind _foundation_triangular_box_extend (`self.FOUNDATION_TRIANGULAR_BOX_EXTEND`))
  (bind _wall_box_extent (`self.WALL_BOX_EXTENT`))
  (bind _wall_box_extent_2 (`self.WALL_BOX_EXTENT`))
  (bind _wall_box_extent_3 (`self.WALL_BOX_EXTENT`))
  (bind _foundation_box_extent (`self.FOUNDATION_BOX_EXTENT`))
  (bind _wall_box_extent_4 (`self.WALL_BOX_EXTENT`))
  (bind _floor_box_extent (`self.FLOOR_BOX_EXTENT`))
  (bind _floor_triangular_box_extent (`self.FLOOR_TRIANGULAR_BOX_EXTENT`))
  (bind _floor_box_extent_2 (`self.FLOOR_BOX_EXTENT`))
  (`self.K2_AttachToComponent` (`self.AttachedBuilding`) (`|GetArrayItem` (`/Game/Skyway/Core/Building/AC_Building_Base.AllBuildingSockets` (`self.AttachedBuilding`)) (`KismetMathLibrary.Conv_ByteToInt` (`self.CollisionPosition`))) _returnvalue_19 _returnvalue_19 _returnvalue_19)
  (`self.SetBoxExtent` (select `/Game/Skyway/Core/Building/E_BuildingCollisionPosition` (`self.CollisionPosition`) :`NewEnumerator1` _foundation_box_extent :`NewEnumerator2` _foundation_box_extent :`NewEnumerator3` _foundation_box_extent :`NewEnumerator4` _foundation_box_extent :`NewEnumerator5` (`self.LADDER_BOX_EXTENT`) :`NewEnumerator6` _wall_box_extent :`NewEnumerator7` _wall_box_extent :`NewEnumerator8` _wall_box_extent :`NewEnumerator9` _wall_box_extent :`NewEnumerator10` _foundation_triangular_box_extend :`NewEnumerator11` _foundation_triangular_box_extend :`NewEnumerator12` _foundation_triangular_box_extend :`NewEnumerator13` _wall_box_extent_4 :`NewEnumerator14` _wall_box_extent_4 :`NewEnumerator15` _wall_box_extent_4 :`NewEnumerator16` _floor_box_extent :`NewEnumerator17` _floor_box_extent :`NewEnumerator18` _floor_box_extent :`NewEnumerator19` _floor_box_extent :`NewEnumerator20` _wall_box_extent_2 :`NewEnumerator21` _wall_box_extent_2 :`NewEnumerator22` _wall_box_extent_2 :`NewEnumerator23` _wall_box_extent_2 :`NewEnumerator24` (`self.LADDER_BOX_EXTENT`) :`NewEnumerator25` _floor_triangular_box_extent :`NewEnumerator26` _floor_triangular_box_extent :`NewEnumerator27` _floor_triangular_box_extent :`NewEnumerator28` _wall_box_extent_3 :`NewEnumerator29` _wall_box_extent_3 :`NewEnumerator30` _wall_box_extent_3 :`NewEnumerator31` (`self.LADDER_BOX_EXTENT`) :`NewEnumerator32` (`self.FLOOR_BOX_EXTENT`) :`NewEnumerator33` (`self.WALL_BOX_EXTENT`) :`NewEnumerator34` _floor_box_extent_2 :`NewEnumerator35` _floor_box_extent_2))
  (`self.SetCollisionResponseToChannel` (select `/Game/Skyway/Core/Building/E_BuildingCollisionPosition` (`self.CollisionPosition`) :`NewEnumerator1` _returnvalue_4 :`NewEnumerator2` _returnvalue_4 :`NewEnumerator3` _returnvalue_4 :`NewEnumerator4` _returnvalue_4 :`NewEnumerator5` (enumliteral `ECollisionChannel` "ECC_GameTraceChannel5") :`NewEnumerator6` _returnvalue_5 :`NewEnumerator7` _returnvalue_5 :`NewEnumerator8` _returnvalue_5 :`NewEnumerator9` _returnvalue_5 :`NewEnumerator10` _returnvalue_6 :`NewEnumerator11` _returnvalue_6 :`NewEnumerator12` _returnvalue_6 :`NewEnumerator13` _returnvalue_7 :`NewEnumerator14` _returnvalue_7 :`NewEnumerator15` _returnvalue_7 :`NewEnumerator16` _returnvalue_8 :`NewEnumerator17` _returnvalue_8 :`NewEnumerator18` _returnvalue_8 :`NewEnumerator19` _returnvalue_8 :`NewEnumerator20` _returnvalue_9 :`NewEnumerator21` _returnvalue_9 :`NewEnumerator22` _returnvalue_9 :`NewEnumerator23` _returnvalue_9 :`NewEnumerator24` (enumliteral `ECollisionChannel` "ECC_GameTraceChannel5") :`NewEnumerator25` _returnvalue_10 :`NewEnumerator26` _returnvalue_10 :`NewEnumerator27` _returnvalue_10 :`NewEnumerator28` _returnvalue_11 :`NewEnumerator29` _returnvalue_11 :`NewEnumerator30` _returnvalue_11 :`NewEnumerator31` (enumliteral `ECollisionChannel` "ECC_GameTraceChannel5") :`NewEnumerator32` (enumliteral `ECollisionChannel` "ECC_GameTraceChannel6") :`NewEnumerator33` (enumliteral `ECollisionChannel` "ECC_GameTraceChannel4") :`NewEnumerator34` _returnvalue_13 :`NewEnumerator35` _returnvalue_13) "ECR_Block")
  (`self.SetCollisionResponseToChannel` (select `/Game/Skyway/Core/Building/E_BuildingCollisionPosition` (`self.CollisionPosition`) :`NewEnumerator1` _returnvalue_12 :`NewEnumerator2` _returnvalue_12 :`NewEnumerator3` _returnvalue_12 :`NewEnumerator4` _returnvalue_12 :`NewEnumerator5` (enumliteral `ECollisionChannel` "ECC_GameTraceChannel5") :`NewEnumerator6` _returnvalue_14 :`NewEnumerator7` _returnvalue_14 :`NewEnumerator8` _returnvalue_14 :`NewEnumerator9` _returnvalue_14 :`NewEnumerator10` _returnvalue :`NewEnumerator11` _returnvalue :`NewEnumerator12` _returnvalue :`NewEnumerator13` _returnvalue_18 :`NewEnumerator14` _returnvalue_18 :`NewEnumerator15` _returnvalue_18 :`NewEnumerator16` _returnvalue_2 :`NewEnumerator17` _returnvalue_2 :`NewEnumerator18` _returnvalue_2 :`NewEnumerator19` _returnvalue_2 :`NewEnumerator20` _returnvalue_3 :`NewEnumerator21` _returnvalue_3 :`NewEnumerator22` _returnvalue_3 :`NewEnumerator23` _returnvalue_3 :`NewEnumerator24` (enumliteral `ECollisionChannel` "ECC_GameTraceChannel5") :`NewEnumerator25` _returnvalue_15 :`NewEnumerator26` _returnvalue_15 :`NewEnumerator27` _returnvalue_15 :`NewEnumerator28` _returnvalue_17 :`NewEnumerator29` _returnvalue_17 :`NewEnumerator30` _returnvalue_17 :`NewEnumerator31` (enumliteral `ECollisionChannel` "ECC_GameTraceChannel5") :`NewEnumerator32` (enumliteral `ECollisionChannel` "ECC_GameTraceChannel7") :`NewEnumerator33` (enumliteral `ECollisionChannel` "ECC_GameTraceChannel4") :`NewEnumerator34` _returnvalue_16 :`NewEnumerator35` _returnvalue_16) "ECR_Block"))

(fn `UpdateCollisionEnabled`
  (locals (L_ObjectTypes :type "Array of EObjectTypeQuery Enum") (L_HitResult :type "HitResult Structure") (L_DisableCollision :type Boolean :default false) (L_BuildingsIgnore :type "Array of PrimitiveComponent Class Reference"))
  (bind _returnvalue (`self.K2_GetComponentLocation`))
  (bind _array (`|MakeArray` "/Game/Skyway/Core/Building/ShipBuildings/AC_Building_Foundation.AC_Building_Foundation_C" "/Game/Skyway/Core/Building/ShipBuildings/AC_Building_Foundation_Triangular.AC_Building_Foundation_Triangular_C" "/Game/Skyway/Core/Building/ShipBuildings/AC_Building_Floor.AC_Building_Floor_C" "/Game/Skyway/Core/Building/ShipBuildings/AC_Building_Floor_Triangular.AC_Building_Floor_Triangular_C" :!type "/Game/Skyway/Core/Building/AC_Building_Base Class Reference"))
  (bind (_bblockinghit _binitialoverlap _time _distance _location _impactpoint _normal _impactnormal _physmat _hitactor _hitcomponent) (`GameplayStatics.BreakHitResult` (`local.L_HitResult`)))
  (set `local.L_BuildingsIgnore` (select `ETraceTypeQuery` (`.TraceChannel_12_CAB0E44C44736E1176497C93D8BC6B36` (break `/Game/Skyway/Core/Inventory/S_Building_Info` (`self.AttachedBuildingInfo`))) :`TraceTypeQuery5` _array :`TraceTypeQuery6` _array))
  (bind _outhits (`KismetSystemLibrary.BoxTraceMultiForObjects` :`Start` _returnvalue :`End` _returnvalue :`HalfSize` (`self.BoxExtent`) :`Orientation` (`/Game/Skyway/Core/Engine/MLBP_Defaults.DEFAULT`) :`ObjectTypes` (`local.L_ObjectTypes`) :`DrawDebugType` (`/Game/Skyway/Core/Engine/MLBP_Defaults.DEFAULT`) :`bIgnoreSelf` false))
  (for _array_element _outhits
    (set `local.L_HitResult` _array_element)
    (if (not (`local.L_DisableCollision`))
      (set `local.L_DisableCollision` (and (or _bblockinghit _binitialoverlap) (!= _hitcomponent self) (`KismetArrayLibrary.Array_Contains` (`local.L_BuildingsIgnore`) (`GameplayStatics.GetObjectClass` (`.HitComponent` (`GameplayStatics.BreakHitResult` (`local.L_HitResult`)))))))
      (else
        (break))))
  (`self.SetCollisionEnabled` (select `bool` (`local.L_DisableCollision`) :`false` "QueryOnly" :`true` "NoCollision" :!type "ECollisionEnabled Enum")))