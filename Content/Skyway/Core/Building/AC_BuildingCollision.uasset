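; Box collision component that marks a position on a building piece (foundation, floor, wall, ladder variants) for modular building.
; BeginPlay routes through server and multicast events to UpdateBuildingCollision, which attaches it to the building's socket.
; That function uses the CollisionPosition enum to pick box extent and blocked trace channels, pairing square with triangular channels.
; CalculateWorldLocation, unused here, computes per-position offsets; remote Tick prints debug extents.
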(event `UpdateBuildingCollision_SERVER`
  (`self.UpdateBuildingCollision_MULTI`))

(event `UpdateBuildingCollision_MULTI`
  (`self.UpdateBuildingCollision`))

(event `self.ReceiveBeginPlay`
  (`self.UpdateBuildingCollision_SERVER`))

(event `self.ReceiveTick`
  (params (DeltaSeconds :type "Float (single-precision)"))
  (`/Engine/EditorBlueprintResources/ActorComponentMacros.Switch Has Authority`
    (:`Remote`
      (`KismetSystemLibrary.PrintString` (`KismetStringLibrary.Concat_StrStr` (`KismetSystemLibrary.GetDisplayName` self) "----------" (`KismetStringLibrary.Conv_VectorToString` (`self.BoxExtent`))) true true (struct :`G` 0.66 :`B` 1.0 :`A` 1.0) 0.0))))

(fn `CalculateWorldLocation`
  (returns (ReturnValue :type "Vector Structure"))
  (return (+ (`self.K2_GetComponentLocation`) (* (`self.GetForwardVector`) (.x (select `/Game/Skyway/Core/Building/E_BuildingCollisionPosition` (`self.CollisionPosition`) :`NewEnumerator1` (`self.FOUNDATION_LOC_F`) :`NewEnumerator2` (`self.FOUNDATION_LOC_B`) :`NewEnumerator3` (`self.FOUNDATION_LOC_L`) :`NewEnumerator4` (`self.FOUNDATION_LOC_R`) :`NewEnumerator5` (`self.FOUNDATION_LADDER_LOC`) :`NewEnumerator6` (`self.FOUNDATION_WALL_LOC_F`) :`NewEnumerator7` (`self.FOUNDATION_WALL_LOC_B`) :`NewEnumerator8` (`self.FOUNDATION_WALL_LOC_L`) :`NewEnumerator9` (`self.FOUNDATION_WALL_LOC_R`) :`NewEnumerator10` (`self.FOUNDATION_TRIANGULAR_LOC_B`) :`NewEnumerator11` (`self.FOUNDATION_TRIANGULAR_LOC_L`) :`NewEnumerator12` (`self.FOUNDATION_TRIANGULAR_LOC_R`) :`NewEnumerator13` (`self.FOUNDATION_TRIANGULAR_WALL_LOC_B`) :`NewEnumerator14` (`self.FOUNDATION_TRIANGULAR_WALL_LOC_L`) :`NewEnumerator15` (`self.FOUNDATION_TRIANGULAR_WALL_LOC_R`) :`NewEnumerator16` (`self.FLOOR_LOC_F`) :`NewEnumerator17` (`self.FLOOR_LOC_B`) :`NewEnumerator18` (`self.FLOOR_LOC_L`) :`NewEnumerator19` (`self.FLOOR_LOC_R`) :`NewEnumerator20` (`self.FLOOR_WALL_LOC_F`) :`NewEnumerator21` (`self.FLOOR_WALL_LOC_B`) :`NewEnumerator22` (`self.FLOOR_WALL_LOC_L`) :`NewEnumerator23` (`self.FLOOR_WALL_LOC_R`) :`NewEnumerator24` (`self.FLOOR_LADDER_LOC`) :`NewEnumerator25` (`self.FLOOR_TRIANGULAR_LOC_B`) :`NewEnumerator26` (`self.FLOOR_TRIANGULAR_LOC_L`) :`NewEnumerator27` (`self.FLOOR_TRIANGULAR_LOC_R`) :`NewEnumerator28` (`self.FLOOR_TRIANGULAR_WALL_LOC_B`) :`NewEnumerator29` (`self.FLOOR_TRIANGULAR_WALL_LOC_L`) :`NewEnumerator30` (`self.FLOOR_TRIANGULAR_WALL_LOC_R`) :`NewEnumerator31` (`self.LADDER_LOC`) :`NewEnumerator32` (`self.LADDER_FLOOR_LOC`) :`NewEnumerator33` (`self.WALL_LOC`) :`NewEnumerator34` (`self.WALL_FLOOR_LOC_L`) :`NewEnumerator35` (`self.WALL_FLOOR_LOC_R`)))) (* (`self.GetRightVector`) (.y (select `/Game/Skyway/Core/Building/E_BuildingCollisionPosition` (`self.CollisionPosition`) :`NewEnumerator1` (`self.FOUNDATION_LOC_F`) :`NewEnumerator2` (`self.FOUNDATION_LOC_B`) :`NewEnumerator3` (`self.FOUNDATION_LOC_L`) :`NewEnumerator4` (`self.FOUNDATION_LOC_R`) :`NewEnumerator5` (`self.FOUNDATION_LADDER_LOC`) :`NewEnumerator6` (`self.FOUNDATION_WALL_LOC_F`) :`NewEnumerator7` (`self.FOUNDATION_WALL_LOC_B`) :`NewEnumerator8` (`self.FOUNDATION_WALL_LOC_L`) :`NewEnumerator9` (`self.FOUNDATION_WALL_LOC_R`) :`NewEnumerator10` (`self.FOUNDATION_TRIANGULAR_LOC_B`) :`NewEnumerator11` (`self.FOUNDATION_TRIANGULAR_LOC_L`) :`NewEnumerator12` (`self.FOUNDATION_TRIANGULAR_LOC_R`) :`NewEnumerator13` (`self.FOUNDATION_TRIANGULAR_WALL_LOC_B`) :`NewEnumerator14` (`self.FOUNDATION_TRIANGULAR_WALL_LOC_L`) :`NewEnumerator15` (`self.FOUNDATION_TRIANGULAR_WALL_LOC_R`) :`NewEnumerator16` (`self.FLOOR_LOC_F`) :`NewEnumerator17` (`self.FLOOR_LOC_B`) :`NewEnumerator18` (`self.FLOOR_LOC_L`) :`NewEnumerator19` (`self.FLOOR_LOC_R`) :`NewEnumerator20` (`self.FLOOR_WALL_LOC_F`) :`NewEnumerator21` (`self.FLOOR_WALL_LOC_B`) :`NewEnumerator22` (`self.FLOOR_WALL_LOC_L`) :`NewEnumerator23` (`self.FLOOR_WALL_LOC_R`) :`NewEnumerator24` (`self.FLOOR_LADDER_LOC`) :`NewEnumerator25` (`self.FLOOR_TRIANGULAR_LOC_B`) :`NewEnumerator26` (`self.FLOOR_TRIANGULAR_LOC_L`) :`NewEnumerator27` (`self.FLOOR_TRIANGULAR_LOC_R`) :`NewEnumerator28` (`self.FLOOR_TRIANGULAR_WALL_LOC_B`) :`NewEnumerator29` (`self.FLOOR_TRIANGULAR_WALL_LOC_L`) :`NewEnumerator30` (`self.FLOOR_TRIANGULAR_WALL_LOC_R`) :`NewEnumerator31` (`self.LADDER_LOC`) :`NewEnumerator32` (`self.LADDER_FLOOR_LOC`) :`NewEnumerator33` (`self.WALL_LOC`) :`NewEnumerator34` (`self.WALL_FLOOR_LOC_L`) :`NewEnumerator35` (`self.WALL_FLOOR_LOC_R`)))) (* (`self.GetUpVector`) (.z (select `/Game/Skyway/Core/Building/E_BuildingCollisionPosition` (`self.CollisionPosition`) :`NewEnumerator1` (`self.FOUNDATION_LOC_F`) :`NewEnumerator2` (`self.FOUNDATION_LOC_B`) :`NewEnumerator3` (`self.FOUNDATION_LOC_L`) :`NewEnumerator4` (`self.FOUNDATION_LOC_R`) :`NewEnumerator5` (`self.FOUNDATION_LADDER_LOC`) :`NewEnumerator6` (`self.FOUNDATION_WALL_LOC_F`) :`NewEnumerator7` (`self.FOUNDATION_WALL_LOC_B`) :`NewEnumerator8` (`self.FOUNDATION_WALL_LOC_L`) :`NewEnumerator9` (`self.FOUNDATION_WALL_LOC_R`) :`NewEnumerator10` (`self.FOUNDATION_TRIANGULAR_LOC_B`) :`NewEnumerator11` (`self.FOUNDATION_TRIANGULAR_LOC_L`) :`NewEnumerator12` (`self.FOUNDATION_TRIANGULAR_LOC_R`) :`NewEnumerator13` (`self.FOUNDATION_TRIANGULAR_WALL_LOC_B`) :`NewEnumerator14` (`self.FOUNDATION_TRIANGULAR_WALL_LOC_L`) :`NewEnumerator15` (`self.FOUNDATION_TRIANGULAR_WALL_LOC_R`) :`NewEnumerator16` (`self.FLOOR_LOC_F`) :`NewEnumerator17` (`self.FLOOR_LOC_B`) :`NewEnumerator18` (`self.FLOOR_LOC_L`) :`NewEnumerator19` (`self.FLOOR_LOC_R`) :`NewEnumerator20` (`self.FLOOR_WALL_LOC_F`) :`NewEnumerator21` (`self.FLOOR_WALL_LOC_B`) :`NewEnumerator22` (`self.FLOOR_WALL_LOC_L`) :`NewEnumerator23` (`self.FLOOR_WALL_LOC_R`) :`NewEnumerator24` (`self.FLOOR_LADDER_LOC`) :`NewEnumerator25` (`self.FLOOR_TRIANGULAR_LOC_B`) :`NewEnumerator26` (`self.FLOOR_TRIANGULAR_LOC_L`) :`NewEnumerator27` (`self.FLOOR_TRIANGULAR_LOC_R`) :`NewEnumerator28` (`self.FLOOR_TRIANGULAR_WALL_LOC_B`) :`NewEnumerator29` (`self.FLOOR_TRIANGULAR_WALL_LOC_L`) :`NewEnumerator30` (`self.FLOOR_TRIANGULAR_WALL_LOC_R`) :`NewEnumerator31` (`self.LADDER_LOC`) :`NewEnumerator32` (`self.LADDER_FLOOR_LOC`) :`NewEnumerator33` (`self.WALL_LOC`) :`NewEnumerator34` (`self.WALL_FLOOR_LOC_L`) :`NewEnumerator35` (`self.WALL_FLOOR_LOC_R`)))))))

(fn `UpdateBuildingCollision`
  (bind _returnvalue (enumliteral `ECollisionChannel` "ECC_GameTraceChannel2"))
  (bind _returnvalue_2 (enumliteral `ECollisionChannel` "ECC_GameTraceChannel7"))
  (bind _returnvalue_3 (enumliteral `ECollisionChannel` "ECC_GameTraceChannel4"))
  (bind _returnvalue_4 (enumliteral `ECollisionChannel` "ECC_GameTraceChannel2"))
  (bind _returnvalue_5 (enumliteral `ECollisionChannel` "ECC_GameTraceChannel4"))
  (bind _returnvalue_6 (enumliteral `ECollisionChannel` "ECC_GameTraceChannel3"))
  (bind _returnvalue_7 (enumliteral `ECollisionChannel` "ECC_GameTraceChannel4"))
  (bind _returnvalue_8 (enumliteral `ECollisionChannel` "ECC_GameTraceChannel6"))
  (bind _returnvalue_9 (enumliteral `ECollisionChannel` "ECC_GameTraceChannel4"))
  (bind _returnvalue_10 (enumliteral `ECollisionChannel` "ECC_GameTraceChannel7"))
  (bind _returnvalue_11 (enumliteral `ECollisionChannel` "ECC_GameTraceChannel4"))
  (bind _returnvalue_12 (enumliteral `ECollisionChannel` "ECC_GameTraceChannel3"))
  (bind _returnvalue_13 (enumliteral `ECollisionChannel` "ECC_GameTraceChannel6"))
  (bind _returnvalue_14 (enumliteral `ECollisionChannel` "ECC_GameTraceChannel4"))
  (bind _returnvalue_15 (enumliteral `ECollisionChannel` "ECC_GameTraceChannel6"))
  (bind _returnvalue_16 (enumliteral `ECollisionChannel` "ECC_GameTraceChannel7"))
  (bind _returnvalue_17 (enumliteral `ECollisionChannel` "ECC_GameTraceChannel4"))
  (bind _returnvalue_18 (enumliteral `ECollisionChannel` "ECC_GameTraceChannel4"))
  (bind _returnvalue_19 (`/Game/Skyway/Core/Engine/MLBP_Defaults.DEFAULT`))
  (bind _foundation_triangular_box_extend (`self.FOUNDATION_TRIANGULAR_BOX_EXTEND`))
  (bind _wall_box_extent (`self.WALL_BOX_EXTENT`))
  (bind _wall_box_extent_2 (`self.WALL_BOX_EXTENT`))
  (bind _wall_box_extent_3 (`self.WALL_BOX_EXTENT`))
  (bind _foundation_box_extent (`self.FOUNDATION_BOX_EXTENT`))
  (bind _wall_box_extent_4 (`self.WALL_BOX_EXTENT`))
  (bind _floor_box_extent (`self.FLOOR_BOX_EXTENT`))
  (bind _floor_triangular_box_extent (`self.FLOOR_TRIANGULAR_BOX_EXTENT`))
  (bind _floor_box_extent_2 (`self.FLOOR_BOX_EXTENT`))
  (set `self.CollisionPosition` (`self.CollisionPosition`))
  (set `self.AttachedBuilding` (`self.AttachedBuilding`))
  (`self.K2_AttachToComponent` (`self.AttachedBuilding`) (`self.CollisionSocketName`) _returnvalue_19 _returnvalue_19 _returnvalue_19)
  (`self.SetBoxExtent` (select `/Game/Skyway/Core/Building/E_BuildingCollisionPosition` (`self.CollisionPosition`) :`NewEnumerator1` _foundation_box_extent :`NewEnumerator2` _foundation_box_extent :`NewEnumerator3` _foundation_box_extent :`NewEnumerator4` _foundation_box_extent :`NewEnumerator5` (`self.LADDER_BOX_EXTENT`) :`NewEnumerator6` _wall_box_extent :`NewEnumerator7` _wall_box_extent :`NewEnumerator8` _wall_box_extent :`NewEnumerator9` _wall_box_extent :`NewEnumerator10` _foundation_triangular_box_extend :`NewEnumerator11` _foundation_triangular_box_extend :`NewEnumerator12` _foundation_triangular_box_extend :`NewEnumerator13` _wall_box_extent_4 :`NewEnumerator14` _wall_box_extent_4 :`NewEnumerator15` _wall_box_extent_4 :`NewEnumerator16` _floor_box_extent :`NewEnumerator17` _floor_box_extent :`NewEnumerator18` _floor_box_extent :`NewEnumerator19` _floor_box_extent :`NewEnumerator20` _wall_box_extent_2 :`NewEnumerator21` _wall_box_extent_2 :`NewEnumerator22` _wall_box_extent_2 :`NewEnumerator23` _wall_box_extent_2 :`NewEnumerator24` (`self.LADDER_BOX_EXTENT`) :`NewEnumerator25` _floor_triangular_box_extent :`NewEnumerator26` _floor_triangular_box_extent :`NewEnumerator27` _floor_triangular_box_extent :`NewEnumerator28` _wall_box_extent_3 :`NewEnumerator29` _wall_box_extent_3 :`NewEnumerator30` _wall_box_extent_3 :`NewEnumerator31` (`self.LADDER_BOX_EXTENT`) :`NewEnumerator32` (`self.FLOOR_BOX_EXTENT`) :`NewEnumerator33` (`self.WALL_BOX_EXTENT`) :`NewEnumerator34` _floor_box_extent_2 :`NewEnumerator35` _floor_box_extent_2))
  (`KismetSystemLibrary.PrintString` "Set Box Extent" true true (struct :`G` 0.66 :`B` 1.0 :`A` 1.0) 10.0)
  (`self.SetCollisionResponseToChannel` (select `/Game/Skyway/Core/Building/E_BuildingCollisionPosition` (`self.CollisionPosition`) :`NewEnumerator1` _returnvalue_4 :`NewEnumerator2` _returnvalue_4 :`NewEnumerator3` _returnvalue_4 :`NewEnumerator4` _returnvalue_4 :`NewEnumerator5` (enumliteral `ECollisionChannel` "ECC_GameTraceChannel5") :`NewEnumerator6` _returnvalue_5 :`NewEnumerator7` _returnvalue_5 :`NewEnumerator8` _returnvalue_5 :`NewEnumerator9` _returnvalue_5 :`NewEnumerator10` _returnvalue_6 :`NewEnumerator11` _returnvalue_6 :`NewEnumerator12` _returnvalue_6 :`NewEnumerator13` _returnvalue_7 :`NewEnumerator14` _returnvalue_7 :`NewEnumerator15` _returnvalue_7 :`NewEnumerator16` _returnvalue_8 :`NewEnumerator17` _returnvalue_8 :`NewEnumerator18` _returnvalue_8 :`NewEnumerator19` _returnvalue_8 :`NewEnumerator20` _returnvalue_9 :`NewEnumerator21` _returnvalue_9 :`NewEnumerator22` _returnvalue_9 :`NewEnumerator23` _returnvalue_9 :`NewEnumerator24` (enumliteral `ECollisionChannel` "ECC_GameTraceChannel5") :`NewEnumerator25` _returnvalue_10 :`NewEnumerator26` _returnvalue_10 :`NewEnumerator27` _returnvalue_10 :`NewEnumerator28` _returnvalue_11 :`NewEnumerator29` _returnvalue_11 :`NewEnumerator30` _returnvalue_11 :`NewEnumerator31` (enumliteral `ECollisionChannel` "ECC_GameTraceChannel5") :`NewEnumerator32` (enumliteral `ECollisionChannel` "ECC_GameTraceChannel6") :`NewEnumerator33` (enumliteral `ECollisionChannel` "ECC_GameTraceChannel4") :`NewEnumerator34` _returnvalue_13 :`NewEnumerator35` _returnvalue_13) "ECR_Block")
  (`self.SetCollisionResponseToChannel` (select `/Game/Skyway/Core/Building/E_BuildingCollisionPosition` (`self.CollisionPosition`) :`NewEnumerator1` _returnvalue_12 :`NewEnumerator2` _returnvalue_12 :`NewEnumerator3` _returnvalue_12 :`NewEnumerator4` _returnvalue_12 :`NewEnumerator5` (enumliteral `ECollisionChannel` "ECC_GameTraceChannel5") :`NewEnumerator6` _returnvalue_14 :`NewEnumerator7` _returnvalue_14 :`NewEnumerator8` _returnvalue_14 :`NewEnumerator9` _returnvalue_14 :`NewEnumerator10` _returnvalue :`NewEnumerator11` _returnvalue :`NewEnumerator12` _returnvalue :`NewEnumerator13` _returnvalue_18 :`NewEnumerator14` _returnvalue_18 :`NewEnumerator15` _returnvalue_18 :`NewEnumerator16` _returnvalue_2 :`NewEnumerator17` _returnvalue_2 :`NewEnumerator18` _returnvalue_2 :`NewEnumerator19` _returnvalue_2 :`NewEnumerator20` _returnvalue_3 :`NewEnumerator21` _returnvalue_3 :`NewEnumerator22` _returnvalue_3 :`NewEnumerator23` _returnvalue_3 :`NewEnumerator24` (enumliteral `ECollisionChannel` "ECC_GameTraceChannel5") :`NewEnumerator25` _returnvalue_15 :`NewEnumerator26` _returnvalue_15 :`NewEnumerator27` _returnvalue_15 :`NewEnumerator28` _returnvalue_17 :`NewEnumerator29` _returnvalue_17 :`NewEnumerator30` _returnvalue_17 :`NewEnumerator31` (enumliteral `ECollisionChannel` "ECC_GameTraceChannel5") :`NewEnumerator32` (enumliteral `ECollisionChannel` "ECC_GameTraceChannel7") :`NewEnumerator33` (enumliteral `ECollisionChannel` "ECC_GameTraceChannel4") :`NewEnumerator34` _returnvalue_16 :`NewEnumerator35` _returnvalue_16) "ECR_Block"))