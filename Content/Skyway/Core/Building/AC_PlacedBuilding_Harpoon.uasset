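; Placed-building component for the Skyway harpoon that detects whether an island lies beneath it.
; While active, it box-traces 3000 units along its local down axis every tick, ignoring its owner and drawing debug for one frame.
; A blocking hit on a BP_Island_Base child sets the FindIsland flag, which clears when none is found.
; CanActivateEnergy simply returns the Active state, independent of island detection.
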(event `self.ReceiveTick`
  (params (DeltaSeconds :type "Float (single-precision)"))
  (`parent.ReceiveTick` DeltaSeconds)
  (`self.FindIsland`))

(fn `CanActivateEnergy`
  (returns (ReturnValue :type Boolean))
  (return (`self.Active`)))

(fn `FindIsland`
  (locals (L_Start :type "Vector Structure" :default (0.0 0.0 0.0)) (L_End :type "Vector Structure") (L_Find :type Boolean :default false))
  (if (`self.Active`)
    (set `local.L_Start` (`self.K2_GetComponentLocation`))
    (set `local.L_End` (+ (`local.L_Start`) (* (`self.GetUpVector`) -3000.0)))
    (bind _outhits (`KismetSystemLibrary.BoxTraceMulti` (`local.L_Start`) (`local.L_End`) (32.0 32.0 1.0) (struct) "TraceTypeQuery1" false (`|MakeArray` (`self.GetOwner`)) "ForOneFrame"))
    (for _array_element _outhits
      (bind (_bblockinghit _binitialoverlap _time _distance _location _impactpoint _normal _impactnormal _physmat _hitactor) (`GameplayStatics.BreakHitResult` _array_element))
      (if _bblockinghit
        (if (`KismetMathLibrary.ClassIsChildOf` (`GameplayStatics.GetObjectClass` _hitactor) "/Game/Skyway/Art/Islands/BP_Island_Base.BP_Island_Base_C")
          (set `local.L_Find` true))))
    (if (!= (`local.L_Find`) (`self.bFindIsland`))
      (set `self.bFindIsland` (`local.L_Find`)))))