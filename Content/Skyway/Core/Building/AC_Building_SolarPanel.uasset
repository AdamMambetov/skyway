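; AC_Building_SolarPanel is the solar panel building Blueprint, which flags an energy shortage.
; Each Tick runs the parent Tick, then checks the combined input and output energy speed against the stored Energy.
; When the net speed is negative and Energy is depleted, it calls EnergyLack with that net speed, repeating every frame the condition holds.
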(event `self.ReceiveTick`
  (params (DeltaSeconds :type "Float (single-precision)"))
  (`parent.ReceiveTick` DeltaSeconds)
  (if (and (< (+ (`self.InputEnergySpeed`) (`self.OutputEnergySpeed`)) 0.0) (<= (`self.Energy`) 0.0))
    (`self.EnergyLack` (+ (`self.InputEnergySpeed`) (`self.OutputEnergySpeed`)))))