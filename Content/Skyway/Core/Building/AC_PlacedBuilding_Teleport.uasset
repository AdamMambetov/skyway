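; Placed-building teleport component that sends a player from a ship down to an island below it.
; While active, each tick runs a downward box trace to detect an island and store the hit location.
; A box collision created at BeginPlay asks the overlapping main character's controller to teleport to that location when an island is found.
; On destruction, the owning ship base destroys the box through a server call.
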(event `self.ReceiveBeginPlay`
  (`parent.ReceiveBeginPlay`)
  (bind _returnvalue (`|AddComponentByClass` :`self` (`self.GetOwner`) :`Class` "/Script/Engine.BoxComponent"))
  (bind _output_get (set `self.BoxCollision` _returnvalue))
  (`self.K2_AttachToComponent` _output_get self (`self.BoxCollisionSocket`) "SnapToTarget" "SnapToTarget" "SnapToTarget" true)
  (add `PrimitiveComponent.OnComponentBeginOverlap` (`self.BoxCollision`) (`|CreateDelegate` :!event `OnBoxCollisionBeginOverlap_Event`))
  (add `PrimitiveComponent.OnComponentEndOverlap` (`self.BoxCollision`) (`|CreateDelegate` :!event `OnBoxCollisionEndOverlap_Event`)))

(event `self.ReceiveTick`
  (params (DeltaSeconds :type "Float (single-precision)"))
  (`parent.ReceiveTick` DeltaSeconds)
  (`self.FindIsland`))

(event `self.ReceiveEndPlay`
  (params (EndPlayReason :type "EEndPlayReason Enum" :default "Destroyed"))
  (switch `EEndPlayReason` EndPlayReason
    (:`Destroyed`
      (bind _asbp_ship_base (cast `/Game/Skyway/Core/Ship/BP_Ship_Base` (`self.GetOwner`)))
      (`/Game/Skyway/Core/Ship/BP_Ship_Base.DestroyComponent_SERVER` _asbp_ship_base (`self.BoxCollision`)))))

(fn `CanActivateEnergy`
  (returns (ReturnValue :type Boolean))
  (return (`self.Active`)))

(fn `FindIsland`
  (locals (L_Start :type "Vector Structure" :default (0.0 0.0 0.0)) (L_End :type "Vector Structure") (L_Find :type Boolean :default false))
  (if (`self.Active`)
    (set `local.L_Start` (`self.K2_GetComponentLocation`))
    (set `local.L_End` (+ (`local.L_Start`) (* (`self.GetUpVector`) -3000.0)))
    (bind _outhits (`KismetSystemLibrary.BoxTraceMulti` (`local.L_Start`) (`local.L_End`) (100.0 100.0 1.0) (struct) "TraceTypeQuery1" false (`|MakeArray` (`self.GetOwner`)) "ForOneFrame"))
    (for _array_element _outhits
      (bind (_bblockinghit _binitialoverlap _time _distance _location _impactpoint _normal _impactnormal _physmat _hitactor) (`GameplayStatics.BreakHitResult` _array_element))
      (if _bblockinghit
        (if (`KismetMathLibrary.ClassIsChildOf` (`GameplayStatics.GetObjectClass` _hitactor) "/Game/Skyway/Art/Islands/BP_Island_Base.BP_Island_Base_C")
          (set `local.L_Find` true)
          (set `self.IslandLocation` _location))))
    (if (!= (`local.L_Find`) (`self.bFindIsland`))
      (set `self.bFindIsland` (`local.L_Find`)))
    (elif (!= (`self.Active`) (`self.bFindIsland`))
      (set `self.bFindIsland` (`/Game/Skyway/Core/Engine/MLBP_Defaults.DEFAULT`))
      (set `self.IslandLocation` (`/Game/Skyway/Core/Engine/MLBP_Defaults.DEFAULT`)))))

(fn `OnBoxCollisionBeginOverlap_Event`
  (params (OverlappedComponent :type "PrimitiveComponent Object Reference") (OtherActor :type "Actor Object Reference") (OtherComp :type "PrimitiveComponent Object Reference") (OtherBodyIndex :type Integer) (bFromSweep :type Boolean) (SweepResult :type "HitResult Structure (by ref)"))
  (if (== "/Game/Skyway/Core/Characters/BP_MainCharacter.BP_MainCharacter_C" (`GameplayStatics.GetObjectClass` (`local.OtherActor`)))
    (`|ExecutionSequence`
      (:`then_1`
        (if (`self.bFindIsland`)
          (message `/Game/Skyway/Core/Engine/BPI_PlayerController.TeleportPlayerToIsland` (`Pawn.GetController` (cast `Pawn` (`local.OtherActor`) :!pure true)) (`self.IslandLocation`)))))))

(fn `OnBoxCollisionEndOverlap_Event`
  (params (OverlappedComponent :type "PrimitiveComponent Object Reference") (OtherActor :type "Actor Object Reference") (OtherComp :type "PrimitiveComponent Object Reference") (OtherBodyIndex :type Integer)))