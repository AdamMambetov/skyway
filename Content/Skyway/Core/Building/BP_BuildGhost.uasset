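; BP_BuildGhost is the building preview actor that shows the selected buildable's mesh, tinted green or red for whether it can be built.
; Tick swaps the mesh when it differs from CurrentBuildingInfo's item mesh, then resets the tint to red.
; SetMeshColor applies the green or red material to every slot, and IsGhostGreen reports buildability by comparing the first slot to the green material.
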(event `self.ReceiveTick`
  (params (DeltaSeconds :type "Float (single-precision)"))
  (bind ((`StaticMesh_55_DD99137048858773BCC1349BF67B1BCE` _staticmesh)) (break `/Game/Skyway/Core/Inventory/S_Item_Info` (`.ItemInfo_2_96BFBB67441ABC75F13542B20097FC01` (break `/Game/Skyway/Core/Inventory/S_Building_Info` (`self.CurrentBuildingInfo`)))))
  (`parent.ReceiveTick` DeltaSeconds)
  (if (!= (`StaticMeshComponent.StaticMesh` (`self.Mesh`)) _staticmesh)
    (`StaticMeshComponent.SetStaticMesh` (`self.Mesh`) _staticmesh)
    (`self.SetMeshColor` false)))

(fn `IsGhostGreen`
  (returns (ReturnValue :type Boolean))
  (return (== (`PrimitiveComponent.GetMaterial` (`self.Mesh`) 0) (`self.GreenColor`))))

(fn `SetMeshColor`
  (params (bCanBuild :type Boolean))
  (for (_ _array_index) (`MeshComponent.GetMaterials` (`self.Mesh`))
    (`PrimitiveComponent.SetMaterial` (`self.Mesh`) _array_index (select `bool` (`local.bCanBuild`) :`false` (`self.RedColor`) :`true` (`self.GreenColor`)))))

(fn `UserConstructionScript`)