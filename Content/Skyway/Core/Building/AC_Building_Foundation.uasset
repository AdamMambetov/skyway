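; Foundation building component for Skyway that creates the collision boxes marking where neighboring foundations, walls and a ladder line up with a foundation.
; SpawnCollisions extends the parent version, creating foundation and wall boxes on four sides plus one ladder box, each with a debug collision.
; Each group gets its own extent and blocks its own custom trace channels, so traces can tell piece types apart.
; ReturnBoxes exposes all nine boxes as an array.
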(fn `ReturnBoxes`
  (returns (Boxes :type "Array of BoxComponent Object Reference"))
  (return (`|MakeArray` (`self.FoundationCollisionForward`) (`self.FoundationCollisionRight`) (`self.FoundationCollisionBackward`) (`self.FoundationCollisionLeft`) (`self.LadderCollison`) (`self.WallCollisionForward`) (`self.WallCollisionBackward`) (`self.WallCollisionLeft`) (`self.WallCollisionRight`))))

(fn `SpawnCollisions`
  (`parent.SpawnCollisions`)
  (`|ExecutionSequence`
    (:`then_0`
      ;[1 1 1] Foundation Forward
      (bind _returnvalue (`self.CreateCollision` (`self.FOUNDATION_LOCATION_FORWARD`) (`self.FOUNDATION_ROTATION_FORWARD`)))
      (bind _output_get (set `self.FoundationCollisionForward` _returnvalue))
      (`self.CreateDebugCollision` _output_get "Forward"))
    (:`then_1`
      ;[1 1 1] Foundation Backward
      (bind _returnvalue_2 (`self.CreateCollision` (`self.FOUNDATION_LOCATION_BACKWARD`) (`self.FOUNDATION_ROTATION_BACKWARD`)))
      (bind _output_get_2 (set `self.FoundationCollisionBackward` _returnvalue_2))
      (`self.CreateDebugCollision` _output_get_2 "Backward"))
    (:`then_2`
      ;[1 1 1] Foundation Left
      (bind _returnvalue_3 (`self.CreateCollision` (`self.FOUNDATION_LOCATION_LEFT`) (`self.FOUNDATION_ROTATION_LEFT`)))
      (bind _output_get_3 (set `self.FoundationCollisionLeft` _returnvalue_3))
      (`self.CreateDebugCollision` _output_get_3 "Left"))
    (:`then_3`
      ;[1 1 1] Foundation Right
      (bind _returnvalue_4 (`self.CreateCollision` (`self.FOUNDATION_LOCATION_RIGHT`) (`self.FOUNDATION_ROTATION_RIGHT`)))
      (bind _output_get_4 (set `self.FoundationCollisionRight` _returnvalue_4))
      (`self.CreateDebugCollision` _output_get_4 "Right"))
    (:`then_4`
      ;[1 1 1] Ladder
      (bind _returnvalue_5 (`self.CreateCollision` (`self.LADDER_LOCATION`) (`self.LADDER_ROTATION`)))
      (bind _output_get_5 (set `self.LadderCollison` _returnvalue_5))
      (`self.CreateDebugCollision` _output_get_5 "Ladder"))
    (:`then_5`
      ;[1 1 1] Wall Forward
      (bind _returnvalue_6 (`self.CreateCollision` (`self.WALL_LOCATION_FORWARD`) (`self.WALL_ROTATION_FORWARD`)))
      (bind _output_get_6 (set `self.WallCollisionForward` _returnvalue_6))
      (`self.CreateDebugCollision` _output_get_6 "Forward"))
    (:`then_6`
      ;[1 1 1] Wall Backward
      (bind _returnvalue_7 (`self.CreateCollision` (`self.WALL_LOCATION_BACKWARD`) (`self.WALL_ROTATION_BACKWARD`)))
      (bind _output_get_7 (set `self.WallCollisionBackward` _returnvalue_7))
      (`self.CreateDebugCollision` _output_get_7 "Backward"))
    (:`then_7`
      ;[1 1 1] Wall Left
      (bind _returnvalue_8 (`self.CreateCollision` (`self.WALL_LOCATION_LEFT`) (`self.WALL_ROTATION_LEFT`)))
      (bind _output_get_8 (set `self.WallCollisionLeft` _returnvalue_8))
      (`self.CreateDebugCollision` _output_get_8 "Left"))
    (:`then_8`
      ;[1 1 1] Wall Right
      (bind _returnvalue_9 (`self.CreateCollision` (`self.WALL_LOCATION_RIGHT`) (`self.WALL_ROTATION_RIGHT`)))
      (bind _output_get_9 (set `self.WallCollisionRight` _returnvalue_9))
      (`self.CreateDebugCollision` _output_get_9 "Right"))
    (:`then_9`
      ;[1 1 1] Foundation Default Settings
      (`BoxComponent.SetBoxExtent` (`self.FoundationCollisionBackward`) (`self.FOUNDATION_BOX_EXTENT`) true)
      (`BoxComponent.SetBoxExtent` (`self.FoundationCollisionForward`) (`self.FOUNDATION_BOX_EXTENT`) true)
      (`BoxComponent.SetBoxExtent` (`self.FoundationCollisionLeft`) (`self.FOUNDATION_BOX_EXTENT`) true)
      (`BoxComponent.SetBoxExtent` (`self.FoundationCollisionRight`) (`self.FOUNDATION_BOX_EXTENT`) true)
      (`self.SetCollisionResponseToChannel` (`self.FoundationCollisionForward`) "ECC_GameTraceChannel2" "ECR_Block")
      (`self.SetCollisionResponseToChannel` (`self.FoundationCollisionBackward`) "ECC_GameTraceChannel2" "ECR_Block")
      (`self.SetCollisionResponseToChannel` (`self.FoundationCollisionLeft`) "ECC_GameTraceChannel2" "ECR_Block")
      (`self.SetCollisionResponseToChannel` (`self.FoundationCollisionRight`) "ECC_GameTraceChannel2" "ECR_Block")
      (`self.SetCollisionResponseToChannel` (`self.FoundationCollisionForward`) "ECC_GameTraceChannel3" "ECR_Block")
      (`self.SetCollisionResponseToChannel` (`self.FoundationCollisionBackward`) "ECC_GameTraceChannel3" "ECR_Block")
      (`self.SetCollisionResponseToChannel` (`self.FoundationCollisionLeft`) "ECC_GameTraceChannel3" "ECR_Block")
      (`self.SetCollisionResponseToChannel` (`self.FoundationCollisionRight`) "ECC_GameTraceChannel3" "ECR_Block"))
    (:`then_10`
      ;[1 1 1] Wall Default Settings
      (`BoxComponent.SetBoxExtent` (`self.WallCollisionForward`) (`self.WALL_BOX_EXTENT`) true)
      (`BoxComponent.SetBoxExtent` (`self.WallCollisionBackward`) (`self.WALL_BOX_EXTENT`) true)
      (`BoxComponent.SetBoxExtent` (`self.WallCollisionLeft`) (`self.WALL_BOX_EXTENT`) true)
      (`BoxComponent.SetBoxExtent` (`self.WallCollisionRight`) (`self.WALL_BOX_EXTENT`) true)
      (`self.SetCollisionResponseToChannel` (`self.WallCollisionForward`) "ECC_GameTraceChannel4" "ECR_Block")
      (`self.SetCollisionResponseToChannel` (`self.WallCollisionBackward`) "ECC_GameTraceChannel4" "ECR_Block")
      (`self.SetCollisionResponseToChannel` (`self.WallCollisionLeft`) "ECC_GameTraceChannel4" "ECR_Block")
      (`self.SetCollisionResponseToChannel` (`self.WallCollisionRight`) "ECC_GameTraceChannel4" "ECR_Block"))
    (:`then_11`
      ;[1 1 1] Ladder Default Settings
      (`BoxComponent.SetBoxExtent` (`self.LadderCollison`) (`self.LADDER_BOX_EXTENT`) true)
      (`self.SetCollisionResponseToChannel` (`self.LadderCollison`) "ECC_GameTraceChannel5" "ECR_Block"))))