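; AC_Building_Furnace is a building component for a furnace that holds pieces to recycle and materials in storage.
; On BeginPlay it adds storage and crafting components to its owner, with a Recycle container and a Storage container.
; CanActivateEnergy resolves the first piece's recipe through data tables, then checks input, energy, second Recycle slot room, and a matching or empty Storage slot.
; SpendEnergy only calls the parent.
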(event `self.ReceiveBeginPlay`
  (`parent.ReceiveBeginPlay`)
  (bind _returnvalue (`|AddComponentByClass` :`self` (`self.GetOwner`) :`Class` "/Game/Skyway/Core/Inventory/AC_Storage.AC_Storage_C" :`InitSlotContainers` (`|MakeArray` (make `/Game/Skyway/Core/Inventory/S_SlotContainer_Info` :`Id` (struct :`TagName` "SlotContainer.Recycle") :`Type` "NewEnumerator6" :`StoredItemTypes` (struct :`GameplayTags` (struct :`(TagName` "Item.Piece")))) (make `/Game/Skyway/Core/Inventory/S_SlotContainer_Info` :`Id` (struct :`TagName` "SlotContainer.Storage") :`StoredItemTypes` (struct :`GameplayTags` (struct :`(TagName` "Item.Material")))))))
  (set `self.Storage` _returnvalue)
  (bind _returnvalue_2 (`|AddComponentByClass` (`self.GetOwner`) "/Game/Skyway/Core/Crafting/AC_Crafting.AC_Crafting_C"))
  (set `self.Crafting` _returnvalue_2))

(fn `CanActivateEnergy`
  (returns (ReturnValue :type Boolean))
  (bind _returnarray (`/Game/Skyway/Core/Inventory/AC_Storage.GetSlotsAtItemType` (`self.Storage`) (struct :`TagName` "SlotContainer.Recycle") "NewEnumerator5"))
  (bind ((`Amount_49_D1E29AF04498C178B74986AAD5610193` _amount) (`MaxAmount_42_B9C41EB0416DBFA24E1E75A6CD16E5AA` _maxamount)) (break `/Game/Skyway/Core/Inventory/S_Item_Info` (`.ItemInfo_14_7E8F48144F0F01654500E084A85436C5` (break `/Game/Skyway/Core/Inventory/S_Slot_Info` (`|GetArrayItem` _returnarray 1)))))
  (bind ((`Amount_49_D1E29AF04498C178B74986AAD5610193` _amount_2) (`ID_71_BA06E0BD4E97D16461377CB9BF36CE2D` _id)) (break `/Game/Skyway/Core/Inventory/S_Item_Info` (`.ItemInfo_14_7E8F48144F0F01654500E084A85436C5` (break `/Game/Skyway/Core/Inventory/S_Slot_Info` (`|GetArrayItem` (`/Game/Skyway/Core/Inventory/AC_Storage.GetSlotsAtItemType` (`self.Storage`) (struct :`TagName` "SlotContainer.Storage") "NewEnumerator5"))))))
  (bind _returnvalue (`|GetDataTableRow` "/Game/Skyway/Core/Inventory/DT_Pieces.DT_Pieces" (`BlueprintGameplayTagLibrary.GetTagName` (`.ID_71_BA06E0BD4E97D16461377CB9BF36CE2D` (break `/Game/Skyway/Core/Inventory/S_Item_Info` (`.ItemInfo_14_7E8F48144F0F01654500E084A85436C5` (break `/Game/Skyway/Core/Inventory/S_Slot_Info` (`|GetArrayItem` (`/Game/Skyway/Core/Inventory/AC_Storage.GetSlotsAtItemType` (`self.Storage`) (struct :`TagName` "SlotContainer.Recycle") "NewEnumerator5"))))))))
    (:`then`
      (bind _returnvalue_2 (`|GetDataTableRow` "/Game/Skyway/Core/Crafting/DT_Recipes.DT_Recipes" (`BlueprintGameplayTagLibrary.GetTagName` (`.RecipeId_25_3797D7844273B4CF8F7EB1842ED1659C` (break `/Game/Skyway/Core/Inventory/S_Piece_Info` _returnvalue))))
        (:`then`
          (return (and (> (`.Amount_49_D1E29AF04498C178B74986AAD5610193` (break `/Game/Skyway/Core/Inventory/S_Item_Info` (`.ItemInfo_14_7E8F48144F0F01654500E084A85436C5` (break `/Game/Skyway/Core/Inventory/S_Slot_Info` (`|GetArrayItem` _returnarray))))) 0) (or (== _amount 0) (< _amount _maxamount)) (> (`self.Energy`) 1.0) (or (== (`.Result_23_1B532DAD43B20A155E0A209CC428568B` (break `/Game/Skyway/Core/Crafting/S_Recipe` _returnvalue_2)) _id) (< _amount_2 1)))))))))

(fn `SpendEnergy`
  (`parent.SpendEnergy`))