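; Experience component that tracks player level, skill points and a Flash currency.
; Adding experience recurses through level-ups, relying on the Level RepNotify to grant a skill point, show the new-level widget, reset experience and raise the linear threshold.
; Flash changes fire an update event, gains show a popup, and losses clamp at zero.
; Only Flash persists in the SaveGame, keyed by player name, and loading writes it straight back.
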(event `self.ReceiveTick`
  (params (DeltaSeconds :type "Float (single-precision)")))

(event `/Game/Skyway/Core/Engine/BPI_CanSave.SaveToPlayer`
  (params (SaveGame :type "SaveGame Object Reference"))
  (bind (_returnvalue _playerinfo) (message `/Game/Skyway/Core/Engine/BPI_SaveGame.LoadPlayer` SaveGame (`FileManager.GetPlayerName`)))
  (if _returnvalue
    (bind _structout (setmembers `/Game/Skyway/Core/Engine/S_PlayerInfo` :`StructRef` _playerinfo :`FlashCount` (`self.Flash`)))
    (message `/Game/Skyway/Core/Engine/BPI_SaveGame.SavePlayer` SaveGame _structout)
    (else
      (bind _structout_2 (setmembers `/Game/Skyway/Core/Engine/S_PlayerInfo` :`StructRef` (`/Game/Skyway/Core/Engine/MLBP_Defaults.DEFAULT`) :`Name` (`FileManager.GetPlayerName`) :`FlashCount` (`self.Flash`)))
      (message `/Game/Skyway/Core/Engine/BPI_SaveGame.SavePlayer` SaveGame _structout_2))))

(event `/Game/Skyway/Core/Engine/BPI_CanSave.LoadToPlayer`
  (params (SaveGame :type "SaveGame Object Reference"))
  (bind (_returnvalue _playerinfo) (message `/Game/Skyway/Core/Engine/BPI_SaveGame.LoadPlayer` SaveGame (`FileManager.GetPlayerName`)))
  (if _returnvalue
    (set `self.Flash` (`.FlashCount_32_991FC9B74667AFC7FB9137A14ECB074D` (break `/Game/Skyway/Core/Engine/S_PlayerInfo` _playerinfo))))
  (`/Game/Skyway/Core/Engine/BPI_CanSave.SaveToPlayer` SaveGame))

(fn `AddExpereance`
  (params (Expereance :type "Float (double-precision)"))
  (locals (L_NeedExp :type "Float (double-precision)") (NewLocalVar_0 :type "Float (double-precision)" :default -0.256))
  (bind _expereance (`local.Expereance`))
  (bind _output_get (set `local.L_NeedExp` (- (`self.ExpereanceToNextLevel`) (`self.CurrentExpereance`))))
  (if (or (> _expereance _output_get) (`KismetMathLibrary.NearlyEqual_FloatFloat` _expereance _output_get))
    (set `self.Level` (+ (`self.Level`) 1))
    (`self.AddExpereance` (- (`local.Expereance`) (`local.L_NeedExp`)))
    (else
      (set `self.CurrentExpereance` (+ (`self.CurrentExpereance`) (`local.Expereance`))))))

(fn `AddFlash`
  (params (Flash :type Integer))
  (set `self.Flash` (+ Flash (`self.Flash`)))
  (`self.OnFlashCountUpdate`)
  (bind _returnvalue (`|CreateWidget` "/Game/Skyway/Core/UI/Expereance/WBP_FlashGetting.WBP_FlashGetting_C" null Flash))
  (`UserWidget.AddToViewport` _returnvalue 100))

(fn `DecrementSkillPoints`
  (`/Engine/EditorBlueprintResources/StandardMacros.DecrementInt` (`self.SkillPoints`)))

(fn `DiminishFlash`
  (params (Flash :type Integer))
  (bind _returnvalue (- (`self.Flash`) Flash))
  (set `self.Flash` (select `bool` (> _returnvalue 0) :`true` _returnvalue))
  (`self.OnFlashCountUpdate`))

(fn `OnRep_Level`
  (`/Engine/EditorBlueprintResources/StandardMacros.IncrementInt` (`self.SkillPoints`)
    (:`  `
      (bind _returnvalue (`|CreateWidget` "/Game/Skyway/Core/UI/Expereance/WBP_NewLevel.WBP_NewLevel_C"))
      (`UserWidget.AddToViewport` _returnvalue 0)
      (set `self.ExpereanceToNextLevel` (+ (* (`self.Level`) 250.0) 1000.0))
      (set `self.CurrentExpereance` 0.0))))