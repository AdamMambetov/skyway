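; Base AI controller that tracks the closest perceived actor as the pawn's enemy and feeds combat state to the Blackboard.
; On possess it resets BattleState.
; While the pawn lives, each tick writes its attack state, the enemy's last position and the nearest perceived actor, which also becomes the focus.
; Prediction sense stimuli from AI Perception update a separate predicted location key.
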(event `self.ReceivePossess`
  (params (PossessedPawn :type "Pawn Object Reference"))
  (bind _blackboard (`self.Blackboard`)
    (:`then`
      (`BlackboardComponent.SetValueAsEnum` _blackboard "BattleState" 0))
    (:`else`)))

(event `self.ReceiveTick`
  (params (DeltaSeconds :type "Float (single-precision)"))
  (if (not (`/Game/Skyway/Core/Stats/AC_StatComponent.IsDead` (`self.GetComponentByClass` (`self.K2_GetPawn`) "/Game/Skyway/Core/Stats/AC_StatComponent.AC_StatComponent_C")))
    (`self.InAttackUpdate`)
    (`self.Enemy Last Pos Update`)
    (`self.EnemyActorUpdate`)))

(event `self.AIPerception.OnTargetPerceptionUpdated`
  (params (Actor :type "Actor Object Reference") (Stimulus :type "AIStimulus Structure"))
  (bind _returnvalue (`AIPerceptionSystem.GetSenseClassForStimulus` Stimulus))
  (if (== _returnvalue "/Script/AIModule.AISense_Prediction")
    (bind _blackboard (`self.Blackboard`)
      (:`then`
        (`BlackboardComponent.SetValueAsVector` _blackboard "PredictLocation" (`.StimulusLocation` (break `AIStimulus` Stimulus))))
      (:`else`))))

(fn `Enemy Last Pos Update`
  (bind _blackboard (`self.Blackboard`)
    (:`then`
      (bind _asactor (cast `Actor` (`BlackboardComponent.GetValueAsObject` _blackboard "Enemy") :!pure true))
      (`/Engine/EditorBlueprintResources/StandardMacros.IsValid` _asactor
        (:`Is Valid`
          (`BlackboardComponent.SetValueAsVector` _blackboard "LastEnemyPos" (`self.K2_GetActorLocation` _asactor)))))
    (:`else`)))

(fn `EnemyActorUpdate`
  (bind _closestenemy (`self.GetClosestEnemyBySense` null))
  (bind _returnvalue (`AIBlueprintHelperLibrary.GetBlackboard` null))
  (`/Engine/EditorBlueprintResources/StandardMacros.IsValid` _returnvalue
    (:`Is Valid`
      (`/Engine/EditorBlueprintResources/StandardMacros.IsValid` _closestenemy
        (:`Is Valid`
          (`BlackboardComponent.SetValueAsObject` _returnvalue "Enemy" _closestenemy)
          (`self.K2_SetFocus` _closestenemy))
        (:`Is Not Valid`
          (`BlackboardComponent.SetValueAsObject` _returnvalue "Enemy" null))))))

(fn `GetClosestEnemyBySense`
  (params (SenseToUse :type "AISense Class Reference"))
  (returns (ClosestEnemy :type "Actor Object Reference"))
  (locals (BestDistance :type "Float (double-precision)" :default 9999999999999.0) (BestEnemy :type "Actor Object Reference"))
  (for _array_element (`AIPerceptionComponent.GetPerceivedActors` (`self.AIPerception`) SenseToUse)
    (bind _returnvalue (`KismetMathLibrary.Vector_Distance` (`self.K2_GetActorLocation` _array_element) (`self.K2_GetActorLocation` (`self.K2_GetPawn`))))
    (if (< _returnvalue (`local.BestDistance`))
      (set `local.BestEnemy` _array_element)
      (set `local.BestDistance` _returnvalue)))
  (return (`local.BestEnemy`)))

(fn `InAttackUpdate`
  (bind _blackboard (`self.Blackboard`)
    (:`then`
      (`BlackboardComponent.SetValueAsBool` _blackboard "InAttack" (select `/Game/Skyway/Core/Attack/E_AttackState` (`/Game/Skyway/Core/Attack/AC_Attack.AttackState` (`self.GetComponentByClass` (`self.K2_GetPawn`) "/Game/Skyway/Core/Attack/AC_Attack.AC_Attack_C")) :`NewEnumerator1` true)))
    (:`else`)))

(fn `UserConstructionScript`)