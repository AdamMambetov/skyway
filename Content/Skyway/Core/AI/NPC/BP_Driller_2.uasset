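; BP_Driller_2 is a flying, laser-armed NPC that keeps pace with the player ship (BP_Ship_Test).
; Each tick it closes to FlyRadius at reduced vertical speed and then matches ship velocity, unless the blackboard InStrafe flag is set.
; Strafes add their velocity to the ship's until the set distance is reached.
; It also requests AI prediction of the blackboard Enemy's position, timed by distance over projectile speed.
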(event `self.ReceiveBeginPlay`
  (`parent.ReceiveBeginPlay`)
  (`/Game/Skyway/Core/Inventory/AC_Storage.AddItemToSlotContainer` (`self.Inventory`) (struct :`TagName` "SlotContainer.Weapon") (struct :`TagName` "Item.Weapon.Laser") 1)
  (bind _returnvalue (`GameplayStatics.GetActorOfClass` "/Game/Skyway/Core/Ship/BP_Ship_Test.BP_Ship_Test_C"))
  (set `self.PlayerShipRef` _returnvalue))

(event `self.ReceiveTick`
  (params (DeltaSeconds :type "Float (single-precision)"))
  (bind _returnvalue (`AIBlueprintHelperLibrary.GetAIController` self))
  (bind _returnvalue_2 (`BlackboardComponent.GetValueAsObject` (`AIController.Blackboard` _returnvalue) "Enemy"))
  (bind _asactor (cast `Actor` _returnvalue_2 :!pure true))
  (`parent.ReceiveTick` DeltaSeconds)
  (if (`BlackboardComponent.GetValueAsBool` (`AIController.Blackboard` (`AIBlueprintHelperLibrary.GetAIController` self)) "InStrafe")
    (`self.Strafe`)
    (else
      (`self.TakePos`)))
  (`/Engine/EditorBlueprintResources/StandardMacros.IsValid` _returnvalue_2
    (:`Is Valid`
      (`AISense_Prediction.RequestControllerPredictionEvent` _returnvalue _asactor (/ (`self.GetDistanceTo` self _asactor) (`.ProjectileSpeed_21_69F9401441B1F6E861D3B990F0B6DCF6` (break `/Game/Skyway/Core/Inventory/S_Weapon_Info` (`/Game/Skyway/Core/Attack/AC_Attack.GetWeaponInfo` (`self.Attack`)))))))))

(fn `Strafe`
  (bind _playershipref (`self.PlayerShipRef`))
  (if (`KismetMathLibrary.NearlyEqual_FloatFloat` (`KismetMathLibrary.Vector_Distance` (`self.K2_GetActorLocation`) (`self.StrafeStartLocation`)) (`self.Strafe Distance`) 10.0)
    (`BlackboardComponent.SetValueAsBool` (`AIController.Blackboard` (`AIBlueprintHelperLibrary.GetAIController` self)) "InStrafe" false)
    (else
      (set `MovementComponent.Velocity` (+ (`self.StrafeVelocity`) (* (`/Game/Skyway/Core/Ship/BP_Ship_Base.Speed` _playershipref) (`/Game/Skyway/Core/Ship/BP_Ship_Base.Direction` _playershipref))) (`self.CharacterMovement`)))))

(fn `StrafeActivate`
  (params (StrafeDirection :type "Vector Structure") (StrafeDistance :type "Float (double-precision)") (StrafeSpeed :type "Float (double-precision)"))
  (locals (L_StartLocation :type "Vector Structure" :default (0.0 0.0 0.0)))
  (set `self.Strafe Distance` StrafeDistance)
  (set `self.StrafeStartLocation` (`self.K2_GetActorLocation`))
  (set `self.StrafeVelocity` (* StrafeDirection StrafeSpeed))
  (`BlackboardComponent.SetValueAsBool` (`AIController.Blackboard` (`AIBlueprintHelperLibrary.GetAIController` self)) "InStrafe" true))

(fn `StrafeDeactivate`
  (`BlackboardComponent.SetValueAsBool` (`AIController.Blackboard` (`AIBlueprintHelperLibrary.GetAIController` self)) "InStrafe" false)
  (set `self.StrafeStartLocation` (0.0 0.0 0.0))
  (set `self.Strafe Distance` 0.0)
  (set `self.StrafeVelocity` (0.0 0.0 0.0)))

(fn `TakePos`
  (bind _returnvalue (`self.K2_GetActorLocation`))
  (bind _charactermovement (`self.CharacterMovement`))
  (bind _flyradius (`self.FlyRadius`))
  (bind _playershipref (`self.PlayerShipRef`))
  (bind _returnvalue_2 (`self.K2_GetActorLocation` _playershipref))
  (bind _speed (`/Game/Skyway/Core/Ship/BP_Ship_Base.Speed` _playershipref))
  (bind _returnvalue_3 (`KismetMathLibrary.Vector_Distance` _returnvalue_2 _returnvalue))
  (bind _returnvalue_4 (+ _speed (`self.FlyRadius`)))
  (bind (_returnvalue_x _returnvalue_y _returnvalue_z) (`KismetMathLibrary.BreakVector` (* (`KismetMathLibrary.GetDirectionUnitVector` _returnvalue _returnvalue_2) _returnvalue_4)))
  (if (or (`KismetMathLibrary.NearlyEqual_FloatFloat` _returnvalue_3 _flyradius (* _returnvalue_4 (`GameplayStatics.GetWorldDeltaSeconds`))) (< _returnvalue_3 _flyradius))
    (set `MovementComponent.Velocity` (* (`/Game/Skyway/Core/Ship/BP_Ship_Base.Direction` _playershipref) _speed) _charactermovement)
    (else
      (set `MovementComponent.Velocity` (`KismetMathLibrary.MakeVector` _returnvalue_x _returnvalue_y (/ _returnvalue_z 2.0)) _charactermovement))))

(fn `UserConstructionScript`
  (`parent.UserConstructionScript`))