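; Base NPC enemy character with a health bar widget, AI perception and leader-pose body meshes.
; Each tick it sets walk speed from the blackboard BattleState and sphere-traces with two radii to update the enemy Overlap key.
; On death it ragdolls, completes the player's first-kill task, awards experience flashes and expires.
; Damage hit sounds are tiered, but health updates before the comparison, so only the lightest plays.
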(event `self.ReceiveBeginPlay`
  (bind _widget (`self.Widget`))
  (bind _returnvalue (`|CreateWidget` "/Game/Skyway/Core/UI/Enemy/WBP_EnemyHpBar.WBP_EnemyHpBar_C" null self))
  (`WidgetComponent.SetWidget` _widget _returnvalue)
  (`WidgetComponent.SetDrawSize` _widget (268.0 42.0))
  (`AIPerceptionComponent.RequestStimuliListenerUpdate` (`AIController.GetAIPerceptionComponent` (`AIBlueprintHelperLibrary.GetAIController` self)))
  (add `/Game/Skyway/Core/Stats/AC_StatComponent.OnStatCurrentValueChange` (`self.StatComponent`) (`|CreateDelegate` :!event `OnTakeDamage`))
  (set `self.CurrentHelth` (`.CurrentValue_4_DE51577F455957135DBA8EAD967FB78D` (break `/Game/Skyway/Core/Stats/S_StatInfo` (`.StatInfo` (`/Game/Skyway/Core/Stats/AC_StatComponent.GetStatInfoById` (`self.StatComponent`) (struct :`TagName` "Stat.Health")))))))

(event `self.ReceiveTick`
  (params (DeltaSeconds :type "Float (single-precision)"))
  (`self.UpdateMaxWalkSpeed`)
  (if (not (`/Game/Skyway/Core/Stats/AC_StatComponent.IsDead` (`self.StatComponent`)))
    (`self.SetNeedToTakePosition`)
    (else
      (`/Engine/EditorBlueprintResources/StandardMacros.DoOnce` false
        (:`Completed`
          (`self.SetLifeSpan` 3.0)
          (`/Game/Skyway/Core/Expereance/AC_Expereance.AddFlash` (`self.GetComponentByClass` (`GameplayStatics.GetPlayerPawn` 0) "/Game/Skyway/Core/Expereance/AC_Expereance.AC_Expereance_C") (`KismetMathLibrary.RandomIntegerInRange` 2 3))
          (`self.OnNpcDeth` self))))))

(event `self.StatComponent.OnStatReachedZero`
  (params (StatId :type "GameplayTag Structure"))
  (bind _returnvalue (`BlackboardComponent.GetValueAsObject` (`AIBlueprintHelperLibrary.GetBlackboard` (`AIBlueprintHelperLibrary.GetAIController` self)) "Enemy"))
  (`|SwitchGameplayTag` StatId
    (:`Stat.Health`
      (`PrimitiveComponent.SetSimulatePhysics` (`self.Mesh`) true)
      (set `SkeletalMeshComponent.bPauseAnims` true (`self.Mesh`))
      (`/Engine/EditorBlueprintResources/StandardMacros.IsValid` _returnvalue
        (:`Is Valid`
          (bind _asbp_main_character (cast `/Game/Skyway/Core/Characters/BP_MainCharacter` _returnvalue))
          (`/Game/Skyway/Core/Tasks/AC_Task.CompleteActionById` (`/Game/Skyway/Core/Characters/BP_MainCharacter.Task` _asbp_main_character) (struct :`TagName` "Action.KillFirstNpc") true))))))

(event `OnTakeDamage`
  (params (StatId :type "GameplayTag Structure") (CurrentValue :type "Float (double-precision)"))
  (bind _sound (`self.Sound`))
  (bind _sound_2 (`self.Sound`))
  (bind _sound_3 (`self.Sound`))
  (bind _returnvalue (- (`self.CurrentHelth`) CurrentValue))
  (if (and (`BlueprintGameplayTagLibrary.MatchesTag` StatId (struct :`TagName` "Stat.Health")) (not (`/Game/Skyway/Core/Stats/AC_StatComponent.IsDead` (`self.StatComponent`))))
    (set `self.CurrentHelth` CurrentValue)
    (if (> _returnvalue 50.0)
      (`AudioComponent.SetSound` _sound_2 "/Game/Skyway/Audio/Cues/HittingRobot_3_Cue.HittingRobot_3_Cue")
      (`AudioComponent.Play` _sound_2 0.0)
      (elif (> _returnvalue 30.0)
        (`AudioComponent.SetSound` _sound_3 "/Game/Skyway/Audio/Cues/HittingRobot_2_Cue.HittingRobot_2_Cue")
        (`AudioComponent.Play` _sound_3 0.0)
        (else
          (`AudioComponent.SetSound` _sound "/Game/Skyway/Audio/Cues/HittingRobot_1_Cue.HittingRobot_1_Cue")
          (`AudioComponent.Play` _sound 0.0))))))

(event `self.OnWeaponCollisionBeginOverlapEvent`
  (params (OverlappedComponent :type "PrimitiveComponent Object Reference") (OtherActor :type "Actor Object Reference") (OtherComp :type "PrimitiveComponent Object Reference") (OtherBodyIndex :type Integer) (bFromSweep :type Boolean) (SweepResult :type "HitResult Structure (by ref)"))
  (bind _asbase_character (cast `BaseCharacter` OtherActor))
  (`self.Recoil` _asbase_character 0.1))

(fn `GetWeaponDamage`
  (returns (ReturnValue :type "Float (single-precision)"))
  (return (`.Damage_9_E157A1A343752171738AF58207467496` (break `/Game/Skyway/Core/Inventory/S_Weapon_Info` (`/Game/Skyway/Core/Attack/AC_Attack.GetWeaponInfo` (`self.Attack`))))))

(fn `SetNeedToTakePosition`
  (locals (L_HalfSize :type "Float (double-precision)") (L_HitEnemy :type Boolean))
  (bind _returnvalue (`self.K2_GetActorLocation`))
  (bind _returnvalue_2 (`AIBlueprintHelperLibrary.GetBlackboard` (`AIBlueprintHelperLibrary.GetAIController` self)))
  (`/Engine/EditorBlueprintResources/StandardMacros.IsValid` _returnvalue_2
    (:`Is Valid`
      (if (`BlackboardComponent.GetValueAsBool` _returnvalue_2 (`KismetStringLibrary.Conv_StringToName` "Overlap"))
        (set `local.L_HalfSize` (`self.MaxOverlapRadius`))
        (else
          (set `local.L_HalfSize` (`self.MinOverlapRadius`))))
      (bind (_outhits _returnvalue_3) (`KismetSystemLibrary.SphereTraceMultiForObjects` _returnvalue _returnvalue (`local.L_HalfSize`) (`|MakeArray` "ObjectTypeQuery3" "ObjectTypeQuery8" "ObjectTypeQuery9" :!type "EObjectTypeQuery Enum")))
      (if _returnvalue_3
        (set `local.L_HitEnemy` false)
        (for _array_element _outhits
          (if (== (`.HitActor` (`GameplayStatics.BreakHitResult` _array_element)) (`BlackboardComponent.GetValueAsObject` (`AIBlueprintHelperLibrary.GetBlackboard` (`AIBlueprintHelperLibrary.GetAIController` self)) (`KismetStringLibrary.Conv_StringToName` "Enemy")))
            (set `local.L_HitEnemy` true)
            (break)))
        (`BlackboardComponent.SetValueAsBool` (`AIBlueprintHelperLibrary.GetBlackboard` (`AIBlueprintHelperLibrary.GetAIController` self)) (`KismetStringLibrary.Conv_StringToName` "Overlap") (`local.L_HitEnemy`))
        (else
          (`BlackboardComponent.SetValueAsBool` (`AIBlueprintHelperLibrary.GetBlackboard` (`AIBlueprintHelperLibrary.GetAIController` self)) (`KismetStringLibrary.Conv_StringToName` "Overlap") false))))))

(fn `UpdateMaxWalkSpeed`
  (set `CharacterMovementComponent.MaxWalkSpeed` (select `/Game/Skyway/Core/AI/E_BattleState` (cast `/Game/Skyway/Core/AI/E_BattleState` (`BlackboardComponent.GetValueAsEnum` (`AIBlueprintHelperLibrary.GetBlackboard` (`AIBlueprintHelperLibrary.GetAIController` self)) "BattleState")) :`NewEnumerator2` (`self.PatrolSpeed`) :`NewEnumerator0` (`self.RushSpeed`) :`NewEnumerator1` (`self.BattleSpeed`) :`NewEnumerator3` (`self.ChaseSpeed`) :!type "Float (single-precision)") (`self.CharacterMovement`)))

(fn `UserConstructionScript`
  (`SkinnedMeshComponent.SetLeaderPoseComponent` (`self.Dop`) (`self.Mesh`) false false)
  (`SkinnedMeshComponent.SetLeaderPoseComponent` (`self.Second`) (`self.Mesh`) false false)
  (`SkinnedMeshComponent.SetLeaderPoseComponent` (`self.Hook`) (`self.Mesh`) false false)
  (`self.SpawnDefaultController`))