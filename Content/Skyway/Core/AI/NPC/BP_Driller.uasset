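; Driller NPC character that starts with a laser weapon and leads its shots at enemies.
; On BeginPlay it adds the laser to its inventory's weapon slot.
; Each tick, while the Blackboard holds a valid Enemy, it requests an AI perception prediction of that actor's future position.
; The prediction time is distance divided by the weapon's projectile speed, estimating where the target will be on impact.
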(event `self.ReceiveBeginPlay`
  (`parent.ReceiveBeginPlay`)
  (`/Game/Skyway/Core/Inventory/AC_Storage.AddItemToSlotContainer` (`self.Inventory`) (struct :`TagName` "SlotContainer.Weapon") (struct :`TagName` "Item.Weapon.Laser") 1))

(event `self.ReceiveTick`
  (params (DeltaSeconds :type "Float (single-precision)"))
  (bind _returnvalue (`AIBlueprintHelperLibrary.GetAIController` self))
  (bind _returnvalue_2 (`BlackboardComponent.GetValueAsObject` (`AIController.Blackboard` _returnvalue) "Enemy"))
  (bind _asactor (cast `Actor` _returnvalue_2 :!pure true))
  (`parent.ReceiveTick` DeltaSeconds)
  (`/Engine/EditorBlueprintResources/StandardMacros.IsValid` _returnvalue_2
    (:`Is Valid`
      (`AISense_Prediction.RequestControllerPredictionEvent` _returnvalue _asactor (/ (`self.GetDistanceTo` self _asactor) (`.ProjectileSpeed_21_69F9401441B1F6E861D3B990F0B6DCF6` (break `/Game/Skyway/Core/Inventory/S_Weapon_Info` (`/Game/Skyway/Core/Attack/AC_Attack.GetWeaponInfo` (`self.Attack`)))))))))

(event `self.OnWeaponCollisionBeginOverlapEvent`
  (params (OverlappedComponent :type "PrimitiveComponent Object Reference") (OtherActor :type "Actor Object Reference") (OtherComp :type "PrimitiveComponent Object Reference") (OtherBodyIndex :type Integer) (bFromSweep :type Boolean) (SweepResult :type "HitResult Structure (by ref)")))

(fn `UserConstructionScript`
  (`parent.UserConstructionScript`))