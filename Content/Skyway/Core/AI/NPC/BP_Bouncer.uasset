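; BP_Bouncer is an NPC character, by its name a bouncer, that fights with fists.
; On BeginPlay it adds a fist weapon to its inventory's weapon slot.
; While alive, it sets its widget's visibility each tick from the AI blackboard's Overlap flag.
; When its weapon collision overlaps another BaseCharacter, it calls Recoil on that character.
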(event `self.ReceiveBeginPlay`
  (`parent.ReceiveBeginPlay`)
  (`/Game/Skyway/Core/Inventory/AC_Storage.AddItemToSlotContainer` (`self.Inventory`) (struct :`TagName` "SlotContainer.Weapon") (struct :`TagName` "Item.Weapon.Fist") 1))

(event `self.ReceiveTick`
  (params (DeltaSeconds :type "Float (single-precision)"))
  (`parent.ReceiveTick` DeltaSeconds)
  (if (not (`/Game/Skyway/Core/Stats/AC_StatComponent.IsDead` (`self.StatComponent`)))
    (`SceneComponent.SetVisibility` (`self.Widget`) (`BlackboardComponent.GetValueAsBool` (`AIBlueprintHelperLibrary.GetBlackboard` (`AIBlueprintHelperLibrary.GetAIController` self)) "Overlap") true)))

(event `self.OnWeaponCollisionBeginOverlapEvent`
  (params (OverlappedComponent :type "PrimitiveComponent Object Reference") (OtherActor :type "Actor Object Reference") (OtherComp :type "PrimitiveComponent Object Reference") (OtherBodyIndex :type Integer) (bFromSweep :type Boolean) (SweepResult :type "HitResult Structure (by ref)"))
  (bind _asbase_character (cast `BaseCharacter` OtherActor))
  (`self.Recoil` _asbase_character 0.5))

(fn `UserConstructionScript`
  (`parent.UserConstructionScript`))