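; BP_BaseNPC is a base NPC Blueprint that reports nearby pawns to its AI.
; Every tick it runs a debug-drawn box trace for Pawn objects around its location and writes the result to the "Overlap" Blackboard bool, if a Blackboard is valid.
; The construction script sets Mesh as master pose for the Dop, Second and Hook components, so the modular parts share its animation.
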(event `self.ReceiveBeginPlay`)

(event `self.ReceiveTick`
  (params (DeltaSeconds :type "Float (single-precision)"))
  (bind _returnvalue (`self.K2_GetActorLocation`))
  (bind _returnvalue_2 (`AIBlueprintHelperLibrary.GetBlackboard` (`AIBlueprintHelperLibrary.GetAIController` self)))
  (bind (_outhit _returnvalue_3) (`KismetSystemLibrary.BoxTraceSingleForObjects` :`Start` _returnvalue :`End` _returnvalue :`HalfSize` (250.0 250.0 250.0) :`ObjectTypes` (`|MakeArray` "ObjectTypeQuery3" :!type "EObjectTypeQuery Enum") :`DrawDebugType` "ForOneFrame"))
  (`/Engine/EditorBlueprintResources/StandardMacros.IsValid` _returnvalue_2
    (:`Is Valid`
      (`BlackboardComponent.SetValueAsBool` _returnvalue_2 (`KismetStringLibrary.Conv_StringToName` "Overlap") _returnvalue_3))))

(fn `UserConstructionScript`
  (`SkinnedMeshComponent.SetLeaderPoseComponent` (`self.Dop`) (`self.Mesh`) false)
  (`SkinnedMeshComponent.SetLeaderPoseComponent` (`self.Second`) (`self.Mesh`) false)
  (`SkinnedMeshComponent.SetLeaderPoseComponent` (`self.Hook`) (`self.Mesh`) false))