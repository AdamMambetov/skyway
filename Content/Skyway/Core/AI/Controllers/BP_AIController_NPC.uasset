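; AI controller for NPC pawns that feeds combat state and perception results into the Blackboard.
; On possess it caches the pawn's stat and attack components, then while the pawn lives, Tick updates InAttack, last enemy position and Enemy.
; Enemy and focus follow the closest sighted actor, with flying robots otherwise focusing the player ship.
; Damage stimuli also set or clear Enemy, and prediction stimuli write PredictLocation.
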(event `self.ReceivePossess`
  (params (PossessedPawn :type "Pawn Object Reference"))
  (bind _blackboard (`self.Blackboard`)
    (:`then`
      (`BlackboardComponent.SetValueAsEnum` _blackboard "BattleState" 0)
      (set `self.PawnStatComp` (`self.GetComponentByClass` (`self.K2_GetPawn`) "/Game/Skyway/Core/Stats/AC_StatComponent.AC_StatComponent_C"))
      (set `self.PawnAttackComp` (`self.GetComponentByClass` (`self.K2_GetPawn`) "/Game/Skyway/Core/Attack/AC_Attack.AC_Attack_C")))
    (:`else`)))

(event `self.ReceiveTick`
  (params (DeltaSeconds :type "Float (single-precision)"))
  (bind _pawnstatcomp (`self.PawnStatComp`)
    (:`then`
      (if (not (`/Game/Skyway/Core/Stats/AC_StatComponent.IsDead` _pawnstatcomp))
        (`self.InAttackUpdate`)
        (`self.Enemy Last Pos Update`)
        (`self.EnemyActorUpdate`)))
    (:`else`)))

(event `self.AIPerception.OnTargetPerceptionUpdated`
  (params (Actor :type "Actor Object Reference") (Stimulus :type "AIStimulus Structure"))
  (bind _returnvalue (`AIPerceptionSystem.GetSenseClassForStimulus` Stimulus))
  (`|ExecutionSequence`
    (:`then_0`
      (if (== _returnvalue "/Script/AIModule.AISense_Prediction")
        (bind _blackboard (`self.Blackboard`)
          (:`then`
            (`BlackboardComponent.SetValueAsVector` _blackboard "PredictLocation" (`.StimulusLocation` (break `AIStimulus` Stimulus))))
          (:`else`))
        (else
          (goto _label :!via `Reset`))))
    (:`then_1`
      (if (== _returnvalue "/Script/AIModule.AISense_Damage")
        (bind _blackboard_2 (`self.Blackboard`)
          (:`then`
            (if (not (`/Game/Skyway/Core/Stats/AC_StatComponent.IsDead` (`self.GetComponentByClass` Actor "/Game/Skyway/Core/Stats/AC_StatComponent.AC_StatComponent_C")))
              (`BlackboardComponent.SetValueAsObject` _blackboard_2 "Enemy" Actor)
              (`/Engine/EditorBlueprintResources/StandardMacros.DoOnce` false :!label _label)
              (else
                (`BlackboardComponent.SetValueAsObject` _blackboard_2 "Enemy" null)
                (goto _label :!via `Reset`))))
          (:`else`))
        (else
          (goto _label :!via `Reset`))))))

(fn `Enemy Last Pos Update`
  (bind _blackboard (`self.Blackboard`)
    (:`then`
      (bind _asactor (cast `Actor` (`BlackboardComponent.GetValueAsObject` _blackboard "Enemy") :!pure true))
      (`/Engine/EditorBlueprintResources/StandardMacros.IsValid` _asactor
        (:`Is Valid`
          (`BlackboardComponent.SetValueAsVector` _blackboard "LastEnemyPos" (`self.K2_GetActorLocation` _asactor)))))
    (:`else`)))

(fn `EnemyActorUpdate`
  (bind _closestenemy (`self.GetClosestEnemyBySense` "/Script/AIModule.AISense_Sight"))
  (bind _returnvalue (`AIBlueprintHelperLibrary.GetBlackboard` null))
  (`/Engine/EditorBlueprintResources/StandardMacros.IsValid` _returnvalue
    (:`Is Valid`
      (`/Engine/EditorBlueprintResources/StandardMacros.IsValid` _closestenemy
        (:`Is Valid`
          (`BlackboardComponent.SetValueAsObject` _returnvalue "Enemy" _closestenemy)
          (`self.K2_SetFocus` _closestenemy))
        (:`Is Not Valid`
          (`BlackboardComponent.SetValueAsObject` _returnvalue "Enemy" null)
          (`self.K2_SetFocus` null)
          (bind _asbp_flying_robot (cast `/Game/Skyway/Core/AI/NPC/BP_FlyingRobot` (`self.K2_GetPawn`)))
          (`self.K2_SetFocus` (`/Game/Skyway/Core/AI/NPC/BP_FlyingRobot.PlayerShipRef` _asbp_flying_robot)))))))

(fn `GetClosestEnemyBySense`
  (params (SenseToUse :type "AISense Class Reference"))
  (returns (ClosestEnemy :type "Actor Object Reference"))
  (locals (BestDistance :type "Float (double-precision)" :default 9999999999999.0) (BestEnemy :type "Actor Object Reference"))
  ; TODO: Раньше в 5.0 была функция GetPerceivedActors
  (bind _outactors (`AIPerceptionComponent.GetCurrentlyPerceivedActors` (`self.AIPerception`) SenseToUse))
  (for _array_element _outactors
    (bind _returnvalue (`KismetMathLibrary.Vector_Distance` (`self.K2_GetActorLocation` _array_element) (`self.K2_GetActorLocation` (`self.K2_GetPawn`))))
    (if (< _returnvalue (`local.BestDistance`))
      (set `local.BestEnemy` _array_element)
      (set `local.BestDistance` _returnvalue)))
  (return (`local.BestEnemy`)))

(fn `InAttackUpdate`
  (bind _blackboard (`self.Blackboard`)
    (:`then`
      (`BlackboardComponent.SetValueAsBool` _blackboard "InAttack" (select `/Game/Skyway/Core/Attack/E_AttackState` (`/Game/Skyway/Core/Attack/AC_Attack.AttackState` (`self.PawnAttackComp`)) :`NewEnumerator1` true)))
    (:`else`)))

(fn `UserConstructionScript`)