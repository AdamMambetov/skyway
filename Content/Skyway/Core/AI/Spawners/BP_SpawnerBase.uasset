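; Base NPC spawner that keeps a randomly sized group of actors spawned at random navmesh points within a radius.
; A looping timer, paused by Tick at the target count, drives spawning; deaths can free slots for respawn.
; Deactivating SpawnActive despawns the group once and retargets to the tracked remaining count; EndPlay also destroys spawned actors.
; Init, which would claim a tagged NavMeshBoundsVolume, is never called.
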(event `self.ReceiveBeginPlay`
  (bind _output_get (set `self.ActorToSpawnCount` (`KismetMathLibrary.RandomIntegerInRange` (`self.MinAmountOfSpawnActor`) (`self.MaxAmountOfSpawnActor`))))
  (set `self.CurrentActorCount` _output_get)
  (bind _returnvalue (`GameplayStatics.GetActorOfClass` "/Script/NavigationSystem.RecastNavMesh"))
  (set `self.RecastNavMesh` _returnvalue)
  (if (!= (`self.SpawnedActorCount`) (`self.ActorToSpawnCount`))
    (`KismetSystemLibrary.Delay` 1.0)
    (bind _returnvalue_2 (`KismetSystemLibrary.K2_SetTimerDelegate` (`|CreateDelegate` :!event `Spawn Actor in Radius`) (`self.SpawnInterval`) true))
    (set `self.SpawnTimerHandle` _returnvalue_2)))

(event `self.ReceiveTick`
  (params (DeltaSeconds :type "Float (single-precision)"))
  (if (< (`self.SpawnedActorCount`) (`self.ActorToSpawnCount`))
    (`KismetSystemLibrary.K2_UnPauseTimerHandle` (`self.SpawnTimerHandle`))
    (else
      (`KismetSystemLibrary.K2_PauseTimerHandle` (`self.SpawnTimerHandle`))))
  (if (`self.SpawnActive`)
    (goto _label :!via `Reset`)
    (else
      (`/Engine/EditorBlueprintResources/StandardMacros.DoOnce` false :!label _label
        (:`Completed`
          (set `self.ActorToSpawnCount` (`self.CurrentActorCount`))
          (for _array_element (`self.SpawnedActors`)
            (`self.K2_DestroyActor` _array_element))
          (`KismetArrayLibrary.Array_Clear` (`self.SpawnedActors`))
          (set `self.SpawnedActorCount` 0))))))

(event `self.ReceiveEndPlay`
  (params (EndPlayReason :type "EEndPlayReason Enum" :default "Destroyed"))
  (`parent.ReceiveEndPlay` EndPlayReason)
  (for _array_element (`self.SpawnedActors`)
    (`/Engine/EditorBlueprintResources/StandardMacros.IsValid` _array_element
      (:`Is Valid`
        (`self.K2_DestroyActor` _array_element)))))

(event `OnNpcDeth_Event`
  (params (DestroyedActor :type "Actor Object Reference"))
  (`/Engine/EditorBlueprintResources/StandardMacros.DecrementInt` (`self.CurrentActorCount`)
    (:`  `
      (if (`self.RespawnActorAfterDeth`)
        (`/Engine/EditorBlueprintResources/StandardMacros.DecrementInt` (`self.SpawnedActorCount`))))))

(fn `Init`
  (bind _spawnradius (`self.SpawnRadius`))
  (bind _returnvalue (* 2.0 _spawnradius))
  (bind _returnvalue_2 (`GameplayStatics.GetActorOfClass` "/Script/NavigationSystem.RecastNavMesh"))
  (set `self.RecastNavMesh` _returnvalue_2)
  (bind _outactors (`GameplayStatics.GetAllActorsOfClassWithTag` "/Script/NavigationSystem.NavMeshBoundsVolume" "Free"))
  (set `self.NavMesh` (`|GetArrayItem` _outactors))
  (`KismetArrayLibrary.Array_RemoveItem` (`Actor.Tags` (`self.NavMesh`)) "Free")
  (`self.K2_SetActorLocation` (`self.NavMesh`) (`self.K2_GetActorLocation`) false false)
  (`self.SetActorScale3D` (`self.NavMesh`) (`KismetMathLibrary.MakeVector` _returnvalue _returnvalue _spawnradius)))

(fn `Spawn Actor in Radius`
  (bind (_randomlocation _returnvalue) (`NavigationSystemV1.K2_GetRandomLocationInNavigableRadius` (`self.K2_GetActorLocation`) (`self.SpawnRadius`) (`self.RecastNavMesh`) null))
  (if (and (< (`self.SpawnedActorCount`) (`self.ActorToSpawnCount`)) (`self.SpawnActive`))
    (if _returnvalue
      (bind _returnvalue_2 (`|SpawnActorFromClass` (`self.ActorClass`) (`KismetMathLibrary.MakeTransform` _randomlocation) "AlwaysSpawn" "OverrideRootScale" null null))
      (add `self.OnDestroyed` _returnvalue_2 (`|CreateDelegate` :!event `OnNpcDeth_Event`))
      (`KismetArrayLibrary.Array_Add` (`self.SpawnedActors`) _returnvalue_2)
      (`/Engine/EditorBlueprintResources/StandardMacros.IncrementInt` (`self.SpawnedActorCount`)
        (:`  `
          (`self.OnActorSpawned` _returnvalue_2)
          (return))))))

(fn `UserConstructionScript`
  (bind _returnvalue (`self.K2_GetActorLocation`))
  (`KismetSystemLibrary.SphereTraceMultiForObjects` :`Start` _returnvalue :`End` _returnvalue :`Radius` (`self.SpawnRadius`) :`ObjectTypes` (`|MakeArray` "ObjectTypeQuery1" :!type "EObjectTypeQuery Enum") :`DrawTime` 1.0))