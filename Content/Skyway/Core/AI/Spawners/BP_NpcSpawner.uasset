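; BP_NpcSpawner is a child spawner that spawns NPCs of randomly chosen types and assigns them a team.
; It picks a random tag from NpcToSpawn and looks up the actor class in DT_Npc, at BeginPlay and again after each spawn.
; The spawn logic comes from the parent class, whose OnActorSpawned event is used to set each spawned BP_BaseNPC's ID to the spawner's TeamId.
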(event `self.ReceiveBeginPlay`
  (`self.SetRandomActorClass`)
  (`parent.ReceiveBeginPlay`)
  (add `self.OnActorSpawned` (delegate `OnNpcSpawned_Event`)))

(event `OnNpcSpawned_Event` :!signature `self.OnActorSpawned`
  (params (SpawnedActor :type "Actor Object Reference"))
  (`self.SetRandomActorClass`)
  (`/Engine/EditorBlueprintResources/StandardMacros.IsValid` SpawnedActor
    (:`Is Valid`
      (bind _asbp_base_npc (cast `/Game/Skyway/Core/AI/NPC/BP_BaseNPC` SpawnedActor))
      (set `BaseCharacter.ID` (`self.TeamId`) _asbp_base_npc))))

(fn `SetRandomActorClass`
  (bind _returnvalue (`|GetDataTableRow` "/Game/Skyway/Core/AI/NPC/DT_Npc.DT_Npc" (`BlueprintGameplayTagLibrary.GetTagName` (`KismetArrayLibrary.Array_Random` (`self.NpcToSpawn`))))
    (:`then`
      (set `self.ActorClass` (`.Class_6_AC49EED748CFDB709E67A695DBCC2AE6` (break `/Game/Skyway/Core/AI/NPC/S_NpcInfo` _returnvalue))))))

(fn `Spawn Actor in Radius`
  (`parent.Spawn Actor in Radius`)
  (return))

(fn `UserConstructionScript`
  (`parent.UserConstructionScript`))