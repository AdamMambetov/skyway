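; Base NPC spawner that extends a parent radius actor spawner to spawn random NPC types for a team.
; It picks a random tag from NpcToSpawn and looks up its class in DT_Npc, re-rolling at begin play and after each spawn.
; Spawned BP_BaseNPC actors receive the TeamId and a death binding.
; When respawn is enabled, a death re-rolls the class and decrements the parent's spawn count.
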(event `self.ReceiveBeginPlay`
  (`self.SetRandomActorClass`)
  (`parent.ReceiveBeginPlay`)
  (add `self.OnActorSpawned` (delegate `OnNpcSpawned_Event`)))

(event `OnNpcSpawned_Event` :!signature `self.OnActorSpawned`
  (params (SpawnedActor :type "Actor Object Reference"))
  (`self.SetRandomActorClass`)
  (bind _asbp_base_npc (cast `/Game/Skyway/Core/AI/NPS/BP_BaseNPC` SpawnedActor))
  (add `/Game/Skyway/Core/AI/NPS/BP_BaseNPC.OnNpcDeth` _asbp_base_npc (delegate `OnNpcDeth_Event`))
  (set `BaseCharacter.ID` (`self.TeamId`) _asbp_base_npc))

(event `OnNpcDeth_Event`
  (if (`self.RespawnNpcAfterDeth`)
    (`self.SetRandomActorClass`)
    (`/Engine/EditorBlueprintResources/StandardMacros.DecrementInt` (`self.SpawnedActorCount`))))

(fn `SetRandomActorClass`
  (bind _returnvalue (`|GetDataTableRow` "/Game/Skyway/Core/AI/NPS/DT_Npc.DT_Npc" (`BlueprintGameplayTagLibrary.GetTagName` (`KismetArrayLibrary.Array_Random` (`self.NpcToSpawn`))))
    (:`then`
      (set `self.ActorClass` (`.Class_6_AC49EED748CFDB709E67A695DBCC2AE6` (break `/Game/Skyway/Core/AI/NPS/S_NpcInfo` _returnvalue))))))

(fn `SpawnActorInRadius`
  (`parent.SpawnActorInRadius`))

(fn `UserConstructionScript`
  (`parent.UserConstructionScript`))