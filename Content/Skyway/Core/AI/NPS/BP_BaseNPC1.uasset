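; BP_BaseNPC1 is a base NPC character that starts with a fist weapon, shares the main mesh pose with its extra mesh parts, and ragdolls when a stat depletes.
; Each tick, the blackboard BattleState selects walk speed.
; While alive, it box-traces around itself to set the blackboard Overlap flag when EnemyActor is near.
; The box doubles in size while Overlap is set, giving the check hysteresis.
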(event `self.ReceiveBeginPlay`
  (`/Game/Skyway/Core/Inventory/AC_Storage.AddItemToSlotContainer` (`self.Inventory`) (struct :`TagName` "SlotContainer.Weapon") (struct :`TagName` "Item.Weapon.Fist") 1))

(event `self.ReceiveTick`
  (params (DeltaSeconds :type "Float (single-precision)"))
  (set `CharacterMovementComponent.MaxWalkSpeed` (select `/Game/Skyway/Core/AI/E_BattleState` (cast `/Game/Skyway/Core/AI/E_BattleState` (`BlackboardComponent.GetValueAsEnum` (`AIBlueprintHelperLibrary.GetBlackboard` (`AIBlueprintHelperLibrary.GetAIController` self)) "BattleState")) :`NewEnumerator2` (`self.PatrolSpeed`) :`NewEnumerator0` (`self.RushSpeed`) :`NewEnumerator1` (`self.BattleSpeed`) :`NewEnumerator3` (`self.ChaseSpeed`) :!type "Float (single-precision)") (`self.CharacterMovement`))
  (if (not (`/Game/Skyway/Core/Stats/AC_StatComponent.IsDead` (`self.StatComponent`)))
    (`self.SetNeedToTakePosition`)))

(event `self.StatComponent.OnStatReachedZero`
  (params (StatId :type "GameplayTag Structure"))
  (`|SwitchGameplayTag` StatId
    (:`Stat.Health`
      (`PrimitiveComponent.SetSimulatePhysics` (`self.Mesh`) true)
      (set `SkeletalMeshComponent.bPauseAnims` true (`self.Mesh`)))))

(fn `SetNeedToTakePosition`
  (locals (L_HalfSize :type "Vector Structure" :default (200.0 200.0 200.0)))
  (bind _returnvalue (`self.K2_GetActorLocation`))
  (bind _returnvalue_2 (`KismetStringLibrary.Conv_StringToName` "Overlap"))
  (bind _returnvalue_3 (`AIBlueprintHelperLibrary.GetBlackboard` (`AIBlueprintHelperLibrary.GetAIController` self)))
  (bind _returnvalue_4 (`AIBlueprintHelperLibrary.GetBlackboard` (`AIBlueprintHelperLibrary.GetAIController` self)))
  (`/Engine/EditorBlueprintResources/StandardMacros.IsValid` _returnvalue_4
    (:`Is Valid`
      (if (`BlackboardComponent.GetValueAsBool` _returnvalue_4 (`KismetStringLibrary.Conv_StringToName` "Overlap"))
        (set `local.L_HalfSize` (600.0 600.0 600.0))
        (else
          (set `local.L_HalfSize` (300.0 300.0 300.0) :!label _label))))
    (:`Is Not Valid`
      (goto _label)))
  (bind (_outhits _returnvalue_5) (`KismetSystemLibrary.BoxTraceMultiForObjects` :`Start` _returnvalue :`End` _returnvalue :`HalfSize` (`local.L_HalfSize`) :`ObjectTypes` (`|MakeArray` "ObjectTypeQuery3" "ObjectTypeQuery8" "ObjectTypeQuery9" :!type "EObjectTypeQuery Enum") :`DrawDebugType` "ForOneFrame"))
  (if _returnvalue_5
    (for _array_element _outhits
      (if (== (`.HitActor` (`GameplayStatics.BreakHitResult` _array_element)) (`BlackboardComponent.GetValueAsObject` (`AIBlueprintHelperLibrary.GetBlackboard` (`AIBlueprintHelperLibrary.GetAIController` self)) (`KismetStringLibrary.Conv_StringToName` "EnemyActor")))
        (`BlackboardComponent.SetValueAsBool` _returnvalue_3 _returnvalue_2 true)
        (break)
        (else
          (`BlackboardComponent.SetValueAsBool` _returnvalue_3 _returnvalue_2 false :!label _label_2))))
    (else
      (goto _label_2))))

(fn `UserConstructionScript`
  (`SkinnedMeshComponent.SetLeaderPoseComponent` (`self.Dop`) (`self.Mesh`) false)
  (`SkinnedMeshComponent.SetLeaderPoseComponent` (`self.Second`) (`self.Mesh`) false)
  (`SkinnedMeshComponent.SetLeaderPoseComponent` (`self.Hook`) (`self.Mesh`) false))