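; Base AI NPC character with modular meshes, an overhead health bar and stat-driven damage and death.
; Each tick sets walk speed from the Blackboard BattleState and sphere-traces for the Blackboard Enemy, using min/max radii as hysteresis for the Overlap key.
; While alive, Overlap controls health bar visibility.
; Health changes apply backward force scaled by damage; a depleted stat triggers ragdoll, and death removes the bar and fires a one-time notification.
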(event `self.ReceiveBeginPlay`
  (bind _widget (`self.Widget`))
  (bind _returnvalue (`|CreateWidget` "/Game/Skyway/Core/UI/Enemy/EnemyHpBar.EnemyHpBar_C" null self))
  (`WidgetComponent.SetWidget` _widget _returnvalue)
  (`WidgetComponent.SetDrawSize` _widget (268.0 42.0))
  (`AIPerceptionComponent.RequestStimuliListenerUpdate` (`AIController.GetAIPerceptionComponent` (`AIBlueprintHelperLibrary.GetAIController` self)))
  (add `/Game/Skyway/Core/Stats/AC_StatComponent.OnStatCurrentValueChange` (`self.StatComponent`) (`|CreateDelegate` :!event `OnTakeDamage`))
  (set `self.CurrentHelth` (`.CurrentValue_4_DE51577F455957135DBA8EAD967FB78D` (break `/Game/Skyway/Core/Stats/S_StatInfo` (`.StatInfo` (`/Game/Skyway/Core/Stats/AC_StatComponent.GetStatInfoById` (`self.StatComponent`) (struct :`TagName` "Stat.Health")))))))

(event `self.ReceiveTick`
  (params (DeltaSeconds :type "Float (single-precision)"))
  (`self.UpdateMaxWalkSpeed`)
  (if (not (`/Game/Skyway/Core/Stats/AC_StatComponent.IsDead` (`self.StatComponent`)))
    (`self.SetNeedToTakePosition`)
    (`SceneComponent.SetVisibility` (`self.Widget`) (`BlackboardComponent.GetValueAsBool` (`AIBlueprintHelperLibrary.GetBlackboard` (`AIBlueprintHelperLibrary.GetAIController` self)) "Overlap") true)
    (else
      (bind _widget (`self.Widget`)
        (:`then`
          (`ActorComponent.K2_DestroyComponent` _widget))
        (:`else`
          _))
      (`/Engine/EditorBlueprintResources/StandardMacros.DoOnce` false
        (:`Completed`
          (`self.OnNpcDeth`))))))

(event `self.StatComponent.OnStatReachedZero`
  (params (StatId :type "GameplayTag Structure"))
  (`|SwitchGameplayTag` StatId
    (:`Stat.Health`
      (`PrimitiveComponent.SetSimulatePhysics` (`self.Mesh`) true)
      (set `SkeletalMeshComponent.bPauseAnims` true (`self.Mesh`)))))

(event `OnTakeDamage`
  (params (StatId :type "GameplayTag Structure") (CurrentValue :type "Float (double-precision)"))
  (if (and (`BlueprintGameplayTagLibrary.MatchesTag` StatId (struct :`TagName` "Stat.Health")) (not (`/Game/Skyway/Core/Stats/AC_StatComponent.IsDead` (`self.StatComponent`))))
    (`CharacterMovementComponent.AddForce` (`self.CharacterMovement`) (* (`self.GetActorForwardVector`) -1.0 2000000.0 (- (`self.CurrentHelth`) CurrentValue)))
    (set `self.CurrentHelth` CurrentValue)
    (`KismetSystemLibrary.PrintString` "Hello")))

(fn `SetNeedToTakePosition`
  (locals (L_HalfSize :type "Float (double-precision)") (L_HitEnemy :type Boolean))
  (bind _returnvalue (`self.K2_GetActorLocation`))
  (bind _returnvalue_2 (`AIBlueprintHelperLibrary.GetBlackboard` (`AIBlueprintHelperLibrary.GetAIController` self)))
  (`/Engine/EditorBlueprintResources/StandardMacros.IsValid` _returnvalue_2
    (:`Is Valid`
      (if (`BlackboardComponent.GetValueAsBool` _returnvalue_2 (`KismetStringLibrary.Conv_StringToName` "Overlap"))
        (set `local.L_HalfSize` (`self.MaxOverlapRadius`))
        (else
          (set `local.L_HalfSize` (`self.MinOverlapRadius`))))
      (bind (_outhits _returnvalue_3) (`KismetSystemLibrary.SphereTraceMultiForObjects` _returnvalue _returnvalue (`local.L_HalfSize`) (`|MakeArray` "ObjectTypeQuery3" "ObjectTypeQuery8" "ObjectTypeQuery9" :!type "EObjectTypeQuery Enum")))
      (if _returnvalue_3
        (set `local.L_HitEnemy` false)
        (for _array_element _outhits
          (if (== (`.HitActor` (`GameplayStatics.BreakHitResult` _array_element)) (`BlackboardComponent.GetValueAsObject` (`AIBlueprintHelperLibrary.GetBlackboard` (`AIBlueprintHelperLibrary.GetAIController` self)) (`KismetStringLibrary.Conv_StringToName` "Enemy")))
            (set `local.L_HitEnemy` true)
            (break)))
        (`BlackboardComponent.SetValueAsBool` (`AIBlueprintHelperLibrary.GetBlackboard` (`AIBlueprintHelperLibrary.GetAIController` self)) (`KismetStringLibrary.Conv_StringToName` "Overlap") (`local.L_HitEnemy`))
        (else
          (`BlackboardComponent.SetValueAsBool` (`AIBlueprintHelperLibrary.GetBlackboard` (`AIBlueprintHelperLibrary.GetAIController` self)) (`KismetStringLibrary.Conv_StringToName` "Overlap") false))))))

(fn `UpdateMaxWalkSpeed`
  (set `CharacterMovementComponent.MaxWalkSpeed` (select `/Game/Skyway/Core/AI/E_BattleState` (cast `/Game/Skyway/Core/AI/E_BattleState` (`BlackboardComponent.GetValueAsEnum` (`AIBlueprintHelperLibrary.GetBlackboard` (`AIBlueprintHelperLibrary.GetAIController` self)) "BattleState")) :`NewEnumerator2` (`self.PatrolSpeed`) :`NewEnumerator0` (`self.RushSpeed`) :`NewEnumerator1` (`self.BattleSpeed`) :`NewEnumerator3` (`self.ChaseSpeed`) :!type "Float (single-precision)") (`self.CharacterMovement`)))

(fn `UserConstructionScript`
  (`SkinnedMeshComponent.SetLeaderPoseComponent` (`self.Dop`) (`self.Mesh`) false)
  (`SkinnedMeshComponent.SetLeaderPoseComponent` (`self.Second`) (`self.Mesh`) false)
  (`SkinnedMeshComponent.SetLeaderPoseComponent` (`self.Hook`) (`self.Mesh`) false)
  (`self.SpawnDefaultController`))