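; Base NPC Blueprint that tells its AI, through the blackboard, whether its enemy is close by.
; Construction slaves the Dop, Second and Hook meshes to the main Mesh as master pose.
; Every tick a box trace around the NPC searches for the blackboard's EnemyActor and writes the Overlap key.
; The box grows while Overlap is true, giving hysteresis so the flag does not flicker at the edge.
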(event `self.ReceiveBeginPlay`)

(event `self.ReceiveTick`
  (params (DeltaSeconds :type "Float (single-precision)"))
  (`self.SetNeedToTakePosition`))

(fn `SetNeedToTakePosition`
  (locals (L_HalfSize :type "Vector Structure" :default (0.0 0.0 0.0)))
  (bind _returnvalue (`self.K2_GetActorLocation`))
  (bind _returnvalue_2 (`KismetStringLibrary.Conv_StringToName` "Overlap"))
  (bind _returnvalue_3 (`AIBlueprintHelperLibrary.GetBlackboard` (`AIBlueprintHelperLibrary.GetAIController` self)))
  (bind _returnvalue_4 (`AIBlueprintHelperLibrary.GetBlackboard` (`AIBlueprintHelperLibrary.GetAIController` self)))
  (`/Engine/EditorBlueprintResources/StandardMacros.IsValid` _returnvalue_4
    (:`Is Valid`
      (if (`BlackboardComponent.GetValueAsBool` _returnvalue_4 (`KismetStringLibrary.Conv_StringToName` "Overlap"))
        (set `local.L_HalfSize` (450.0 450.0 450.0))
        (else
          (set `local.L_HalfSize` (200.0 200.0 200.0))))
      (bind _outhits (`KismetSystemLibrary.BoxTraceMultiForObjects` _returnvalue _returnvalue (`local.L_HalfSize`) (struct) (`|MakeArray` "ObjectTypeQuery3" "ObjectTypeQuery8" "ObjectTypeQuery9" :!type "EObjectTypeQuery Enum")))
      (for _array_element _outhits
        (bind _returnvalue_5 (== (`.HitActor` (`GameplayStatics.BreakHitResult` _array_element)) (`BlackboardComponent.GetValueAsObject` (`AIBlueprintHelperLibrary.GetBlackboard` (`AIBlueprintHelperLibrary.GetAIController` self)) (`KismetStringLibrary.Conv_StringToName` "EnemyActor"))))
        (if _returnvalue_5
          (break)))
      (if _returnvalue_5
        (`BlackboardComponent.SetValueAsBool` _returnvalue_3 _returnvalue_2 true)
        (else
          (`BlackboardComponent.SetValueAsBool` _returnvalue_3 _returnvalue_2 false))))))

(fn `UserConstructionScript`
  (`SkinnedMeshComponent.SetLeaderPoseComponent` (`self.Dop`) (`self.Mesh`) false)
  (`SkinnedMeshComponent.SetLeaderPoseComponent` (`self.Second`) (`self.Mesh`) false)
  (`SkinnedMeshComponent.SetLeaderPoseComponent` (`self.Hook`) (`self.Mesh`) false))