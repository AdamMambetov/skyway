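; Actor component that manages its owner's tag-identified stats, such as Health and Energy.
; It builds the stat array from initial values on BeginPlay and subtracts incoming damage from Health.
; Changes are clamped between zero and max, then relayed through server and multicast events to a value-changed dispatcher.
; Tick regenerates Energy through a server event, only between Ultra Dynamic Sky's dawn and dusk, making it daylight-driven.
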(event `self.ReceiveBeginPlay`
  (`self.InitStats_SERVER`)
  (add `Actor.OnTakeAnyDamage` (`self.GetOwner`) (`|CreateDelegate` :!event `OnTakeAnyDamage_Event`))
  (bind _returnvalue (`GameplayStatics.GetActorOfClass` "/Game/UltraDynamicSky/Blueprints/Ultra_Dynamic_Sky.Ultra_Dynamic_Sky_C"))
  (set `self.UltraDynamicSkyRef` _returnvalue))

(event `self.ReceiveTick`
  (params (DeltaSeconds :type "Float (single-precision)"))
  (`self.RegenStats_SERVER`))

(event `OnTakeAnyDamage_Event`
  (params (DamagedActor :type "Actor Object Reference") (Damage :type "Float (single-precision)") (DamageType :type "DamageType Object Reference") (InstigatedBy :type "Controller Object Reference") (DamageCauser :type "Actor Object Reference"))
  (`self.ChangeStatValueById` (struct :`TagName` "Stat.Health") Damage))

(event `OnStartCurrentValueChange_SERVER`
  (params (StatId :type "GameplayTag Structure") (CurrentValue :type "Float (double-precision)"))
  (`self.OnStartCurrentValueChange_MULTI` StatId CurrentValue))

(event `OnStartCurrentValueChange_MULTI`
  (params (StatId :type "GameplayTag Structure") (CurrentValue :type "Float (double-precision)"))
  (`self.OnStatCurrentValueChange` StatId CurrentValue))

(event `InitStats_SERVER`
  (`self.InitStats`))

(event `ChangeStatValueById_SERVER`
  (params (Id :type "GameplayTag Structure") (Value :type "Float (double-precision)"))
  (`self.ChangeStatValueById` Id Value))

(event `RegenStats_SERVER`
  (`self.RegenStats`))

(fn `CanEnergyRegenerate`
  (returns (ReturnValue :type Boolean))
  (bind (_returnvalue _statinfo) (`self.GetStatInfoById` (struct :`TagName` "Stat.Energy")))
  (bind _ultradynamicskyref (`self.UltraDynamicSkyRef`))
  (bind ((`CurrentValue_4_DE51577F455957135DBA8EAD967FB78D` _currentvalue) (`MaxValue_5_3CC336414940E22148AD9A97F33F72D7` _maxvalue) (`bCanRegenerate_12_DA1BA7624075C2D48F2FF7B502F8F507` _bcanregenerate)) (break `/Game/Skyway/Core/Stats/S_StatInfo` _statinfo))
  (bind _time_of_day (`/Game/UltraDynamicSky/Blueprints/Ultra_Dynamic_Sky.Time of Day` _ultradynamicskyref))
  (if _returnvalue
    (return (and (< _currentvalue _maxvalue) _bcanregenerate (> _time_of_day (`/Game/UltraDynamicSky/Blueprints/Ultra_Dynamic_Sky.Dawn Time` _ultradynamicskyref)) (< _time_of_day (`/Game/UltraDynamicSky/Blueprints/Ultra_Dynamic_Sky.Dusk Time` _ultradynamicskyref))))))

(fn `ChangeStatValueById`
  (params (Id :type "GameplayTag Structure") (Value :type "Float (double-precision)"))
  (locals (L_StatInfo :type "/Game/Skyway/Core/Stats/S_StatInfo Structure") (L_StatIndex :type Integer))
  (bind ((`CurrentValue_4_DE51577F455957135DBA8EAD967FB78D` _currentvalue) (`MaxValue_5_3CC336414940E22148AD9A97F33F72D7` _maxvalue)) (break `/Game/Skyway/Core/Stats/S_StatInfo` (`local.L_StatInfo`)))
  (bind ((`CurrentValue_4_DE51577F455957135DBA8EAD967FB78D` _currentvalue_2) (`ID_9_CB03B1114A36A3A49D84BCBA5584296D` _id)) (break `/Game/Skyway/Core/Stats/S_StatInfo` (`local.L_StatInfo`)))
  (for (_array_element _array_index) (`self.Stats`)
    (if (== (`.ID_9_CB03B1114A36A3A49D84BCBA5584296D` (break `/Game/Skyway/Core/Stats/S_StatInfo` _array_element)) (`local.Id`))
      (`|ExecutionSequence`
        (:`then_0`
          (set `local.L_StatInfo` _array_element)
          (set `local.L_StatIndex` _array_index))
        (:`then_1`
          (`self.CompareCurrentValue` (`local.L_StatInfo`) (`local.Value`)
            (:`<`
              (if (> (`.CurrentValue_4_DE51577F455957135DBA8EAD967FB78D` (break `/Game/Skyway/Core/Stats/S_StatInfo` (`local.L_StatInfo`))) 0.0)
                (setmembers `/Game/Skyway/Core/Stats/S_StatInfo` :`StructRef` (`local.L_StatInfo`) :`CurrentValue` 0.0)
                (else
                  (return))))
            (:`><`
              (setmembers `/Game/Skyway/Core/Stats/S_StatInfo` :`StructRef` (`local.L_StatInfo`) :`CurrentValue` (- (`.CurrentValue_4_DE51577F455957135DBA8EAD967FB78D` (break `/Game/Skyway/Core/Stats/S_StatInfo` (`local.L_StatInfo`))) (`local.Value`))))
            (:`>`
              (if (< _currentvalue _maxvalue)
                (setmembers `/Game/Skyway/Core/Stats/S_StatInfo` :`StructRef` (`local.L_StatInfo`) :`CurrentValue` (`.MaxValue_5_3CC336414940E22148AD9A97F33F72D7` (break `/Game/Skyway/Core/Stats/S_StatInfo` (`local.L_StatInfo`))))
                (else
                  (return))))))
        (:`then_2`
          (`KismetArrayLibrary.Array_Set` (`self.Stats`) (`local.L_StatIndex`) (`local.L_StatInfo`))
          (`self.OnStartCurrentValueChange_SERVER` _id _currentvalue_2)
          (return))))))

(fn `GetStatInfoById`
  (params (Id :type "GameplayTag Structure" :default (struct :`TagName` "Stat")))
  (returns (ReturnValue :type Boolean) (StatInfo :type "/Game/Skyway/Core/Stats/S_StatInfo Structure"))
  (for _array_element (`self.Stats`)
    (if (== (`.ID_9_CB03B1114A36A3A49D84BCBA5584296D` (break `/Game/Skyway/Core/Stats/S_StatInfo` _array_element)) (`local.Id`))
      (return true _array_element))))

(fn `InitStats`
  (locals (L_StatInfo :type "/Game/Skyway/Core/Stats/S_StatInfo Structure"))
  (bind _l_statinfo (`local.L_StatInfo`))
  (bind ((`MaxValue_5_3CC336414940E22148AD9A97F33F72D7` _maxvalue) (`ID_9_CB03B1114A36A3A49D84BCBA5584296D` _id)) (break `/Game/Skyway/Core/Stats/S_StatInfo` (`local.L_StatInfo`)))
  (bind ((`CurrentValue_4_DE51577F455957135DBA8EAD967FB78D` _currentvalue) (`MaxValue_5_3CC336414940E22148AD9A97F33F72D7` _maxvalue_2)) (break `/Game/Skyway/Core/Stats/S_StatInfo` (`local.L_StatInfo`)))
  (`KismetArrayLibrary.Array_Clear` (`self.Stats`))
  (for _array_element (`self.InitialStats`)
    (set `local.L_StatInfo` _array_element)
    (if (and (> _maxvalue 0.0) (`/Game/Skyway/Core/Engine/FLBP_Defaults.IsValidStatId` _id))
      (if (> _currentvalue _maxvalue_2)
        (setmembers `/Game/Skyway/Core/Stats/S_StatInfo` :`StructRef` _l_statinfo :`CurrentValue` (`.MaxValue_5_3CC336414940E22148AD9A97F33F72D7` (break `/Game/Skyway/Core/Stats/S_StatInfo` _l_statinfo))))
      (`KismetArrayLibrary.Array_Add` (`self.Stats`) (`local.L_StatInfo`)))))

(fn `RegenStats`
  (locals (L_Stat :type "/Game/Skyway/Core/Stats/S_StatInfo Structure"))
  (for _array_element (`self.Stats`)
    (set `local.L_Stat` _array_element)
    (`|SwitchGameplayTag` (`.ID_9_CB03B1114A36A3A49D84BCBA5584296D` (break `/Game/Skyway/Core/Stats/S_StatInfo` (`local.L_Stat`)))
      (:`Stat.Energy`
        (if (`self.CanEnergyRegenerate`)
          (`self.ChangeStatValueById` (`.ID_9_CB03B1114A36A3A49D84BCBA5584296D` (break `/Game/Skyway/Core/Stats/S_StatInfo` (`local.L_Stat`))) (* (* (`.RegenerationRate_17_81ADE5EF4CC47325C6D0A8B76B4F7C99` (break `/Game/Skyway/Core/Stats/S_StatInfo` (`local.L_Stat`))) (`GameplayStatics.GetWorldDeltaSeconds`)) -1.0)))))))