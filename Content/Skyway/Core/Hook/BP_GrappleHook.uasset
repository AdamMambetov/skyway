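; BP_GrappleHook is a grapple hook projectile that flies with an initial burst of speed and an erratic path.
; BeginPlay records the start location and derives a boosted velocity from its Velocity variable.
; Tick blends the boosted velocity down to the base one in fixed per-frame steps, adding random per-axis jitter to ProjectileMovement.
; A check to destroy it beyond the grapple's maximum distance exists but is disconnected.
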(event `self.ReceiveBeginPlay`
  (set `MovementComponent.Velocity` (`self.Velocity`) (`self.ProjectileMovement`))
  (set `self.StartLocation` (`self.K2_GetActorLocation`))
  (set `self.ForceVelocitty` (* (`self.Velocity`) 5.0))
  (set `self.VelocityAlfa` 0.0))

(event `self.ReceiveTick`
  (params (DeltaSeconds :type "Float (single-precision)"))
  (bind _returnvalue (`KismetMathLibrary.RandomFloatInRange` -200.0 200.0))
  (bind (_returnvalue_x _returnvalue_y _returnvalue_z) (`KismetMathLibrary.BreakVector` (`KismetMathLibrary.VLerp` (`self.ForceVelocitty`) (`self.Velocity`) (`self.VelocityAlfa`))))
  (set `MovementComponent.Velocity` (`KismetMathLibrary.MakeVector` (+ _returnvalue_x _returnvalue) (+ _returnvalue_y _returnvalue) (+ _returnvalue_z _returnvalue)) (`self.ProjectileMovement`))
  (if (< (`self.VelocityAlfa`) 1.0)
    (set `self.VelocityAlfa` (+ (`self.VelocityAlfa`) 0.05))))

(fn `UserConstructionScript`)