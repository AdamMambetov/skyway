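; Grappling hook component for the main character that either pulls the player to what the hook hits or reels in objects tagged CanBeGrappled.
; Firing, replicated via server-to-multicast events, spawns a hook and cable; Tick runs a state machine for flight and pulling.
; Distance limits scaled by ProgressBarPercent, or overshooting the anchor, destroy the hook.
; Hook destruction restores movement settings and adds BPI_Item targets to inventory.
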(event `self.ReceiveBeginPlay`
  (bind _asbp_main_character (cast `/Game/Skyway/Core/Characters/BP_MainCharacter` (`self.GetOwner`)))
  (bind _output_get (set `self.MainCharacterRef` _asbp_main_character))
  (set `self.OwnerCharacterMovement` (`Character.CharacterMovement` _output_get)))

(event `self.ReceiveTick`
  (params (DeltaSeconds :type "Float (single-precision)"))
  (switch `/Game/Skyway/Core/Hook/E_HookState` (`self.GrappleState`)
    (:`NewEnumerator0`
      (set `self.Alpha` 0.0))
    (:`NewEnumerator4`)
    (:`NewEnumerator1`
      (`self.Flight`))
    (:`NewEnumerator2`
      (`self.AttachedToTarget`))
    (:`NewEnumerator3`
      (`self.Attached to Object`))))

(event `FireGrapple_SERVER`
  (params (TargetLocation :type "Vector Structure") (LocalOffset :type "Vector Structure") (ProgressBarPercent :type "Float (double-precision)"))
  (`self.FireGrapple_MULTI` TargetLocation LocalOffset ProgressBarPercent))

(event `FireGrapple_MULTI`
  (params (TargetLocation :type "Vector Structure") (LocalOffset :type "Vector Structure") (ProgressBarPercent :type "Float (double-precision)"))
  (`self.FireGrapple` TargetLocation LocalOffset ProgressBarPercent))

(event `OnGrappleDestroyed_SERVER`
  (params (DestroyedActor :type "Actor Object Reference"))
  (`self.OnGrappleDestroyed_MULTI` DestroyedActor))

(event `OnGrappleDestroyed_MULTI`
  (params (DestroyedActor :type "Actor Object Reference"))
  (`self.OnGrappleDestroyed` DestroyedActor))

(fn `Attached to Object`
  (bind _alpha (`self.Alpha`))
  (bind _maxgrapplespeed (`self.MaxGrappleSpeed`))
  (bind _hitactor (`self.HitActor`))
  (bind _returnvalue (- (`self.CalculateCableLength`) 1500.0))
  (`Actor.SetLifeSpan` _hitactor (`Actor.InitialLifeSpan` _hitactor))
  (if (<= _alpha 1.0)
    (set `self.Alpha` (+ _alpha (`self.AlphaSpeed`))))
  (set `self.GrappleSpeed` (`KismetMathLibrary.Lerp` _maxgrapplespeed (- _maxgrapplespeed (- (`self.MaxGrappleSpeed`) 2000.0)) (`self.Alpha`)))
  (`Actor.K2_AttachToActor` (`self.GrappleHook`) (`self.HitActor`) "StaticMesh" "SnapToTarget" "SnapToTarget" "SnapToTarget" true)
  (bind _grapplecable (`self.GrappleCable`)
    (:`then`
      (if (< _returnvalue 0.0)
        (bind _cablecomponent (`CableActor.CableComponent` _grapplecable))
        (set `CableComponent.CableLength` 0.0 _cablecomponent)
        (else
          (set `CableComponent.CableLength` _returnvalue _cablecomponent)))
      (`Actor.K2_AddActorWorldOffset` (`self.HitActor`) (* (* (* (`self.ToGrappleHook`) -1.0) (`self.GrappleSpeed`)) (`GameplayStatics.GetWorldDeltaSeconds`)) false false)
      (`self.TryToDestroyCable`))
    (:`else`)))

(fn `AttachedToTarget`
  (bind _returnvalue (- (`self.CalculateCableLength`) 1500.0))
  (`self.GrappleHook`
    (:`then`
      (bind _ownercharactermovement (`self.OwnerCharacterMovement`)
        (:`then`
          (set `MovementComponent.Velocity` (* (`self.ToGrappleHook`) (+ (* (`self.GrappleSpeed`) (`GameplayStatics.GetWorldDeltaSeconds`)) 0.001)) _ownercharactermovement)
          (bind _grapplecable (`self.GrappleCable`)
            (:`then`
              (if (< _returnvalue 0.0)
                (bind _cablecomponent (`CableActor.CableComponent` _grapplecable))
                (set `CableComponent.CableLength` 0.0 _cablecomponent)
                (else
                  (set `CableComponent.CableLength` _returnvalue _cablecomponent)))
              (`CharacterMovementComponent.AddForce` (`self.OwnerCharacterMovement`) (* (`self.ToGrappleHook`) 1000000.0))
              (`self.TryToDestroyCable`))
            (:`else`)))
        (:`else`)))
    (:`else`)))

(fn `CancelGrapple`
  (bind _grapplehook (`self.GrappleHook`)
    (:`then`
      (`Actor.K2_DestroyActor` _grapplehook))
    (:`else`)))

(fn `FireGrapple`
  (params (TargetLocation :type "Vector Structure") (LocalOffset :type "Vector Structure") (ProgressBarPercent :type "Float (double-precision)"))
  (locals (L_SpawnLocation :type "Vector Structure" :default (0.0 0.0 0.0)))
  (set `self.ProgressBarPercent` ProgressBarPercent)
  (if (not (`self.IsUse?`))
    (set `self.GrappleState` "NewEnumerator1")
    (set `local.L_SpawnLocation` (`SceneComponent.GetSocketLocation` (`Character.Mesh` (`self.MainCharacterRef`)) "HookSocket"))
    (set `self.FireDirection` (`KismetMathLibrary.GetDirectionUnitVector` (`local.L_SpawnLocation`) (`local.TargetLocation`)))
    (bind _returnvalue (`|SpawnActorFromClass` "/Game/Skyway/Core/Hook/BP_GrappleHook.BP_GrappleHook_C" (`KismetMathLibrary.MakeTransform` (`local.L_SpawnLocation`) (`KismetMathLibrary.FindLookAtRotation` (`local.L_SpawnLocation`) (`local.TargetLocation`)) (3.0 3.0 3.0)) "Undefined" "OverrideRootScale" null (* (`self.FireDirection`) (* (`self.HookSpeed`) (`GameplayStatics.GetWorldDeltaSeconds`))) null))
    (bind _output_get (set `self.GrappleHook` _returnvalue))
    (add `Actor.OnActorHit` _output_get (`|CreateDelegate` :!event `OnGrappleHit`))
    (add `Actor.OnDestroyed` (`self.GrappleHook`) (`|CreateDelegate` :!event `OnGrappleDestroyed_SERVER`))
    (bind _returnvalue_2 (`|SpawnActorFromClass` "/Game/Skyway/Core/Hook/BP_GrappleCable.BP_GrappleCable_C" (`KismetMathLibrary.MakeTransform` (`local.L_SpawnLocation`) (`/Game/Skyway/Core/Engine/MLBP_Defaults.DEFAULT`) (`/Game/Skyway/Core/Engine/MLBP_Defaults.DEFAULT_SCALE`)) "Undefined" "OverrideRootScale" null null))
    (set `self.GrappleCable` _returnvalue_2)
    (set `CharacterMovementComponent.MaxWalkSpeed` 150.0 (`self.OwnerCharacterMovement`))
    (bind _ascharacter (cast `Character` (`self.GetOwner`)))
    (`Actor.K2_AttachToComponent` (`self.GrappleCable`) (`Character.Mesh` _ascharacter) "HookSocket" "SnapToTarget" "SnapToTarget" "SnapToTarget" true)
    (`CableComponent.SetAttachEndTo` (`CableActor.CableComponent` (`self.GrappleCable`)) (`self.GrappleHook`) "None" "None")
    (set `CableComponent.EndLocation` (`/Game/Skyway/Core/Engine/MLBP_Defaults.DEFAULT`) (`CableActor.CableComponent` (`self.GrappleCable`)))))

(fn `Flight`
  (bind _returnvalue (- (`self.CalculateCableLength`) 1500.0))
  (bind _grapplecable (`self.GrappleCable`)
    (:`then`
      (if (< _returnvalue 0.0)
        (bind _cablecomponent (`CableActor.CableComponent` _grapplecable))
        (set `CableComponent.CableLength` 0.0 _cablecomponent)
        (else
          (set `CableComponent.CableLength` _returnvalue _cablecomponent)))
      (if (> (`self.CalculateCableLength`) (+ (`self.MinGrappleDistace`) 1000.0))
        (`self.TryToDestroyCable`)))
    (:`else`)))

(fn `IsUse?`
  (returns (ReturnValue :type Boolean))
  (return (select `/Game/Skyway/Core/Hook/E_HookState` (`self.GrappleState`) :`NewEnumerator1` true :`NewEnumerator2` true :`NewEnumerator3` true)))

(fn `OnGrappleDestroyed`
  (params (DestroyedActor :type "Actor Object Reference"))
  (set `self.GrappleHook` null)
  (set `self.GrappleState` "NewEnumerator0")
  (`|ExecutionSequence`
    (:`then_0`
      (bind _grapplecable (`self.GrappleCable`)
        (:`then`
          (`Actor.K2_DestroyActor` _grapplecable)
          (set `self.GrappleCable` null))
        (:`else`)))
    (:`then_1`
      (bind _ascharacter (cast `Character` (`self.GetOwner`)))
      (bind _charactermovement (`Character.CharacterMovement` _ascharacter))
      (set `CharacterMovementComponent.GroundFriction` 8.0 _charactermovement)
      (set `CharacterMovementComponent.GravityScale` 3.0 _charactermovement)
      (set `CharacterMovementComponent.AirControl` 1.0 _charactermovement)
      (set `CharacterMovementComponent.MaxWalkSpeed` 600.0 _charactermovement))
    (:`then_2`
      (bind _hitactor (`self.HitActor`)
        (:`then`
          (if (`KismetSystemLibrary.DoesImplementInterface` _hitactor "/Game/Skyway/Core/Inventory/BPI_Item.BPI_Item_C")
            (bind (_id _amount) (message `/Game/Skyway/Core/Inventory/BPI_Item.GetItemIdAndAmount` _hitactor))
            (`/Game/Skyway/Core/Inventory/AC_Inventory.AddItem` (`/Game/Skyway/Core/Characters/BP_MainCharacter.Inventory` (`self.MainCharacterRef`)) _id _amount)
            (`Actor.K2_DestroyActor` (`self.HitActor`))))
        (:`else`)))))

(fn `OnGrappleHit`
  (params (SelfActor :type "Actor Object Reference") (OtherActor :type "Actor Object Reference") (NormalImpulse :type "Vector Structure") (Hit :type "HitResult Structure (by ref)"))
  (`Actor.SetLifeSpan` (`self.GrappleHook`) 9999999.0)
  (set `self.HitActor` (`.HitActor` (`GameplayStatics.BreakHitResult` Hit)))
  (if (not (`Actor.ActorHasTag` (`self.HitActor`) "CanBeGrappled"))
    (`Actor.K2_AttachToActor` (`self.GrappleHook`) (`self.HitActor`) "None" "KeepWorld" "KeepWorld" "KeepWorld" true)
    (set `self.GrappleState` "NewEnumerator2")
    (bind _ascharacter (cast `Character` (`self.GetOwner`)))
    (bind _charactermovement (`Character.CharacterMovement` _ascharacter))
    (set `CharacterMovementComponent.GroundFriction` 0.0 _charactermovement)
    (set `CharacterMovementComponent.GravityScale` 0.0 _charactermovement)
    (set `CharacterMovementComponent.AirControl` 1.0 _charactermovement)
    (set `CharacterMovementComponent.MaxWalkSpeed` 1500.0 _charactermovement)
    (set `self.InitialHookDirection2D` (`self.ToGrappleHook2D`))
    (else
      (set `self.GrappleState` "NewEnumerator3"))))

(fn `OnRep_GrappleState`
  (`self.OnGrappleStateChanged` (`self.GrappleState`)))

(fn `TryToDestroyCable`
  (bind _returnvalue (`KismetMathLibrary.Vector_Distance` (`Actor.K2_GetActorLocation` (`self.GrappleHook`)) (`Actor.K2_GetActorLocation` (`self.GetOwner`))))
  (if (or (> _returnvalue (* (`self.MaxGrappleDistace`) (`self.ProgressBarPercent`))) (< _returnvalue (`self.MinGrappleDistace`)))
    (`Actor.K2_DestroyActor` (`self.GrappleHook`))
    (elif (and (< (`KismetMathLibrary.Dot_VectorVector` (`self.InitialHookDirection2D`) (`self.ToGrappleHook2D`)) 0.0) (`|EnumInequality` (`self.GrappleState`) "NewEnumerator1") (`|EnumInequality` (`self.GrappleState`) "NewEnumerator3"))
      (`Actor.K2_DestroyActor` (`self.GrappleHook`)))))