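; Grappling hook equipment that either pulls the player to a surface or reels tagged objects in.
; Activate line-traces from the camera, attaches the hook to the hit actor, shows the cable and picks the mode by the CanBeGrappled tag.
; Tick drives player velocity or offsets the object toward the housing.
; Player overlap with the cancel trigger resets the hook and destroys any tagged hooked object.
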(event `self.ReceiveTick`
  (params (DeltaSeconds :type "Float (single-precision)"))
  (switch `/Game/Skyway/Core/Hook/Old/E_HookOperatingModes` (`self.OperatingMode`)
    (:`NewEnumerator1`
      (`self.PullPlayer`))
    (:`NewEnumerator2`
      (`self.PullObject` DeltaSeconds))))

(event `self.HookCancelTrigger.OnComponentBeginOverlap`
  (params (OverlappedComponent :type "PrimitiveComponent Object Reference") (OtherActor :type "Actor Object Reference") (OtherComp :type "PrimitiveComponent Object Reference") (OtherBodyIndex :type Integer) (bFromSweep :type Boolean) (SweepResult :type "HitResult Structure (by ref)"))
  (if (== OtherActor (`self.MainCharacterRef`))
    (`self.Cancel`)
    (bind _hookedobject (`self.HookedObject`)
      (:`then`
        (if (`self.ActorHasTag` _hookedobject "CanBeGrappled")
          (`self.K2_DestroyActor` _hookedobject)))
      (:`else`))))

(fn `Activate`
  (locals (L_HitLocation :type "Vector Structure" :default (0.0 0.0 0.0)))
  (`parent.Activate`)
  (`self.MainCharacterRef`
    (:`then`
      _)
    (:`else`
      (bind _asbp_main_character (cast `/Game/Skyway/Core/Characters/BP_MainCharacter` (`GameplayStatics.GetPlayerCharacter` 0)))
      (set `self.MainCharacterRef` _asbp_main_character)))
  (bind (_returnvalue _hitresult) (`self.CheckForHit`))
  (if _returnvalue
    (bind (_bblockinghit _binitialoverlap _time _distance _location _impactpoint _normal _impactnormal _physmat _hitactor) (`GameplayStatics.BreakHitResult` _hitresult))
    (set `local.L_HitLocation` _impactpoint)
    (set `self.HookedObject` _hitactor)
    (`self.FireHook` (`local.L_HitLocation`))
    (if (`self.ActorHasTag` (`self.HookedObject`) "CanBeGrappled")
      (set `self.OperatingMode` "NewEnumerator2")
      (else
        (set `self.OperatingMode` "NewEnumerator1")
        (`Character.Jump` (`self.MainCharacterRef`))))))

(fn `Cancel`
  (`parent.Cancel`)
  (set `self.OperatingMode` "NewEnumerator0")
  (`SceneComponent.K2_AttachToComponent` (`self.Hook`) (`self.Housing`) "None" "SnapToTarget" "SnapToTarget" "SnapToTarget" true)
  (`SceneComponent.K2_SetRelativeLocation` (`self.Hook`) (23.0 2.0 0.0) false false)
  (`SceneComponent.SetVisibility` (`self.Cable`) false false))

(fn `CheckForHit`
  (returns (ReturnValue :type Boolean) (HitResult :type "HitResult Structure"))
  (bind _returnvalue (`GameplayStatics.GetPlayerCameraManager` 0))
  (bind _returnvalue_2 (`PlayerCameraManager.GetCameraLocation` _returnvalue))
  (bind (_outhit _returnvalue_3) (`KismetSystemLibrary.LineTraceSingle` _returnvalue_2 (+ _returnvalue_2 (* (`self.GetActorForwardVector` _returnvalue) 10000.0)) "TraceTypeQuery1"))
  (return _returnvalue_3 _outhit))

(fn `FireHook`
  (params (HitLocation :type "Vector Structure"))
  (`SceneComponent.K2_SetWorldLocation` (`self.Hook`) HitLocation false false)
  (`SceneComponent.K2_AttachToComponent` (`self.Hook`) (`Actor.RootComponent` (`self.HookedObject`)) "None" "KeepWorld" "KeepWorld" "KeepWorld" true)
  (`SceneComponent.SetVisibility` (`self.Cable`) true false))

(fn `PullObject`
  (params (`Delta T` :type "Float (double-precision)"))
  (`self.K2_AddActorWorldOffset` (`self.HookedObject`) (* (* (`KismetMathLibrary.GetDirectionUnitVector` (`SceneComponent.K2_GetComponentLocation` (`self.Hook`)) (`SceneComponent.K2_GetComponentLocation` (`self.Housing`))) (`self.GrappleSpeed`)) `Delta T`) false false))

(fn `PullPlayer`
  (set `MovementComponent.Velocity` (* (`KismetMathLibrary.GetDirectionUnitVector` (`PlayerCameraManager.GetCameraLocation` (`GameplayStatics.GetPlayerCameraManager` 0)) (`SceneComponent.K2_GetComponentLocation` (`self.Hook`))) (`self.GrappleSpeed`)) (`Character.CharacterMovement` (`self.MainCharacterRef`))))

(fn `UserConstructionScript`
  (`parent.UserConstructionScript`))