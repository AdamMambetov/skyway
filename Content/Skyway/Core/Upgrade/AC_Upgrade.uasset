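; Actor component that manages and activates the owner's upgrades, loaded from DT_Upgrades on BeginPlay.
; ActivateUpgradeById flags an inactive upgrade active, fires OnUpgradeActivate and completes the first-upgrade training task if current.
; A gameplay tag switch sends Health and Energy boosts to the stat component as modifiers and nearly removes grapple cooldown for Hook Boost 4.
; Other boost accumulation is disconnected, so GetAllBoosts returns variables this graph never updates.
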(event `self.ReceiveBeginPlay`
  (`self.InitUpgrades`)
  (set `self.OwnerStatComp` (`Actor.GetComponentByClass` (`self.GetOwner`) "/Game/Skyway/Core/Stats/AC_StatComponent.AC_StatComponent_C"))
  (set `self.OwnerTaskComp` (`Actor.GetComponentByClass` (`self.GetOwner`) "/Game/Skyway/Core/Tasks/AC_Task.AC_Task_C"))
  (set `self.OwnerGrappleComp` (`Actor.GetComponentByClass` (`self.GetOwner`) "/Game/Skyway/Core/Hook/AC_Grapple.AC_Grapple_C")))

(fn `ActivateUpgradeById`
  (params (UpgradeId :type "GameplayTag Structure"))
  (locals (L_Boost :type "Float (double-precision)"))
  (bind _upgrades (`self.Upgrades`))
  (bind ((`Name_20_6A0B85594A90E217E69136BD90667BBB` _name) (`Description_23_45A6D4084E9E6C459822DB8CCD80DB08` _description) (`Task_37_F243B44D4B614EEEE1517DBCEF91E53D` _task) (`CurrentTaskIndex_11_0FD1030F4BBB9E7445CBB486176018B2` _currenttaskindex)) (break `/Game/Skyway/Core/Tasks/S_TaskChain` (`/Game/Skyway/Core/Tasks/AC_Task.CurrentTaskChain` (`self.OwnerTaskComp`))))
  (for (_array_element _array_index) _upgrades
    (if (== (`.Id_16_C698D4794DE27ACE1B0B23BCD391E817` (break `/Game/Skyway/Core/Upgrade/S_UpgradeInfo` _array_element)) (`local.UpgradeId`))
      (bind _output (`|GetArrayItem` _upgrades _array_index))
      (if (not (`.Active_17_6D9C8D4E44A3DD3B5F8CC699650D749E` (break `/Game/Skyway/Core/Upgrade/S_UpgradeInfo` _output)))
        (bind _structout (setmembers `/Game/Skyway/Core/Upgrade/S_UpgradeInfo` :`StructRef` _output :`Active` true))
        (`self.OnUpgradeActivate` _array_element)
        (if (!= (`.CurrentTaskIndex_11_0FD1030F4BBB9E7445CBB486176018B2` (break `/Game/Skyway/Core/Tasks/S_TaskChain` (`/Game/Skyway/Core/Tasks/AC_Task.CurrentTaskChain` (`self.OwnerTaskComp`)))) -1)
          (if (== (`.TaskId_2_190FDDB94B36C38E21D7B5BFECC34D3A` (break `/Game/Skyway/Core/Tasks/S_Task` (`|GetArrayItem` _task _currenttaskindex))) (struct :`TagName` "Task.Train.10_FirstUpgrade"))
            (`/Game/Skyway/Core/Tasks/AC_Task.CompleteCurrentTask` (`self.OwnerTaskComp`))))
        (bind ((`Id_16_C698D4794DE27ACE1B0B23BCD391E817` _id) (`Boost_25_3AEF6CD8438A5F47E7722B95C6709CCE` _boost)) (break `/Game/Skyway/Core/Upgrade/S_UpgradeInfo` _structout))
        (set `local.L_Boost` _boost)
        (`|SwitchGameplayTag` _id
          (:`Upgrade.EnergyBoost.1`
            (`/Game/Skyway/Core/Stats/AC_StatComponent.AddStatModifier` (`self.OwnerStatComp`) (make `/Game/Skyway/Core/Stats/S_StatModifier` :`Id` (struct :`TagName` "Stat.Energy") :`Value` (`local.L_Boost`) :`Type` "NewEnumerator1" :`TypeContainer` (struct :`GameplayTags` (struct :`(TagName` "StatModifier.Immediately")))) :!label _label))
          (:`Upgrade.EnergyBoost.2`
            (`/Game/Skyway/Core/Stats/AC_StatComponent.AddStatModifier` (`self.OwnerStatComp`) (make `/Game/Skyway/Core/Stats/S_StatModifier` :`Id` (struct :`TagName` "Stat.Energy") :`Value` (`local.L_Boost`) :`Type` "NewEnumerator2" :`TypeContainer` (struct :`GameplayTags` (struct :`(TagName` "StatModifier.Immediately")))) :!label _label_2))
          (:`Upgrade.EnergyBoost.3`
            (goto _label))
          (:`Upgrade.EnergyBoost.4`
            (goto _label_2))
          (:`Upgrade.HealthBoost.1`
            (`/Game/Skyway/Core/Stats/AC_StatComponent.AddStatModifier` (`self.OwnerStatComp`) (make `/Game/Skyway/Core/Stats/S_StatModifier` :`Id` (struct :`TagName` "Stat.Health") :`Value` (`local.L_Boost`) :`Type` "NewEnumerator1" :`TypeContainer` (struct :`GameplayTags` (struct :`(TagName` "StatModifier.Immediately")))) :!label _label_3))
          (:`Upgrade.HealthBoost.2`
            (`/Game/Skyway/Core/Stats/AC_StatComponent.AddStatModifier` (`self.OwnerStatComp`) (make `/Game/Skyway/Core/Stats/S_StatModifier` :`Id` (struct :`TagName` "Stat.Health") :`Value` (`local.L_Boost`) :`Type` "NewEnumerator2" :`TypeContainer` (struct :`GameplayTags` (struct :`(TagName` "StatModifier.Immediately")))) :!label _label_4))
          (:`Upgrade.HealthBoost.3`
            (goto _label_3))
          (:`Upgrade.HealthBoost.4`
            (goto _label_4))
          (:`Upgrade.HookBoost.4`
            (set `/Game/Skyway/Core/Hook/AC_Grapple.HookCooldown` 0.001 (`self.OwnerGrappleComp`))))))))

(fn `GetAllBoosts`
  (returns (MeleeDamageBoost :type "Float (double-precision)") (RangeDamageBoost :type "Float (double-precision)") (HookDistanceBoost :type "Float (double-precision)") (MaxHealthBoost :type "Float (double-precision)") (HpRegenBoost :type "Float (double-precision)") (MaxEnergyBoost :type "Float (double-precision)") (EnergyRegenBoost :type "Float (double-precision)") (HookSpeedBoost :type "Float (double-precision)") (MeleeAttackInterval :type "Float (double-precision)") (RangeAttackInterval :type "Float (double-precision)") (HookNoCooldown :type Boolean))
  (return (`self.MeleeDamageBoost`) (`self.RangeDamageBoost`) (`self.HookDistanceBoost`) (`self.MaxHealthBoost`) (`self.HpRegenBoost`) (`self.MaxEnergyBoost`) (`self.EnergyRegenBoost`) (`self.HookSpeedBoost`) (`self.MeleeAttackInterval`) (`self.RangeAttackInterval`) (`self.HookNoCooldown`)))

(fn `InitUpgrades`
  (bind _outrownames (`DataTableFunctionLibrary.GetDataTableRowNames` "/Game/Skyway/Core/Upgrade/DT_Upgrades.DT_Upgrades"))
  (for _array_element _outrownames
    (bind _returnvalue (`|GetDataTableRow` "/Game/Skyway/Core/Upgrade/DT_Upgrades.DT_Upgrades" _array_element)
      (:`then`
        (`KismetArrayLibrary.Array_Add` (`self.Upgrades`) _returnvalue)))))