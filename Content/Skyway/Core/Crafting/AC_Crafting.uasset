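; Actor component that handles recipe crafting and timed recipe research, with recipes built from DT_Recipes at BeginPlay.
; Craft requests check ingredients in the requester's storage, consume them immediately or on timer completion, then add the result, optionally to a chosen slot container.
; Research runs on a pausable timer whose remaining time Tick writes into the recipe; studying marks it learned and plays a sound.
; Recipe state saves and loads per player name.
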(event `self.ReceiveBeginPlay`
  (`self.GenerateRecipes`)
  (set `self.OwnerInventoryComp` (`Actor.GetComponentByClass` (`self.GetOwner`) "/Game/Skyway/Core/Inventory/AC_Inventory.AC_Inventory_C"))
  (set `self.OwnerSoundComp` (`Actor.GetComponentByClass` (`self.GetOwner`) "/Script/Engine.AudioComponent"))
  (set `self.OwnerTaskComp` (`Actor.GetComponentByClass` (`self.GetOwner`) "/Game/Skyway/Core/Tasks/AC_Task.AC_Task_C")))

(event `/Game/Skyway/Core/Engine/BPI_CanSave.SaveToPlayer`
  (params (SaveGame :type "SaveGame Object Reference"))
  (if (`self.bIsLoaded`)
    (bind (_returnvalue _playerinfo) (message `/Game/Skyway/Core/Engine/BPI_SaveGame.LoadPlayer` SaveGame (`FileManager.GetPlayerName`)))
    (if _returnvalue
      (bind _structout (setmembers `/Game/Skyway/Core/Engine/S_PlayerInfo` :`StructRef` _playerinfo :`Recipes` (`self.Recipes`)))
      (message `/Game/Skyway/Core/Engine/BPI_SaveGame.SavePlayer` SaveGame _structout)
      (else
        (message `/Game/Skyway/Core/Engine/BPI_SaveGame.SavePlayer` SaveGame (make `/Game/Skyway/Core/Engine/S_PlayerInfo` :`Name` (`FileManager.GetPlayerName`) :`Recipes` (`self.Recipes`)))))))

(event `/Game/Skyway/Core/Engine/BPI_CanSave.LoadToPlayer`
  (params (SaveGame :type "SaveGame Object Reference"))
  (bind (_returnvalue _playerinfo) (message `/Game/Skyway/Core/Engine/BPI_SaveGame.LoadPlayer` SaveGame (`FileManager.GetPlayerName`)))
  (if _returnvalue
    (set `self.Recipes` (`.Recipes_22_0074517948EB326546F88F9F96EB172B` (break `/Game/Skyway/Core/Engine/S_PlayerInfo` _playerinfo))))
  (set `self.bIsLoaded` true))

(event `self.ReceiveTick`
  (params (DeltaSeconds :type "Float (single-precision)"))
  (bind _currentresearchrecipeindex (`self.CurrentResearchRecipeIndex`))
  (bind _recipes (`self.Recipes`))
  (if (`KismetArrayLibrary.Array_IsValidIndex` _recipes _currentresearchrecipeindex)
    (if (and (!= (`KismetMathLibrary.FTrunc` (`KismetSystemLibrary.K2_GetTimerRemainingTimeHandle` (`self.ResearchHandle`))) (`.CurrentTimeToResearch_44_4D3C11784BD9CEF843A8BFA18AA9DFCD` (break `/Game/Skyway/Core/Crafting/S_Recipe` (`|GetArrayItem` _recipes _currentresearchrecipeindex)))) (`KismetSystemLibrary.K2_IsValidTimerHandle` (`self.ResearchHandle`)))
      (setmembers `/Game/Skyway/Core/Crafting/S_Recipe` :`StructRef` (`|GetArrayItem` (`self.Recipes`) (`self.CurrentResearchRecipeIndex`)) :`CurrentTimeToResearch` (`KismetMathLibrary.FCeil` (`KismetSystemLibrary.K2_GetTimerRemainingTimeHandle` (`self.ResearchHandle`))))
      (`self.OnRecipeUpdated`))))

(fn `ActivateStudy`
  (params (RecipeId :type "GameplayTag Structure"))
  (if (not (not (`KismetSystemLibrary.K2_IsValidTimerHandle` (`self.ResearchHandle`))))
    (`self.PauseStudy`))
  (for (_array_element _array_index) (`self.Recipes`)
    (bind ((`MaxTimeToResearch_43_65FF67AA4038AC2441B30181BF42CB4B` _maxtimetoresearch) (`CurrentTimeToResearch_44_4D3C11784BD9CEF843A8BFA18AA9DFCD` _currenttimetoresearch) (`Id_12_889ED428442C5949D1161581D23E95DC` _id)) (break `/Game/Skyway/Core/Crafting/S_Recipe` _array_element))
    (if (== _id RecipeId)
      (bind _returnvalue (`KismetSystemLibrary.K2_SetTimerDelegate` (`|CreateDelegate` :!event `StudyCurrentRecipe`) (+ (`KismetMathLibrary.Conv_IntToDouble` _currenttimetoresearch) 1e-05)))
      (set `self.ResearchHandle` _returnvalue)
      (set `self.CurrentResearchRecipe` _array_element)
      (set `self.CurrentResearchRecipeIndex` _array_index))))

(fn `CanCraftItemsByRecipeId`
  (params (RecipeId :type "GameplayTag Structure") (Num :type Integer) (RequesterStorage :type "/Game/Skyway/Core/Inventory/AC_Storage Object Reference"))
  (returns (ReturnValue :type Boolean) (MissingItems :type "Array of GameplayTag Structure"))
  (locals (L_CanCraft :type Boolean) (L_MissingItems :type "Array of GameplayTag Structure"))
  (`|GetDataTableRow` "/Game/Skyway/Core/Crafting/DT_Recipes.DT_Recipes" (`BlueprintGameplayTagLibrary.GetTagName` (`local.RecipeId`))
    (:`then`
      (set `local.L_CanCraft` true)
      (if (and (> (`local.Num`) 0) (`KismetSystemLibrary.IsValid` (`local.RequesterStorage`)) (`BlueprintGameplayTagLibrary.MatchesTag` (`local.RecipeId`) (struct :`TagName` "Recipe")))
        (bind _returnvalue (`|GetDataTableRow` "/Game/Skyway/Core/Crafting/DT_Recipes.DT_Recipes" (`BlueprintGameplayTagLibrary.GetTagName` (`local.RecipeId`)))
          (:`then`
            (bind ((`MaxTimeToResearch_43_65FF67AA4038AC2441B30181BF42CB4B` _maxtimetoresearch) (`CurrentTimeToResearch_44_4D3C11784BD9CEF843A8BFA18AA9DFCD` _currenttimetoresearch) (`TimeToCraft_35_5D3BB99F4D0DE280AE270D8C06CE8397` _timetocraft) (`Items_19_C6E91E9B484DDB55EE95BABEFCBE6FFB` _items)) (break `/Game/Skyway/Core/Crafting/S_Recipe` _returnvalue))
            (bind _keys (`BlueprintMapLibrary.Map_Keys` _items))
            (bind _values (`BlueprintMapLibrary.Map_Values` _items))
            (set `local.L_MissingItems` _keys)
            (for (_array_element _array_index) _keys
              (bind _returnvalue_2 (`/Game/Skyway/Core/Inventory/AC_Inventory.FindCountItemById` (`local.RequesterStorage`) _array_element))
              (if (< _returnvalue_2 (* (`|GetArrayItem` _values _array_index) (`local.Num`)))
                (set `local.L_CanCraft` false)
                (else
                  (`KismetArrayLibrary.Array_RemoveItem` (`local.L_MissingItems`) _array_element))))
            (if (`self.CraftActive`)
              (return false (`local.L_MissingItems`))
              (else
                (return (`local.L_CanCraft`) (`local.L_MissingItems`))))))))))

(fn `Craft`
  (if (`self.InstantlyRemoveResources`)
    (bind _returnvalue (`|GetDataTableRow` "/Game/Skyway/Core/Crafting/DT_Recipes.DT_Recipes" (`BlueprintGameplayTagLibrary.GetTagName` (`self.CurrentRecipeId`)))
      (:`then`
        (if (`BlueprintGameplayTagLibrary.MatchesTag` (`self.SlotContainerId`) (struct :`TagName` "SlotContainer"))
          (bind ((`MaxTimeToResearch_43_65FF67AA4038AC2441B30181BF42CB4B` _maxtimetoresearch) (`CurrentTimeToResearch_44_4D3C11784BD9CEF843A8BFA18AA9DFCD` _currenttimetoresearch) (`TimeToCraft_35_5D3BB99F4D0DE280AE270D8C06CE8397` _timetocraft) (`Result_23_1B532DAD43B20A155E0A209CC428568B` _result)) (break `/Game/Skyway/Core/Crafting/S_Recipe` _returnvalue))
          (bind (_returnvalue_2 _rest) (`/Game/Skyway/Core/Inventory/AC_Storage.AddItemToSlotContainer` (`self.RequesterStorage`) (`self.SlotContainerId`) _result (`self.Num`)))
          (if (`KismetMathLibrary.Conv_IntToBool` _rest)
            (`/Game/Skyway/Core/Inventory/AC_Inventory.AddItem` (`self.RequesterStorage`) _result _rest))
          (else
            (`/Game/Skyway/Core/Inventory/AC_Inventory.AddItem` (`self.RequesterStorage`) _result (`self.Num`))))
        (`self.StopCraft`)
        (`self.CraftEnd`)))
    (else
      (`self.Remove Items for Craft` (`self.CurrentRecipeId`) (`self.RequesterStorage`) (`self.Num`))
      (bind _returnvalue_3 (`|GetDataTableRow` "/Game/Skyway/Core/Crafting/DT_Recipes.DT_Recipes" (`BlueprintGameplayTagLibrary.GetTagName` (`self.CurrentRecipeId`)))
        (:`then`
          (if (`BlueprintGameplayTagLibrary.MatchesTag` (`self.SlotContainerId`) (struct :`TagName` "SlotContainer"))
            (bind ((`MaxTimeToResearch_43_65FF67AA4038AC2441B30181BF42CB4B` _maxtimetoresearch_2) (`CurrentTimeToResearch_44_4D3C11784BD9CEF843A8BFA18AA9DFCD` _currenttimetoresearch_2) (`Result_23_1B532DAD43B20A155E0A209CC428568B` _result_2)) (break `/Game/Skyway/Core/Crafting/S_Recipe` _returnvalue_3))
            (bind (_returnvalue_4 _rest_2) (`/Game/Skyway/Core/Inventory/AC_Storage.AddItemToSlotContainer` (`self.RequesterStorage`) (`self.SlotContainerId`) _result_2 (`self.Num`)))
            (if (`KismetMathLibrary.Conv_IntToBool` _rest_2)
              (`/Game/Skyway/Core/Inventory/AC_Inventory.AddItem` (`self.RequesterStorage`) _result_2 _rest_2))
            (else
              (`/Game/Skyway/Core/Inventory/AC_Inventory.AddItem` (`self.RequesterStorage`) _result_2 (`self.Num`))))
          (`self.StopCraft`)
          (`self.CraftEnd`))))))

(fn `CraftPause`
  (`KismetSystemLibrary.K2_PauseTimerHandle` (`self.CraftTimerHandle`)))

(fn `CraftRequest`
  (params (RecipeId :type "GameplayTag Structure" :default (struct :`TagName` "Recipe")) (Num :type Integer :default 1) (RequesterStorage :type "/Game/Skyway/Core/Inventory/AC_Storage Object Reference") (InstantlyRemoveResources :type Boolean) (SlotContainerId :type "GameplayTag Structure"))
  (returns (ReturnValue :type Boolean) (MissingItems :type "Array of GameplayTag Structure"))
  (bind (_returnvalue _missingitems) (`self.CanCraftItemsByRecipeId` RecipeId Num RequesterStorage))
  (if _returnvalue
    (set `self.InstantlyRemoveResources` InstantlyRemoveResources)
    (if (`local.InstantlyRemoveResources`)
      (`self.Remove Items for Craft` (`local.RecipeId`) (`local.RequesterStorage`) (`local.Num`)))
    (bind _returnvalue_2 (`|GetDataTableRow` "/Game/Skyway/Core/Crafting/DT_Recipes.DT_Recipes" (`BlueprintGameplayTagLibrary.GetTagName` (`local.RecipeId`)))
      (:`then`
        (bind ((`MaxTimeToResearch_43_65FF67AA4038AC2441B30181BF42CB4B` _maxtimetoresearch) (`CurrentTimeToResearch_44_4D3C11784BD9CEF843A8BFA18AA9DFCD` _currenttimetoresearch) (`TimeToCraft_35_5D3BB99F4D0DE280AE270D8C06CE8397` _timetocraft) (`Id_12_889ED428442C5949D1161581D23E95DC` _id)) (break `/Game/Skyway/Core/Crafting/S_Recipe` _returnvalue_2))
        (set `self.CurrentRecipeId` _id)
        (set `self.Num` (`local.Num`))
        (set `self.RequesterStorage` (`local.RequesterStorage`))
        (set `self.CraftActive` true)
        (set `self.SlotContainerId` (`local.SlotContainerId`))
        (bind _returnvalue_3 (`KismetSystemLibrary.K2_SetTimer` null "Craft" _timetocraft))
        (set `self.CraftTimerHandle` _returnvalue_3)
        (`self.CraftBegin`)
        (return true)))
    (else
      (return false _missingitems))))

(fn `CraftUnpause`
  (`KismetSystemLibrary.K2_UnPauseTimerHandle` (`self.CraftTimerHandle`)))

(fn `FindAndRemoveItemsById`
  (params (ItemId :type "GameplayTag Structure") (Storage :type "/Game/Skyway/Core/Inventory/AC_Storage Object Reference") (Num :type Integer))
  (returns (ReturnValue :type Boolean))
  (locals (L_NumItemsForRemove :type Integer))
  (set `local.L_NumItemsForRemove` Num)
  (bind (_arrayindex _arrayelement) (`/Engine/EditorBlueprintResources/StandardMacros.ReverseForEachLoop` (`/Game/Skyway/Core/Inventory/AC_Storage.GetSlotContainers` (`local.Storage`)))
    (:`LoopBody`
      (for _array_element (`.Slots_13_F3D539BF4555F142E47575834D8A86C6` (break `/Game/Skyway/Core/Inventory/S_SlotContainer_Info` _arrayelement))
        (bind ((`Amount_49_D1E29AF04498C178B74986AAD5610193` _amount) (`ID_71_BA06E0BD4E97D16461377CB9BF36CE2D` _id)) (break `/Game/Skyway/Core/Inventory/S_Item_Info` (`.ItemInfo_14_7E8F48144F0F01654500E084A85436C5` (break `/Game/Skyway/Core/Inventory/S_Slot_Info` _array_element))))
        (if (== _id (`local.ItemId`))
          (if (< _amount (`local.L_NumItemsForRemove`))
            (set `local.L_NumItemsForRemove` (- (`local.L_NumItemsForRemove`) _amount))
            (`/Game/Skyway/Core/Inventory/AC_Storage.RemoveSlot` (`local.Storage`) _array_element _amount)
            (else
              (bind _breturnvalue (`/Game/Skyway/Core/Inventory/AC_Storage.RemoveSlot` (`local.Storage`) _array_element (`local.L_NumItemsForRemove`)))
              (return _breturnvalue))))))))

(fn `GenerateRecipes`
  (`KismetArrayLibrary.Array_Clear` (`self.Recipes`))
  (bind _outrownames (`DataTableFunctionLibrary.GetDataTableRowNames` "/Game/Skyway/Core/Crafting/DT_Recipes.DT_Recipes"))
  (for _array_element _outrownames
    (bind _returnvalue (`|GetDataTableRow` "/Game/Skyway/Core/Crafting/DT_Recipes.DT_Recipes" _array_element)
      (:`then`
        (`KismetArrayLibrary.Array_Add` (`self.Recipes`) _returnvalue)))))

(fn `GetRecipeById`
  (params (RecipeId :type "GameplayTag Structure"))
  (returns (ReturnValue :type "/Game/Skyway/Core/Crafting/S_Recipe Structure"))
  (for _array_element (`self.Recipes`)
    (if (== (`.Id_12_889ED428442C5949D1161581D23E95DC` (break `/Game/Skyway/Core/Crafting/S_Recipe` _array_element)) RecipeId)
      (return _array_element))))

(fn `GetRecipesByCategory`
  (params (Category :type "/Game/Skyway/Core/Crafting/E_RecypeCategory Enum" :default "NewEnumerator0"))
  (returns (RecipesByCategory :type "Array of /Game/Skyway/Core/Crafting/S_Recipe Structure"))
  (locals (L_RecipesByCategory :type "Array of /Game/Skyway/Core/Crafting/S_Recipe Structure"))
  (for _array_element (`self.Recipes`)
    (if (`|EnumEquality` (`.RecipeCategory_26_03CBAE084F7969C4FB154F9D3B388559` (break `/Game/Skyway/Core/Crafting/S_Recipe` _array_element)) (`local.Category`))
      (`KismetArrayLibrary.Array_Add` (`local.L_RecipesByCategory`) _array_element)))
  (return (`local.L_RecipesByCategory`)))

(fn `PauseStudy`
  (bind _recipes (`self.Recipes`))
  (if (`BlueprintGameplayTagLibrary.IsGameplayTagValid` (`.Id_12_889ED428442C5949D1161581D23E95DC` (break `/Game/Skyway/Core/Crafting/S_Recipe` (`self.CurrentResearchRecipe`))))
    (for (_array_element _array_index) _recipes
      (if (== (`.Id_12_889ED428442C5949D1161581D23E95DC` (break `/Game/Skyway/Core/Crafting/S_Recipe` _array_element)) (`.Id_12_889ED428442C5949D1161581D23E95DC` (break `/Game/Skyway/Core/Crafting/S_Recipe` (`self.CurrentResearchRecipe`))))
        (setmembers `/Game/Skyway/Core/Crafting/S_Recipe` :`StructRef` (`|GetArrayItem` _recipes _array_index) :`CurrentTimeToResearch` (`KismetMathLibrary.FCeil` (`KismetSystemLibrary.K2_GetTimerRemainingTimeHandle` (`self.ResearchHandle`))))
        (`KismetSystemLibrary.K2_PauseTimerHandle` (`self.ResearchHandle`))))))

(fn `Remove Items for Craft`
  (params (RecipeId :type "GameplayTag Structure") (Storage :type "/Game/Skyway/Core/Inventory/AC_Storage Object Reference") (Num :type Integer))
  (bind _returnvalue (`|GetDataTableRow` "/Game/Skyway/Core/Crafting/DT_Recipes.DT_Recipes" (`BlueprintGameplayTagLibrary.GetTagName` RecipeId))
    (:`then`
      (bind ((`MaxTimeToResearch_43_65FF67AA4038AC2441B30181BF42CB4B` _maxtimetoresearch) (`CurrentTimeToResearch_44_4D3C11784BD9CEF843A8BFA18AA9DFCD` _currenttimetoresearch) (`TimeToCraft_35_5D3BB99F4D0DE280AE270D8C06CE8397` _timetocraft) (`Items_19_C6E91E9B484DDB55EE95BABEFCBE6FFB` _items)) (break `/Game/Skyway/Core/Crafting/S_Recipe` _returnvalue))
      (bind _keys (`BlueprintMapLibrary.Map_Keys` _items))
      (bind _values (`BlueprintMapLibrary.Map_Values` _items))
      (for (_array_element _array_index) _keys
        (`self.FindAndRemoveItemsById` _array_element (`local.Storage`) (* (`|GetArrayItem` _values _array_index) (`local.Num`)))))))

(fn `StopCraft`
  (set `self.CraftActive` false)
  (`KismetSystemLibrary.K2_ClearAndInvalidateTimerHandle` (`self.CraftTimerHandle`)))

(fn `StudyCurrentRecipe`
  (bind _recipes (`self.Recipes`))
  (bind ((`Id_12_889ED428442C5949D1161581D23E95DC` _id)) (break `/Game/Skyway/Core/Crafting/S_Recipe` (`self.CurrentResearchRecipe`)))
  (`self.OnStudyRecipe` _id)
  (`self.OnRecipeUpdated`)
  (for (_array_element _array_index) _recipes
    (if (== (`.Id_12_889ED428442C5949D1161581D23E95DC` (break `/Game/Skyway/Core/Crafting/S_Recipe` _array_element)) _id)
      (setmembers `/Game/Skyway/Core/Crafting/S_Recipe` :`StructRef` (`|GetArrayItem` _recipes _array_index) :`Studyied` true)
      (`AudioComponent.SetSound` (`self.OwnerSoundComp`) "/Game/Skyway/Audio/Cues/изучение-навыка_Cue.изучение-навыка_Cue")
      (`AudioComponent.Play` (`self.OwnerSoundComp`) 0.0))))