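; Base world pickup actor that shows an item's mesh and a floating icon, both looked up from its initial item ID.
; The construction script sets the mesh, while BeginPlay and player respawn events create the icon widget.
; Once the world loads, Tick keeps the icon above the pickup facing the player.
; Unhooked pickups, detected by root child count, destroy themselves when too far from their owner.
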(event `self.ReceiveTick`
  (params (DeltaSeconds :type "Float (single-precision)"))
  (bind _returnvalue (`self.GetOwner`))
  (`parent.ReceiveTick` DeltaSeconds)
  (bind _gm_main (`self.GM_Main`)
    (:`then`
      (if (`/Game/Skyway/Core/Engine/GM_Main.bWorldLoaded` _gm_main)
        (`SceneComponent.K2_SetWorldLocationAndRotation` (`self.Widget`) (+ (`self.K2_GetActorLocation`) (0.0 0.0 80.0)) (`KismetMathLibrary.FindLookAtRotation` (`SceneComponent.K2_GetComponentLocation` (`self.Widget`)) (`self.K2_GetActorLocation` (`GameplayStatics.GetPlayerPawn` 0))) false false)
        (if (== 2 (`SceneComponent.GetNumChildrenComponents` (`self.DefaultSceneRoot`)))
          (`/Engine/EditorBlueprintResources/StandardMacros.IsValid` _returnvalue
            (:`Is Valid`
              (if (> (`KismetMathLibrary.Vector_Distance` (`self.K2_GetActorLocation` _returnvalue) (`SceneComponent.K2_GetComponentLocation` (`self.StaticMesh`))) 5000.0)
                (`self.K2_DestroyActor`)))))))
    (:`else`)))

(event `self.ReceiveBeginPlay`
  (bind _asgm_main (cast `/Game/Skyway/Core/Engine/GM_Main` (`GameplayStatics.GetGameMode`)))
  (bind _output_get (set `self.GM_Main` _asgm_main))
  (add `/Game/Skyway/Core/Engine/GM_Main.OnPlayerRespawn` _output_get (`|CreateDelegate` :!event `OnPlayerRespawn_Event`))
  (bind (_returnvalue _iteminfo) (`/Game/Skyway/Core/Engine/FLBP_Defaults.GetItemInfoById` (`self.InitialID`)))
  (bind _returnvalue_2 (`|CreateWidget` "/Game/Skyway/Core/UI/WBP_ItemIcon.WBP_ItemIcon_C" (`GameplayStatics.GetPlayerController` 0) (`.Icon_69_E7C0F30049DDB94441E17A93C556C0EF` (break `/Game/Skyway/Core/Inventory/S_Item_Info` _iteminfo))))
  (`WidgetComponent.SetWidget` (`self.Widget`) _returnvalue_2))

(event `OnPlayerRespawn_Event`
  (bind (_returnvalue _iteminfo) (`/Game/Skyway/Core/Engine/FLBP_Defaults.GetItemInfoById` (`self.InitialID`)))
  (bind _returnvalue_2 (`|CreateWidget` "/Game/Skyway/Core/UI/WBP_ItemIcon.WBP_ItemIcon_C" (`GameplayStatics.GetPlayerController` 0) (`.Icon_69_E7C0F30049DDB94441E17A93C556C0EF` (break `/Game/Skyway/Core/Inventory/S_Item_Info` _iteminfo))))
  (`WidgetComponent.SetWidget` (`self.Widget`) _returnvalue_2))

(fn `UserConstructionScript`
  (`parent.UserConstructionScript`)
  (bind (_returnvalue _iteminfo) (`/Game/Skyway/Core/Engine/FLBP_Defaults.GetItemInfoById` (`self.InitialID`)))
  (if _returnvalue
    (`StaticMeshComponent.SetStaticMesh` (`self.StaticMesh`) (`.StaticMesh_55_DD99137048858773BCC1349BF67B1BCE` (break `/Game/Skyway/Core/Inventory/S_Item_Info` _iteminfo)))
    (else
      (`KismetSystemLibrary.PrintString` "Row Not Found!" true true (struct :`R` 1.0 :`B` 0.018015 :`A` 1.0)))))