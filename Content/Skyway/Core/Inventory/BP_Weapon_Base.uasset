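; BP_Weapon_Base is a base weapon Blueprint that deals melee damage through a box collision.
; Construction loads WeaponInfo from the DT_Weapons row named by the InitialID tag and sets its initial item amount.
; Attack, which only handles the Fist type, enables query-only collision, and hits on non-owner actors apply the weapon's damage.
; SERVER-suffixed events wrap attacking and collision toggling, with nothing here switching collision off automatically.
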(event `Attack_SERVER`
  (`self.Attack`))

(event `EnableCollision_SERVER`
  (`self.EnableCollision`))

(event `DisableCollision_SERVER`
  (`self.DisableCollision`))

(event `self.BoxCollision.OnComponentHit`
  (params (HitComponent :type "PrimitiveComponent Object Reference") (OtherActor :type "Actor Object Reference") (OtherComp :type "PrimitiveComponent Object Reference") (NormalImpulse :type "Vector Structure") (Hit :type "HitResult Structure (by ref)"))
  (if (!= OtherActor (`self.GetOwner`))
    (`GameplayStatics.ApplyDamage` OtherActor (`.Damage_9_E157A1A343752171738AF58207467496` (break `/Game/Skyway/Core/Inventory/S_Weapon_Info` (`self.WeaponInfo`))))))

(fn `Attack`
  (switch `/Game/Skyway/Core/Inventory/E_WeaponType` (`.WeaponType_6_742DF51A4E96C15CAA15F3A5D0E18F2C` (break `/Game/Skyway/Core/Inventory/S_Weapon_Info` (`self.WeaponInfo`)))
    (:`NewEnumerator0`
      (`self.EnableCollision_SERVER`))))

(fn `DisableCollision`
  (if (`PrimitiveComponent.K2_IsCollisionEnabled` (`self.BoxCollision`))
    (`PrimitiveComponent.SetCollisionEnabled` (`self.BoxCollision`) "NoCollision")))

(fn `EnableCollision`
  (if (not (`PrimitiveComponent.K2_IsCollisionEnabled` (`self.BoxCollision`)))
    (`PrimitiveComponent.SetCollisionEnabled` (`self.BoxCollision`) "QueryOnly")))

(fn `UserConstructionScript`
  (`parent.UserConstructionScript`)
  (bind _returnvalue (`|GetDataTableRow` "/Game/Skyway/Core/Inventory/DT_Weapons.DT_Weapons" (`BlueprintGameplayTagLibrary.GetTagName` (`self.InitialID`)))
    (:`then`
      (bind _output_get (set `self.WeaponInfo` _returnvalue))
      (setmembers `/Game/Skyway/Core/Inventory/S_Item_Info` :`StructRef` (`.ItemInfo_11_1C9DECE349EB7A8AE9502F90F742809E` (break `/Game/Skyway/Core/Inventory/S_Weapon_Info` _output_get)) :`Amount` (`self.InitialAmount`)))))