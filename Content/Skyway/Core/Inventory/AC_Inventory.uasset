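; Inventory component child that drives the Recycle container, filling its output slot from whatever is placed in the input slot.
; BeginPlay binds a slot-update handler that reacts to Recycle slot 0, looking up the item in DT_Pieces and its recipe in DT_Recipes.
; Slot 1 receives the recipe result, scaled as input amount divided by the first ingredient quantity, or clears when input empties, via a server setter.
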(event `self.ReceiveBeginPlay`
  (`parent.ReceiveBeginPlay`)
  (add `self.OnSlotUpdated` (`|CreateDelegate` :!event `OnSlotUpdated_Event`)))

(fn `OnSlotUpdated_Event`
  (params (SlotInfo :type "/Game/Skyway/Core/Inventory/S_Slot_Info Structure"))
  (switch `/Game/Skyway/Core/Inventory/E_SlotType` (`.Type_32_DA6EC9A74765E8D199FD1FABBE3B74F3` (break `/Game/Skyway/Core/Inventory/S_Slot_Info` SlotInfo))
    (:`NewEnumerator6`
      (if (== (`.Index_20_9AE11B3243796F89520F24AEAC51F772` (break `/Game/Skyway/Core/Inventory/S_Slot_Info` (`local.SlotInfo`))) 0)
        (if (> (`.Amount_49_D1E29AF04498C178B74986AAD5610193` (break `/Game/Skyway/Core/Inventory/S_Item_Info` (`.ItemInfo_14_7E8F48144F0F01654500E084A85436C5` (break `/Game/Skyway/Core/Inventory/S_Slot_Info` (`local.SlotInfo`))))) 0)
          (bind _returnvalue (`|GetDataTableRow` "/Game/Skyway/Core/Inventory/DT_Pieces.DT_Pieces" (`BlueprintGameplayTagLibrary.GetTagName` (`.ID_71_BA06E0BD4E97D16461377CB9BF36CE2D` (break `/Game/Skyway/Core/Inventory/S_Item_Info` (`.ItemInfo_14_7E8F48144F0F01654500E084A85436C5` (break `/Game/Skyway/Core/Inventory/S_Slot_Info` (`local.SlotInfo`)))))))
            (:`then`
              (bind _returnvalue_2 (`|GetDataTableRow` "/Game/Skyway/Core/Crafting/DT_Recipes.DT_Recipes" (`BlueprintGameplayTagLibrary.GetTagName` (`.RecipeId_25_3797D7844273B4CF8F7EB1842ED1659C` (break `/Game/Skyway/Core/Inventory/S_Piece_Info` _returnvalue))))
                (:`then`
                  (bind ((`Items_19_C6E91E9B484DDB55EE95BABEFCBE6FFB` _items) (`Result_23_1B532DAD43B20A155E0A209CC428568B` _result)) (break `/Game/Skyway/Core/Crafting/S_Recipe` _returnvalue_2))
                  (bind _values (`BlueprintMapLibrary.Map_Values` _items))
                  (bind (_returnvalue_3 _iteminfo) (`/Game/Skyway/Core/Engine/FLBP_Defaults.GetItemInfoById` _result))
                  (bind _structout (setmembers `/Game/Skyway/Core/Inventory/S_Item_Info` :`StructRef` _iteminfo :`Amount` (/ (`.Amount_49_D1E29AF04498C178B74986AAD5610193` (break `/Game/Skyway/Core/Inventory/S_Item_Info` (`.ItemInfo_14_7E8F48144F0F01654500E084A85436C5` (break `/Game/Skyway/Core/Inventory/S_Slot_Info` (`local.SlotInfo`))))) (`|GetArrayItem` _values))))
                  (bind _structout_2 (setmembers `/Game/Skyway/Core/Inventory/S_Slot_Info` :`StructRef` (`|GetArrayItem` (`self.GetSlotsAtItemType` (struct :`TagName` "SlotContainer.Recycle") (`/Game/Skyway/Core/Engine/MLBP_Defaults.DEFAULT`)) 1) :`ItemInfo` _structout))
                  (`self.SetSlotsElem_SERVER` _structout_2 (struct :`TagName` "SlotContainer.Recycle"))))))
          (else
            (bind _structout_3 (setmembers `/Game/Skyway/Core/Inventory/S_Slot_Info` :`StructRef` (`|GetArrayItem` (`self.GetSlotsAtItemType` (struct :`TagName` "SlotContainer.Recycle") (`/Game/Skyway/Core/Engine/MLBP_Defaults.DEFAULT`)) 1) :`ItemInfo` (`self.EMPTY_ITEM`)))
            (`self.SetSlotsElem_SERVER` _structout_3 (struct :`TagName` "SlotContainer.Recycle"))))))))