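; AC_Storage is an inventory storage component, shown here through the helper functions that validate slots in its StorageSlots array.
; A slot is valid when it is in the array, its amount exceeds the default sentinel, and it is either empty or holds a valid item ID with an amount above empty.
; IsSlotEmpty builds on that check, while IsValidSlotAtIndex repeats it by index and slot type, with only Inventory wired.
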(fn `IsSlotEmpty`
  (params (SlotInfo :type "/Game/Skyway/Core/Inventory/S_Slot_Info Structure"))
  (returns (ReturnValue :type Boolean) (Empty :type Boolean))
  (locals (L_SlotInfo :type "/Game/Skyway/Core/Inventory/S_Slot_Info Structure"))
  (if (`self.IsValidSlot` SlotInfo)
    (return true (and (== (`.Amount_49_D1E29AF04498C178B74986AAD5610193` (break `/Game/Skyway/Core/Inventory/S_Item_Info` (`.ItemInfo_14_7E8F48144F0F01654500E084A85436C5` (break `/Game/Skyway/Core/Inventory/S_Slot_Info` (`local.SlotInfo`))))) (`self.EMPTY_SLOT_VALUE`)) (not (`BlueprintGameplayTagLibrary.IsGameplayTagValid` (`.ID_71_BA06E0BD4E97D16461377CB9BF36CE2D` (break `/Game/Skyway/Core/Inventory/S_Item_Info` (`.ItemInfo_14_7E8F48144F0F01654500E084A85436C5` (break `/Game/Skyway/Core/Inventory/S_Slot_Info` (`local.SlotInfo`)))))))))
    (else
      (return false false))))

(fn `IsValidSlot`
  (params (SlotInfo :type "/Game/Skyway/Core/Inventory/S_Slot_Info Structure"))
  (returns (ReturnValue :type Boolean))
  (bind ((`Amount_49_D1E29AF04498C178B74986AAD5610193` _amount) (`ID_71_BA06E0BD4E97D16461377CB9BF36CE2D` _id)) (break `/Game/Skyway/Core/Inventory/S_Item_Info` (`.ItemInfo_14_7E8F48144F0F01654500E084A85436C5` (break `/Game/Skyway/Core/Inventory/S_Slot_Info` (`local.SlotInfo`)))))
  (return (and (`KismetArrayLibrary.Array_Contains` (`self.StorageSlots`) (`local.SlotInfo`)) (> (`.Amount_49_D1E29AF04498C178B74986AAD5610193` (break `/Game/Skyway/Core/Inventory/S_Item_Info` (`.ItemInfo_14_7E8F48144F0F01654500E084A85436C5` (break `/Game/Skyway/Core/Inventory/S_Slot_Info` (`local.SlotInfo`))))) (`self.DEFAULT_AMOUNT_VALUE`)) (or (and (== (`.Amount_49_D1E29AF04498C178B74986AAD5610193` (break `/Game/Skyway/Core/Inventory/S_Item_Info` (`.ItemInfo_14_7E8F48144F0F01654500E084A85436C5` (break `/Game/Skyway/Core/Inventory/S_Slot_Info` (`local.SlotInfo`))))) (`self.EMPTY_SLOT_VALUE`)) (not (`BlueprintGameplayTagLibrary.IsGameplayTagValid` _id))) (and (`/Game/Skyway/Core/Engine/FLBP_Defaults.IsValidItemId` _id) (> _amount (`self.EMPTY_SLOT_VALUE`)))))))

(fn `IsValidSlotAtIndex`
  (params (Index :type Integer) (Type :type "/Game/Skyway/Core/Inventory/E_SlotType Enum" :default "NewEnumerator0"))
  (returns (ReturnValue :type Boolean) (Slots :type "Array of /Game/Skyway/Core/Inventory/S_Slot_Info Structure") (Slot :type "/Game/Skyway/Core/Inventory/S_Slot_Info Structure"))
  (locals (L_SearchingSlotsArray :type "Array of /Game/Skyway/Core/Inventory/S_Slot_Info Structure") (L_SlotInfo :type "/Game/Skyway/Core/Inventory/S_Slot_Info Structure"))
  (bind ((`Amount_49_D1E29AF04498C178B74986AAD5610193` _amount) (`ID_71_BA06E0BD4E97D16461377CB9BF36CE2D` _id)) (break `/Game/Skyway/Core/Inventory/S_Item_Info` (`.ItemInfo_14_7E8F48144F0F01654500E084A85436C5` (break `/Game/Skyway/Core/Inventory/S_Slot_Info` (`local.L_SlotInfo`)))))
  (bind ((`Amount_49_D1E29AF04498C178B74986AAD5610193` _amount_2)) (break `/Game/Skyway/Core/Inventory/S_Item_Info` (`.ItemInfo_14_7E8F48144F0F01654500E084A85436C5` (break `/Game/Skyway/Core/Inventory/S_Slot_Info` (`local.L_SlotInfo`)))))
  (set `local.L_SearchingSlotsArray` (select `/Game/Skyway/Core/Inventory/E_SlotType` (`local.Type`) :`NewEnumerator1` (`self.StorageSlots`)))
  (set `local.L_SlotInfo` (select `/Game/Skyway/Core/Inventory/E_SlotType` (`local.Type`) :`NewEnumerator1` (`|GetArrayItem` (`self.StorageSlots`) (`local.Index`))))
  (return (and (`KismetArrayLibrary.Array_Contains` (`local.L_SearchingSlotsArray`) (`local.L_SlotInfo`)) (> _amount_2 (`self.DEFAULT_AMOUNT_VALUE`)) (or (and (== _amount_2 (`self.EMPTY_SLOT_VALUE`)) (not (`BlueprintGameplayTagLibrary.IsGameplayTagValid` _id))) (and (`/Game/Skyway/Core/Engine/FLBP_Defaults.IsValidItemId` _id) (> _amount (`self.EMPTY_SLOT_VALUE`))))) (`local.L_SearchingSlotsArray`) (`local.L_SlotInfo`)))